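; Cinematic controller that stages a scripted gate-opening encounter between Marines and Hormagant enemies through externally callable events.
; OpenGates raises the gate by a per-update timeline offset and, after a delay, sends all Marines forward via AIMoveTo; MoveActors runs only the march.
; The first finished move passes a DoOnce to trigger the Warrior taunt, randomized-speed enemy threats and Marine montages.
; AttackBody separately plays the attacking enemy's melee montage.
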(event `AttackBody`
  (`Character.PlayAnimMontage` (`self.AttackingEnemy`) "/Game/WH40Assets/Tyranids/Animations/Montages/AM_Hormagant_AttackMelee1.AM_Hormagant_AttackMelee1" 1.0 "None"))

(event `OpenGates`
  (bind _staticmeshcomponent (`StaticMeshActor.StaticMeshComponent` (`self.GateActor`)))
  (`|ExecutionSequence`
    (:`then_0`
      (`Timeline|Timeline` :!via `PlayFromStart`
        (:`Update`
          (`SceneComponent.K2_SetWorldLocation` _staticmeshcomponent (+ (`SceneComponent.K2_GetComponentLocation` _staticmeshcomponent) (0.0 0.0 3.0)) false false))))
    (:`then_1`
      (`KismetSystemLibrary.Delay` 4.0 :!label _label)
      (for _array_element (`self.MarinesActors`)
        (`AITask_MoveTo.AIMoveTo` (`AIBlueprintHelperLibrary.GetAIController` _array_element) (- (`SceneComponent.K2_GetComponentLocation` (`Character.Mesh` _array_element)) (`KismetMathLibrary.MakeVector` 0.0 (`KismetMathLibrary.RandomFloatInRange` -2200.0 -2400.0))) null
          (:`OnMoveFinished`
            (`/Engine/EditorBlueprintResources/StandardMacros.DoOnce` false
              (:`Completed`
                (`KismetSystemLibrary.Delay` 0.5)
                (`Character.PlayAnimMontage` (`self.WarriorActor`) "/Game/WH40Assets/Tyranids/Animations/Montages/AM_Warrior_Taunt.AM_Warrior_Taunt" 1.0 "None")
                (`|ExecutionSequence`
                  (:`then_0`
                    (`KismetSystemLibrary.Delay` 1.0)
                    (for _array_element_2 (`self.BaseEnemiesArray`)
                      (`Character.PlayAnimMontage` _array_element_2 "/Game/WH40Assets/Tyranids/Animations/Montages/AM_Hormagant_Threaten.AM_Hormagant_Threaten" (`KismetMathLibrary.RandomFloatInRange` 0.8 1.2) "None")))
                  (:`then_1`
                    (`Character.PlayAnimMontage` (`|GetArrayItem` (`self.MarinesActors`) 4) "/Game/WH40Assets/SpaceMarines/Animations/Montages/AM_SM_Spawn.AM_SM_Spawn" 1.0 "None")
                    (`KismetSystemLibrary.Delay` 0.2)
                    (`Character.PlayAnimMontage` (`|GetArrayItem` (`self.MarinesActors`) 2) "/Game/WH40Assets/SpaceMarines/Animations/Montages/AM_SM_Reload_Pistol.AM_SM_Reload_Pistol" 1.0 "None")))))))))))

(event `MoveActors`
  (goto _label))

(fn `UserConstructionScript`)