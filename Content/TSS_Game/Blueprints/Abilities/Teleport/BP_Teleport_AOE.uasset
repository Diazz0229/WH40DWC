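; BP_Teleport_AOE is a teleport ability area actor that shows a decal, then fades it out and destroys itself.
; On BeginPlay it creates a dynamic decal material, waits briefly, then a looping timer steps the Opacity parameter down until it drops below zero.
; CheckCritAndDealDamage has an empty body, with its crit-roll and damage nodes left disconnected, so the actor deals no damage.
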(event `self.ReceiveBeginPlay`
  (bind _returnvalue (`DecalComponent.CreateDynamicMaterialInstance` (`self.Decal`)))
  (set `self.DynamicMaterial` _returnvalue)
  (`KismetSystemLibrary.Delay` 3.0)
  (`KismetSystemLibrary.K2_SetTimerDelegate` (delegate `LowerOpacity`) 0.1 true))

(event `LowerOpacity`
  (bind _dynamicmaterial (`self.DynamicMaterial`))
  (bind _returnvalue (`MaterialInstanceDynamic.K2_GetScalarParameterValue` _dynamicmaterial "Opacity"))
  (if (>= _returnvalue 0.0)
    (`MaterialInstanceDynamic.SetScalarParameterValue` _dynamicmaterial "Opacity" (- _returnvalue 0.1))
    (else
      (`KismetSystemLibrary.K2_PauseTimer` null "LowerOpacity")
      (`self.K2_DestroyActor`))))

(fn `CheckCritAndDealDamage`
  (params (DamageTarget :type "Actor Object Reference") (PlController :type "/Game/TSS_Game/Blueprints/System/BP_PlayerController Object Reference") (Source :type "/Game/TSS_Game/Blueprints/System/BP_CharacterBase Object Reference")))

(fn `UserConstructionScript`)