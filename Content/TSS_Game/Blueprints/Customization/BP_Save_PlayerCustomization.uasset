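; Player customization save game that holds per-class armor and equipment loadouts and the player's unlocked equipment.
; InitialSaveGame builds default loadouts from DataTable rows for five classes (Tactical, Assault, Devastator, ranged and melee Apothecary) via shared TEMP arrays, with Apothecary-specific armor presets.
; ConvertSavedNames, called from the lobby controller, turns saved names into unlocked equipment by searching each equipment table in turn.
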(event `InitialSaveGame`
  (params (SaveVersion :type Integer))
  (`KismetArrayLibrary.Array_Clear` (`self.SaveData_Slot1`))
  (`KismetArrayLibrary.Array_Clear` (`self.TEMP_PlayerCustomizationVisual`))
  (`KismetArrayLibrary.Array_Clear` (`self.TEMP_PlayerEquipment`))
  (set `self.LastPlayedClass` "NewEnumerator0")
  (set `self.SaveVersion` SaveVersion)
  (`KismetArrayLibrary.Array_Clear` (`self.TEMP_PlayerCustomizationVisual`))
  (bind _returnvalue (`|GetDataTableRow` "/Game/TSS_Game/Blueprints/Customization/DT_ArmorList_Helmets.DT_ArmorList_Helmets" "BaseHelmet")
    (:`then`
      (`KismetArrayLibrary.Array_Add` (`self.TEMP_PlayerCustomizationVisual`) _returnvalue)
      (bind _returnvalue_2 (`|GetDataTableRow` "/Game/TSS_Game/Blueprints/Customization/DT_ArmorList_Backpack.DT_ArmorList_Backpack" "BaseBackpack")
        (:`then`
          (`KismetArrayLibrary.Array_Add` (`self.TEMP_PlayerCustomizationVisual`) _returnvalue_2)
          (bind _returnvalue_3 (`|GetDataTableRow` "/Game/TSS_Game/Blueprints/Customization/DT_ArmorList_Hands.DT_ArmorList_Hands" "BaseHands")
            (:`then`
              (`KismetArrayLibrary.Array_Add` (`self.TEMP_PlayerCustomizationVisual`) _returnvalue_3)
              (bind _returnvalue_4 (`|GetDataTableRow` "/Game/TSS_Game/Blueprints/Customization/DT_ArmorList_Legs.DT_ArmorList_Legs" "Base_Legs")
                (:`then`
                  (`KismetArrayLibrary.Array_Add` (`self.TEMP_PlayerCustomizationVisual`) _returnvalue_4)
                  (bind _returnvalue_5 (`|GetDataTableRow` "/Game/TSS_Game/Blueprints/Customization/DT_ArmorList_Shoulders_LT.DT_ArmorList_Shoulders_LT" "BaseLeftShoulder")
                    (:`then`
                      (`KismetArrayLibrary.Array_Add` (`self.TEMP_PlayerCustomizationVisual`) _returnvalue_5)
                      (bind _returnvalue_6 (`|GetDataTableRow` "/Game/TSS_Game/Blueprints/Customization/DT_ArmorList_Shoulders_RT.DT_ArmorList_Shoulders_RT" "BaseRightShoulder")
                        (:`then`
                          (`KismetArrayLibrary.Array_Add` (`self.TEMP_PlayerCustomizationVisual`) _returnvalue_6)
                          (bind _returnvalue_7 (`|GetDataTableRow` "/Game/TSS_Game/Blueprints/Customization/DT_ArmorList_Torso.DT_ArmorList_Torso" "BaseChest")
                            (:`then`
                              (`KismetArrayLibrary.Array_Add` (`self.TEMP_PlayerCustomizationVisual`) _returnvalue_7)
                              (`|ExecutionSequence`
                                (:`then_0`
                                  ;[1 1 1] Tactical base equipment
                                  (bind _returnvalue_8 (`|GetDataTableRow` "/Game/TSS_Game/Blueprints/Customization/DT_EQP_WPN_Primary.DT_EQP_WPN_Primary" "BaseBolter")
                                    (:`then`
                                      (`KismetArrayLibrary.Array_AddUnique` (`self.TEMP_PlayerEquipment`) _returnvalue_8)
                                      (`KismetArrayLibrary.Array_AddUnique` (`self.PlayerUnlocked_Equipment`) _returnvalue_8)
                                      (bind _returnvalue_9 (`|GetDataTableRow` "/Game/TSS_Game/Blueprints/Customization/DT_EQP_WPN_SecondaryMelee.DT_EQP_WPN_SecondaryMelee" "BaseKnife")
                                        (:`then`
                                          (`KismetArrayLibrary.Array_AddUnique` (`self.TEMP_PlayerEquipment`) _returnvalue_9)
                                          (`KismetArrayLibrary.Array_AddUnique` (`self.PlayerUnlocked_Equipment`) _returnvalue_9)
                                          (bind _returnvalue_10 (`|GetDataTableRow` "/Game/TSS_Game/Blueprints/Customization/DT_EQP_WPN_SecondaryPistols.DT_EQP_WPN_SecondaryPistols" "BasePistol")
                                            (:`then`
                                              (`KismetArrayLibrary.Array_AddUnique` (`self.TEMP_PlayerEquipment`) _returnvalue_10)
                                              (`KismetArrayLibrary.Array_AddUnique` (`self.PlayerUnlocked_Equipment`) _returnvalue_10)
                                              (bind _returnvalue_11 (`|GetDataTableRow` "/Game/TSS_Game/Blueprints/Customization/DT_EQP_Chapter.DT_EQP_Chapter" "RelicHealth")
                                                (:`then`
                                                  (`KismetArrayLibrary.Array_AddUnique` (`self.TEMP_PlayerEquipment`) _returnvalue_11)
                                                  (`KismetArrayLibrary.Array_AddUnique` (`self.PlayerUnlocked_Equipment`) _returnvalue_11)
                                                  (bind _returnvalue_12 (`|GetDataTableRow` "/Game/TSS_Game/Blueprints/Customization/DT_EQP_Equipment.DT_EQP_Equipment" "FragGrenade_1")
                                                    (:`then`
                                                      (`KismetArrayLibrary.Array_AddUnique` (`self.TEMP_PlayerEquipment`) _returnvalue_12)
                                                      (`KismetArrayLibrary.Array_AddUnique` (`self.PlayerUnlocked_Equipment`) _returnvalue_12)
                                                      (`KismetArrayLibrary.Array_AddUnique` (`self.SaveData_Slot1`) (make `/Game/TSS_Game/Blueprints/Customization/ST_SaveGame_CustomizationData` "NewEnumerator0" (`self.TEMP_PlayerCustomizationVisual`) (`self.TEMP_PlayerEquipment`) _returnvalue_12))
                                                      (`KismetArrayLibrary.Array_Clear` (`self.TEMP_PlayerEquipment`)))))))))))))
                                (:`then_1`
                                  ;[1 1 1] AssaultBaseEquipment
                                  (bind _returnvalue_13 (`|GetDataTableRow` "/Game/TSS_Game/Blueprints/Customization/DT_EQP_WPN_SecondaryPistols.DT_EQP_WPN_SecondaryPistols" "BasePistol")
                                    (:`then`
                                      (`KismetArrayLibrary.Array_AddUnique` (`self.TEMP_PlayerEquipment`) _returnvalue_13)
                                      (bind _returnvalue_14 (`|GetDataTableRow` "/Game/TSS_Game/Blueprints/Customization/DT_EQP_WPN_SecondaryMelee.DT_EQP_WPN_SecondaryMelee" "Chainsword")
                                        (:`then`
                                          (`KismetArrayLibrary.Array_AddUnique` (`self.TEMP_PlayerEquipment`) _returnvalue_14)
                                          (`KismetArrayLibrary.Array_AddUnique` (`self.PlayerUnlocked_Equipment`) _returnvalue_14)
                                          (bind _returnvalue_15 (`|GetDataTableRow` "/Game/TSS_Game/Blueprints/Customization/DT_EQP_Equipment.DT_EQP_Equipment" "MedkitLight")
                                            (:`then`
                                              (`KismetArrayLibrary.Array_AddUnique` (`self.TEMP_PlayerEquipment`) _returnvalue_15)
                                              (`KismetArrayLibrary.Array_AddUnique` (`self.PlayerUnlocked_Equipment`) _returnvalue_15)
                                              (bind _returnvalue_16 (`|GetDataTableRow` "/Game/TSS_Game/Blueprints/Customization/DT_EQP_Chapter.DT_EQP_Chapter" "RelicHealth")
                                                (:`then`
                                                  (`KismetArrayLibrary.Array_AddUnique` (`self.TEMP_PlayerEquipment`) _returnvalue_16)
                                                  (`KismetArrayLibrary.Array_AddUnique` (`self.PlayerUnlocked_Equipment`) _returnvalue_16)
                                                  (bind _returnvalue_17 (`|GetDataTableRow` "/Game/TSS_Game/Blueprints/Customization/DT_EQP_Equipment.DT_EQP_Equipment" "FragGrenade_1")
                                                    (:`then`
                                                      (`KismetArrayLibrary.Array_AddUnique` (`self.TEMP_PlayerEquipment`) _returnvalue_17)
                                                      (`KismetArrayLibrary.Array_AddUnique` (`self.SaveData_Slot1`) (make `/Game/TSS_Game/Blueprints/Customization/ST_SaveGame_CustomizationData` "NewEnumerator1" (`self.TEMP_PlayerCustomizationVisual`) (`self.TEMP_PlayerEquipment`) _returnvalue_17 _returnvalue_15))
                                                      (`KismetArrayLibrary.Array_Clear` (`self.TEMP_PlayerEquipment`)))))))))))))
                                (:`then_2`
                                  ;[1 1 1] Devastator base equipment
                                  (bind _returnvalue_18 (`|GetDataTableRow` "/Game/TSS_Game/Blueprints/Customization/DT_EQP_WPN_Primary.DT_EQP_WPN_Primary" "Heavy_Bolter")
                                    (:`then`
                                      (`KismetArrayLibrary.Array_AddUnique` (`self.TEMP_PlayerEquipment`) _returnvalue_18)
                                      (`KismetArrayLibrary.Array_AddUnique` (`self.PlayerUnlocked_Equipment`) _returnvalue_18)
                                      (bind _returnvalue_19 (`|GetDataTableRow` "/Game/TSS_Game/Blueprints/Customization/DT_EQP_Equipment.DT_EQP_Equipment" "FragGrenade_1")
                                        (:`then`
                                          (`KismetArrayLibrary.Array_AddUnique` (`self.TEMP_PlayerEquipment`) _returnvalue_19)
                                          (bind _returnvalue_20 (`|GetDataTableRow` "/Game/TSS_Game/Blueprints/Customization/DT_EQP_Chapter.DT_EQP_Chapter" "RelicHealth")
                                            (:`then`
                                              (`KismetArrayLibrary.Array_AddUnique` (`self.TEMP_PlayerEquipment`) _returnvalue_20)
                                              (`KismetArrayLibrary.Array_AddUnique` (`self.PlayerUnlocked_Equipment`) _returnvalue_20)
                                              (`KismetArrayLibrary.Array_AddUnique` (`self.SaveData_Slot1`) (make `/Game/TSS_Game/Blueprints/Customization/ST_SaveGame_CustomizationData` "NewEnumerator4" (`self.TEMP_PlayerCustomizationVisual`) (`self.TEMP_PlayerEquipment`) _returnvalue_19))
                                              (`KismetArrayLibrary.Array_Clear` (`self.TEMP_PlayerEquipment`)))))))))
                                (:`then_3`
                                  ;[1 1 1] ApothRange base equipment
                                  (bind _returnvalue_21 (`|GetDataTableRow` "/Game/TSS_Game/Blueprints/Customization/DT_EQP_WPN_Primary.DT_EQP_WPN_Primary" "BaseBolter")
                                    (:`then`
                                      (`KismetArrayLibrary.Array_AddUnique` (`self.TEMP_PlayerEquipment`) _returnvalue_21)
                                      (`KismetArrayLibrary.Array_AddUnique` (`self.PlayerUnlocked_Equipment`) _returnvalue_21)
                                      (bind _returnvalue_22 (`|GetDataTableRow` "/Game/TSS_Game/Blueprints/Customization/DT_EQP_WPN_SecondaryMelee.DT_EQP_WPN_SecondaryMelee" "Narthecium1")
                                        (:`then`
                                          (`KismetArrayLibrary.Array_AddUnique` (`self.TEMP_PlayerEquipment`) _returnvalue_22)
                                          (`KismetArrayLibrary.Array_AddUnique` (`self.PlayerUnlocked_Equipment`) _returnvalue_22)
                                          (bind _returnvalue_23 (`|GetDataTableRow` "/Game/TSS_Game/Blueprints/Customization/DT_EQP_WPN_SecondaryPistols.DT_EQP_WPN_SecondaryPistols" "BasePistol")
                                            (:`then`
                                              (`KismetArrayLibrary.Array_AddUnique` (`self.TEMP_PlayerEquipment`) _returnvalue_23)
                                              (`KismetArrayLibrary.Array_AddUnique` (`self.PlayerUnlocked_Equipment`) _returnvalue_23)
                                              (bind _returnvalue_24 (`|GetDataTableRow` "/Game/TSS_Game/Blueprints/Customization/DT_EQP_Chapter.DT_EQP_Chapter" "RelicHealth")
                                                (:`then`
                                                  (`KismetArrayLibrary.Array_AddUnique` (`self.TEMP_PlayerEquipment`) _returnvalue_24)
                                                  (`KismetArrayLibrary.Array_AddUnique` (`self.PlayerUnlocked_Equipment`) _returnvalue_24)
                                                  (bind _returnvalue_25 (`|GetDataTableRow` "/Game/TSS_Game/Blueprints/Customization/DT_EQP_Equipment.DT_EQP_Equipment" "HealingStimulator")
                                                    (:`then`
                                                      (`KismetArrayLibrary.Array_AddUnique` (`self.TEMP_PlayerEquipment`) _returnvalue_25)
                                                      (`KismetArrayLibrary.Array_AddUnique` (`self.PlayerUnlocked_Equipment`) _returnvalue_25)
                                                      (`KismetArrayLibrary.Array_Clear` (`self.TEMP_PlayerCustomizationVisual`))
                                                      (bind _returnvalue_26 (`|GetDataTableRow` "/Game/TSS_Game/Blueprints/Customization/DT_ArmorList_Helmets.DT_ArmorList_Helmets" "Helmet_MKVII_Apothecary")
                                                        (:`then`
                                                          (`KismetArrayLibrary.Array_Add` (`self.TEMP_PlayerCustomizationVisual`) _returnvalue_26)
                                                          (bind _returnvalue_27 (`|GetDataTableRow` "/Game/TSS_Game/Blueprints/Customization/DT_ArmorList_Backpack.DT_ArmorList_Backpack" "Backpack_Apothecary")
                                                            (:`then`
                                                              (`KismetArrayLibrary.Array_Add` (`self.TEMP_PlayerCustomizationVisual`) _returnvalue_27)
                                                              (bind _returnvalue_28 (`|GetDataTableRow` "/Game/TSS_Game/Blueprints/Customization/DT_ArmorList_Hands.DT_ArmorList_Hands" "BaseHands")
                                                                (:`then`
                                                                  (`KismetArrayLibrary.Array_Add` (`self.TEMP_PlayerCustomizationVisual`) _returnvalue_28)
                                                                  (bind _returnvalue_29 (`|GetDataTableRow` "/Game/TSS_Game/Blueprints/Customization/DT_ArmorList_Legs.DT_ArmorList_Legs" "Legs_MKVII_Apothecary")
                                                                    (:`then`
                                                                      (`KismetArrayLibrary.Array_Add` (`self.TEMP_PlayerCustomizationVisual`) _returnvalue_29)
                                                                      (bind _returnvalue_30 (`|GetDataTableRow` "/Game/TSS_Game/Blueprints/Customization/DT_ArmorList_Shoulders_LT.DT_ArmorList_Shoulders_LT" "BaseLeftShoulder")
                                                                        (:`then`
                                                                          (`KismetArrayLibrary.Array_Add` (`self.TEMP_PlayerCustomizationVisual`) _returnvalue_30)
                                                                          (bind _returnvalue_31 (`|GetDataTableRow` "/Game/TSS_Game/Blueprints/Customization/DT_ArmorList_Shoulders_RT.DT_ArmorList_Shoulders_RT" "BaseRightShoulder")
                                                                            (:`then`
                                                                              (`KismetArrayLibrary.Array_Add` (`self.TEMP_PlayerCustomizationVisual`) _returnvalue_31)
                                                                              (bind _returnvalue_32 (`|GetDataTableRow` "/Game/TSS_Game/Blueprints/Customization/DT_ArmorList_Torso.DT_ArmorList_Torso" "BaseChest")
                                                                                (:`then`
                                                                                  (`KismetArrayLibrary.Array_Add` (`self.TEMP_PlayerCustomizationVisual`) _returnvalue_32)
                                                                                  (`KismetArrayLibrary.Array_Add` (`self.TEMP_PlayerCustomizationVisual`) (make `/Game/TSS_Game/Blueprints/Customization/ST_CustItem` :`Name` "NartheciumNoMelee" :`Icon` null :`SkelMesh` (`|MakeArray` "/Game/Characters/SpaceMarine/BodyParts/Pelvis/IM_XX_PelvisAddLT_ApothecaryReductor01/Models/SK_IM_XX_PelvisAddLT_ApothecaryReductor01.SK_IM_XX_PelvisAddLT_ApothecaryReductor01" "/Game/Characters/SpaceMarine/BodyParts/Pelvis/IM_XX_PelvisAddRT_ApothecaryReductor01/Models/SK_IM_XX_PelvisAddRT_ApothecaryReductor01.SK_IM_XX_PelvisAddRT_ApothecaryReductor01" :!type "SkeletalMesh Object Reference") :`SlotTag` "NewEnumerator10"))
                                                                                  (`KismetArrayLibrary.Array_AddUnique` (`self.SaveData_Slot1`) (make `/Game/TSS_Game/Blueprints/Customization/ST_SaveGame_CustomizationData` "NewEnumerator2" (`self.TEMP_PlayerCustomizationVisual`) (`self.TEMP_PlayerEquipment`) _returnvalue_25))
                                                                                  (`KismetArrayLibrary.Array_Clear` (`self.TEMP_PlayerEquipment`)))))))))))))))))))))))))))
                                (:`then_4`
                                  ;[1 1 1] ApothMeleeBaseEquipment
                                  (bind _returnvalue_33 (`|GetDataTableRow` "/Game/TSS_Game/Blueprints/Customization/DT_EQP_WPN_SecondaryPistols.DT_EQP_WPN_SecondaryPistols" "BasePistol")
                                    (:`then`
                                      (`KismetArrayLibrary.Array_AddUnique` (`self.TEMP_PlayerEquipment`) _returnvalue_33)
                                      (bind _returnvalue_34 (`|GetDataTableRow` "/Game/TSS_Game/Blueprints/Customization/DT_EQP_WPN_SecondaryMelee.DT_EQP_WPN_SecondaryMelee" "Chainsword")
                                        (:`then`
                                          (`KismetArrayLibrary.Array_AddUnique` (`self.TEMP_PlayerEquipment`) _returnvalue_34)
                                          (`KismetArrayLibrary.Array_AddUnique` (`self.PlayerUnlocked_Equipment`) _returnvalue_34)
                                          (bind _returnvalue_35 (`|GetDataTableRow` "/Game/TSS_Game/Blueprints/Customization/DT_EQP_Equipment.DT_EQP_Equipment" "HealingStimulator")
                                            (:`then`
                                              (`KismetArrayLibrary.Array_AddUnique` (`self.TEMP_PlayerEquipment`) _returnvalue_35)
                                              (`KismetArrayLibrary.Array_AddUnique` (`self.PlayerUnlocked_Equipment`) _returnvalue_35)
                                              (bind _returnvalue_36 (`|GetDataTableRow` "/Game/TSS_Game/Blueprints/Customization/DT_EQP_Chapter.DT_EQP_Chapter" "RelicHealth")
                                                (:`then`
                                                  (`KismetArrayLibrary.Array_AddUnique` (`self.TEMP_PlayerEquipment`) _returnvalue_36)
                                                  (`KismetArrayLibrary.Array_AddUnique` (`self.PlayerUnlocked_Equipment`) _returnvalue_36)
                                                  (`KismetArrayLibrary.Array_Clear` (`self.TEMP_PlayerCustomizationVisual`))
                                                  (bind _returnvalue_37 (`|GetDataTableRow` "/Game/TSS_Game/Blueprints/Customization/DT_ArmorList_Helmets.DT_ArmorList_Helmets" "Helmet_MKVII_Apothecary")
                                                    (:`then`
                                                      (`KismetArrayLibrary.Array_Add` (`self.TEMP_PlayerCustomizationVisual`) _returnvalue_37)
                                                      (bind _returnvalue_38 (`|GetDataTableRow` "/Game/TSS_Game/Blueprints/Customization/DT_ArmorList_Backpack.DT_ArmorList_Backpack" "Backpack_Apothecary")
                                                        (:`then`
                                                          (`KismetArrayLibrary.Array_Add` (`self.TEMP_PlayerCustomizationVisual`) _returnvalue_38)
                                                          (bind _returnvalue_39 (`|GetDataTableRow` "/Game/TSS_Game/Blueprints/Customization/DT_ArmorList_Hands.DT_ArmorList_Hands" "BaseHands")
                                                            (:`then`
                                                              (`KismetArrayLibrary.Array_Add` (`self.TEMP_PlayerCustomizationVisual`) _returnvalue_39)
                                                              (bind _returnvalue_40 (`|GetDataTableRow` "/Game/TSS_Game/Blueprints/Customization/DT_ArmorList_Legs.DT_ArmorList_Legs" "Legs_MKVII_Apothecary")
                                                                (:`then`
                                                                  (`KismetArrayLibrary.Array_Add` (`self.TEMP_PlayerCustomizationVisual`) _returnvalue_40)
                                                                  (bind _returnvalue_41 (`|GetDataTableRow` "/Game/TSS_Game/Blueprints/Customization/DT_ArmorList_Shoulders_LT.DT_ArmorList_Shoulders_LT" "BaseLeftShoulder")
                                                                    (:`then`
                                                                      (`KismetArrayLibrary.Array_Add` (`self.TEMP_PlayerCustomizationVisual`) _returnvalue_41)
                                                                      (bind _returnvalue_42 (`|GetDataTableRow` "/Game/TSS_Game/Blueprints/Customization/DT_ArmorList_Shoulders_RT.DT_ArmorList_Shoulders_RT" "BaseRightShoulder")
                                                                        (:`then`
                                                                          (`KismetArrayLibrary.Array_Add` (`self.TEMP_PlayerCustomizationVisual`) _returnvalue_42)
                                                                          (bind _returnvalue_43 (`|GetDataTableRow` "/Game/TSS_Game/Blueprints/Customization/DT_ArmorList_Torso.DT_ArmorList_Torso" "BaseChest")
                                                                            (:`then`
                                                                              (`KismetArrayLibrary.Array_Add` (`self.TEMP_PlayerCustomizationVisual`) _returnvalue_43)
                                                                              (`KismetArrayLibrary.Array_Add` (`self.TEMP_PlayerCustomizationVisual`) (make `/Game/TSS_Game/Blueprints/Customization/ST_CustItem` "NartheciumNoMelee" null (`|MakeArray` "/Game/Characters/SpaceMarine/BodyParts/Pelvis/IM_XX_PelvisAddLT_ApothecaryReductor01/Models/SK_IM_XX_PelvisAddLT_ApothecaryReductor01.SK_IM_XX_PelvisAddLT_ApothecaryReductor01" "/Game/Characters/SpaceMarine/BodyParts/Pelvis/IM_XX_PelvisAddRT_ApothecaryReductor01/Models/SK_IM_XX_PelvisAddRT_ApothecaryReductor01.SK_IM_XX_PelvisAddRT_ApothecaryReductor01" :!type "SkeletalMesh Object Reference") (`|MakeArray` "/Game/WH40Assets/Weapons/Narthecium/SM_Narthecium_v01.SM_Narthecium_v01" :!type "StaticMesh Object Reference") "NewEnumerator10" (`|MakeArray` "joint_ForearmRT" :!type "Name")))
                                                                              (`KismetArrayLibrary.Array_AddUnique` (`self.SaveData_Slot1`) (make `/Game/TSS_Game/Blueprints/Customization/ST_SaveGame_CustomizationData` "NewEnumerator3" (`self.TEMP_PlayerCustomizationVisual`) (`self.TEMP_PlayerEquipment`) _returnvalue_35))
                                                                              (`KismetArrayLibrary.Array_Clear` (`self.TEMP_PlayerEquipment`)))))))))))))))))))))))))))))))))))))))))

(event `ConvertSavedNames`
  (params (PlayerController :type "/Game/TSS_Game/Blueprints/System/BP_PlayerControllerLobby Object Reference"))
  (bind _unlockedequipmentnames (`self.UnlockedEquipmentNames`))
  (if (`KismetArrayLibrary.Array_IsNotEmpty` _unlockedequipmentnames)
    (for _array_element _unlockedequipmentnames
      (bind _st_equipment (`self.F_GetEquipmentTableRow_Workaround` _array_element))
      (`KismetArrayLibrary.Array_AddUnique` (`self.PlayerUnlocked_Equipment`) _st_equipment)))
  (`/Game/TSS_Game/Blueprints/System/BP_PlayerControllerLobby.SavedNamesConverted` PlayerController))

(fn `F_GetEquipmentTableRow_Workaround`
  (params (RowName :type Name))
  (returns (`ST Equipment` :type "/Game/TSS_Game/Blueprints/Customization/ST_EQP_Item Structure"))
  (bind _returnvalue (`|GetDataTableRow` "/Game/TSS_Game/Blueprints/Customization/DT_EQP_WPN_Primary.DT_EQP_WPN_Primary" RowName)
    (:`then`
      (return _returnvalue))
    (:`RowNotFound`
      (bind _returnvalue_2 (`|GetDataTableRow` "/Game/TSS_Game/Blueprints/Customization/DT_EQP_WPN_SecondaryMelee.DT_EQP_WPN_SecondaryMelee" RowName)
        (:`then`
          (return _returnvalue_2))
        (:`RowNotFound`
          (bind _returnvalue_3 (`|GetDataTableRow` "/Game/TSS_Game/Blueprints/Customization/DT_EQP_Equipment.DT_EQP_Equipment" RowName)
            (:`then`
              (return _returnvalue_3))
            (:`RowNotFound`
              (bind _returnvalue_4 (`|GetDataTableRow` "/Game/TSS_Game/Blueprints/Customization/DT_EQP_Chapter.DT_EQP_Chapter" RowName)
                (:`then`
                  (return _returnvalue_4))
                (:`RowNotFound`
                  (bind _returnvalue_5 (`|GetDataTableRow` "/Game/TSS_Game/Blueprints/Customization/DT_EQP_ChapOther.DT_EQP_ChapOther" RowName)
                    (:`then`
                      (return _returnvalue_5))
                    (:`RowNotFound`
                      (bind _returnvalue_6 (`|GetDataTableRow` "/Game/TSS_Game/Blueprints/Customization/DT_EQP_WPN_SecondaryPistols.DT_EQP_WPN_SecondaryPistols" RowName)
                        (:`then`
                          (return _returnvalue_6))
                        (:`RowNotFound`
                          (`KismetSystemLibrary.PrintString` null "BP_Save_PlayerCust: Could not get player equipment from any table!" true true (struct :`R` 1.0 :`A` 1.0) 4.0))))))))))))))