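; Healing stimulator equipment component: a limited-use medkit used on the owner's equipment target, or on the owner if none.
; Slot input passes a state and ammo check, cancels reloading, then plays a self or ally heal montage, mirrored to other clients via server-to-multicast events.
; Montage notifies revive wounded targets and award exp; the local client requests a stackable heal-over-time buff, clears bleeding and toxins, and spends ammo.
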(event `self.ReceiveBeginPlay`
  ;[1 1 1] BeginPlay
  (`parent.ReceiveBeginPlay`))

(event `EnhancedInput|/Game/TSS_Game/Blueprints/EnhancedInput/InputAction_EQP1`
  (params (ActionValue :type Boolean) (ElapsedSeconds :type "Float (double-precision)") (TriggeredSeconds :type "Float (double-precision)") (InputAction :type "InputAction Object Reference" :default "/Game/TSS_Game/Blueprints/EnhancedInput/InputAction_EQP1.InputAction_EQP1"))
  (bind _ownercharref (`self.OwnerCharRef`))
  (bind _player_controller_ref (`self.Player Controller Ref`))
  (bind _targetactor (`self.TargetActor`))
  (bind _ownercharref_2 (`self.OwnerCharRef`))
  (bind _ownercharref_3 (`self.OwnerCharRef`))
  (bind _targetactor_2 (`self.TargetActor`))
  (bind _equippedweapon (`/Game/TSS_Game/Blueprints/System/BP_CharacterBase.EquippedWeapon` _ownercharref))
  (bind _equipment_target (`/Game/TSS_Game/Blueprints/System/BP_CharacterBase.Equipment_Target` (`self.OwnerCharRef`)))
  ;[1 1 1] Throw logic
  (:`Started`
    (bind _canuse (`self.CheckSlotKey` 0))
    (if _canuse
      (if (or (`/Game/TSS_Game/Blueprints/System/BP_CharacterBase.IsMeleeAttacking` _ownercharref) (`/Game/TSS_Game/Blueprints/System/BP_CharacterBase.IsDead` _ownercharref) (`/Game/TSS_Game/Blueprints/System/BP_CharacterBase.IsSprinting?` _ownercharref) (`/Game/TSS_Game/Blueprints/System/BP_CharacterBase.IsEvading?` _ownercharref) (`/Game/TSS_Game/Blueprints/System/BP_CharacterBase.IsUsingEquipment?` _ownercharref) (`/Game/TSS_Game/Blueprints/System/BP_CharacterBase.IsInputDisabled?` _ownercharref)) :!label _label
        _
        (elif (> (`self.AmmoCur`) 0)
          (if (`/Game/TSS_Game/Blueprints/Weapons/Base/BP_WeaponBase.isReloading` _equippedweapon)
            (set `/Game/TSS_Game/Blueprints/Weapons/Base/BP_WeaponBase.isReloading` false _equippedweapon))
          (`/Engine/EditorBlueprintResources/StandardMacros.IsValid` _equipment_target
            (:`Is Valid`
              (bind _asbp_character_base (cast `/Game/TSS_Game/Blueprints/System/BP_CharacterBase` _equipment_target))
              (set `self.TargetActor` _asbp_character_base))
            (:`Is Not Valid`
              (set `self.TargetActor` (`self.OwnerCharRef`))))
          (`self.SV_Use` (`self.TargetActor`))
          (if (== (`self.OwnerCharRef`) (`self.TargetActor`)) :!label _label_2
            (set `self.Montage to Play` "/Game/WH40Assets/SpaceMarines/Animations/Montages/AM_SM_HealSelf.AM_SM_HealSelf")
            (else
              (set `self.Montage to Play` "/Game/WH40Assets/SpaceMarines/Animations/Montages/AM_SM_HealApoth.AM_SM_HealApoth")))
          (bind _notifyname (`|PlayMontage` (`Character.Mesh` _ownercharref_2) (`self.Montage to Play`) 1.2)
            (:`then`
              (`/Game/TSS_Game/Blueprints/System/BP_CharacterBase.Hide WPNIn Main Hand` _ownercharref_2 true)
              (`/Game/TSS_Game/Blueprints/System/BP_CharacterBase.Hide WPNIn Secondary Hand` _ownercharref_2 true)
              (set `/Game/TSS_Game/Blueprints/System/BP_CharacterBase.IsUsingEquipment?` true (`self.OwnerCharRef`)))
            (:`OnCompleted`
              (`/Game/TSS_Game/Blueprints/System/BP_CharacterBase.Hide WPNIn Main Hand` _ownercharref_2 false :!label _label_3)
              (`/Game/TSS_Game/Blueprints/System/BP_CharacterBase.Hide WPNIn Secondary Hand` _ownercharref_2 false)
              (set `/Game/TSS_Game/Blueprints/System/BP_CharacterBase.IsUsingEquipment?` false (`self.OwnerCharRef`)))
            (:`OnInterrupted`
              (goto _label_3))
            (:`OnNotifyBegin`
              (if (`/Game/TSS_Game/Blueprints/System/BP_CharacterBase.IsWounded?` _targetactor_2)
                (`/Game/TSS_Game/Blueprints/System/BP_CharacterBase.LC_WoundedHealed` _targetactor_2 1.3)
                (`self.LC_AddExpToOwner`))
              (if (and (== _notifyname "Heal_start") (`Pawn.IsLocallyControlled` (`self.OwnerCharRef`)))
                (message `/Game/TSS_Game/Blueprints/AbilitySystem/BuffSystem/Base/BPI_Buffable.Attach Buff Request` (`self.Player Controller Ref`) (make `/Game/TSS_Game/Blueprints/AbilitySystem/BuffSystem/ST_BuffSettingsMSG` (`self.TargetActor`) "/Game/TSS_Game/Blueprints/AbilitySystem/BuffSystem/AC_Buff_Healing.AC_Buff_Healing_C" 1 (`self.OwnerCharRef`) true -6.0 -6.0 5.0 1.0))
                (set `/Game/TSS_Game/Blueprints/System/BP_CharacterBase.IsUsingEquipment?` false _ownercharref_3)
                (if (`/Game/TSS_Game/Blueprints/System/BP_CharacterBase.IsWounded?` (`self.TargetActor`))
                  (`/Game/TSS_Game/Blueprints/System/BP_CharacterBase.Speech_Say` _ownercharref_3 "NewEnumerator9" false 80.0)
                  (else
                    (`/Game/TSS_Game/Blueprints/System/BP_CharacterBase.Speech_Say` _ownercharref_3 "NewEnumerator3" false 80.0)))
                (`/Engine/EditorBlueprintResources/StandardMacros.DecrementInt` (`self.AmmoCur`)
                  (:`  `
                    (message `/Game/TSS_Game/Blueprints/AbilitySystem/BuffSystem/Base/BPI_Buffable.Detach Buff Request` _player_controller_ref "/Game/TSS_Game/Blueprints/AbilitySystem/BuffSystem/AC_Buff_Bleeding.AC_Buff_Bleeding_C" _targetactor false)
                    (message `/Game/TSS_Game/Blueprints/AbilitySystem/BuffSystem/Base/BPI_Buffable.Detach Buff Request` _player_controller_ref "/Game/TSS_Game/Blueprints/AbilitySystem/BuffSystem/AC_Buff_Toxins.AC_Buff_Toxins_C" _targetactor false))))))
          (else
            (`GameplayStatics.PlaySound2D` "/Game/TSS_Game/SFX/UI/SC_ERROR.SC_ERROR" 1.0 1.0 0.0 null null)))))))

(event `EnhancedInput|/Game/TSS_Game/Blueprints/EnhancedInput/InputAction_EQP2`
  (params (ActionValue :type Boolean) (ElapsedSeconds :type "Float (double-precision)") (TriggeredSeconds :type "Float (double-precision)") (InputAction :type "InputAction Object Reference" :default "/Game/TSS_Game/Blueprints/EnhancedInput/InputAction_EQP2.InputAction_EQP2"))
  ;[1 1 1] Throw logic
  (:`Started`
    (bind _canuse (`self.CheckSlotKey` 1))
    (if _canuse
      (goto _label))))

(event `SV_Use`
  (params (TargetActor :type "/Game/TSS_Game/Blueprints/System/BP_CharacterBase Object Reference"))
  ;[1 1 1] Throw logic
  (`self.MC_Use` TargetActor))

(event `MC_Use`
  (params (TargetActor :type "/Game/TSS_Game/Blueprints/System/BP_CharacterBase Object Reference"))
  ;[1 1 1] Throw logic
  (if (not (`Pawn.IsLocallyControlled` (`self.OwnerCharRef`)))
    (set `self.TargetActor` TargetActor)
    (goto _label_2)))