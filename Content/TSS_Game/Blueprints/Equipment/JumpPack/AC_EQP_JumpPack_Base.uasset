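; Base jump pack equipment component for a fuel-limited leap to the cursor, ending in a ground-slam AOE scaled from melee weapon damage.
; Holding the equipment key shows a mouse-following marker; release launches the character up, then toward the target via montages, ignoring pawn collision.
; A capsule hit triggers the slam and restores collision.
; The owning client drives jump and landing, mirrored through server-to-multicast events; fuel recharges after a delay.
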(event `self.ReceiveBeginPlay`
  (bind _ownercharref (`self.OwnerCharRef`))
  ;[1 1 1] BeginPlay
  (`parent.ReceiveBeginPlay`)
  (set `/Game/TSS_Game/Blueprints/System/BP_CharacterBase.EvadeRollMontage` "/Game/WH40Assets/SpaceMarines/Animations/Montages/AS_SM_JumpPack_Evade_N.AS_SM_JumpPack_Evade_N" _ownercharref)
  (set `/Game/TSS_Game/Blueprints/System/BP_CharacterBase.IsJumppack` true _ownercharref)
  (add `PrimitiveComponent.OnComponentHit` (`Character.CapsuleComponent` _ownercharref) (delegate `OnCapsuleHit`))
  (set `/Game/TSS_Game/Blueprints/System/BP_CharacterBase.JumpPackRef` self _ownercharref))

(event `OnCapsuleHit`
  (params (HitComponent :type "PrimitiveComponent Object Reference") (OtherActor :type "Actor Object Reference") (OtherComp :type "PrimitiveComponent Object Reference") (NormalImpulse :type "Vector Structure") (Hit :type "HitResult Structure (by ref)"))
  (bind _ownercharref (`self.OwnerCharRef`))
  (bind _ownercharref_2 (`self.OwnerCharRef`))
  (bind _wpn_melee (`/Game/TSS_Game/Blueprints/System/BP_CharacterBase.WPN_Melee` _ownercharref))
  (bind _returnvalue (`SceneComponent.K2_GetComponentLocation` (`Character.Mesh` _ownercharref_2)))
  ;[1 1 1] Hit after jump
  (if (`Pawn.IsLocallyControlled` (`self.OwnerCharRef`))
    (`/Engine/EditorBlueprintResources/StandardMacros.DoOnce` true :!label _label
      (:`Completed`
        (`self.SV_HitEvent`)
        (`Character.LaunchCharacter` _ownercharref_2 (0.0 0.0 -5000.0) false true :!label _label_2)
        (`Character.PlayAnimMontage` _ownercharref_2 "/Game/WH40Assets/SpaceMarines/Animations/Montages/AS_SM_JumpPack_FlyHit.AS_SM_JumpPack_FlyHit" 1.5 "None")
        (`self.JumpFinish`)
        (bind _outhit (`KismetSystemLibrary.LineTraceSingleForObjects` _returnvalue (- _returnvalue (0.0 0.0 10000.0)) (`|MakeArray` "ObjectTypeQuery1" "ObjectTypeQuery2" :!type "EObjectTypeQuery Enum")))
        (bind (_bblockinghit _binitialoverlap _time _distance _location) (`GameplayStatics.BreakHitResult` _outhit))
        (`NiagaraFunctionLibrary.SpawnSystemAtLocation` "/Game/VFX/Upgrade/N_AS_Smoke_Placement_Square.N_AS_Smoke_Placement_Square" _location)
        (`/Engine/EditorBlueprintResources/StandardMacros.IsValid` _wpn_melee
          (:`Is Valid`
            (`|SpawnActorFromClass` "/Game/TSS_Game/Blueprints/Weapons/Base/BP_JumpPackLand_AOE.BP_JumpPackLand_AOE_C" (`KismetMathLibrary.Conv_VectorToTransform` _location) "AlwaysSpawn" "MultiplyWithRoot" null "NewEnumerator0" (`self.Player Controller Ref`) _ownercharref (* (`/Game/TSS_Game/Blueprints/Weapons/Base/BP_WeaponBase.DamageMin` _wpn_melee) (`self.DamageMultiplier`)) (* (`/Game/TSS_Game/Blueprints/Weapons/Base/BP_WeaponBase.DamageMax` _wpn_melee) (`self.DamageMultiplier`)) (`/Game/TSS_Game/Blueprints/Weapons/Base/BP_WeaponBase.CritChance` _wpn_melee) (`/Game/TSS_Game/Blueprints/Weapons/Base/BP_WeaponBase.CritMultiplier` _wpn_melee) null) ; Always damages as melee
            (`self.SetIsReplicated` (`Character.CharacterMovement` _ownercharref) true)))))))

(event `SV_HitEvent`
  ;[1 1 1] Throw logic
  (`self.MC_HitEvent`))

(event `MC_HitEvent`
  ;[1 1 1] Throw logic
  (if (not (`Pawn.IsLocallyControlled` (`self.OwnerCharRef`)))
    (goto _label_2)))

(event `EnhancedInput|/Game/TSS_Game/Blueprints/EnhancedInput/InputAction_EQP1`
  (params (ActionValue :type Boolean) (ElapsedSeconds :type "Float (double-precision)") (TriggeredSeconds :type "Float (double-precision)") (InputAction :type "InputAction Object Reference" :default "/Game/TSS_Game/Blueprints/EnhancedInput/InputAction_EQP1.InputAction_EQP1"))
  (bind _ownercharref (`self.OwnerCharRef`))
  (bind _ownercharref_2 (`self.OwnerCharRef`))
  (bind _ownercharref_3 (`self.OwnerCharRef`))
  (bind _ownercharref_4 (`self.OwnerCharRef`))
  (bind _ownercharref_5 (`self.OwnerCharRef`))
  (bind _ownercharref_6 (`self.OwnerCharRef`))
  (bind _ownercharref_7 (`self.OwnerCharRef`))
  (bind _ownercharref_8 (`self.OwnerCharRef`))
  (bind _ownercharref_9 (`self.OwnerCharRef`))
  (bind _equippedweapon (`/Game/TSS_Game/Blueprints/System/BP_CharacterBase.EquippedWeapon` _ownercharref))
  (bind _mesh (`Character.Mesh` _ownercharref_3))
  (bind _mesh_2 (`Character.Mesh` _ownercharref_5))
  (bind _mouselocation (`/Game/TSS_Game/Blueprints/System/BP_CharacterBase.MouseLocation` _ownercharref_9))
  ;[1 1 1] Throw logic
  (:`Started`
    (bind _canuse (`self.CheckSlotKey` 0))
    (if _canuse
      (if (>= (`self.Fuel Current`) (`self.FuelUsedHeavyJump`)) :!label _label_3
        (bind _returnvalue (`|SpawnActorFromClass` "/Game/TSS_Game/Blueprints/Equipment/JumpPack/BP_JumpPack_Target.BP_JumpPack_Target_C" (`KismetMathLibrary.Conv_VectorToTransform` _mouselocation) "Undefined" "MultiplyWithRoot" null null))
        (bind _output_get (set `self.TargetMarker` _returnvalue))
        (`KismetSystemLibrary.K2_SetTimer` null "CalculatePath" (`self.PredictPathDuration`) true)
        (`Actor.SetActorHiddenInGame` _output_get true)
        (else
          (`self.RemoveTargetMarker`)
          (`GameplayStatics.PlaySound2D` "/Game/TSS_Game/SFX/UI/SC_ERROR.SC_ERROR" 1.0 1.0 0.0 null null)))))
  (:`Completed`
    (bind _canuse_2 (`self.CheckSlotKey` 0))
    (if _canuse_2
      (if (>= (`self.Fuel Current`) (`self.FuelUsedHeavyJump`)) :!label _label_4
        (if (or (`/Game/TSS_Game/Blueprints/System/BP_CharacterBase.IsMeleeAttacking` _ownercharref) (`/Game/TSS_Game/Blueprints/System/BP_CharacterBase.IsDead` _ownercharref) (`/Game/TSS_Game/Blueprints/System/BP_CharacterBase.IsEvading?` _ownercharref) (`/Game/TSS_Game/Blueprints/System/BP_CharacterBase.IsInputDisabled?` _ownercharref))
          (`self.RemoveTargetMarker` :!label _label_5)
          (elif (> (`self.AmmoCur`) 0)
            (set `/Game/TSS_Game/Blueprints/System/BP_CharacterBase.IsMeleeAttacking` true _ownercharref)
            (if (`/Game/TSS_Game/Blueprints/Weapons/Base/BP_WeaponBase.isReloading` _equippedweapon)
              (set `/Game/TSS_Game/Blueprints/Weapons/Base/BP_WeaponBase.isReloading` false _equippedweapon))
            (if (`/Game/TSS_Game/Blueprints/System/BP_CharacterBase.IsSprinting?` _ownercharref)
              (`/Game/TSS_Game/Blueprints/System/BP_CharacterBase.SprintEnd` _ownercharref true false))
            (`/Game/TSS_Game/Blueprints/System/BP_CharacterBase.InstantRotationToMouse` _ownercharref_9)
            (bind _output_get_2 (set `self.JumpTarget` _mouselocation))
            (bind _output_get_3 (set `self.JumpStart` (`SceneComponent.K2_GetComponentLocation` (`Character.Mesh` _ownercharref_9))))
            (`self.SV_JumpBegin` _output_get_2 _output_get_3)
            (`self.RemoveTargetMarker`)
            (`/Game/TSS_Game/Blueprints/System/BP_CharacterBase.CustomDisableInput` _ownercharref_8 2.5)
            (`self.SpendFuel` (`self.FuelUsedHeavyJump`))
            (`self.SetIsReplicated` (`Character.CharacterMovement` _ownercharref_8) false)
            (bind _notifyname (`|PlayMontage` (`Character.Mesh` _ownercharref_8) "/Game/WH40Assets/SpaceMarines/Animations/Montages/AS_SM_JumpPack_FlyUp.AS_SM_JumpPack_FlyUp")
              (:`OnCompleted`
                (`|ExecutionSequence`
                  (:`then_0`
                    (goto _label :!via `Reset`))
                  (:`then_1`
                    (`|PlayMontage` (`Character.Mesh` _ownercharref_7) "/Game/WH40Assets/SpaceMarines/Animations/Montages/AS_SM_JumpPack_FlyDown.AS_SM_JumpPack_FlyDown" :!label _label_6
                      (:`then`
                        (`Character.LaunchCharacter` (`self.OwnerCharRef`) (* (`KismetMathLibrary.GetForwardVector` (`KismetMathLibrary.FindLookAtRotation` (`SceneComponent.K2_GetComponentLocation` (`Character.CapsuleComponent` _ownercharref_7)) (`self.JumpTarget`))) (`self.SideVelocity`)) false false)
                        (`SceneComponent.K2_AttachToComponent` (`/Game/TSS_Game/Blueprints/System/BP_CharacterBase.Exhaust1` _ownercharref_3) _mesh "joint_Thruster_LTSocket" "KeepRelative" "KeepRelative" "KeepRelative" true)
                        (`SceneComponent.K2_AttachToComponent` (`/Game/TSS_Game/Blueprints/System/BP_CharacterBase.Exhaust2` _ownercharref_3) _mesh "joint_Thruster_RTSocket" "KeepRelative" "KeepRelative" "KeepRelative" true)
                        (`self.Activate` (`/Game/TSS_Game/Blueprints/System/BP_CharacterBase.Exhaust1` _ownercharref_2) true)
                        (`self.Activate` (`/Game/TSS_Game/Blueprints/System/BP_CharacterBase.Exhaust2` _ownercharref_2) true))))))
              (:`OnNotifyBegin`
                (if (== _notifyname "Jump_Start")
                  (for _array_element (`|MakeArray` (`Character.CapsuleComponent` _ownercharref_6) (`Character.Mesh` _ownercharref_6) :!type "PrimitiveComponent Object Reference") :!label _label_7
                    (`PrimitiveComponent.SetCollisionResponseToChannel` _array_element "ECC_GameTraceChannel2" "ECR_Ignore")
                    (`PrimitiveComponent.SetCollisionResponseToChannel` _array_element "ECC_Pawn" "ECR_Ignore")
                    (`PrimitiveComponent.SetCollisionResponseToChannel` _array_element "ECC_WorldDynamic" "ECR_Ignore"))
                  (`Character.LaunchCharacter` _ownercharref_7 (`KismetMathLibrary.MakeVector` 0.0 0.0 (`self.UpVelocity`)) false false)
                  (`Character.LaunchCharacter` (`self.OwnerCharRef`) (`KismetMathLibrary.MakeVector` 0.0 0.0 (`self.UpVelocity`)) false false)
                  (`SceneComponent.K2_AttachToComponent` (`/Game/TSS_Game/Blueprints/System/BP_CharacterBase.Exhaust1` _ownercharref_5) _mesh_2 "joint_Thruster_LTSocket" "KeepRelative" "KeepRelative" "KeepRelative" true)
                  (`SceneComponent.K2_AttachToComponent` (`/Game/TSS_Game/Blueprints/System/BP_CharacterBase.Exhaust2` _ownercharref_5) _mesh_2 "joint_Thruster_RTSocket" "KeepRelative" "KeepRelative" "KeepRelative" true)
                  (`self.Activate` (`/Game/TSS_Game/Blueprints/System/BP_CharacterBase.Exhaust1` _ownercharref_4) true)
                  (`self.Activate` (`/Game/TSS_Game/Blueprints/System/BP_CharacterBase.Exhaust2` _ownercharref_4) true)
                  (`NiagaraFunctionLibrary.SpawnSystemAtLocation` "/Game/VFX/Upgrade/N_AS_Smoke_Placement_Square.N_AS_Smoke_Placement_Square" (`self.JumpStart`)))))
            (else
              (`GameplayStatics.PlaySound2D` "/Game/TSS_Game/SFX/UI/SC_ERROR.SC_ERROR" 1.0 1.0 0.0 null null)
              (goto _label_5))))
        (else
          (`self.RemoveTargetMarker`)
          (`GameplayStatics.PlaySound2D` "/Game/TSS_Game/SFX/UI/SC_ERROR.SC_ERROR" 1.0 1.0 0.0 null null))))))

(event `EnhancedInput|/Game/TSS_Game/Blueprints/EnhancedInput/InputAction_EQP2`
  (params (ActionValue :type Boolean) (ElapsedSeconds :type "Float (double-precision)") (TriggeredSeconds :type "Float (double-precision)") (InputAction :type "InputAction Object Reference" :default "/Game/TSS_Game/Blueprints/EnhancedInput/InputAction_EQP2.InputAction_EQP2"))
  ;[1 1 1] Throw logic
  (:`Started`
    (bind _canuse (`self.CheckSlotKey` 1))
    (if _canuse
      (goto _label_3)))
  (:`Completed`
    (bind _canuse_2 (`self.CheckSlotKey` 1))
    (if _canuse_2
      (goto _label_4))))

(event `JumpFinish`
  (bind _ownercharref (`self.OwnerCharRef`))
  ;[1 1 1] Throw logic
  (for _array_element (`|MakeArray` (`Character.CapsuleComponent` _ownercharref) (`Character.Mesh` _ownercharref) :!type "PrimitiveComponent Object Reference")
    (`PrimitiveComponent.SetCollisionResponseToChannel` _array_element "ECC_GameTraceChannel2" "ECR_Block")
    (`PrimitiveComponent.SetCollisionResponseToChannel` _array_element "ECC_Pawn" "ECR_Block")
    (`PrimitiveComponent.SetCollisionResponseToChannel` _array_element "ECC_WorldDynamic" "ECR_Block"))
  (`KismetSystemLibrary.Delay` 1.0)
  (set `/Game/TSS_Game/Blueprints/System/BP_CharacterBase.IsMeleeAttacking` false (`self.OwnerCharRef`)))

(event `SV_JumpBegin`
  (params (JumpTarget :type "Vector Structure") (JumpStart :type "Vector Structure"))
  ;[1 1 1] Throw logic
  (`self.MC_JumpBegin` JumpTarget JumpStart))

(event `MC_JumpBegin`
  (params (JumpTarget :type "Vector Structure") (JumpStart :type "Vector Structure"))
  (bind _ownercharref (`self.OwnerCharRef`))
  ;[1 1 1] Throw logic
  (if (not (`Pawn.IsLocallyControlled` (`self.OwnerCharRef`)))
    (set `/Game/TSS_Game/Blueprints/System/BP_CharacterBase.IsMeleeAttacking` true (`self.OwnerCharRef`))
    (`/Engine/EditorBlueprintResources/StandardMacros.IsValid` _ownercharref
      (:`Is Valid`
        (set `self.JumpTarget` JumpTarget)
        (set `self.JumpStart` JumpStart)
        (bind _notifyname (`|PlayMontage` (`Character.Mesh` _ownercharref) "/Game/WH40Assets/SpaceMarines/Animations/Montages/AS_SM_JumpPack_FlyUp.AS_SM_JumpPack_FlyUp")
          (:`OnCompleted`
            (goto _label_6))
          (:`OnNotifyBegin`
            (if (== _notifyname "Jump_Start")
              (goto _label_7))))))))

(event `self.SpendFuel`
  (params (SpentFuel :type "Float (double-precision)"))
  ;[1 1 1] Fuel usage
  (`parent.SpendFuel` SpentFuel)
  (`self.FuelResetDelayTimer`))

(event `RemoveTargetMarker`
  (bind _targetmarker (`self.TargetMarker`))
  ;[1 1 1] CalculatePath
  (`/Engine/EditorBlueprintResources/StandardMacros.IsValid` _targetmarker
    (:`Is Valid`
      (`Actor.K2_DestroyActor` _targetmarker))))

(event `CalculatePath`
  (bind _ownercharref (`self.OwnerCharRef`))
  (bind _targetmarker (`self.TargetMarker`))
  ;[1 1 1] CalculatePath
  (if (or (`/Game/TSS_Game/Blueprints/System/BP_CharacterBase.IsMeleeAttacking` _ownercharref) (`/Game/TSS_Game/Blueprints/System/BP_CharacterBase.IsEvading?` _ownercharref) (`/Game/TSS_Game/Blueprints/System/BP_CharacterBase.IsInputDisabled?` _ownercharref))
    (`/Engine/EditorBlueprintResources/StandardMacros.IsValid` _targetmarker
      (:`Is Valid`
        (`Actor.SetActorHiddenInGame` _targetmarker true)))
    (else
      (`/Engine/EditorBlueprintResources/StandardMacros.IsValid` (`self.OwnerCharRef`)
        (:`Is Valid`
          (`/Engine/EditorBlueprintResources/StandardMacros.IsValid` _targetmarker
            (:`Is Valid`
              (`Actor.SetActorHiddenInGame` _targetmarker false)
              (`Actor.K2_TeleportTo` :`self` _targetmarker :`DestLocation` (`/Game/TSS_Game/Blueprints/System/BP_CharacterBase.MouseLocation` (`self.OwnerCharRef`))))))))))

(event `FuelResetDelayTimer`
  ;[1 1 1] Fuel usage
  (`self.FuelStopRecharge`)
  (`KismetSystemLibrary.K2_SetTimerDelegate` (delegate `FuelRechargeBegin`) (`self.FuelRechargeDelay`)))

(event `FuelRechargeBegin`
  ;[1 1 1] Fuel usage
  (if (not (`/Game/TSS_Game/Blueprints/System/BP_CharacterBase.IsDead` (`self.OwnerCharRef`)))
    (`KismetSystemLibrary.K2_SetTimerDelegate` (delegate `FuelRechargeTick`) (`self.FuelRechargeSpeed`) true)))

(event `FuelRechargeTick`
  (bind _fuelmax (`self.FuelMax`))
  ;[1 1 1] Fuel usage
  (if (>= (`self.Fuel Current`) _fuelmax)
    (`self.FuelStopRecharge`)
    (else
      (set `self.Fuel Current` (`KismetMathLibrary.FClamp` (+ (`self.Fuel Current`) 1.0) 0.0 _fuelmax)))))

(event `FuelStopRecharge`
  ;[1 1 1] Fuel usage
  (`KismetSystemLibrary.K2_PauseTimer` null "FuelRechargeTick"))