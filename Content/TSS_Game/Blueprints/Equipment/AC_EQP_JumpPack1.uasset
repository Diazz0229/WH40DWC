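; Jump pack equipment component that, on BeginPlay, gives the owning character the jump pack evade montage and sets its IsJumppack flag.
; It also carries grenade-throw logic with mouse-distance pitch, predicted-path markers and server-to-multicast replication, but local throw and preview chains are disconnected.
; Slot inputs still reach CheckIfCanThrow on release, which can set IsMeleeAttacking, cancel reloading or play an error sound without launching anything.
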(event `CalculatePath`
  ;[1 1 1] Predict throw path
)

(event `self.ReceiveBeginPlay`
  (bind _ownercharref (`self.OwnerCharRef`))
  ;[1 1 1] BeginPlay
  (`parent.ReceiveBeginPlay`)
  (set `/Game/TSS_Game/Blueprints/System/BP_CharacterBase.EvadeRollMontage` "/Game/WH40Assets/SpaceMarines/Animations/Montages/AS_SM_JumpPack_Evade_N.AS_SM_JumpPack_Evade_N" _ownercharref)
  (set `/Game/TSS_Game/Blueprints/System/BP_CharacterBase.IsJumppack` true _ownercharref))

(event `EnhancedInput|/Game/TSS_Game/Blueprints/EnhancedInput/InputAction_EQP1`
  (params (ActionValue :type Boolean) (ElapsedSeconds :type "Float (double-precision)") (TriggeredSeconds :type "Float (double-precision)") (InputAction :type "InputAction Object Reference" :default "/Game/TSS_Game/Blueprints/EnhancedInput/InputAction_EQP1.InputAction_EQP1"))
  (bind _ownercharref (`self.OwnerCharRef`))
  (bind _equippedweapon (`/Game/TSS_Game/Blueprints/System/BP_CharacterBase.EquippedWeapon` _ownercharref))
  ;[1 1 1] Throw logic
  (:`Started`
    (bind _canuse (`self.CheckSlotKey` 0))
    (if _canuse
      (if (> (`self.AmmoCur`) 0) :!label _label
        _)))
  (:`Completed`
    (bind _canuse_2 (`self.CheckSlotKey` 0))
    (if _canuse_2
      (`KismetSystemLibrary.K2_PauseTimer` null "CalculatePath" :!label _label_2)
      (if (or (`/Game/TSS_Game/Blueprints/System/BP_CharacterBase.IsMeleeAttacking` _ownercharref) (`/Game/TSS_Game/Blueprints/System/BP_CharacterBase.IsDead` _ownercharref) (`/Game/TSS_Game/Blueprints/System/BP_CharacterBase.IsSprinting?` _ownercharref) (`/Game/TSS_Game/Blueprints/System/BP_CharacterBase.IsEvading?` _ownercharref))
        _
        (elif (> (`self.AmmoCur`) 0)
          (set `/Game/TSS_Game/Blueprints/System/BP_CharacterBase.IsMeleeAttacking` true _ownercharref)
          (if (`/Game/TSS_Game/Blueprints/Weapons/Base/BP_WeaponBase.isReloading` _equippedweapon)
            (set `/Game/TSS_Game/Blueprints/Weapons/Base/BP_WeaponBase.isReloading` false _equippedweapon))
          (else
            (`GameplayStatics.PlaySound2D` "/Game/TSS_Game/SFX/UI/SC_ERROR.SC_ERROR" 1.0 1.0 0.0 null null)))))))

(event `EnhancedInput|/Game/TSS_Game/Blueprints/EnhancedInput/InputAction_EQP2`
  (params (ActionValue :type Boolean) (ElapsedSeconds :type "Float (double-precision)") (TriggeredSeconds :type "Float (double-precision)") (InputAction :type "InputAction Object Reference" :default "/Game/TSS_Game/Blueprints/EnhancedInput/InputAction_EQP2.InputAction_EQP2"))
  ;[1 1 1] Throw logic
  (:`Started`
    (bind _canuse (`self.CheckSlotKey` 1))
    (if _canuse
      (goto _label)))
  (:`Completed`
    (bind _canuse_2 (`self.CheckSlotKey` 1))
    (if _canuse_2
      (goto _label_2))))

(event `SV_ThrowGrenade`
  (params (ThrowTopAngle :type "Float (single-precision)"))
  ;[1 1 1] Throw logic
  (`self.MC_ThrowGrenade` ThrowTopAngle))

(event `MC_ThrowGrenade`
  (params (ThrowTopAngle :type "Float (single-precision)"))
  (bind _ownercharref (`self.OwnerCharRef`))
  (bind _ownercharref_2 (`self.OwnerCharRef`))
  (bind (_returnvalue_roll _returnvalue_pitch _returnvalue_yaw) (`KismetMathLibrary.BreakRotator` (`SceneComponent.K2_GetComponentRotation` (`Character.CapsuleComponent` _ownercharref_2))))
  ;[1 1 1] Throw logic
  (set `self.ThrowTopAngle` ThrowTopAngle)
  (`/Engine/EditorBlueprintResources/StandardMacros.IsValid` _ownercharref
    (:`Is Valid`
      (if (not (`Pawn.IsLocallyControlled` _ownercharref))
        (`self.Hide WPNIn Secondary Hand` false)
        (bind _notifyname (`|PlayMontage` (`Character.Mesh` (`self.OwnerCharRef`)) "/Game/WH40Assets/SpaceMarines/Animations/Montages/AM_SM_GrenadeThrow.AM_SM_GrenadeThrow")
          (:`OnCompleted`
            (`self.Hide WPNIn Secondary Hand` false :!label _label_3))
          (:`OnInterrupted`
            (goto _label_3))
          (:`OnNotifyBegin`
            (if (== _notifyname "Throw_start")
              (`|SpawnActorFromClass` "/Game/TSS_Game/Blueprints/Equipment/Grenades/BP_EQP_Grenade_Frag.BP_EQP_Grenade_Frag_C" (`KismetMathLibrary.MakeTransform` (`SceneComponent.K2_GetComponentLocation` (`/Game/TSS_Game/Blueprints/System/BP_CharacterBase.BulletSpawnLocation` _ownercharref_2)) (`KismetMathLibrary.MakeRotator` _returnvalue_roll (`self.ThrowTopAngle`) _returnvalue_yaw)) "Undefined" "MultiplyWithRoot" null 99.0 (`self.Projectile Velocity`) 5.0 2.0 (`self.Damage Type`) 2.0 (`self.OwnerCharRef`) 150.0 null))))))))