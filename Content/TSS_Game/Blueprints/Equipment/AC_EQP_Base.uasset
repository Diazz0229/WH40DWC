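; Base actor component for character equipment, holding shared ammo, fuel, damage and crit stats.
; On BeginPlay it caches default stats, optionally spawns its visual actor on a mesh socket, fills ammo and triggers the customizable character's next equipment attachment.
; For locally controlled, activatable equipment, it matches its class to the controller's slots, registers on the character, then updates HUD and perk classes.
; SpendFuel clamps fuel; input handlers are empty stubs.
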(event `self.ReceiveBeginPlay`
  (bind _ownercharref (`self.OwnerCharRef`))
  (bind _ownercharref_2 (`self.OwnerCharRef`))
  ;[1 1 1] BeginPlay
  (bind _asbp_character_base (cast `/Game/TSS_Game/Blueprints/System/BP_CharacterBase` (`self.GetOwner`)))
  (bind _output_get (set `self.OwnerCharRef` _asbp_character_base))
  (set `self.Crit Chance_Default` (`self.Crit Chance`))
  (set `self.FuelMax_Default` (`self.FuelMax`))
  (set `self.DamageMin_Default` (`self.DamageMin`))
  (set `self.DamageMax_Default` (`self.DamageMax`))
  (set `self.Crit Multiplier_Default` (`self.Crit Multiplier`))
  (set `self.AmmoMax_Default` (`self.AmmoMax`))
  (if (`self.IsVisuallyAttached?`)
    (`self.EQP Show Equipment` (`self.AttachedSocket`) _output_get))
  (set `self.AmmoCur` (`self.AmmoMax`))
  (bind _asbp_character_cust_v_1 (cast `/Game/TSS_Game/Blueprints/System/BP_Character_Cust_v1` _ownercharref))
  (`/Game/TSS_Game/Blueprints/System/BP_Character_Cust_v1.AttachNextEquipment` _asbp_character_cust_v_1)
  (if (and (`Pawn.IsLocallyControlled` _ownercharref) (`self.IsActivatable?`))
    (bind _asbp_player_controller (cast `/Game/TSS_Game/Blueprints/System/BP_PlayerController` (`GameplayStatics.GetPlayerController` 0)))
    (bind _output_get_2 (set `self.Player Controller Ref` _asbp_player_controller))
    (for (_array_element _array_index) (`/Game/TSS_Game/Blueprints/System/BP_PlayerController.EQP_Slots` _output_get_2)
      (bind (_name _icon _description _equipmentcomponent) (break `/Game/TSS_Game/Blueprints/Customization/ST_EQP_Item` _array_element))
      (if (== (`GameplayStatics.GetObjectClass` self) _equipmentcomponent)
        (`KismetArrayLibrary.Array_Set` (`/Game/TSS_Game/Blueprints/System/BP_CharacterBase.EQP_Slots` (`self.OwnerCharRef`)) _array_index self true)
        (set `self.EQP Name` _name)
        (set `self.CharUsedSlot` (- _array_index 1))))
    (`/Game/TSS_Game/UI/GameHUD/W_PlayerHUD.UpdateEQPSlots` (`/Game/TSS_Game/Blueprints/System/BP_PlayerController.PlayerHUD` (`/Game/TSS_Game/Blueprints/System/BP_CharacterBase.OwningPlayerController` _ownercharref_2)))
    (`/Game/TSS_Game/Blueprints/System/BP_CharacterBase.UpdatePerkClasses` _ownercharref_2 self (`self.PerkClasses`))))

(event `EnhancedInput|/Game/TSS_Game/Blueprints/EnhancedInput/InputAction_EQP1`
  (params (ActionValue :type Boolean) (ElapsedSeconds :type "Float (double-precision)") (TriggeredSeconds :type "Float (double-precision)") (InputAction :type "InputAction Object Reference" :default "/Game/TSS_Game/Blueprints/EnhancedInput/InputAction_EQP1.InputAction_EQP1"))
  ;[1 1 1] BeginPlay
)

(event `EnhancedInput|/Game/TSS_Game/Blueprints/EnhancedInput/InputAction_EQP2`
  (params (ActionValue :type Boolean) (ElapsedSeconds :type "Float (double-precision)") (TriggeredSeconds :type "Float (double-precision)") (InputAction :type "InputAction Object Reference" :default "/Game/TSS_Game/Blueprints/EnhancedInput/InputAction_EQP2.InputAction_EQP2")))

(event `SpendFuel`
  (params (SpentFuel :type "Float (double-precision)"))
  (set `self.Fuel Current` (`KismetMathLibrary.FClamp` (- (`self.Fuel Current`) SpentFuel) 0.0 (`self.FuelMax`))))

(fn `CheckSlotKey`
  (params (KeyIndex :type Integer))
  (returns (CanUse :type Boolean))
  (return (== (`self.CharUsedSlot`) KeyIndex)))

(fn `EQP Show Equipment`
  (params (Socket :type Name) (PawnSlot :type "/Game/TSS_Game/Blueprints/System/BP_CharacterBase Object Reference"))
  (bind _returnvalue (`|SpawnActorFromClass` (`self.AttachedBP`) (`KismetMathLibrary.Conv_VectorToTransform` (`Actor.K2_GetActorLocation` PawnSlot)) "Undefined" "MultiplyWithRoot" null null))
  (`Actor.K2_AttachToComponent` _returnvalue (`Character.Mesh` PawnSlot) Socket "SnapToTarget" "SnapToTarget" "SnapToTarget" true)
  (return))