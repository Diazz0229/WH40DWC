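; Grenade equipment component for a character: holding G previews the throw arc and releasing it throws.
; A looping timer derives pitch from mouse distance, predicts the projectile path and spawns short-lived path and target marker actors.
; Release plays the throw montage, whose Throw_start notify spawns the grenade.
; A server-to-multicast event chain shares the angle, so non-local copies replay the montage and spawn their own grenade.
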(event `self.ReceiveBeginPlay`
  (bind _asbp_character_base (cast `/Game/TSS_Game/Blueprints/System/BP_CharacterBase` (`self.GetOwner`)))
  (set `self.OwnerCharRef` _asbp_character_base))

(event `CalculatePath`
  (bind _projectile_velocity_x (`KismetMathLibrary.BreakVector` (`self.Projectile Velocity`)))
  (bind _ownercharref (`self.OwnerCharRef`))
  (bind (_returnvalue_roll _returnvalue_pitch _returnvalue_yaw) (`KismetMathLibrary.BreakRotator` (`SceneComponent.K2_GetComponentRotation` (`Character.CapsuleComponent` _ownercharref))))
  (`self.CalculateThrowAngle`)
  (bind (_outhit _outpathpositions) (`GameplayStatics.Blueprint_PredictProjectilePath_ByObjectType` (`SceneComponent.K2_GetComponentLocation` (`/Game/TSS_Game/Blueprints/System/BP_CharacterBase.BulletSpawnLocation` _ownercharref)) (* (`KismetMathLibrary.GetForwardVector` (`KismetMathLibrary.MakeRotator` _returnvalue_roll (`self.ThrowTopAngle`) _returnvalue_yaw)) _projectile_velocity_x) true 32.0 (`|MakeArray` "ObjectTypeQuery1" "ObjectTypeQuery2" :!type "EObjectTypeQuery Enum") false (`|MakeArray` (`self.OwnerCharRef`))))
  (for (_array_element _array_index) _outpathpositions
    (if (== _array_index (`KismetArrayLibrary.Array_LastIndex` _outpathpositions))
      (`|SpawnActorFromClass` "/Game/TSS_Game/Blueprints/Equipment/BP_GrenadeThrow_Target.BP_GrenadeThrow_Target_C" (`KismetMathLibrary.Conv_VectorToTransform` _array_element) "Undefined" "MultiplyWithRoot" null (`self.PredictPathDuration`) null)
      (else
        (`|SpawnActorFromClass` "/Game/TSS_Game/Blueprints/Equipment/BP_GrenadeThrow_Path.BP_GrenadeThrow_Path_C" (`KismetMathLibrary.Conv_VectorToTransform` _array_element) "Undefined" "MultiplyWithRoot" null (`self.PredictPathDuration`) null)))))

(event `Key|G`
  (params (Key :type "Key Structure"))
  (bind _ownercharref (`self.OwnerCharRef`))
  (bind (_returnvalue_roll _returnvalue_pitch _returnvalue_yaw) (`KismetMathLibrary.BreakRotator` (`SceneComponent.K2_GetComponentRotation` (`Character.CapsuleComponent` _ownercharref))))
  (:`Pressed`
    (`KismetSystemLibrary.K2_SetTimer` null "CalculatePath" (`self.PredictPathDuration`) true))
  (:`Released`
    (`KismetSystemLibrary.K2_PauseTimer` null "CalculatePath")
    (`self.CalculateThrowAngle`)
    (bind _notifyname (`|PlayMontage` (`Character.Mesh` (`self.OwnerCharRef`)) "/Game/WH40Assets/SpaceMarines/Animations/Montages/AM_SM_GrenadeThrow.AM_SM_GrenadeThrow")
      (:`then`
        (`self.SV_ThrowGrenade` (`self.ThrowTopAngle`)))
      (:`OnNotifyBegin`
        (if (== _notifyname "Throw_start")
          (`|SpawnActorFromClass` "/Game/TSS_Game/Blueprints/Equipment/BP_EQP_Grenade_BASE.BP_EQP_Grenade_BASE_C" (`KismetMathLibrary.MakeTransform` (`SceneComponent.K2_GetComponentLocation` (`/Game/TSS_Game/Blueprints/System/BP_CharacterBase.BulletSpawnLocation` _ownercharref)) (`KismetMathLibrary.MakeRotator` _returnvalue_roll (`self.ThrowTopAngle`) _returnvalue_yaw)) "Undefined" "MultiplyWithRoot" null 99.0 (`self.Projectile Velocity`) 10.0 2.0 (`self.Damage Type`) 2.0 (`self.OwnerCharRef`) 150.0 null :!label _label))))))

(event `SV_ThrowGrenade`
  (params (ThrowTopAngle :type "Float (single-precision)"))
  (`self.MC_ThrowGrenade` ThrowTopAngle))

(event `MC_ThrowGrenade`
  (params (ThrowTopAngle :type "Float (single-precision)"))
  (set `self.ThrowTopAngle` ThrowTopAngle)
  (if (not (`Pawn.IsLocallyControlled` (`self.OwnerCharRef`)))
    (bind _notifyname (`|PlayMontage` (`Character.Mesh` (`self.OwnerCharRef`)) "/Game/WH40Assets/SpaceMarines/Animations/Montages/AM_SM_GrenadeThrow.AM_SM_GrenadeThrow")
      (:`OnNotifyBegin`
        (if (== _notifyname "Throw_start")
          (goto _label))))))