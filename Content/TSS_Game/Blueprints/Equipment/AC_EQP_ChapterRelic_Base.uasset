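; Base equipment component for Chapter Relics, giving the owning character an optional visual and a perk.
; On BeginPlay it caches the owner and, if visually attached, spawns the relic actor snapped to a mesh socket.
; It then calls AttachNextEquipment on Cust_v1 characters, continuing only if that cast succeeds.
; On the server, it finally grants the attached perk through the owner's player controller.
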(event `self.ReceiveBeginPlay`
  (bind _asbp_character_base (cast `/Game/TSS_Game/Blueprints/System/BP_CharacterBase` (`self.GetOwner`)))
  (bind _output_get (set `self.OwnerCharRef` _asbp_character_base))
  (if (`self.IsVisuallyAttached?`)
    (`self.EQP Show Equipment` (`self.AttachedSocket`) _output_get))
  (bind _asbp_character_cust_v_1 (cast `/Game/TSS_Game/Blueprints/System/BP_Character_Cust_v1` (`self.OwnerCharRef`)))
  (`/Game/TSS_Game/Blueprints/System/BP_Character_Cust_v1.AttachNextEquipment` _asbp_character_cust_v_1)
  (if (`KismetSystemLibrary.IsServer`)
    (bind _asbp_player_controller (cast `/Game/TSS_Game/Blueprints/System/BP_PlayerController` (`Pawn.GetController` _output_get)))
    (`/Game/TSS_Game/Blueprints/System/BP_PlayerController.AddPerkToCharacter` _asbp_player_controller (`self.AttachedPerk`))))

(fn `EQP Show Equipment`
  (params (Socket :type Name) (PawnSlot :type "/Game/TSS_Game/Blueprints/System/BP_CharacterBase Object Reference"))
  (bind _returnvalue (`|SpawnActorFromClass` (`self.AttachedBP`) (`KismetMathLibrary.Conv_VectorToTransform` (`Actor.K2_GetActorLocation` PawnSlot)) "Undefined" "MultiplyWithRoot" null null))
  (`Actor.K2_AttachToComponent` _returnvalue (`Character.Mesh` PawnSlot) Socket "SnapToTarget" "SnapToTarget" "SnapToTarget" true)
  (return))