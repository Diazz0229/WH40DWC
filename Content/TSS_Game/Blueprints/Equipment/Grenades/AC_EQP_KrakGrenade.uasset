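; Krak grenade equipment component or actor that lets the owning character aim and throw a grenade from either equipment slot.
; Holding the slot input runs a looping timer that spawns predicted-path and target markers, with launch pitch derived from mouse distance.
; Release checks character state and ammo, then plays the throw montage, whose notify spawns the grenade.
; A server-to-multicast event replays montage and spawn on non-local instances, so each spawns its own grenade.
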(event `CalculatePath`
  (bind _ownercharref (`self.OwnerCharRef`))
  (bind _projectile_velocity_x (`KismetMathLibrary.BreakVector` (`self.Projectile Velocity`)))
  (bind (_returnvalue_roll _returnvalue_pitch _returnvalue_yaw) (`KismetMathLibrary.BreakRotator` (`SceneComponent.K2_GetComponentRotation` (`Character.CapsuleComponent` _ownercharref))))
  ;[1 1 1] Predict throw path
  (if (not (or (`/Game/TSS_Game/Blueprints/System/BP_CharacterBase.IsSprinting?` _ownercharref) (`/Game/TSS_Game/Blueprints/System/BP_CharacterBase.IsMeleeAttacking` _ownercharref) (`/Game/TSS_Game/Blueprints/System/BP_CharacterBase.IsEvading?` _ownercharref)))
    (`self.CalculateThrowAngle`)
    (bind (_outhit _outpathpositions) (`GameplayStatics.Blueprint_PredictProjectilePath_ByObjectType` (`SceneComponent.K2_GetComponentLocation` (`/Game/TSS_Game/Blueprints/System/BP_CharacterBase.BulletSpawnLocation` _ownercharref)) (* (`KismetMathLibrary.GetForwardVector` (`KismetMathLibrary.MakeRotator` _returnvalue_roll (`self.ThrowTopAngle`) _returnvalue_yaw)) _projectile_velocity_x) true 32.0 (`|MakeArray` "ObjectTypeQuery1" "ObjectTypeQuery2" :!type "EObjectTypeQuery Enum") false (`self.TraceIgnoreActors`)))
    (for (_array_element _array_index) _outpathpositions
      (if (== _array_index (`KismetArrayLibrary.Array_LastIndex` _outpathpositions))
        (`|SpawnActorFromClass` "/Game/TSS_Game/Blueprints/Equipment/GrenadeBase/BP_GrenadeThrow_Target.BP_GrenadeThrow_Target_C" (`KismetMathLibrary.Conv_VectorToTransform` _array_element) "Undefined" "MultiplyWithRoot" null (`self.PredictPathDuration`) null)
        (else
          (`|SpawnActorFromClass` "/Game/TSS_Game/Blueprints/Equipment/GrenadeBase/BP_GrenadeThrow_Path.BP_GrenadeThrow_Path_C" (`KismetMathLibrary.Conv_VectorToTransform` _array_element) "Undefined" "MultiplyWithRoot" null (`self.PredictPathDuration`) null))))))

(event `self.ReceiveBeginPlay`
  (bind _ownercharref (`self.OwnerCharRef`))
  (bind _wpn_primary (`/Game/TSS_Game/Blueprints/System/BP_CharacterBase.WPN_Primary` _ownercharref))
  (bind _wpn_secondary (`/Game/TSS_Game/Blueprints/System/BP_CharacterBase.WPN_Secondary` _ownercharref))
  (bind _wpn_melee (`/Game/TSS_Game/Blueprints/System/BP_CharacterBase.WPN_Melee` _ownercharref))
  ;[1 1 1] BeginPlay
  (`parent.ReceiveBeginPlay`)
  (`/Engine/EditorBlueprintResources/StandardMacros.IsValid` _wpn_primary
    (:`Is Valid`
      (`KismetArrayLibrary.Array_AddUnique` (`self.TraceIgnoreActors`) _wpn_primary))
    (:`Is Not Valid`
      _))
  (`/Engine/EditorBlueprintResources/StandardMacros.IsValid` _wpn_secondary
    (:`Is Valid`
      (`KismetArrayLibrary.Array_AddUnique` (`self.TraceIgnoreActors`) _wpn_secondary))
    (:`Is Not Valid`
      _))
  (`/Engine/EditorBlueprintResources/StandardMacros.IsValid` _wpn_melee
    (:`Is Valid`
      _)
    (:`Is Not Valid`
      _))
  (`KismetArrayLibrary.Array_AddUnique` (`self.TraceIgnoreActors`) _wpn_melee))

(event `EnhancedInput|/Game/TSS_Game/Blueprints/EnhancedInput/InputAction_EQP1`
  (params (ActionValue :type Boolean) (ElapsedSeconds :type "Float (double-precision)") (TriggeredSeconds :type "Float (double-precision)") (InputAction :type "InputAction Object Reference" :default "/Game/TSS_Game/Blueprints/EnhancedInput/InputAction_EQP1.InputAction_EQP1"))
  (bind _ownercharref (`self.OwnerCharRef`))
  (bind _ownercharref_2 (`self.OwnerCharRef`))
  (bind _equippedweapon (`/Game/TSS_Game/Blueprints/System/BP_CharacterBase.EquippedWeapon` _ownercharref))
  (bind (_returnvalue_roll _returnvalue_pitch _returnvalue_yaw) (`KismetMathLibrary.BreakRotator` (`SceneComponent.K2_GetComponentRotation` (`Character.CapsuleComponent` _ownercharref_2))))
  ;[1 1 1] Throw logic
  (:`Started`
    (bind _canuse (`self.CheckSlotKey` 0))
    (if _canuse
      (if (> (`self.AmmoCur`) 0) :!label _label
        (`KismetSystemLibrary.K2_SetTimer` null "CalculatePath" (`self.PredictPathDuration`) true))))
  (:`Completed`
    (bind _canuse_2 (`self.CheckSlotKey` 0))
    (if _canuse_2
      (`KismetSystemLibrary.K2_PauseTimer` null "CalculatePath" :!label _label_2)
      (if (or (`/Game/TSS_Game/Blueprints/System/BP_CharacterBase.IsMeleeAttacking` _ownercharref) (`/Game/TSS_Game/Blueprints/System/BP_CharacterBase.IsDead` _ownercharref) (`/Game/TSS_Game/Blueprints/System/BP_CharacterBase.IsSprinting?` _ownercharref) (`/Game/TSS_Game/Blueprints/System/BP_CharacterBase.IsEvading?` _ownercharref) (`/Game/TSS_Game/Blueprints/System/BP_CharacterBase.IsInputDisabled?` _ownercharref))
        _
        (elif (> (`self.AmmoCur`) 0)
          (set `/Game/TSS_Game/Blueprints/System/BP_CharacterBase.IsMeleeAttacking` true _ownercharref)
          (if (`/Game/TSS_Game/Blueprints/Weapons/Base/BP_WeaponBase.isReloading` _equippedweapon)
            (set `/Game/TSS_Game/Blueprints/Weapons/Base/BP_WeaponBase.isReloading` false _equippedweapon))
          (if true
            (`self.CalculateThrowAngle`)
            (bind _notifyname (`|PlayMontage` (`Character.Mesh` (`self.OwnerCharRef`)) "/Game/WH40Assets/SpaceMarines/Animations/Montages/AM_SM_GrenadeThrow.AM_SM_GrenadeThrow")
              (:`then`
                (`self.SV_ThrowGrenade` (`self.ThrowTopAngle`))
                (`/Game/TSS_Game/Blueprints/System/BP_CharacterBase.Hide WPNIn Secondary Hand` (`self.OwnerCharRef`) true))
              (:`OnCompleted`
                (`/Game/TSS_Game/Blueprints/System/BP_CharacterBase.Hide WPNIn Secondary Hand` (`self.OwnerCharRef`) true :!label _label_3))
              (:`OnInterrupted`
                (goto _label_3))
              (:`OnNotifyBegin`
                (if (== _notifyname "Throw_start")
                  (set `/Game/TSS_Game/Blueprints/System/BP_CharacterBase.IsMeleeAttacking` false _ownercharref_2)
                  (`/Engine/EditorBlueprintResources/StandardMacros.DecrementInt` (`self.AmmoCur`)
                    (:`  `
                      (`|SpawnActorFromClass` "/Game/TSS_Game/Blueprints/Equipment/Grenades/BP_EQP_Grenade_Krak.BP_EQP_Grenade_Krak_C" (`KismetMathLibrary.MakeTransform` (`SceneComponent.K2_GetComponentLocation` (`/Game/TSS_Game/Blueprints/System/BP_CharacterBase.BulletSpawnLocation` _ownercharref_2)) (`KismetMathLibrary.MakeRotator` _returnvalue_roll (`self.ThrowTopAngle`) _returnvalue_yaw)) "Undefined" "MultiplyWithRoot" null (`self.DamageMin`) (`self.Projectile Velocity`) (`self.Crit Chance`) (`self.Crit Multiplier`) (`self.Damage Type`) (`self.Explode Delay`) (`self.OwnerCharRef`) (`self.DamageMax`) (`self.ActiveRadius`) null :!label _label_4)))))))
          (else
            (`GameplayStatics.PlaySound2D` "/Game/TSS_Game/SFX/UI/SC_ERROR.SC_ERROR" 1.0 1.0 0.0 null null)))))))

(event `EnhancedInput|/Game/TSS_Game/Blueprints/EnhancedInput/InputAction_EQP2`
  (params (ActionValue :type Boolean) (ElapsedSeconds :type "Float (double-precision)") (TriggeredSeconds :type "Float (double-precision)") (InputAction :type "InputAction Object Reference" :default "/Game/TSS_Game/Blueprints/EnhancedInput/InputAction_EQP2.InputAction_EQP2"))
  ;[1 1 1] Throw logic
  (:`Started`
    (bind _canuse (`self.CheckSlotKey` 1))
    (if _canuse
      (goto _label)))
  (:`Completed`
    (bind _canuse_2 (`self.CheckSlotKey` 1))
    (if _canuse_2
      (goto _label_2))))

(event `SV_ThrowGrenade`
  (params (ThrowTopAngle :type "Float (single-precision)"))
  ;[1 1 1] Throw logic
  (`self.MC_ThrowGrenade` ThrowTopAngle))

(event `MC_ThrowGrenade`
  (params (ThrowTopAngle :type "Float (single-precision)"))
  ;[1 1 1] Throw logic
  (set `self.ThrowTopAngle` ThrowTopAngle)
  (if (not (`Pawn.IsLocallyControlled` (`self.OwnerCharRef`)))
    (`/Game/TSS_Game/Blueprints/System/BP_CharacterBase.Hide WPNIn Secondary Hand` (`self.OwnerCharRef`) false)
    (bind _notifyname (`|PlayMontage` (`Character.Mesh` (`self.OwnerCharRef`)) "/Game/WH40Assets/SpaceMarines/Animations/Montages/AM_SM_GrenadeThrow.AM_SM_GrenadeThrow")
      (:`OnCompleted`
        (`/Game/TSS_Game/Blueprints/System/BP_CharacterBase.Hide WPNIn Secondary Hand` (`self.OwnerCharRef`) false :!label _label_5))
      (:`OnInterrupted`
        (goto _label_5))
      (:`OnNotifyBegin`
        (if (== _notifyname "Throw_start")
          (goto _label_4))))))