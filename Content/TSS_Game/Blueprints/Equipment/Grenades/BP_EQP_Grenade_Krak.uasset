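; Krak grenade projectile actor that detonates after a fuse delay or on contact with a living, damageable enemy.
; BeginPlay launches it via ProjectileMovement, and the timer, hit and sphere-overlap paths share a DoOnce so it explodes once.
; Detonation stops movement, spawns BP_GrenadeExplosion_Krak with damage, crit, radius and owner data, then destroys the grenade shortly afterwards.
; Its impulse and crit-damage helper functions are not called from the event graph.
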(event `self.ReceiveBeginPlay`
  (bind _returnvalue_location (`KismetMathLibrary.BreakTransform` (`self.GetTransform`)))
  (bind _sphere_radius (`self.Sphere Radius`))
  (bind _grenadedamagemin (`self.GrenadeDamageMin`))
  (bind _projectilemovement (`self.ProjectileMovement`))
  (bind _owner_character (`self.Owner Character`))
  (bind _grenadedamagemax (`self.GrenadeDamageMax`))
  (bind _damage_type (`self.Damage Type`))
  (bind _crit_chance (`self.Crit Chance`))
  (bind _crit_multiplier (`self.Crit Multiplier`))
  (bind _owningplayercontroller (`/Game/TSS_Game/Blueprints/System/BP_CharacterBase.OwningPlayerController` _owner_character))
  (`ProjectileMovementComponent.SetVelocityInLocalSpace` (`self.ProjectileMovement`) (`self.ProjectileVelocity`))
  (`PrimitiveComponent.SetCollisionResponseToChannel` (`self.Sphere`) "ECC_WorldDynamic" "ECR_Overlap")
  (set `self.ProjectileMovementComponent` (`self.ProjectileMovement`))
  (`KismetSystemLibrary.Delay` (`self.ExplodeDelay`))
  (`/Engine/EditorBlueprintResources/StandardMacros.DoOnce` false :!label _label
    (:`Completed`
      (`/Engine/EditorBlueprintResources/StandardMacros.IsValid` _projectilemovement
        (:`Is Valid`
          (`ActorComponent.Deactivate` _projectilemovement))
        (:`Is Not Valid`
          _))
      (`/Engine/EditorBlueprintResources/StandardMacros.IsValid` _owningplayercontroller
        (:`Is Valid`
          (`|SpawnActorFromClass` "/Game/TSS_Game/Blueprints/Weapons/Base/BP_GrenadeExplosion_Krak.BP_GrenadeExplosion_Krak_C" (`KismetMathLibrary.MakeTransform` _returnvalue_location (`KismetMathLibrary.MakeRotator` 0.0 0.0 (`KismetMathLibrary.RandomFloatInRange` 0.0 360.0))) "Undefined" "MultiplyWithRoot" null _damage_type _owningplayercontroller _owner_character _grenadedamagemin _grenadedamagemax _crit_chance _crit_multiplier 0.0 0.0 _sphere_radius null))
        (:`Is Not Valid`
          (`|SpawnActorFromClass` "/Game/TSS_Game/Blueprints/Weapons/Base/BP_GrenadeExplosion_Krak.BP_GrenadeExplosion_Krak_C" (`KismetMathLibrary.MakeTransform` _returnvalue_location (`KismetMathLibrary.MakeRotator` 0.0 0.0 (`KismetMathLibrary.RandomFloatInRange` 0.0 360.0))) "Undefined" "MultiplyWithRoot" null _damage_type null _owner_character _grenadedamagemin _grenadedamagemax _crit_chance _crit_multiplier 0.0 0.0 _sphere_radius null)))
      (`KismetSystemLibrary.Delay` 0.5)
      (`self.K2_DestroyActor`))))

(event `self.ReceiveHit`
  (params (MyComp :type "PrimitiveComponent Object Reference") (Other :type "Actor Object Reference") (OtherComp :type "PrimitiveComponent Object Reference") (bSelfMoved :type Boolean) (HitLocation :type "Vector Structure") (HitNormal :type "Vector Structure") (NormalImpulse :type "Vector Structure") (Hit :type "HitResult Structure (by ref)"))
  (bind (_bblockinghit _binitialoverlap _time _distance _location _impactpoint _normal _impactnormal _physmat _hitactor) (`GameplayStatics.BreakHitResult` Hit))
  (bind _hit_actor (`self.Hit Actor`))
  (set `self.Other Comp` OtherComp)
  (set `self.Hit Actor` _hitactor)
  (set `self.ImpactLocation` _location)
  (if (and (`KismetSystemLibrary.DoesImplementInterface` _hit_actor "/Game/TSS_Game/Blueprints/System/BPI_Damagable.BPI_Damagable_C") (not (`self.ActorHasTag` _hit_actor "Dead")) (`self.ActorHasTag` _hit_actor "Enemy")) :!label _label_2
    (goto _label)))

(event `self.Sphere.OnComponentBeginOverlap`
  (params (OverlappedComponent :type "PrimitiveComponent Object Reference") (OtherActor :type "Actor Object Reference") (OtherComp :type "PrimitiveComponent Object Reference") (OtherBodyIndex :type Integer) (bFromSweep :type Boolean) (SweepResult :type "HitResult Structure (by ref)"))
  (set `self.Other Comp` OtherComp)
  (set `self.Hit Actor` OtherActor)
  (set `self.ImpactLocation` (`.Location` (`GameplayStatics.BreakHitResult` SweepResult)))
  (goto _label_2))

(fn `ApplyPhysics`
  (params (OtherComponent :type "PrimitiveComponent Object Reference"))
  (`/Engine/EditorBlueprintResources/StandardMacros.IsValid` OtherComponent
    (:`Is Valid`
      (if (`SceneComponent.IsSimulatingPhysics` OtherComponent "None")
        (`PrimitiveComponent.AddImpulseAtLocation` OtherComponent (* (`self.GetVelocity`) (`self.ProjectileImpulseStrenght`)) (`self.K2_GetActorLocation`) "None")
        (return)
        (else
          (return))))
    (:`Is Not Valid`
      (return))))

(fn `CheckCritAndDealDamage`
  (params (DamageTarget :type "Actor Object Reference") (Target :type "/Game/TSS_Game/Blueprints/System/BP_PlayerController Object Reference") (Source :type "/Game/TSS_Game/Blueprints/System/BP_CharacterBase Object Reference"))
  (bind _grenadedamagemin (`self.GrenadeDamageMin`))
  (if (<= (`KismetMathLibrary.RandomFloatInRange` 0.0 100.0) (`self.Crit Chance`))
    (set `self.GrenadeDamageMin` (* (`self.GrenadeDamageMin`) (`self.Crit Multiplier`)))
    (`/Game/TSS_Game/Blueprints/System/BP_PlayerController.DealDamage` Target DamageTarget _grenadedamagemin Source true (`self.Damage Type`) 0.0 0.0)
    (else
      (`/Game/TSS_Game/Blueprints/System/BP_PlayerController.DealDamage` Target DamageTarget _grenadedamagemin Source false (`self.Damage Type`) 0.0 0.0))))

(fn `UserConstructionScript`)