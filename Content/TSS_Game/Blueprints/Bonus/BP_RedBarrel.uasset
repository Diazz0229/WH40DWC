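; BP_RedBarrel is an explosive barrel with a physics-simulated cylinder that reacts to a damage interaction event.
; The event activates the barrel's particle system immediately and triggers the spawn step after a two-second delay.
; Both steps route through Server-named events to multicast events, the spawn one creating BP_Explosion at the barrel's location and destroying the barrel.
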(event `self.ReceiveBeginPlay`
  (`PrimitiveComponent.SetSimulatePhysics` (`self.Cylinder`) true))

(event `Multicast_Spawn`
  (`|SpawnActorFromClass` "/Game/TSS_Game/Blueprints/Weapons/Base/BP_Explosion.BP_Explosion_C" (`KismetMathLibrary.MakeTransform` (`self.K2_GetActorLocation`)) "AlwaysSpawn" "OverrideRootScale" null null)
  (`self.K2_DestroyActor`))

(event `/Game/TSS_Game/Blueprints/System/BPI_Damagable.DamageIntercation`
  (params (`Damage dealt` :type "Float (double-precision)") (Source :type "Object Object Reference") (`IsMulticast?` :type Boolean))
  (`|ExecutionSequence`
    (:`then_0`
      (`KismetSystemLibrary.Delay` 2.0)
      (`self.ServerSpawn`))
    (:`then_1`
      (`self.ServerActivateParticle`))))

(event `ServerSpawn`
  (`self.Multicast_Spawn`))

(event `ServerActivateParticle`
  (`self.MulticastParticle`))

(event `MulticastParticle`
  (`ActorComponent.Activate` (`self.ParticleSystem`) false))

(fn `UserConstructionScript`)