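; Background tracer emitter actor that simulates distant gunfire by spawning BP_BackgroundTracer actors in intermittent bursts.
; From BeginPlay, a timer waits a random interval, then runs AttackSequence, which fires SpawnTracer on a fast looping timer for a random duration.
; The sequence then pauses that timer by function name and schedules the next burst.
; Each tracer spawns at the Direction component's transform, with random Spread applied to roll, pitch and yaw.
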(event `self.ReceiveBeginPlay`
  (`KismetSystemLibrary.K2_SetTimerDelegate` (delegate `AttackSequence`) (`KismetMathLibrary.RandomFloatInRange` 1.0 6.0) :!label _label))

(event `AttackSequence`
  (`KismetSystemLibrary.K2_SetTimerDelegate` (delegate `SpawnTracer`) 0.1 true)
  (`KismetSystemLibrary.Delay` (`KismetMathLibrary.RandomFloatInRange` 1.0 3.0))
  (`KismetSystemLibrary.K2_PauseTimer` null "SpawnTracer")
  (goto _label))

(event `SpawnTracer`
  (bind _spread (`self.Spread`))
  (bind _returnvalue (`KismetMathLibrary.RandomFloatInRange` _spread (* _spread -1.0)))
  (`|SpawnActorFromClass` "/Game/TSS_Game/Blueprints/Bonus/BP_BackgroundTracer.BP_BackgroundTracer_C" (`KismetMathLibrary.MakeTransform` (.location (`SceneComponent.K2_GetComponentToWorld` (`self.Direction`))) (`KismetMathLibrary.MakeRotator` (+ (.roll (.rotation (`SceneComponent.K2_GetComponentToWorld` (`self.Direction`)))) _returnvalue) (+ (.pitch (.rotation (`SceneComponent.K2_GetComponentToWorld` (`self.Direction`)))) _returnvalue) (+ (.yaw (.rotation (`SceneComponent.K2_GetComponentToWorld` (`self.Direction`)))) _returnvalue)) (.scale (`SceneComponent.K2_GetComponentToWorld` (`self.Direction`)))) "Undefined" "MultiplyWithRoot" null null))

(fn `UserConstructionScript`)