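; Warrior enemy AI character with melee attacks, toxic grenade throws, enrage and a hard-landing roar.
; A proximity sphere drives charge, heavy claw or light sword attacks, with montage notifies opening single-hit-per-target damage windows.
; Random timers trigger line-of-sight grenade throws and, once first damaged, recurring enrages that give itself a charge mutation and nearby enemies a speed mutation.
; Server events make most decisions, while MC events play montages and effects.
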(event `SV_RetryAttack`
  ;[1 1 1] Claw/Sword Attack
  (`/Engine/EditorBlueprintResources/StandardMacros.DoOnce` false :!label _label
    (:`Completed`
      (`self.RotateToPlayer`)
      (`self.CheckForOverlappingPlayers`
        (:`ActorsFound`
          (`/Engine/EditorBlueprintResources/ActorMacros.Switch Has Authority`
            (:`Authority`
              (`Controller.StopMovement` (`AIBlueprintHelperLibrary.GetAIController` self)))
            (:`Remote`
              _))
          (set `self.isAttacking` true)
          (if (`self.IsCharging`)
            (`self.MC_ChargeAttack`)
            (elif (== (`KismetMathLibrary.RandomIntegerInRange` 0 1) 0)
              (`self.MC_HeavyAttck`)
              (else
                (`self.MC_LightAttack`)))))
        (:`GroupIsEmpty`
          (`self.ResetAttack`))))))

(event `MC_ChargeAttack`
  ;[1 1 1] Claw/Sword Attack
  (`KismetArrayLibrary.Array_Clear` (`self.ActorsAlreadyHit`))
  (bind _notifyname (`|PlayMontage` (`self.Mesh`) "/Game/WH40Assets/Tyranids/Animations/Montages/AM_Warrior_Attack_Charge.AM_Warrior_Attack_Charge" 1.2)
    (:`OnCompleted`
      (set `self.isAttacking` false :!label _label_2)
      (`/Engine/EditorBlueprintResources/ActorMacros.Switch Has Authority`
        (:`Authority`
          (`self.ResetAttack`))
        (:`Remote`
          _))
      (set `self.IsClawAttack` false :!label _label_3))
    (:`OnInterrupted`
      (goto _label_2))
    (:`OnNotifyBegin`
      (if (== _notifyname "AttackBegin")
        (set `self.IsClawAttack` true)
        (elif (== _notifyname "EffectBegin")
          (`ActorComponent.SetActive` (`self.ClawEffect1`) true true)
          (`ActorComponent.SetActive` (`self.ClawEffect2`) true true)
          (else
            (goto _label_3)))))))

(event `self.AttackTracerSphere.OnComponentBeginOverlap`
  (params (OverlappedComponent :type "PrimitiveComponent Object Reference") (OtherActor :type "Actor Object Reference") (OtherComp :type "PrimitiveComponent Object Reference") (OtherBodyIndex :type Integer) (bFromSweep :type Boolean) (SweepResult :type "HitResult Structure (by ref)"))
  ;[1 1 1] Claw/Sword Attack
  (`/Engine/EditorBlueprintResources/ActorMacros.Switch Has Authority`
    (:`Authority`
      (bind _asbp_character_base (cast `/Game/TSS_Game/Blueprints/System/BP_CharacterBase` OtherActor)) ; Choose only players
      (if (not (`self.ActorHasTag` _asbp_character_base "Dead"))
        (`KismetSystemLibrary.K2_SetTimerDelegate` (delegate `SV_RetryAttack`) (`self.AttacksDelay`) true)
        (goto _label)))))

(event `MC_HeavyAttck`
  ;[1 1 1] Claw/Sword Attack
  (`KismetArrayLibrary.Array_Clear` (`self.ActorsAlreadyHit`))
  (bind _notifyname (`|PlayMontage` (`self.Mesh`) "/Game/WH40Assets/Tyranids/Animations/Montages/AM_Warrior_Attack_Heavy.AM_Warrior_Attack_Heavy")
    (:`OnCompleted`
      (set `self.isAttacking` false :!label _label_4)
      (`/Engine/EditorBlueprintResources/ActorMacros.Switch Has Authority`
        (:`Authority`
          (`self.ResetAttack`))
        (:`Remote`
          _))
      (set `self.IsClawAttack` false :!label _label_5))
    (:`OnInterrupted`
      (goto _label_4))
    (:`OnNotifyBegin`
      (if (== _notifyname "AttackBegin")
        (set `self.IsClawAttack` true)
        (elif (== _notifyname "EffectBegin")
          (`ActorComponent.SetActive` (`self.ClawEffect1`) true true)
          (`ActorComponent.SetActive` (`self.ClawEffect2`) true true)
          (else
            (goto _label_5)))))))

(event `ResetAttack`
  ;[1 1 1] Claw/Sword Attack
  (goto _label :!via `Reset`))

(event `MC_LightAttack`
  ;[1 1 1] Claw/Sword Attack
  (`KismetArrayLibrary.Array_Clear` (`self.ActorsAlreadyHit`))
  (bind _notifyname (`|PlayMontage` (`self.Mesh`) "/Game/WH40Assets/Tyranids/Animations/Montages/AM_Warrior_Attack_LightAttack.AM_Warrior_Attack_LightAttack")
    (:`OnCompleted`
      (set `self.isAttacking` false :!label _label_6)
      (`/Engine/EditorBlueprintResources/ActorMacros.Switch Has Authority`
        (:`Authority`
          (`self.ResetAttack`))
        (:`Remote`
          _))
      (set `self.SwordAttack` false :!label _label_7))
    (:`OnInterrupted`
      (goto _label_6))
    (:`OnNotifyBegin`
      (if (== _notifyname "AttackBegin")
        (set `self.SwordAttack` true)
        (elif (== _notifyname "EffectBegin")
          (`ActorComponent.SetActive` (`self.SwordEffect3`) true true)
          (else
            (goto _label_7)))))))

(event `self.ClawCollision2.OnComponentBeginOverlap`
  (params (OverlappedComponent :type "PrimitiveComponent Object Reference") (OtherActor :type "Actor Object Reference") (OtherComp :type "PrimitiveComponent Object Reference") (OtherBodyIndex :type Integer) (bFromSweep :type Boolean) (SweepResult :type "HitResult Structure (by ref)"))
  (bind _temp_overlapedactor (`self.TEMP_OverlapedActor`))
  ;[1 1 1] Claw/Sword Attack
  (set `self.TEMP_OverlapedActor` OtherActor)
  (if (and (`self.IsClawAttack`) (not (`self.isDead`)) (not (`KismetArrayLibrary.Array_Contains` (`self.ActorsAlreadyHit`) _temp_overlapedactor))) :!label _label_8
    (cast `/Game/TSS_Game/Blueprints/System/BP_CharacterBase` _temp_overlapedactor) ; Choose only players
    (if (not (or (`self.ActorHasTag` _temp_overlapedactor "Dead") (`self.ActorHasTag` _temp_overlapedactor "Invul")))
      (`KismetArrayLibrary.Array_AddUnique` (`self.ActorsAlreadyHit`) _temp_overlapedactor)
      (message `/Game/TSS_Game/Blueprints/System/BPI_Damagable.DamageIntercation` _temp_overlapedactor (* (`self.Damage Dealt Melee`) 2.0) self true (`self.Damage Type Melee`))
      (`GameplayStatics.PlaySound2D` "/Game/TSS_Game/SFX/Weapon/Melee/Impact_Hard_Slice.Impact_Hard_Slice" 1.0 1.0 0.0 null null))))

(event `self.MC_AttackSequence`
  ;[1 1 1] Claw/Sword Attack
)

(event `self.ClawCollision1.OnComponentBeginOverlap`
  (params (OverlappedComponent :type "PrimitiveComponent Object Reference") (OtherActor :type "Actor Object Reference") (OtherComp :type "PrimitiveComponent Object Reference") (OtherBodyIndex :type Integer) (bFromSweep :type Boolean) (SweepResult :type "HitResult Structure (by ref)"))
  ;[1 1 1] Claw/Sword Attack
  (set `self.TEMP_OverlapedActor` OtherActor)
  (goto _label_8))

(event `self.ClawCollision3.OnComponentBeginOverlap`
  (params (OverlappedComponent :type "PrimitiveComponent Object Reference") (OtherActor :type "Actor Object Reference") (OtherComp :type "PrimitiveComponent Object Reference") (OtherBodyIndex :type Integer) (bFromSweep :type Boolean) (SweepResult :type "HitResult Structure (by ref)"))
  ;[1 1 1] Claw/Sword Attack
  (set `self.TEMP_OverlapedActor` OtherActor)
  (goto _label_8))

(event `self.SwordCollision4.OnComponentBeginOverlap`
  (params (OverlappedComponent :type "PrimitiveComponent Object Reference") (OtherActor :type "Actor Object Reference") (OtherComp :type "PrimitiveComponent Object Reference") (OtherBodyIndex :type Integer) (bFromSweep :type Boolean) (SweepResult :type "HitResult Structure (by ref)"))
  (bind _temp_overlapedactor (`self.TEMP_OverlapedActor`))
  ;[1 1 1] Claw/Sword Attack
  (set `self.TEMP_OverlapedActor` OtherActor)
  (if (and (`self.SwordAttack`) (not (`self.isDead`)) (not (`KismetArrayLibrary.Array_Contains` (`self.ActorsAlreadyHit`) _temp_overlapedactor)))
    (cast `/Game/TSS_Game/Blueprints/System/BP_CharacterBase` _temp_overlapedactor) ; Choose only players
    (if (not (or (`self.ActorHasTag` _temp_overlapedactor "Dead") (`self.ActorHasTag` _temp_overlapedactor "Invul")))
      (`KismetArrayLibrary.Array_AddUnique` (`self.ActorsAlreadyHit`) _temp_overlapedactor)
      (message `/Game/TSS_Game/Blueprints/System/BPI_Damagable.DamageIntercation` _temp_overlapedactor (`self.Damage Dealt Melee`) self true (`self.Damage Type Melee`))
      (`GameplayStatics.PlaySound2D` "/Game/TSS_Game/SFX/Weapon/Melee/Impact_Hard_Slice.Impact_Hard_Slice" 1.0 1.0 0.0 null null))))

(event `/Game/TSS_Game/Blueprints/System/BPI_Damagable.DamageIntercation`
  (params (`Damage dealt` :type "Float (double-precision)") (Source :type "Actor Object Reference") (`IsMulticast?` :type Boolean) (DamageType :type "/Game/TSS_Game/Blueprints/Weapons/E_DamageTypes Enum" :default "NewEnumerator0"))
  ;[1 1 1] Abilities
  (`parent.DamageIntercation` `Damage dealt` Source `IsMulticast?` DamageType)
  (`/Engine/EditorBlueprintResources/ActorMacros.Switch Has Authority`
    (:`Authority`
      (`/Engine/EditorBlueprintResources/StandardMacros.DoOnce` false
        (:`Completed`
          (`KismetSystemLibrary.K2_SetTimerDelegate` (delegate `SV_Enrage`) (`KismetMathLibrary.RandomFloatInRange` 1.0 4.0)))))))

(event `SV_Enrage`
  ;[1 1 1] Abilities
  (`self.MC_Enrage`)
  (`Controller.StopMovement` (`AIBlueprintHelperLibrary.GetAIController` self))
  (`CharacterMovementComponent.SetMovementMode` (`self.CharacterMovement`) "MOVE_None" 0))

(event `MC_Enrage`
  (bind _returnvalue (`self.K2_GetActorLocation`))
  ;[1 1 1] Abilities
  (set `self.isAttacking` true)
  (set `self.IsCharging` true)
  (`|PlayMontage` (`self.Mesh`) "/Game/WH40Assets/Tyranids/Animations/Montages/AM_Warrior_Taunt.AM_Warrior_Taunt"
    (:`then`
      (bind _outhits (`KismetSystemLibrary.SphereTraceMulti` _returnvalue _returnvalue 1000.0 "TraceTypeQuery1"))
      (for _array_element _outhits
        (bind (_bblockinghit _binitialoverlap _time _distance _location _impactpoint _normal _impactnormal _physmat _hitactor) (`GameplayStatics.BreakHitResult` _array_element))
        (if (and (`self.ActorHasTag` _hitactor "Enemy") (`KismetSystemLibrary.DoesImplementInterface` _hitactor "/Game/TSS_Game/Blueprints/AbilitySystem/EnemyMutations/Base/BPI_AttachableMutation.BPI_AttachableMutation_C") (not (`KismetArrayLibrary.Array_Contains` (`self.ActorsAlreadyBuffed`) _hitactor)))
          (message `/Game/TSS_Game/Blueprints/AbilitySystem/EnemyMutations/Base/BPI_AttachableMutation.AttachMutation` _hitactor 1 "/Game/TSS_Game/Blueprints/AbilitySystem/EnemyMutations/AC_Mutation_MSpeed100.AC_Mutation_MSpeed100_C")
          (`KismetArrayLibrary.Array_AddUnique` (`self.ActorsAlreadyBuffed`) _hitactor)))
      (message `/Game/TSS_Game/Blueprints/AbilitySystem/EnemyMutations/Base/BPI_AttachableMutation.AttachMutation` self 1 "/Game/TSS_Game/Blueprints/AbilitySystem/EnemyMutations/AC_Mutation_Charge.AC_Mutation_Charge_C"))
    (:`OnCompleted`
      (`/Engine/EditorBlueprintResources/ActorMacros.Switch Has Authority` :!label _label_9
        (:`Authority`
          (`KismetSystemLibrary.K2_SetTimerDelegate` (delegate `SV_Enrage`) (`KismetMathLibrary.RandomFloatInRange` 30.0 45.0))
          (`CharacterMovementComponent.SetMovementMode` (`self.CharacterMovement`) "MOVE_Walking" 0)
          (set `self.isAttacking` false)
          (set `self.IsCharging` false))))
    (:`OnInterrupted`
      (goto _label_9))))

(event `SV_CheckRangedTargets`
  (bind _target_player_actor (`self.Target Player Actor`))
  (bind _returnvalue (`self.K2_GetActorLocation` self))
  ;[0.4703 1 0.3672] Try to check if player is attackable
  (`/Engine/EditorBlueprintResources/StandardMacros.IsValid` (`self.Target Player Actor`)
    (:`Is Valid`
      _)
    (:`Is Not Valid`
      _))
  (if (not (`self.isDead`))
    (`/Engine/EditorBlueprintResources/StandardMacros.IsValid` _target_player_actor
      (:`Is Valid`
        (`/Engine/EditorBlueprintResources/StandardMacros.DoOnce` false :!label _label_10
          (:`Completed`
            (bind _outhits (`KismetSystemLibrary.LineTraceMultiForObjects` (+ (`self.K2_GetActorLocation` self) (0.0 0.0 180.0)) (+ (`self.K2_GetActorLocation` _target_player_actor) (0.0 0.0 80.0)) (`self.TraceForPawns`) false (`self.Actors to Ignore`)))
            (set `self.RangeTargetFound` false)
            (for _array_element _outhits
              (if (== (`self.Target Player Actor`) (`.HitActor` (`GameplayStatics.BreakHitResult` _array_element)))
                (set `self.RangeTargetFound` true)))
            (`KismetSystemLibrary.K2_SetTimer` null "SV_CheckRangedTargets" (`KismetMathLibrary.RandomFloatInRange` 5.0 25.0))
            (if (`self.RangeTargetFound`)
              (bind _outhits_2 (`KismetSystemLibrary.LineTraceMultiForObjects` (+ (`self.K2_GetActorLocation` self) (0.0 0.0 180.0)) (+ (`self.K2_GetActorLocation` (`self.Target Player Actor`)) (0.0 0.0 80.0)) (`self.TraceForBlockers`))) ; Check for blockers on the way
              (if (`KismetArrayLibrary.Array_IsNotEmpty` _outhits_2)
                (`self.ResetThrowAttack`)
                (else
                  (`Controller.StopMovement` (`AIBlueprintHelperLibrary.GetAIController` self))
                  (`self.MC_ThrowGrenade`)
                  (`self.ResetThrowAttack`)))
              (else
                (bind _outhits_3 (`KismetSystemLibrary.BoxTraceMultiForObjects` _returnvalue _returnvalue (0.0 0.0 0.0) (struct) (`self.TraceForPawns`)))
                (for _array_element_2 _outhits_3
                  (bind (_bblockinghit _binitialoverlap _time _distance _location _impactpoint _normal _impactnormal _physmat _hitactor) (`GameplayStatics.BreakHitResult` _array_element_2))
                  (bind _asbp_character_base (cast `/Game/TSS_Game/Blueprints/System/BP_CharacterBase` _hitactor))
                  (if (`/Game/TSS_Game/Blueprints/System/BP_CharacterBase.IsDead` _asbp_character_base)
                    (set `self.Target Player Actor` null)
                    (`self.ResetThrowAttack`)
                    (else
                      (set `self.Target Player Actor` _hitactor)
                      (`self.ResetThrowAttack`)
                      (`self.SV_CheckRangedTargets`))))
                (`self.ResetThrowAttack`)))))))))

(event `ResetThrowAttack`
  ;[0.4703 1 0.3672] Try to check if player is attackable
  (goto _label_10 :!via `Reset`))

(event `MC_ThrowGrenade`
  (bind _returnvalue (`SceneComponent.K2_GetComponentLocation` (`self.ArrowThrower`)))
  ;[0.4703 1 0.3672] Try to check if player is attackable
  (`self.RotateToPlayer`)
  (set `self.isAttacking` true)
  (`SceneComponent.SetVisibility` (`self.Grenade`) true false)
  (bind _notifyname (`|PlayMontage` (`self.Mesh`) "/Game/WH40Assets/Tyranids/Animations/Montages/AM_Warrior_Attack_Throw.AM_Warrior_Attack_Throw")
    (:`OnCompleted`
      (set `self.isAttacking` false :!label _label_11)
      (`SceneComponent.SetVisibility` (`self.Grenade`) false false)
      (bind _asbp_character_base (cast `/Game/TSS_Game/Blueprints/System/BP_CharacterBase` (`self.Target Player Actor`)))
      (`/Game/TSS_Game/Blueprints/System/BP_CharacterBase.Speech_Say` _asbp_character_base "NewEnumerator2" false 35.0))
    (:`OnInterrupted`
      (goto _label_11))
    (:`OnNotifyBegin`
      (if (== _notifyname "AttackBegin")
        (`|SpawnActorFromClass` "/Game/TSS_Game/Blueprints/Weapons/AI/BP_WPN_GrenadeToxic.BP_WPN_GrenadeToxic_C" (`KismetMathLibrary.MakeTransform` _returnvalue (`KismetMathLibrary.FindLookAtRotation` _returnvalue (+ (`self.K2_GetActorLocation` (`self.Target Player Actor`)) (0.0 0.0 300.0)))) "Undefined" "MultiplyWithRoot" null (`self.GrenadeDamage`) (`self.GrenadeDamageType`) null)
        (`SceneComponent.SetVisibility` (`self.Grenade`) false false)))))

(event `self.ReceiveBeginPlay`
  ;[0.4703 1 0.3672] Try to check if player is attackable
  (`parent.ReceiveBeginPlay`)
  (`KismetSystemLibrary.K2_SetTimerDelegate` (delegate `SV_CheckRangedTargets`) (`KismetMathLibrary.RandomFloatInRange` 5.0 25.0)))

(event `self.CapsuleComponent.OnComponentHit`
  (params (HitComponent :type "PrimitiveComponent Object Reference") (OtherActor :type "Actor Object Reference") (OtherComp :type "PrimitiveComponent Object Reference") (NormalImpulse :type "Vector Structure") (Hit :type "HitResult Structure (by ref)"))
  (bind (_returnvalue_x _returnvalue_y _returnvalue_z) (`KismetMathLibrary.BreakVector` (`CharacterMovementComponent.GetLastUpdateVelocity` (`self.CharacterMovement`))))
  (if (`KismetSystemLibrary.IsServer`)
    (bind _asstatic_mesh_actor (cast `StaticMeshActor` OtherActor))
    (if (<= _returnvalue_z -2000.0)
      (switch `ECollisionChannel` (`PrimitiveComponent.GetCollisionObjectType` (`StaticMeshActor.StaticMeshComponent` _asstatic_mesh_actor))
        (:`ECC_WorldStatic`
          (`self.SV_LandingRoar`))))))

(event `SV_LandingRoar`
  (`self.MC_LandingRoar`)
  (`Controller.StopMovement` (`AIBlueprintHelperLibrary.GetAIController` self))
  (`CharacterMovementComponent.SetMovementMode` (`self.CharacterMovement`) "MOVE_None" 0))

(event `MC_LandingRoar`
  (bind _returnvalue (`SceneComponent.K2_GetComponentLocation` (`self.OriginPoint`)))
  (set `self.isAttacking` true)
  (set `self.IsCharging` true)
  (`|PlayMontage` (`self.Mesh`) "/Game/WH40Assets/Tyranids/Animations/Montages/AM_Warrior_Taunt.AM_Warrior_Taunt"
    (:`then`
      (`NiagaraFunctionLibrary.SpawnSystemAtLocation` "/Game/VFX/Upgrade/N_AS_Smoke_Placement_radial.N_AS_Smoke_Placement_radial" _returnvalue)
      (`GameplayStatics.SpawnSoundAtLocation` "/Game/TSS_Game/SFX/Weapon/HeavyStep3.HeavyStep3" _returnvalue (struct) 2.0 1.0 0.0 "/Game/TSS_Game/SFX/SAS_LocalHits.SAS_LocalHits" null))
    (:`OnCompleted`
      (`CharacterMovementComponent.SetMovementMode` (`self.CharacterMovement`) "MOVE_Walking" 0 :!label _label_12)
      (set `self.isAttacking` false)
      (set `self.IsCharging` false))
    (:`OnInterrupted`
      (goto _label_12))))

(fn `UserConstructionScript`
  (`parent.UserConstructionScript`))