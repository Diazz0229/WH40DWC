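; Elite Hormagant enemy, a child Blueprint that adds a recurring enrage ability, first triggered by taking damage.
; The first hit on the server starts a short random timer; when it fires on a living enemy, AI movement halts and MC_Enrage plays a threaten montage while attaching a speed mutation.
; When the montage completes or is interrupted, the server restores walking, clears the attacking flag and schedules the next enrage after a longer random delay.
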(event `/Game/TSS_Game/Blueprints/System/BPI_Damagable.DamageIntercation`
  (params (`Damage dealt` :type "Float (double-precision)") (Source :type "Actor Object Reference") (`IsMulticast?` :type Boolean) (DamageType :type "/Game/TSS_Game/Blueprints/Weapons/E_DamageTypes Enum" :default "NewEnumerator0"))
  ;[1 1 1] Abilities
  (`parent.DamageIntercation` `Damage dealt` Source `IsMulticast?` DamageType)
  (`/Engine/EditorBlueprintResources/ActorMacros.Switch Has Authority`
    (:`Authority`
      (`/Engine/EditorBlueprintResources/StandardMacros.DoOnce` false
        (:`Completed`
          (`KismetSystemLibrary.K2_SetTimerDelegate` (delegate `SV_Enrage`) (`KismetMathLibrary.RandomFloatInRange` 1.0 4.0)))))))

(event `SV_Enrage`
  ;[1 1 1] Abilities
  (if (not (`self.isDead`))
    (`self.MC_Enrage`)
    (`Controller.StopMovement` (`AIBlueprintHelperLibrary.GetAIController` self))
    (`CharacterMovementComponent.SetMovementMode` (`self.CharacterMovement`) "MOVE_None" 0)))

(event `MC_Enrage`
  ;[1 1 1] Abilities
  (set `self.isAttacking` true)
  (set `self.IsCharging` true)
  (`|PlayMontage` (`self.Mesh`) "/Game/WH40Assets/Tyranids/Animations/Montages/AM_Hormagant_Threaten.AM_Hormagant_Threaten"
    (:`then`
      (message `/Game/TSS_Game/Blueprints/AbilitySystem/EnemyMutations/Base/BPI_AttachableMutation.AttachMutation` self 1 "/Game/TSS_Game/Blueprints/AbilitySystem/EnemyMutations/AC_Mutation_MASpeed50.AC_Mutation_MASpeed50_C"))
    (:`OnCompleted`
      (`/Engine/EditorBlueprintResources/ActorMacros.Switch Has Authority` :!label _label
        (:`Authority`
          (`KismetSystemLibrary.K2_SetTimerDelegate` (delegate `SV_Enrage`) (`KismetMathLibrary.RandomFloatInRange` 30.0 45.0))
          (`CharacterMovementComponent.SetMovementMode` (`self.CharacterMovement`) "MOVE_Walking" 0)
          (set `self.isAttacking` false))))
    (:`OnInterrupted`
      (goto _label))))

(fn `UserConstructionScript`
  (`parent.UserConstructionScript`))