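; Spore Mine enemy that self-destructs into a toxic explosion, built on a parent enemy class.
; Its attack sequence calls the server death event on itself, and both attacking and dying feed one DoOnce-guarded detonation.
; Detonation plays the explode animation, then after a short delay hides the actor and spawns a scaled-down BP_ToxicExplosion at the hitbox, passing its ranged damage settings and itself as buff owner.
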(event `self.MC_AttackSequence`
  (`self.SV_EnemyDead` null "NewEnumerator5")
  (`/Engine/EditorBlueprintResources/StandardMacros.DoOnce` false :!label _label
    (:`Completed`
      (`SkeletalMeshComponent.PlayAnimation` (`self.Mesh`) "/Game/WH40Assets/Tyranids/SporeMine/SporeMine_Explode.SporeMine_Explode" false)
      (`KismetSystemLibrary.Delay` 0.35)
      (`self.SetActorHiddenInGame` true)
      (`|SpawnActorFromClass` "/Game/TSS_Game/Blueprints/Weapons/Base/BP_ToxicExplosion.BP_ToxicExplosion_C" (`KismetMathLibrary.MakeTransform` (`SceneComponent.K2_GetComponentLocation` (`self.Hitbox`)) (struct) (0.8 0.8 0.8)) "Undefined" "MultiplyWithRoot" null (`self.Damage Dealt Range`) (`self.Damage Type Range`) self null))))

(event `self.ReceiveBeginPlay`
  (`parent.ReceiveBeginPlay`))

(event `self.SV_EnemyDead`
  (params (`DMG source cast` :type "/Game/TSS_Game/Blueprints/System/BP_CharacterBase Object Reference") (DamageType :type "/Game/TSS_Game/Blueprints/Weapons/E_DamageTypes Enum" :default "NewEnumerator0"))
  (`parent.SV_EnemyDead` `DMG source cast` DamageType))

(event `self.MC_EnemyDead`
  (params (DamageType :type "/Game/TSS_Game/Blueprints/Weapons/E_DamageTypes Enum" :default "NewEnumerator0"))
  (`parent.MC_EnemyDead` "NewEnumerator0")
  (goto _label))

(fn `UserConstructionScript`
  (`parent.UserConstructionScript`))