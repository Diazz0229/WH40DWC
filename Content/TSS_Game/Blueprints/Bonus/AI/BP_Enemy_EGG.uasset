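; Tyranid egg enemy that, when triggered, glows and then bursts to hatch one or two Spore Mines.
; The attack runs once: a timeline ramps emissive glow and color on dynamic materials, then the server spawns the mines and kills the egg if still alive.
; Death swaps in a broken mesh with toxic explosion and sound; gore parts spawn from a bone list.
; On BeginPlay the server registers it in the game mode's enemy list.
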(event `self.ReceiveBeginPlay`
  (bind _sm_egg (`self.SM_Egg`))
  (for (_array_element _array_index) (`MeshComponent.GetMaterials` _sm_egg)
    (bind _returnvalue (`KismetMaterialLibrary.CreateDynamicMaterialInstance` _array_element))
    (`KismetArrayLibrary.Array_AddUnique` (`self.Materials_Dissolved`) _returnvalue)
    (`PrimitiveComponent.SetMaterial` _sm_egg _array_index _returnvalue))
  (`/Engine/EditorBlueprintResources/ActorMacros.Switch Has Authority`
    (:`Authority`
      (bind _asbp_game_mode_base (cast `/Game/TSS_Game/Blueprints/System/BP_GameModeBase` (`GameplayStatics.GetGameMode`)))
      (bind _output_get (set `self.As BP Game Mode Base` _asbp_game_mode_base))
      (`KismetArrayLibrary.Array_Add` (`/Game/TSS_Game/Blueprints/System/BP_GameModeBase.AllEnemiesArray` _output_get) self))))

(event `self.MC_AttackSequence`
  (`/Engine/EditorBlueprintResources/StandardMacros.DoOnce` false
    (:`Completed`
      (bind (_direction _duration) (`Timeline|Timeline_2` :!via `PlayFromStart`) ; 3 sec init
        (:`Update`
          (for _array_element (`self.Materials_Dissolved`)
            (`MaterialInstanceDynamic.SetScalarParameterValue` _array_element "GlowColorMultiplier" (`KismetMathLibrary.Lerp` 0.0 800.0 _duration))
            (`MaterialInstanceDynamic.SetVectorParameterValue` _array_element "EmissiveGlowColor" (make `LinearColor` (`KismetMathLibrary.Lerp` 0.0 1.0 _duration) (`KismetMathLibrary.Lerp` 1.0 0.0 _duration)))))
        (:`Finished`
          (`/Engine/EditorBlueprintResources/ActorMacros.Switch Has Authority`
            (:`Authority`
              (if (not (`self.isDead`))
                (`self.SpawnSpores`)
                (`self.SV_EnemyDead` null "NewEnumerator5")))))))))

(event `self.MC_EnemyDead`
  (params (DamageType :type "/Game/TSS_Game/Blueprints/Weapons/E_DamageTypes Enum" :default "NewEnumerator0"))
  (bind (_returnvalue_x _returnvalue_y _returnvalue_z) (`KismetMathLibrary.BreakVector` (`SceneComponent.K2_GetComponentLocation` (`self.SM_Egg`))))
  (`StaticMeshComponent.SetStaticMesh` (`self.SM_Egg`) "/Game/WH40Assets/Tyranids/Models/SM_TyranidEgg_broken.SM_TyranidEgg_broken")
  (`GameplayStatics.SpawnEmitterAtLocation` "/Game/TSS_Game/Particles/P_Explosion_Toxic.P_Explosion_Toxic" (`KismetMathLibrary.MakeVector` _returnvalue_x _returnvalue_y (+ _returnvalue_z 50.0)) (struct) (0.5 0.5 0.5))
  (`GameplayStatics.SpawnSoundAtLocation` "/Game/TSS_Game/SFX/Characters/Tyranids/SC_TYR_Sploosh.SC_TYR_Sploosh" (`SceneComponent.K2_GetComponentLocation` (`self.SM_Egg`)) (struct) 1.0 1.0 0.0 null null)
  (`parent.MC_EnemyDead` DamageType))

(event `SpawnSpores`
  (bind (_returnvalue_x _returnvalue_y _returnvalue_z) (`KismetMathLibrary.BreakVector` (`SceneComponent.K2_GetComponentLocation` (`self.SM_Egg`))))
  (for _ (range (+ (`KismetMathLibrary.RandomIntegerInRange` 1 2) 1))
    (`AIBlueprintHelperLibrary.SpawnAIFromClass` "/Game/TSS_Game/Blueprints/Bonus/AI/BPC_Enemy_SporeMine.BPC_Enemy_SporeMine_C" "/Game/TSS_Game/Blueprints/Bonus/AI/TyranidsAI/BT_AI_Basic_Melee.BT_AI_Basic_Melee" (`KismetMathLibrary.MakeVector` _returnvalue_x _returnvalue_y (+ _returnvalue_z 50.0)) (struct) true null)))

(event `self.SpawnGoreBodyParts`
  (bind (_returnvalue_x _returnvalue_y _returnvalue_z) (`KismetMathLibrary.BreakVector` (`SceneComponent.K2_GetComponentLocation` (`self.SM_Egg`))))
  (for _array_element (`self.GoreBoneNames`)
    (`|SpawnActorFromClass` (`.BodyPartBP_6_870A4F174662D9F858F9E0A003252CA6` (break `/Game/TSS_Game/Blueprints/Bonus/AI/ST_GoreBodyParts` _array_element)) (`KismetMathLibrary.MakeTransform` (`KismetMathLibrary.MakeVector` _returnvalue_x _returnvalue_y (+ _returnvalue_z 50.0)) (`KismetMathLibrary.RandomRotator` false)) "Undefined" "MultiplyWithRoot" null null)))

(fn `UserConstructionScript`
  (`parent.UserConstructionScript`))