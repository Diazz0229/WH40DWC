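; BP_Enemy_EGG_cluster is an enemy egg cluster that groups several eggs placed as child actor components.
; Its construction script loops over five child actor components and casts each spawned actor to BP_Enemy_BASE.
; Successful casts are added uniquely to the EggActors array, giving the cluster references to its individual eggs.
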(fn `UserConstructionScript`
  (for _array_element (`|MakeArray` (`self.ChildActor`) (`self.BP_Enemy_EGG_C_3`) (`self.BP_Enemy_EGG_C_2`) (`self.BP_Enemy_EGG_C_5`) (`self.BP_Enemy_EGG_C_4`))
    (bind _asbp_enemy_base (cast `/Game/TSS_Game/Blueprints/Bonus/AI/BP_Enemy_BASE` (`ChildActorComponent.ChildActor` _array_element)))
    (`KismetArrayLibrary.Array_AddUnique` (`self.EggActors`) _asbp_enemy_base)))