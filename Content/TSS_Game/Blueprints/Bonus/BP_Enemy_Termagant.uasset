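; Termagant enemy that attaches a Fleshborer weapon actor on begin play and fires bursts of projectiles at its player target.
; An attack line-traces for the target, then for blockers, moving toward the player when blocked and dropping the target when not found.
; Clear shots start a random-length burst via a self-calling delayed event, with random spread on each projectile's aim.
; A server-to-multicast event replays the burst on remote machines.
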(event `self.ReceiveBeginPlay`
  (bind _mesh (`self.Mesh`))
  ;[1 1 1] Begin play - attach weapon
  (`parent.ReceiveBeginPlay`)
  (bind _returnvalue (`|SpawnActorFromClass` "/Game/TSS_Game/Blueprints/Weapons/AI/BP_AI_WPN_Fleshborer.BP_AI_WPN_Fleshborer_C" (`SceneComponent.K2_GetComponentToWorld` _mesh) "Undefined" "MultiplyWithRoot" null null))
  (bind _output_get (set `self.WeaponMesh` _returnvalue))
  (`self.K2_AttachToComponent` _output_get _mesh "WeaponRT_socket" "SnapToTarget" "SnapToTarget" "SnapToTarget" true)
  (bind _asbp_ai_wpn_fleshborer (cast `/Game/TSS_Game/Blueprints/Weapons/AI/BP_AI_WPN_Fleshborer` _output_get))
  (set `self.Arrow Projectile Spawnpoint` (`/Game/TSS_Game/Blueprints/Weapons/AI/BP_AI_WPN_Fleshborer.Arrow_ProjectileSpawnpoint` _asbp_ai_wpn_fleshborer)))

(event `LC_StartAttackSequence`
  ;[1 1 1] Try to check if player is attackable
  (`/Engine/EditorBlueprintResources/StandardMacros.IsValid` (`self.Target Player Actor`)
    (:`Is Valid`
      (`/Engine/EditorBlueprintResources/StandardMacros.DoOnce` false :!label _label
        (:`Completed`
          (bind _outhits (`KismetSystemLibrary.LineTraceMultiForObjects` (+ (`self.K2_GetActorLocation` (`self.WeaponMesh`)) (0.0 0.0 180.0)) (+ (`self.K2_GetActorLocation` (`self.Target Player Actor`)) (0.0 0.0 80.0)) (`self.TraceForPawns`) false (`self.Actors to Ignore`)))
          (set `self.RangeTargetFound` false)
          (for _array_element _outhits
            (if (== (`self.Target Player Actor`) (`.HitActor` (`GameplayStatics.BreakHitResult` _array_element)))
              (set `self.RangeTargetFound` true)))
          (if (`self.RangeTargetFound`)
            (bind _outhits_2 (`KismetSystemLibrary.LineTraceMultiForObjects` (+ (`self.K2_GetActorLocation` (`self.WeaponMesh`)) (0.0 0.0 180.0)) (+ (`self.K2_GetActorLocation` (`self.Target Player Actor`)) (0.0 0.0 80.0)) (`self.TraceForBlockers`))) ; Check for blockers on the way
            (if (`KismetArrayLibrary.Array_IsNotEmpty` _outhits_2)
              (`self.ResetAttackSequence`)
              (`|AIMoveTo` self (0.0 0.0 0.0) (`self.Target Player Actor`) (`self.MeleeAttackRadius`))
              (else
                (bind _output_get (set `self.RangedShotsAmmount` (`KismetMathLibrary.RandomIntegerInRange` (`self.RangedShotsMin`) (`self.RangedShotsMax`))))
                (`self.ShootProjectile`)
                (`self.RotateToPlayer`)
                (`self.SV_StartAttackSequence` _output_get (`self.Target Player Actor`))))
            (else
              (set `self.Target Player Actor` null)
              (`self.ResetAttackSequence`))))))
    (:`Is Not Valid`
      (goto _label :!via `Reset`))))

(event `ResetAttackSequence`
  ;[1 1 1] Try to check if player is attackable
  (goto _label :!via `Reset`))

(event `ShootProjectile`
  ;[1 1 1] Projectile spawn
  (if (`self.isDead`)
    _
    (elif (<= (`self.RangedShotsAmmount`) 0)
      (set `self.isAttacking` false)
      (`self.ResetAttackSequence`)
      (else
        (set `self.isAttacking` true)
        (`/Engine/EditorBlueprintResources/StandardMacros.IsValid` (`self.Target Player Actor`)
          (:`Is Valid`
            (`self.RotateToPlayer`)
            (bind (_returnvalue_location _returnvalue_rotation) (`self.CalculateProjectileSpawn`))
            (`|SpawnActorFromClass` "/Game/TSS_Game/Blueprints/Weapons/AI/BP_Projectile_EnemyFleshborer.BP_Projectile_EnemyFleshborer_C" (`KismetMathLibrary.MakeTransform` _returnvalue_location _returnvalue_rotation) "Undefined" "MultiplyWithRoot" null (`self.Damage Dealt Range`) self 0 self)
            (`/Engine/EditorBlueprintResources/StandardMacros.DecrementInt` (`self.RangedShotsAmmount`)
              (:`  `
                (`KismetSystemLibrary.Delay` (`self.RangedShotsDelay`))
                (`self.ShootProjectile`)))))))))

(event `SV_StartAttackSequence`
  (params (Shots :type Integer) (`Target Player Actor` :type "Actor Object Reference"))
  (`self.MC_StartAttackSequence` Shots `Target Player Actor`))

(event `MC_StartAttackSequence`
  (params (Shots :type Integer) (`Target Player Actor` :type "Actor Object Reference"))
  (`/Engine/EditorBlueprintResources/ActorMacros.Switch Has Authority`
    (:`Remote`
      (set `self.RangedShotsAmmount` Shots)
      (set `self.Target Player Actor` `Target Player Actor`)
      (`self.ShootProjectile`)
      (`self.RotateToPlayer`))))

(fn `CalculateProjectileSpawn`
  (returns (ReturnValue_Location :type "Vector Structure") (ReturnValue_Rotation :type "Rotator Structure"))
  (bind _spread (`self.Spread`))
  (bind _spread_2 (`self.Spread`))
  (bind _spread_3 (`self.Spread`))
  (bind _returnvalue (`SceneComponent.K2_GetComponentLocation` (`self.Arrow Projectile Spawnpoint`)))
  (bind (_returnvalue_roll _returnvalue_pitch _returnvalue_yaw) (`KismetMathLibrary.BreakRotator` (`KismetMathLibrary.FindLookAtRotation` _returnvalue (`self.K2_GetActorLocation` (`self.Target Player Actor`)))))
  (return _returnvalue (`KismetMathLibrary.MakeRotator` (+ _returnvalue_roll (`KismetMathLibrary.RandomFloatInRange` (* (/ _spread_3 2.0) -1.0) _spread_3)) (+ _returnvalue_pitch (`KismetMathLibrary.RandomFloatInRange` (* (/ _spread_2 2.0) -1.0) (* _spread_2 1.2))) (+ _returnvalue_yaw (`KismetMathLibrary.RandomFloatInRange` (* _spread -1.0) _spread)))))

(fn `UserConstructionScript`
  (`parent.UserConstructionScript`))