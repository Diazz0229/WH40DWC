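; Background enemy that moves toward an end-path actor and then removes itself.
; Shortly after BeginPlay, it casts GoalActor to BP_BackgroundEnemy_EndPath and issues an AI MoveTo with a random point in that actor's box.
; The same MoveTo also receives GoalActor, which takes priority over the random location.
; Destruction follows a fixed delay from when the move is issued, regardless of arrival.
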(event `self.ReceiveBeginPlay`
  (bind _goal_actor (`self.Goal Actor`))
  (`KismetSystemLibrary.Delay` 0.5)
  (bind _asbp_background_enemy_end_path (cast `/Game/TSS_Game/Blueprints/LevelDesign/BP_BackgroundEnemy_EndPath` _goal_actor))
  (bind _box (`/Game/TSS_Game/Blueprints/LevelDesign/BP_BackgroundEnemy_EndPath.Box` _asbp_background_enemy_end_path))
  (`AITask_MoveTo.AIMoveTo` (`AIBlueprintHelperLibrary.GetAIController` self) (`KismetMathLibrary.RandomPointInBoundingBox` (`SceneComponent.K2_GetComponentLocation` _box) (`BoxComponent.BoxExtent` _box)) _goal_actor
    (:`then`
      (`KismetSystemLibrary.Delay` 6.0)
      (`self.K2_DestroyActor`))))

(fn `UserConstructionScript`)