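; BP_FireHazard is a fire hazard actor that deals periodic damage to characters standing inside it.
; Overlapping BP_CharacterBase actors join an array, and each entry triggers an immediate damage pass and starts or restarts a looping half-second timer.
; Each pass sends a small damage amount to every character in the array through DamageIntercationMessage.
; Leaving removes the character, and the timer clears once the array is empty.
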(event `StartDamaging`
  ;[1 1 1] Apply damage to all players inside the fire blueprint
  (for _array_element (`self.PlayerArray`)
    (bind _asbp_character_base (cast `/Game/TSS_Game/Blueprints/System/BP_CharacterBase` _array_element))
    (message `/Game/TSS_Game/Blueprints/System/BPI_Damagable.DamageIntercation` _asbp_character_base 0.1 null false "NewEnumerator0")))

(event `self.ReceiveActorBeginOverlap`
  (params (OtherActor :type "Actor Object Reference"))
  ;[1 1 1] Begin Overlap, add the player to the array and start damaging
  (bind _asbp_character_base (cast `/Game/TSS_Game/Blueprints/System/BP_CharacterBase` OtherActor))
  (`KismetArrayLibrary.Array_Add` (`self.PlayerArray`) _asbp_character_base)
  (`self.StartDamaging`)
  (`KismetSystemLibrary.K2_SetTimer` null "StartDamaging" 0.5 true))

(event `self.ReceiveActorEndOverlap`
  (params (OtherActor :type "Actor Object Reference"))
  (bind _playerarray (`self.PlayerArray`))
  ;[1 1 1] End Overlap, remove the player from the array and stop damaging it
  (bind _asbp_character_base (cast `/Game/TSS_Game/Blueprints/System/BP_CharacterBase` OtherActor))
  (`KismetArrayLibrary.Array_RemoveItem` _playerarray _asbp_character_base)
  (if (<= (`KismetArrayLibrary.Array_Length` _playerarray) 0)
    (`KismetSystemLibrary.K2_ClearTimer` null "StartDamaging")))

(fn `UserConstructionScript`)