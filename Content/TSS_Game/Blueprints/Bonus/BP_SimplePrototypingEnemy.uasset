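; Simple prototyping melee enemy for multiplayer, with optional aggression, roaming and player hunting.
; Looping timers run sphere-trace detection and random target picking to drive AIMoveTo, while attack-sphere overlaps start montages whose notify damages overlapping players.
; Damage passes through server and multicast events, with local prediction for the shooter.
; Death awards score, ragdolls, rolls data-table drops, then shrinks and destroys the actor; unused backup damage events remain.
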(event `self.ReceiveBeginPlay`
  ;[1 1 1] Begin Play
  (`KismetSystemLibrary.Delay` 0.2)
  (`|ExecutionSequence`
    (:`then_0`
      (if (`self.AI_agressive`)
        (`KismetSystemLibrary.K2_SetTimer` null "CheckForPlayerInRadius" 1.0 true)))
    (:`then_1`
      (if (`self.AI_knownPlayerPos`)
        (`KismetSystemLibrary.K2_SetTimer` null "HuntPlayers" 5.0 true)
        (`self.HuntPlayers`)))))

(event `AttackMontageMulticast`
  ;[1 1 1] Attack montage
  (`/Engine/EditorBlueprintResources/StandardMacros.DoOnce` false :!label _label
    (:`Completed`
      (set `self.isAttacking` true)
      (`KismetSystemLibrary.K2_SetTimer` null "AttackMontageMulticast" 1.5 true)
      (`|PlayMontage` (`self.Mesh`) "/Game/WH40Assets/Tyranids/Animations/Montages/AM_Hormagant_AttackMelee1.AM_Hormagant_AttackMelee1"
        (:`then`
          (`KismetSystemLibrary.RetriggerableDelay` 1.5)
          (set `self.isAttacking` false)
          (goto _label :!via `Reset`))
        (:`OnNotifyBegin`
          (for _array_element (`PrimitiveComponent.GetOverlappingActors` (`self.AttackTracerSphere`) "/Game/TSS_Game/Blueprints/System/BP_CharacterBase.BP_CharacterBase_C")
            (if (not (`self.ActorHasTag` _array_element "Invul"))
              (message `/Game/TSS_Game/Blueprints/System/BPI_Damagable.DamageIntercation` _array_element (`self.Damage Dealt`) self true "NewEnumerator0")
              (`GameplayStatics.SpawnSoundAtLocation` "/Game/TSS_Game/SFX/Weapon/Melee/Impact_Punch_Harder01_Cue.Impact_Punch_Harder01_Cue" (`self.K2_GetActorLocation` _array_element) (struct) 0.5 1.0 0.0 null null) ; Firing Sound
            )))))))

(event `self.AttackTracerSphere.OnComponentBeginOverlap`
  (params (OverlappedComponent :type "PrimitiveComponent Object Reference") (OtherActor :type "Actor Object Reference") (OtherComp :type "PrimitiveComponent Object Reference") (OtherBodyIndex :type Integer) (bFromSweep :type Boolean) (SweepResult :type "HitResult Structure (by ref)"))
  ;[1 1 1] Damage Player (overlap with the sphere)
  (cast `/Game/TSS_Game/Blueprints/System/BP_CharacterBase` OtherActor) ; Choose only players
  (`self.AttackMontageMulticast`))

(event `CheckForPlayerInRadius`
  (bind _returnvalue (`self.K2_GetActorLocation`))
  ;[1 1 1] Move to nearest Player
  (if (not (or (`self.isAttacking`) (`self.isDead`)))
    (bind (_outhit _returnvalue_2) (`KismetSystemLibrary.SphereTraceSingleForObjects` _returnvalue (- _returnvalue (0.0 0.0 50.0)) 800.0 (`self.ObjectType`)))
    (if _returnvalue_2
      (set `self.Target Player Actor` (`.HitActor` (`GameplayStatics.BreakHitResult` _outhit)))
      (`/Engine/EditorBlueprintResources/StandardMacros.DoOnce` false :!label _label_2
        (:`Completed`
          (`self.MoveToPlayer` (`self.Target Player Actor`))))
      (else
        ;;[1 1 1] Random Location if no Player has been detected
        (if (`self.AI_roaming`)
          (`AITask_MoveTo.AIMoveTo` (`AIBlueprintHelperLibrary.GetAIController` self) (`NavigationSystemV1.K2_GetRandomReachablePointInRadius` (`self.K2_GetActorLocation`) 500.0 null null) null 10.0 "Default" "Default" true false))))))

(event `self.AttackTracerSphere.OnComponentEndOverlap`
  (params (OverlappedComponent :type "PrimitiveComponent Object Reference") (OtherActor :type "Actor Object Reference") (OtherComp :type "PrimitiveComponent Object Reference") (OtherBodyIndex :type Integer))
  ;[1 1 1] Damage Player (overlap with the sphere)
  (cast `/Game/TSS_Game/Blueprints/System/BP_CharacterBase` OtherActor)
  (`KismetSystemLibrary.K2_ClearTimer` null "AttackMontageMulticast"))

(event `HuntPlayers`
  ;[1 1 1] Move to nearest Player
  (if (not (`KismetSystemLibrary.IsValid` (`self.Target Player Actor`)))
    (bind _outactors (`GameplayStatics.GetAllActorsOfClass` "/Game/TSS_Game/Blueprints/System/BP_CharacterBase.BP_CharacterBase_C"))
    (set `self.Target Player Actor` (`KismetArrayLibrary.Array_Random` _outactors))
    (goto _label_2)))

(event `MoveToPlayer`
  (params (GoalActor :type "Actor Object Reference"))
  ;[1 1 1] Move to nearest Player
  (if (not (and (`self.isDead`) (`self.isAttacking`)))
    (`AITask_MoveTo.AIMoveTo` (`AIBlueprintHelperLibrary.GetAIController` self) (0.0 0.0 0.0) GoalActor (`self.Acceptance Radius`) "Default" "Default" true false
      (:`OnMoveFinished`
        (goto _label_2 :!via `Reset`)))))

(event `/Game/TSS_Game/Blueprints/System/BPI_Damagable.DamageIntercation`
  (params (`Damage dealt` :type "Float (double-precision)") (Source :type "Object Object Reference") (`IsMulticast?` :type Boolean) (DamageType :type "/Game/TSS_Game/Blueprints/Weapons/E_DamageTypes Enum" :default "NewEnumerator0"))
  (bind _dmg_source_cast (`self.DMG source cast`))
  ;[1 1 1] Deals with health and damage stuff
  (bind _asbp_character_base (cast `/Game/TSS_Game/Blueprints/System/BP_CharacterBase` Source))
  (bind _output_get (set `self.DMG source cast` _asbp_character_base))
  (if (and (`self.IsLocallyControlled` _output_get) (not `IsMulticast?`))
    (bind _output_get_2 (set `self.Health` (- (`self.Health`) `Damage dealt`)))
    (`self.LC_EnemyBlood`)
    (if (<= _output_get_2 0.0)
      (`/Engine/EditorBlueprintResources/StandardMacros.DoOnce` false
        (:`Completed`
          (`/Game/TSS_Game/Blueprints/System/BP_PlayerController.SV_KillEnemy` (`/Game/TSS_Game/Blueprints/System/BP_CharacterBase.OwningPlayerController` (`self.DMG source cast`)) self)
          (`self.F_SetCharDead`)))
      (else
        (`self.LC_EnemyBlood`)))
    (elif (not (`self.IsLocallyControlled` _dmg_source_cast))
      (`self.SV_DamageWasDealt` `Damage dealt` _dmg_source_cast))))

(event `SV_DamageWasDealt`
  (params (Damage :type "Float (double-precision)") (`DMG source cast` :type "/Game/TSS_Game/Blueprints/System/BP_CharacterBase Object Reference"))
  ;[1 1 1] Deals with health and damage stuff
  (bind _output_get (set `self.Health` (- (`self.Health`) Damage)))
  (if (<= _output_get 0.0)
    (`self.SV_EnemyDead` (`self.DMG source cast`))
    (else
      (`self.MC_DamageWasDealt` Damage `DMG source cast`))))

(event `MC_DamageWasDealt`
  (params (Damage :type "Float (double-precision)") (`DMG source cast` :type "/Game/TSS_Game/Blueprints/System/BP_CharacterBase Object Reference"))
  ;[1 1 1] Deals with health and damage stuff
  (if (not (`self.IsLocallyControlled` `DMG source cast`))
    (set `self.Health` (- (`self.Health`) Damage)))
  (`self.LC_EnemyBlood`))

(event `LC_EnemyBlood`
  ;[1 1 1] Deals with health and damage stuff
  (`GameplayStatics.SpawnEmitterAtLocation` "/Game/TSS_Game/Particles/P_body_bullet_impact.P_Body_Bullet_Impact" (`SceneComponent.K2_GetComponentLocation` (`self.Hitbox`)) (struct) (5.0 5.0 5.0)))

(event `SV_EnemyDead`
  (params (`DMG source cast` :type "/Game/TSS_Game/Blueprints/System/BP_CharacterBase Object Reference"))
  ;[1 1 1] Deals with health and damage stuff
  (bind _output_get (set `self.DMG source cast` `DMG source cast`))
  (bind _playerstate (`Controller.PlayerState` (`self.GetController` _output_get)))
  (`/Engine/EditorBlueprintResources/StandardMacros.IsValid` _playerstate
    (:`Is Valid`
      (bind _asbp_player_state (cast `/Game/TSS_Game/Blueprints/System/BP_PlayerState` _playerstate))
      (set `/Game/TSS_Game/Blueprints/System/BP_PlayerState.PlayerScore` (+ (`/Game/TSS_Game/Blueprints/System/BP_PlayerState.PlayerScore` _asbp_player_state) 1) _asbp_player_state)
      (set `self.isDead` true)
      (`self.DetachFromControllerPendingDestroy`)
      (`self.MC_EnemyDead`))))

(event `MC_EnemyDead`
  (bind _returnvalue (`KismetMathLibrary.RandomFloatInRange` -100.0 100.0))
  ;[1 1 1] Death - Happens on all clients
  (`self.F_SetCharDead`)
  (`|ExecutionSequence`
    (:`then_0`
      (if (`self.DropsItems?`) :!pinned true
        (bind _outrownames (`DataTableFunctionLibrary.GetDataTableRowNames` "/Game/TSS_Game/Blueprints/Pickup/DT_DropTable_Hormagaunt.DT_DropTable_Hormagaunt"))
        (for _array_element _outrownames
          (bind _returnvalue_2 (`|GetDataTableRow` "/Game/TSS_Game/Blueprints/Pickup/DT_DropTable_Hormagaunt.DT_DropTable_Hormagaunt" _array_element)
            (:`then`
              (if (<= (`KismetMathLibrary.RandomFloatInRange` 0.0 100.0) (`.ChanceToDrop_5_687A509C4FFEF1541AE9659D108160BA` (break `/Game/TSS_Game/Blueprints/Pickup/ST_DropTableStruct` _returnvalue_2)))
                (`|SpawnActorFromClass` (break `/Game/TSS_Game/Blueprints/Pickup/ST_DropTableStruct` _returnvalue_2) (`KismetMathLibrary.MakeTransform` (+ (`self.K2_GetActorLocation`) (`KismetMathLibrary.MakeVector` _returnvalue _returnvalue))) "Undefined" "MultiplyWithRoot" null null)))))))
    (:`then_1`
      (`KismetSystemLibrary.Delay` 5.0)
      (bind (_direction _duration) (`Timeline|Timeline_0` :!via `PlayFromStart`)
        (:`Update`
          (`SceneComponent.SetWorldScale3D` (`self.Mesh`) (`KismetMathLibrary.VLerp` (1.0 1.0 1.0) (0.0 0.0 0.0) _duration)))
        (:`Finished`
          (`self.K2_DestroyActor`))))))

(event `CustomEvent`
  (params (`Damage dealt` :type "Float (double-precision)") (Source :type "Object Object Reference") (`IsMulticast?` :type Boolean))
  (bind _playerstate (`Controller.PlayerState` (`self.GetController` (`self.DMG source cast`))))
  ;[1 1 1] Reserv_copy_deal damage
  (bind _asbp_character_base (cast `/Game/TSS_Game/Blueprints/System/BP_CharacterBase` Source))
  (bind _output_get (set `self.DMG source cast` _asbp_character_base))
  (if (and (`self.IsLocallyControlled` _output_get) (not `IsMulticast?`))
    (bind _output_get_2 (set `self.Health` (- (`self.Health`) `Damage dealt`)))
    (`self.LC_EnemyBlood`)
    (if (<= _output_get_2 0.0)
      (`KismetSystemLibrary.PrintString` (`KismetStringLibrary.Conv_DoubleToString` _output_get_2))
      (`/Engine/EditorBlueprintResources/StandardMacros.DoOnce` false
        (:`Completed`
          (`self.SV_EnemyDead` null)
          (`self.F_SetCharDead`))))
    (else
      (if (`self.IsLocallyControlled` (`self.DMG source cast`))
        (`/Engine/EditorBlueprintResources/ActorMacros.Switch Has Authority`
          (:`Authority`
            _)))
      (set `self.Health` (- (`self.Health`) `Damage dealt`))
      (`self.LC_EnemyBlood`)
      (if (<= (`self.Health`) 0.0)
        (`/Engine/EditorBlueprintResources/StandardMacros.DoOnce` false
          (:`Completed`
            (`self.SV_EnemyDead` null)
            (`/Engine/EditorBlueprintResources/StandardMacros.IsValid` _playerstate
              (:`Is Valid`
                (bind _asbp_player_state (cast `/Game/TSS_Game/Blueprints/System/BP_PlayerState` _playerstate))
                (set `/Game/TSS_Game/Blueprints/System/BP_PlayerState.PlayerScore` (+ (`/Game/TSS_Game/Blueprints/System/BP_PlayerState.PlayerScore` _asbp_player_state) 1) _asbp_player_state)))))))))

(event `CustomEvent_1`
  ;[1 1 1] Reserv_copy_deal damage
  (set `self.isDead` true)
  (`self.DetachFromControllerPendingDestroy`)
  (`self.MC_EnemyDead`))

(event `CustomEvent_2`
  ;[1 1 1] Reserv_copy_deal damage
  (`GameplayStatics.SpawnEmitterAtLocation` "/Game/TSS_Game/Particles/P_body_bullet_impact.P_Body_Bullet_Impact" (`SceneComponent.K2_GetComponentLocation` (`self.Hitbox`)) (struct) (5.0 5.0 5.0)))

(fn `F_SetCharDead`
  (bind _charactermovement (`self.CharacterMovement`))
  (bind _mesh (`self.Mesh`))
  (`MovementComponent.StopMovementImmediately` _charactermovement)
  (`NavMovementComponent.StopActiveMovement` _charactermovement)
  (set `CharacterMovementComponent.MaxWalkSpeed` 0.0 _charactermovement)
  (`KismetArrayLibrary.Array_Add` (`self.Tags`) "Dead")
  (`PrimitiveComponent.SetCollisionResponseToChannel` _mesh "ECC_WorldDynamic" "ECR_Ignore")
  (`PrimitiveComponent.SetCollisionResponseToChannel` _mesh "ECC_GameTraceChannel1" "ECR_Ignore")
  (`PrimitiveComponent.SetCollisionEnabled` (`self.CapsuleComponent`) "NoCollision")
  (`PrimitiveComponent.SetCollisionEnabled` (`self.Hitbox`) "NoCollision")
  (`PrimitiveComponent.SetCollisionEnabled` (`self.AttackTracerSphere`) "NoCollision")
  (`PrimitiveComponent.SetSimulatePhysics` (`self.Mesh`) true)
  (return))

(fn `UserConstructionScript`)