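; Level-placed spawner that creates an ammo crate at its own transform when its SpawnAmmoCrate event is called.
; A FakeCrate placeholder component is destroyed at BeginPlay, leaving the spot empty until a spawn is triggered.
; Each spawn uses the SpawnedActor class and stores the result in AttachedCrate, without attaching it or checking for an existing crate.
; CrateValidation reports whether that stored crate is still valid.
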(event `self.ReceiveBeginPlay`
  (`ActorComponent.K2_DestroyComponent` (`self.FakeCrate`)))

(event `SpawnAmmoCrate`
  (bind _returnvalue (`|SpawnActorFromClass` (`self.SpawnedActor`) (`self.GetTransform`) "Undefined" "MultiplyWithRoot" null null))
  (set `self.AttachedCrate` _returnvalue))

(fn `Crate Validation`
  (returns (IsCrateValid :type Boolean))
  (return (`KismetSystemLibrary.IsValid` (`self.AttachedCrate`))))

(fn `UserConstructionScript`)