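; Level-placed enemy spawner that, while active, spawns regular wave enemies at random points inside its box, leaving bosses to the game mode.
; BeginSpawns sets wave data and limits, adds or levels up a mutation, and starts a looping spawn timer.
; Each tick checks the game mode's enemy count against the cap, then rolls table chances.
; Authority spawns AI with behavior trees, registers them, and attaches accumulated mutations through BPI_AttachableMutation.
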(event `self.ReceiveBeginPlay`
  (`/Engine/EditorBlueprintResources/ActorMacros.Switch Has Authority`
    (:`Authority`
      (`KismetSystemLibrary.Delay` 3.0)
      (if (`self.IsActive?`)
        (bind _asbp_game_mode_base (cast `/Game/TSS_Game/Blueprints/System/BP_GameModeBase` (`GameplayStatics.GetGameMode`))
          (:`then`
            (set `self.GameModeCast` _asbp_game_mode_base))
          (:`CastFailed`
            (`KismetSystemLibrary.PrintString` "BP_EnemySpawner: Couldn't cast to Game mode! " true true (struct :`R` 1.0 :`G` 0.024638 :`A` 1.0) 4.0)))))))

(event `BeginSpawns`
  (params (EnemiesPerSpawn :type Integer) (EnemiesMax :type Integer) (NewMutation :type "/Game/TSS_Game/Blueprints/AbilitySystem/EnemyMutations/Base/AC_Mutation_BASE Class Reference (by ref)") (WaveList :type "/Game/TSS_Game/Blueprints/Bonus/AI/ST_WaveList Structure"))
  (bind _mutationsadded (`self.MutationsAdded`))
  (bind _mutationsadded_2 (`self.MutationsAdded`))
  (`KismetSystemLibrary.K2_SetTimer` null "SpawnEnemies" 1.0 true)
  (set `self.EnemiesSpawned` EnemiesPerSpawn)
  (set `self.EnemiesMax` EnemiesMax)
  (set `self.MutationWasLeveled` false)
  (set `self.Wave List` WaveList)
  (for _array_element _mutationsadded_2
    (bind (_bp_component _level) (break `/Game/TSS_Game/Blueprints/AbilitySystem/EnemyMutations/Base/ST_MutationSettings` _array_element))
    (if (== _bp_component NewMutation)
      (`KismetArrayLibrary.Array_Add` _mutationsadded (make `/Game/TSS_Game/Blueprints/AbilitySystem/EnemyMutations/Base/ST_MutationSettings` NewMutation (+ _level 1)))
      (`KismetArrayLibrary.Array_RemoveItem` _mutationsadded _array_element)
      (set `self.MutationWasLeveled` true)))
  (if (not (`self.MutationWasLeveled`))
    (`KismetArrayLibrary.Array_AddUnique` _mutationsadded_2 (make `/Game/TSS_Game/Blueprints/AbilitySystem/EnemyMutations/Base/ST_MutationSettings` NewMutation 1))))

(event `SpawnEnemies`
  (bind (_enemyclass _spawnchance _behaviortree) (break `/Game/TSS_Game/Blueprints/Bonus/AI/ST_WaveList` (`self.Wave List`)))
  ;[1 1 1] Determine if enemies are not more than max ammount
  (if (`self.IsActive?`)
    (bind _asbp_game_mode_base (cast `/Game/TSS_Game/Blueprints/System/BP_GameModeBase` (`GameplayStatics.GetGameMode`)))
    (if (< (`KismetArrayLibrary.Array_Length` (`/Game/TSS_Game/Blueprints/System/BP_GameModeBase.AllEnemiesArray` _asbp_game_mode_base)) (`self.EnemiesMax`))
      ;[1 1 1] Get Max chance cause table can have >100% chance
      (set `self.MaxSpawnChance` 0)
      (for _array_element (`.SpawnChance_8_F9413F8F4665FBD2F9637EAE00FAAA70` (break `/Game/TSS_Game/Blueprints/Bonus/AI/ST_WaveList` (`self.Wave List`)))
        (set `self.MaxSpawnChance` (+ (`self.MaxSpawnChance`) _array_element))
        ;[1 1 1] Get Wave list table and spawn simple enemies (bosses are spawned directly from game mode)
        (for (_array_element_2 _array_index) _enemyclass
          (for _ (range 1 (+ (`self.EnemiesSpawned`) 1))
            (set `self.RandomSpawnChance` (`KismetMathLibrary.RandomIntegerInRange` 0 (`self.MaxSpawnChance`)))
            (if (<= (`self.RandomSpawnChance`) (`|GetArrayItem` _spawnchance _array_index))
              (`/Engine/EditorBlueprintResources/ActorMacros.Switch Has Authority`
                (:`Authority`
                  (bind _returnvalue (`AIBlueprintHelperLibrary.SpawnAIFromClass` (castclass `Pawn` _array_element_2 :!pure true) (`|GetArrayItem` _behaviortree _array_index) (+ (`KismetMathLibrary.RandomPointInBoundingBox` (`SceneComponent.K2_GetComponentLocation` (`self.DefaultSceneRoot`)) (`BoxComponent.BoxExtent` (`self.Box`))) (0.0 0.0 50.0)) (struct) false null))
                  (bind _output_get (set `self.TEMP_SpawnedEnemy` _returnvalue))
                  (bind _asbp_game_mode_base_2 (cast `/Game/TSS_Game/Blueprints/System/BP_GameModeBase` (`GameplayStatics.GetGameMode`)))
                  (`KismetArrayLibrary.Array_AddUnique` (`/Game/TSS_Game/Blueprints/System/BP_GameModeBase.AllEnemiesArray` _asbp_game_mode_base_2) _output_get)
                  ;[1 1 1] Attach mutations to spawned enemy
                  (if (`KismetSystemLibrary.DoesImplementInterface` _output_get "/Game/TSS_Game/Blueprints/AbilitySystem/EnemyMutations/Base/BPI_AttachableMutation.BPI_AttachableMutation_C")
                    (for _array_element_3 (`self.MutationsAdded`)
                      (bind (_bp_component _level) (break `/Game/TSS_Game/Blueprints/AbilitySystem/EnemyMutations/Base/ST_MutationSettings` _array_element_3))
                      (message `/Game/TSS_Game/Blueprints/AbilitySystem/EnemyMutations/Base/BPI_AttachableMutation.AttachMutation` (`self.TEMP_SpawnedEnemy`) _level _bp_component))))))))))))

(fn `UserConstructionScript`)