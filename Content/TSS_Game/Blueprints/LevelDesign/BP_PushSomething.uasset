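; BP_PushSomething is a pushable pawn that slides briefly when a BP_CharacterBase hits it.
; CalculateDirection snaps the hit normal's yaw, relative to the pawn's yaw, to one of four axis-aligned world directions.
; Tick feeds that direction into AddMovementInput while CanMove is true.
; A DoOnce gate ignores further hits until the half-second delay ends, stops movement and resets it.
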(event `Reset`
  (goto _label :!via `Reset`))

(event `self.ReceiveHit`
  (params (MyComp :type "PrimitiveComponent Object Reference") (Other :type "Actor Object Reference") (OtherComp :type "PrimitiveComponent Object Reference") (bSelfMoved :type Boolean) (HitLocation :type "Vector Structure") (HitNormal :type "Vector Structure") (NormalImpulse :type "Vector Structure") (Hit :type "HitResult Structure (by ref)"))
  (bind _asbp_character_base (cast `/Game/TSS_Game/Blueprints/System/BP_CharacterBase` Other))
  (`/Engine/EditorBlueprintResources/StandardMacros.IsValid` _asbp_character_base
    (:`Is Valid`
      (`/Engine/EditorBlueprintResources/StandardMacros.DoOnce` false :!label _label
        (:`Completed`
          (`self.CalculateDirection` HitNormal)
          (set `self.CanMove` true)
          (`KismetSystemLibrary.RetriggerableDelay` 0.5)
          (set `self.CanMove` false)
          (`self.Reset`))))))

(event `self.ReceiveTick`
  (params (DeltaSeconds :type "Float (single-precision)"))
  (if (`self.CanMove`)
    (`self.AddMovementInput` (`self.Direction`))))

(fn `CalculateDirection`
  (params (InVec :type "Vector Structure"))
  (switch `int` (`KismetMathLibrary.Round` (/ (+ (- (.yaw (`KismetMathLibrary.Conv_VectorToRotator` InVec)) (.yaw (`self.K2_GetActorRotation`))) 180.0) 90.0))
    (:`Default`
      (set `self.Direction` (-1.0 0.0 0.0) :!label _label))
    (:`0`
      (goto _label))
    (:`1`
      (set `self.Direction` (0.0 -1.0 0.0)))
    (:`2`
      (set `self.Direction` (1.0 0.0 0.0)))
    (:`3`
      (set `self.Direction` (0.0 1.0 0.0))))
  (return))

(fn `UserConstructionScript`)