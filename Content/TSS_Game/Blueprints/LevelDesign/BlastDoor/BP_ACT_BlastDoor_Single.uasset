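; BP_ACT_BlastDoor_Single is an activatable level-design blast door that lowers open and enables linked enemy spawners.
; On its first activation, it triggers linked alert lights and plays a Timeline.
; Each Timeline update lowers the mesh by OpenSpeed, making movement depend on update rate.
; At a fixed height threshold it stops, sets the spawners active and calls the parent's activation.
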(event `self.MC_Activate`
  (`self.MC_OpenDoor` (`self.Open Speed`)))

(event `MC_OpenDoor`
  (params (OpenSpeed :type "Float (double-precision)" :default 15.0))
  (bind _blastdoormesh1 (`self.BlastDoorMesh1`))
  (bind (_relativelocation_x _relativelocation_y _relativelocation_z) (`KismetMathLibrary.BreakVector` (`SceneComponent.RelativeLocation` _blastdoormesh1)))
  (`/Engine/EditorBlueprintResources/StandardMacros.DoOnce` false
    (:`Completed`
      (for _array_element (`self.Lamps_0`)
        (bind _asbp_act_alert_lights (cast `/Game/TSS_Game/Blueprints/LevelDesign/BlastDoor/BP_ACT_AlertLights` _array_element))
        (`self.MC_Activate` _asbp_act_alert_lights))
      (`Timeline|Timeline` :!label _label
        (:`Update`
          (`SceneComponent.K2_SetRelativeLocation` _blastdoormesh1 (`KismetMathLibrary.MakeVector` _relativelocation_x _relativelocation_y (- _relativelocation_z OpenSpeed)) false false)
          (if (<= _relativelocation_z 200.0)
            (`self.StopOpening`)
            (for _array_element_2 (`self.NewAISpawns`)
              (bind _asbp_enemy_spawner (cast `/Game/TSS_Game/Blueprints/LevelDesign/Spawners/BP_EnemySpawner` _array_element_2))
              (set `/Game/TSS_Game/Blueprints/LevelDesign/Spawners/BP_EnemySpawner.IsActive?` true _asbp_enemy_spawner))
            (`parent.MC_Activate`)))))))

(event `StopOpening`
  (goto _label :!via `Stop`))

(event `self.ReceiveBeginPlay`
  (`parent.ReceiveBeginPlay`))

(fn `UserConstructionScript`
  (`parent.UserConstructionScript`))