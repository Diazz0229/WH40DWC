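; Alarm beacon actor in the BlastDoor level-design set, with two spotlights and an alarm sound switched by activate and deactivate events.
; MCActivate shows the lights, spins them through RotatingMovement yaw and spawns the attenuated alarm, skipping the sound if IsInitialyActivated is set.
; MCDeactivate halts rotation, hides the lights and stops the stored sound, destroying that manually managed component after a short delay.
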(event `self.MC_Activate`
  (set `RotatingMovementComponent.RotationRate` (struct :`Pitch` 180.0) (`self.RotatingMovement`))
  (`SceneComponent.SetVisibility` (`self.SpotLight1`) true false)
  (`SceneComponent.SetVisibility` (`self.SpotLight`) true false)
  (if (not (`self.IsInitialyActivated?`))
    (bind _returnvalue (`GameplayStatics.SpawnSoundAtLocation` "/Game/TSS_Game/SFX/DecoSounds/SC_Alarm.SC_Alarm" (`SceneComponent.K2_GetComponentLocation` (`self.DefaultSceneRoot`)) (struct) 1.0 1.0 0.0 "/Game/TSS_Game/SFX/SAS_LocalHits.SAS_LocalHits" null false))
    (set `self.SpawnedSound` _returnvalue)))

(event `self.MC_Deactivate`
  (bind _spawnedsound (`self.SpawnedSound`))
  (set `RotatingMovementComponent.RotationRate` (struct) (`self.RotatingMovement`))
  (`SceneComponent.SetVisibility` (`self.SpotLight1`) false false)
  (`SceneComponent.SetVisibility` (`self.SpotLight`) false false)
  (`AudioComponent.Stop` _spawnedsound)
  (`KismetSystemLibrary.Delay` 2.0)
  (`ActorComponent.K2_DestroyComponent` _spawnedsound))

(fn `UserConstructionScript`
  (`parent.UserConstructionScript`))