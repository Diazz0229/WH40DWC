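; BP_Button is a single-use interactable button in the BlastDoor level-design set that triggers a list of linked actors.
; Interaction calls the MC activate event, which validates the interacting character and passes a DoOnce gate.
; It then calls SVActivate on each valid BP_Activatable_Base in ActorsToActivate, hides its light and plays a switch sound at its location.
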(event `self.ReceiveBeginPlay`)

(event `/Game/TSS_Game/Blueprints/System/BPI_Interactive.Interact With Actor`
  (params (CharacterReference :type "/Game/TSS_Game/Blueprints/System/BP_CharacterBase Object Reference"))
  (`self.MC_Activate` CharacterReference))

(event `MC_Activate`
  (params (InputObject :type "Object Object Reference"))
  (`/Engine/EditorBlueprintResources/StandardMacros.IsValid` InputObject
    (:`Is Valid`
      (`/Engine/EditorBlueprintResources/StandardMacros.DoOnce` false
        (:`Completed`
          (for _array_element (`self.ActorsToActivate`)
            (`/Engine/EditorBlueprintResources/StandardMacros.IsValid` _array_element
              (:`Is Valid`
                (bind _asbp_activatable_base (cast `/Game/TSS_Game/Blueprints/LevelDesign/BP_Activatable_Base` _array_element))
                (`/Game/TSS_Game/Blueprints/LevelDesign/BP_Activatable_Base.SV_Activate` _asbp_activatable_base))))
          (`SceneComponent.SetHiddenInGame` (`self.Light`) true false)
          (`GameplayStatics.PlaySoundAtLocation` "/Engine/VREditor/Sounds/UI/Flashlight_Switch.Flashlight_Switch" (`self.K2_GetActorLocation`) (struct) 1.0 1.0 0.0 null null null null))))))

(fn `UserConstructionScript`)