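; Activatable bridge for level design that slides its bridge part along Z from a start height to a target height, despite the "Rotate" naming.
; Activation plays machinery audio and, only once, switches on linked alert lamps and runs a Timeline that adds OpenSpeed each update.
; At the target, it stops motion and sound, turns off the lamps, enables enemy spawners, then activates linked doors after a short delay.
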(event `self.MC_Activate`
  (`self.MC_RotateBridge` (`self.Open Speed`))
  (bind _returnvalue (`GameplayStatics.SpawnSoundAtLocation` "/Game/TSS_Game/SFX/DecoSounds/SC_MachineryWorking.SC_MachineryWorking" (`SceneComponent.K2_GetComponentLocation` (`self.DefaultSceneRoot`)) (struct) 1.5 1.0 0.0 null null false))
  (set `self.SpawnedSound` _returnvalue))

(event `MC_RotateBridge`
  (params (OpenSpeed :type "Float (double-precision)"))
  (bind _bridgepart (`self.BridgePart`))
  (bind (_relativelocation_x _relativelocation_y _relativelocation_z) (`KismetMathLibrary.BreakVector` (`SceneComponent.RelativeLocation` _bridgepart)))
  (bind _returnvalue (+ _relativelocation_z OpenSpeed))
  (`/Engine/EditorBlueprintResources/StandardMacros.DoOnce` false
    (:`Completed`
      (for _array_element (`self.Lamps`)
        (bind _asbp_act_alert_lights (cast `/Game/TSS_Game/Blueprints/LevelDesign/BlastDoor/BP_ACT_AlertLights` _array_element))
        (`self.MC_Activate` _asbp_act_alert_lights))
      (`Timeline|Timeline` :!label _label
        (:`Update`
          (`SceneComponent.K2_SetRelativeLocation` _bridgepart (`KismetMathLibrary.MakeVector` _relativelocation_x _relativelocation_y _returnvalue) false false)
          (if (>= _returnvalue (`self.TargetPosZ`))
            (`self.StopRotating`)
            (bind (_arrayindex _arrayelement) (`/Engine/EditorBlueprintResources/StandardMacros.ReverseForEachLoop` (`self.Lamps`))
              (:`LoopBody`
                (bind _asbp_act_alert_lights_2 (cast `/Game/TSS_Game/Blueprints/LevelDesign/BlastDoor/BP_ACT_AlertLights` _arrayelement))
                (`self.MC_Deactivate` _asbp_act_alert_lights_2))
              (:`Completed`
                (for _array_element_2 (`self.NewAISpawns`)
                  (bind _asbp_enemy_spawner (cast `/Game/TSS_Game/Blueprints/LevelDesign/Spawners/BP_EnemySpawner` _array_element_2))
                  (set `/Game/TSS_Game/Blueprints/LevelDesign/Spawners/BP_EnemySpawner.IsActive?` true _asbp_enemy_spawner))
                (`KismetSystemLibrary.Delay` 2.0)
                (for _array_element_3 (`self.OpenDoors`)
                  (bind _asbp_activatable_base (cast `/Game/TSS_Game/Blueprints/LevelDesign/BP_Activatable_Base` _array_element_3))
                  (`self.MC_Activate` _asbp_activatable_base))))))))))

(event `StopRotating`
  (bind _spawnedsound (`self.SpawnedSound`))
  (`AudioComponent.Stop` _spawnedsound)
  (`ActorComponent.K2_DestroyComponent` _spawnedsound)
  (goto _label :!via `Stop`))

(event `self.ReceiveBeginPlay`
  (bind _bridgepart (`self.BridgePart`))
  (bind (_relativelocation_x _relativelocation_y) (`KismetMathLibrary.BreakVector` (`SceneComponent.RelativeLocation` _bridgepart)))
  (`parent.ReceiveBeginPlay`)
  (`SceneComponent.K2_SetRelativeLocation` _bridgepart (`KismetMathLibrary.MakeVector` _relativelocation_x _relativelocation_y (`self.Start Location Z`)) false false))

(fn `UserConstructionScript`
  (`parent.UserConstructionScript`))