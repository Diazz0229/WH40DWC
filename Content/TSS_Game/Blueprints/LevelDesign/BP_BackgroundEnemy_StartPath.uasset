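; Level-design spawner that continuously feeds background enemies into the level from a box volume and hands each a goal actor.
; On the authority, BeginPlay waits briefly and, if IsActive is set, starts a looping timer that fires SpawnEnemies every half second.
; Each tick rechecks IsActive, spawns a BP_Enemy_Background at a random point in the Box extent around the root, and sets its GoalActor.
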(event `self.ReceiveBeginPlay`
  (`/Engine/EditorBlueprintResources/ActorMacros.Switch Has Authority`
    (:`Authority`
      (`KismetSystemLibrary.Delay` 3.0)
      (if (`self.IsActive?`)
        (`self.BeginSpawns`)))))

(event `BeginSpawns`
  (`KismetSystemLibrary.K2_SetTimer` null "SpawnEnemies" 0.5 true))

(event `SpawnEnemies`
  (if (`self.IsActive?`)
    (`/Engine/EditorBlueprintResources/ActorMacros.Switch Has Authority`
      (:`Authority`
        (bind _returnvalue (`AIBlueprintHelperLibrary.SpawnAIFromClass` "/Game/TSS_Game/Blueprints/Bonus/BP_Enemy_Background.BP_Enemy_Background_C" null (`KismetMathLibrary.RandomPointInBoundingBox` (`SceneComponent.K2_GetComponentLocation` (`self.DefaultSceneRoot`)) (`BoxComponent.BoxExtent` (`self.Box`))) (struct) false null))
        (bind _asbp_enemy_background (cast `/Game/TSS_Game/Blueprints/Bonus/BP_Enemy_Background` _returnvalue))
        (set `/Game/TSS_Game/Blueprints/Bonus/BP_Enemy_Background.Goal Actor` (`self.Goal Actor`) _asbp_enemy_background)))))

(fn `UserConstructionScript`)