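; BP_RaisingLava is a mission hazard actor: lava that rises on demand, damaging players and killing enemies.
; StartLavaRaising plays a Timeline that moves the actor up by RaisingSpeed per update with sweep, until StopLavaRaising.
; DamageBox overlaps track locally controlled characters for looping one-second multicast damage, paused by function name when none remain.
; Overlapping enemies die immediately through a server-only call.
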(event `self.ReceiveBeginPlay`)

(event `StartLavaRaising`
  (params (RaisingSpeed :type "Float (double-precision)"))
  (set `self.RaisingSpeed` RaisingSpeed)
  (`Timeline|Timeline` :!label _label
    (:`Update`
      (`self.K2_AddActorWorldOffset` (`KismetMathLibrary.MakeVector` 0.0 0.0 (`self.RaisingSpeed`)) true))))

(event `DamageActorsInArea`
  (for _array_element (`self.ActorsRecievingDamage`)
    (message `/Game/TSS_Game/Blueprints/System/BPI_Damagable.DamageIntercation` _array_element 75.0 self true "NewEnumerator4")))

(event `StopLavaRaising`
  (goto _label :!via `Stop`))

(event `self.DamageBox.OnComponentBeginOverlap`
  (params (OverlappedComponent :type "PrimitiveComponent Object Reference") (OtherActor :type "Actor Object Reference") (OtherComp :type "PrimitiveComponent Object Reference") (OtherBodyIndex :type Integer) (bFromSweep :type Boolean) (SweepResult :type "HitResult Structure (by ref)"))
  (bind _asbp_character_base (cast `/Game/TSS_Game/Blueprints/System/BP_CharacterBase` OtherActor)
    (:`then`
      (if (`Pawn.IsLocallyControlled` _asbp_character_base)
        (`KismetArrayLibrary.Array_AddUnique` (`self.ActorsRecievingDamage`) OtherActor)
        (`KismetSystemLibrary.K2_SetTimerDelegate` (delegate `DamageActorsInArea`) 1.0 true)))
    (:`CastFailed`
      (bind _asbp_enemy_base (cast `/Game/TSS_Game/Blueprints/Bonus/AI/BP_Enemy_BASE` OtherActor))
      (if (`KismetSystemLibrary.IsServer`)
        (`/Game/TSS_Game/Blueprints/Bonus/AI/BP_Enemy_BASE.SV_EnemyDead` _asbp_enemy_base null "NewEnumerator0")))))

(event `self.DamageBox.OnComponentEndOverlap`
  (params (OverlappedComponent :type "PrimitiveComponent Object Reference") (OtherActor :type "Actor Object Reference") (OtherComp :type "PrimitiveComponent Object Reference") (OtherBodyIndex :type Integer))
  (bind _asbp_character_base (cast `/Game/TSS_Game/Blueprints/System/BP_CharacterBase` OtherActor))
  (`KismetArrayLibrary.Array_RemoveItem` (`self.ActorsRecievingDamage`) _asbp_character_base)
  (if (`KismetArrayLibrary.Array_IsEmpty` (`self.ActorsRecievingDamage`))
    (`KismetSystemLibrary.K2_PauseTimer` null "DamageActorsInArea")))

(fn `UserConstructionScript`)