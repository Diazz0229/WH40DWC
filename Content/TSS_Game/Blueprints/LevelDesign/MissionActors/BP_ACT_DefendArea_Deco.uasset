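; Decor actor for a defend-area mission that moves its MovingPart vertically when activated.
; CustomFloatData acts as a percentage of the travel span, computed as the summed absolute start and target heights, to set the next Z relative to StartLocationZ.
; A Timeline serves as an update ticker, stepping Z by an OpenSpeed-scaled amount per update, independent of delta time, then stopping and snapping at the goal.
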(event `self.MC_Activate`
  (`self.MC_MoveDeco` (`self.Open Speed`)))

(event `MC_MoveDeco`
  (params (OpenSpeed :type "Float (double-precision)"))
  (bind (_relativelocation_x _relativelocation_y _relativelocation_z) (`KismetMathLibrary.BreakVector` (`SceneComponent.RelativeLocation` (`self.MovingPart`))))
  (bind _returnvalue (* (/ (+ (`KismetMathLibrary.Abs` (`self.Start Location Z`)) (`KismetMathLibrary.Abs` (`self.TargetPosZ`))) 500.0) (`self.Open Speed`)))
  (set `self.NextStepPosZ` (+ (`self.Start Location Z`) (* (`self.CustomFloatData`) (/ (+ (`KismetMathLibrary.Abs` (`self.Start Location Z`)) (`KismetMathLibrary.Abs` (`self.TargetPosZ`))) 100.0))))
  (if (not (== (`self.CurPosZ`) (`self.NextStepPosZ`)))
    (`Timeline|Timeline` :!label _label
      (:`Update`
        (if (< (`self.CurPosZ`) (`self.NextStepPosZ`))
          (`self.Set Decor Z Position` (+ _relativelocation_z _returnvalue))
          (if (>= (`self.CurPosZ`) (`self.NextStepPosZ`))
            (`self.StopMoving` :!label _label_2)
            (`self.Set Decor Z Position` (`self.NextStepPosZ`)))
          (else
            (`self.Set Decor Z Position` (- _relativelocation_z _returnvalue))
            (if (<= (`self.CurPosZ`) (`self.NextStepPosZ`))
              (goto _label_2))))))))

(event `StopMoving`
  (goto _label :!via `Stop`))

(event `self.ReceiveBeginPlay`
  (bind _movingpart (`self.MovingPart`))
  (bind (_relativelocation_x _relativelocation_y) (`KismetMathLibrary.BreakVector` (`SceneComponent.RelativeLocation` _movingpart)))
  (`parent.ReceiveBeginPlay`)
  (bind _output_get (set `self.CurPosZ` (`self.Start Location Z`)))
  (`SceneComponent.K2_SetRelativeLocation` _movingpart (`KismetMathLibrary.MakeVector` _relativelocation_x _relativelocation_y _output_get) false false))

(fn `Set Decor Z Position`
  (params (CurPosZ :type "Float (double-precision)"))
  (returns (NewPos :type "Float (double-precision)"))
  (bind _movingpart (`self.MovingPart`))
  (bind (_relativelocation_x _relativelocation_y) (`KismetMathLibrary.BreakVector` (`SceneComponent.RelativeLocation` _movingpart)))
  (bind _output_get (set `self.CurPosZ` CurPosZ))
  (`SceneComponent.K2_SetRelativeLocation` _movingpart (`KismetMathLibrary.MakeVector` _relativelocation_x _relativelocation_y _output_get) false false)
  (return _output_get))

(fn `UserConstructionScript`
  (`parent.UserConstructionScript`))