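; Mission actor for a defend-area objective that fills a percentage while living characters stand inside its box.
; Once activated, a looping timer drops dead characters from the overlap list and adds progress per defender plus a bonus, optionally draining when empty.
; Progress updates a widget indicator and is passed to chained activatables.
; At full, the server notifies the parent mission controller and the area deactivates.
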(event `self.ReceiveBeginPlay`
  (bind _asw_defence_indicator (cast `/Game/TSS_Game/UI/DefenceIndicator/W_DefenceIndicator` (`WidgetComponent.GetWidget` (`self.PercentWidget`))))
  (set `self.Defence Indicator` _asw_defence_indicator))

(event `ActivateDefence`
  (`SceneComponent.SetVisibility` (`self.VisualDefendArea`) true true)
  (`SceneComponent.SetVisibility` (`self.PercentWidget`) true false)
  (`KismetSystemLibrary.K2_SetTimerDelegate` (delegate `CheckPlayers`) (`self.CheckPlayersTimer`) true))

(event `DeactivateDefence`
  (`SceneComponent.SetVisibility` (`self.VisualDefendArea`) false true)
  (`SceneComponent.SetVisibility` (`self.PercentWidget`) false false)
  (`KismetSystemLibrary.K2_PauseTimer` null "CheckPlayers"))

(event `CheckPlayers`
  (bind _output_get (set `self.DefendingPlayers` (`PrimitiveComponent.GetOverlappingActors` (`self.Box`) "/Game/TSS_Game/Blueprints/System/BP_CharacterBase.BP_CharacterBase_C")))
  (if (`KismetArrayLibrary.Array_IsNotEmpty` _output_get)
    (for _array_element (`self.DefendingPlayers`)
      (bind _asbp_character_base (cast `/Game/TSS_Game/Blueprints/System/BP_CharacterBase` _array_element))
      (if (`/Game/TSS_Game/Blueprints/System/BP_CharacterBase.IsDead` _asbp_character_base)
        (`KismetArrayLibrary.Array_RemoveItem` (`self.DefendingPlayers`) _array_element)))
    (if (`KismetArrayLibrary.Array_IsNotEmpty` (`self.DefendingPlayers`))
      (`self.AddPercentToDefence` (`self.BonusPercentPerTick`))
      (else
        (if (`self.ShouldDrainOutWhenEmpty?`) :!label _label
          (`self.AddPercentToDefence` (`self.DrainPercentWhenEmpty`)))))
    (else
      (goto _label))))

(event `AddPercentToDefence`
  (params (`Additional points` :type "Float (double-precision)"))
  (bind _output_get (set `self.DefenceCurPercent` (`KismetMathLibrary.FClamp` (+ (`self.DefenceCurPercent`) (* (`self.PercentGainedPerTick`) (`KismetArrayLibrary.Array_Length` (`self.DefendingPlayers`))) `Additional points`) 0.0 100.0)))
  (`/Game/TSS_Game/UI/DefenceIndicator/W_DefenceIndicator.UpdateValues` (`self.Defence Indicator`) _output_get)
  (for _array_element (`self.ChainActivatables`)
    ;[1 1 1] Send all attached objects percents
    (set `/Game/TSS_Game/Blueprints/LevelDesign/BP_Activatable_Base.CustomFloatData` (`self.DefenceCurPercent`) _array_element)
    (`self.MC_Activate` _array_element))
  (if (>= _output_get 100.0)
    (if (`KismetSystemLibrary.IsServer`)
      (`/Game/TSS_Game/Blueprints/LevelDesign/MissionActors/BP_Act_DefendController.DefenceComplete` (`self.ParentMissionController`)))
    (`self.DeactivateDefence`)))

(fn `UserConstructionScript`
  (`parent.UserConstructionScript`))