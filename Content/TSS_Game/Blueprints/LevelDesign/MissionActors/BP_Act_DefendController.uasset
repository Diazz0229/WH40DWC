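; BP_Act_DefendController is a mission actor that runs a room's defend-points objective.
; MC_InitDefendPoints activates each chained BP_Act_DefendArea and registers itself as its controller.
; DefenceComplete counts finished points; at the required total the server changes the room's win condition, disables enemy spawners and has player controller 0 send a character message to eliminate remaining threats.
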(event `self.ReceiveBeginPlay`)

(event `MC_InitDefendPoints`
  (for _array_element (`self.ChainActivatables`)
    (bind _asbp_act_defend_area (cast `/Game/TSS_Game/Blueprints/LevelDesign/MissionActors/BP_Act_DefendArea` _array_element))
    (`/Game/TSS_Game/Blueprints/LevelDesign/MissionActors/BP_Act_DefendArea.ActivateDefence` _asbp_act_defend_area)
    (set `/Game/TSS_Game/Blueprints/LevelDesign/MissionActors/BP_Act_DefendArea.ParentMissionController` self _asbp_act_defend_area)))

(event `DefenceComplete`
  (bind _parentroom (`self.ParentRoom`))
  (bind (_roomcharinfo_charname _roomcharinfo_charportrait) (break `/Game/TSS_Game/UI/IngameWindows/ST_CharacterDialogInfo` (`/Game/TSS_Game/Blueprints/LevelDesign/ModularRooms/BP_ProcRoom_Base.RoomCharInfo` _parentroom)))
  (`/Engine/EditorBlueprintResources/StandardMacros.IncrementInt` (`self.CompletedDefencePoints`)
    (:`  `
      (if (>= (`self.CompletedDefencePoints`) (`self.RequiredDefencePoints`))
        (if (`KismetSystemLibrary.IsServer`)
          (set `/Game/TSS_Game/Blueprints/LevelDesign/ModularRooms/BP_ProcRoom_Base.WinCondition` "NewEnumerator0" _parentroom)
          (`/Game/TSS_Game/Blueprints/LevelDesign/ModularRooms/BP_ProcRoom_Base.DisableRoomEnemySpawners` _parentroom)
          (bind _asbp_player_controller (cast `/Game/TSS_Game/Blueprints/System/BP_PlayerController` (`GameplayStatics.GetPlayerController` 0)))
          (`/Game/TSS_Game/Blueprints/System/BP_PlayerController.SendCharacterMessage` _asbp_player_controller _roomcharinfo_charportrait _roomcharinfo_charname "Success. Now eliminate the remaining threats in the sector."))))))

(fn `UserConstructionScript`
  (`parent.UserConstructionScript`))