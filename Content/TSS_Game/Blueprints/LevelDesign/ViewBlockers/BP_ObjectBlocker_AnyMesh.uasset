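; View-blocker actor that turns up to six assigned static mesh actors transparent while the locally controlled character overlaps it.
; BeginPlay caches each target's materials, overlap start swaps every slot to M_Transparent, and overlap end or ResetMaterials restores them.
; Any overlapping BP_CharacterBase gets this actor added to its HiddenPropsActors, with no removal here.
; Targets are checked as a nested chain, so an empty slot skips all later ones.
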(event `self.ReceiveBeginPlay`
  (bind _target_4 (`self.Target_4`))
  (bind _target_1 (`self.Target_1`))
  (bind _target_3 (`self.Target_3`))
  (bind _target_2 (`self.Target_2`))
  (bind _target_5 (`self.Target_5`))
  (bind _target_6 (`self.Target_6`))
  (`/Engine/EditorBlueprintResources/StandardMacros.IsValid` _target_1
    (:`Is Valid`
      (for _array_element (`MeshComponent.GetMaterials` (`StaticMeshActor.StaticMeshComponent` _target_1))
        (`KismetArrayLibrary.Array_Add` (`self.Original_Material_1`) _array_element))
      (`/Engine/EditorBlueprintResources/StandardMacros.IsValid` _target_2
        (:`Is Valid`
          (for _array_element_2 (`MeshComponent.GetMaterials` (`StaticMeshActor.StaticMeshComponent` _target_2))
            (`KismetArrayLibrary.Array_Add` (`self.Original_Material_2`) _array_element_2))
          (`/Engine/EditorBlueprintResources/StandardMacros.IsValid` _target_3
            (:`Is Valid`
              (for _array_element_3 (`MeshComponent.GetMaterials` (`StaticMeshActor.StaticMeshComponent` _target_3))
                (`KismetArrayLibrary.Array_Add` (`self.Original_Material_3`) _array_element_3))
              (`/Engine/EditorBlueprintResources/StandardMacros.IsValid` _target_4
                (:`Is Valid`
                  (for _array_element_4 (`MeshComponent.GetMaterials` (`StaticMeshActor.StaticMeshComponent` _target_4))
                    (`KismetArrayLibrary.Array_Add` (`self.Original_Material_4`) _array_element_4))
                  (`/Engine/EditorBlueprintResources/StandardMacros.IsValid` _target_5
                    (:`Is Valid`
                      (for _array_element_5 (`MeshComponent.GetMaterials` (`StaticMeshActor.StaticMeshComponent` _target_5))
                        (`KismetArrayLibrary.Array_Add` (`self.Original_Material_5`) _array_element_5))
                      (`/Engine/EditorBlueprintResources/StandardMacros.IsValid` _target_6
                        (:`Is Valid`
                          (for _array_element_6 (`MeshComponent.GetMaterials` (`StaticMeshActor.StaticMeshComponent` _target_6))
                            (`KismetArrayLibrary.Array_Add` (`self.Original_Material_6`) _array_element_6)))))))))))))))

(event `self.ReceiveActorBeginOverlap`
  (params (OtherActor :type "Actor Object Reference"))
  (bind _target_1 (`self.Target_1`))
  (bind _target_2 (`self.Target_2`))
  (bind _target_3 (`self.Target_3`))
  (bind _target_4 (`self.Target_4`))
  (bind _target_5 (`self.Target_5`))
  (bind _target_6 (`self.Target_6`))
  (bind _staticmeshcomponent (`StaticMeshActor.StaticMeshComponent` _target_6))
  (bind _staticmeshcomponent_2 (`StaticMeshActor.StaticMeshComponent` _target_1))
  (bind _staticmeshcomponent_3 (`StaticMeshActor.StaticMeshComponent` _target_2))
  (bind _staticmeshcomponent_4 (`StaticMeshActor.StaticMeshComponent` _target_3))
  (bind _staticmeshcomponent_5 (`StaticMeshActor.StaticMeshComponent` _target_4))
  (bind _staticmeshcomponent_6 (`StaticMeshActor.StaticMeshComponent` _target_5))
  (bind _asbp_character_base (cast `/Game/TSS_Game/Blueprints/System/BP_CharacterBase` OtherActor))
  (`KismetArrayLibrary.Array_AddUnique` (`/Game/TSS_Game/Blueprints/System/BP_CharacterBase.HiddenPropsActors` _asbp_character_base) self)
  (if (`Pawn.IsLocallyControlled` _asbp_character_base)
    (`/Engine/EditorBlueprintResources/StandardMacros.IsValid` _target_1
      (:`Is Valid`
        (for (_ _array_index) (`MeshComponent.GetMaterials` _staticmeshcomponent_2)
          (`PrimitiveComponent.SetMaterial` _staticmeshcomponent_2 _array_index "/Game/TSS_Game/Materials/M_Transparent.M_Transparent"))
        (`/Engine/EditorBlueprintResources/StandardMacros.IsValid` _target_2
          (:`Is Valid`
            (for (_ _array_index_2) (`MeshComponent.GetMaterials` _staticmeshcomponent_3)
              (`PrimitiveComponent.SetMaterial` _staticmeshcomponent_3 _array_index_2 "/Game/TSS_Game/Materials/M_Transparent.M_Transparent"))
            (`/Engine/EditorBlueprintResources/StandardMacros.IsValid` _target_3
              (:`Is Valid`
                (for (_ _array_index_3) (`MeshComponent.GetMaterials` _staticmeshcomponent_4)
                  (`PrimitiveComponent.SetMaterial` _staticmeshcomponent_4 _array_index_3 "/Game/TSS_Game/Materials/M_Transparent.M_Transparent"))
                (`/Engine/EditorBlueprintResources/StandardMacros.IsValid` _target_4
                  (:`Is Valid`
                    (for (_ _array_index_4) (`MeshComponent.GetMaterials` _staticmeshcomponent_5)
                      (`PrimitiveComponent.SetMaterial` _staticmeshcomponent_5 _array_index_4 "/Game/TSS_Game/Materials/M_Transparent.M_Transparent"))
                    (`/Engine/EditorBlueprintResources/StandardMacros.IsValid` _target_5
                      (:`Is Valid`
                        (for (_ _array_index_5) (`MeshComponent.GetMaterials` _staticmeshcomponent_6)
                          (`PrimitiveComponent.SetMaterial` _staticmeshcomponent_6 _array_index_5 "/Game/TSS_Game/Materials/M_Transparent.M_Transparent"))
                        (`/Engine/EditorBlueprintResources/StandardMacros.IsValid` _target_6
                          (:`Is Valid`
                            (for (_ _array_index_6) (`MeshComponent.GetMaterials` _staticmeshcomponent)
                              (`PrimitiveComponent.SetMaterial` _staticmeshcomponent _array_index_6 "/Game/TSS_Game/Materials/M_Transparent.M_Transparent"))))))))))))))))

(event `ResetMaterials`
  (bind _target_1 (`self.Target_1`))
  (bind _target_2 (`self.Target_2`))
  (bind _target_3 (`self.Target_3`))
  (bind _target_4 (`self.Target_4`))
  (bind _target_5 (`self.Target_5`))
  (bind _target_6 (`self.Target_6`))
  (`/Engine/EditorBlueprintResources/StandardMacros.IsValid` _target_1 :!label _label
    (:`Is Valid`
      (for (_array_element _array_index) (`self.Original_Material_1`)
        (`PrimitiveComponent.SetMaterial` (`StaticMeshActor.StaticMeshComponent` _target_1) _array_index _array_element))
      (`/Engine/EditorBlueprintResources/StandardMacros.IsValid` _target_2
        (:`Is Valid`
          (for (_array_element_2 _array_index_2) (`self.Original_Material_2`)
            (`PrimitiveComponent.SetMaterial` (`StaticMeshActor.StaticMeshComponent` _target_2) _array_index_2 _array_element_2))
          (`/Engine/EditorBlueprintResources/StandardMacros.IsValid` _target_3
            (:`Is Valid`
              (for (_array_element_3 _array_index_3) (`self.Original_Material_3`)
                (`PrimitiveComponent.SetMaterial` (`StaticMeshActor.StaticMeshComponent` _target_3) _array_index_3 _array_element_3))
              (`/Engine/EditorBlueprintResources/StandardMacros.IsValid` _target_4
                (:`Is Valid`
                  (for (_array_element_4 _array_index_4) (`self.Original_Material_4`)
                    (`PrimitiveComponent.SetMaterial` (`StaticMeshActor.StaticMeshComponent` _target_4) _array_index_4 _array_element_4))
                  (`/Engine/EditorBlueprintResources/StandardMacros.IsValid` _target_5
                    (:`Is Valid`
                      (for (_array_element_5 _array_index_5) (`self.Original_Material_5`)
                        (`PrimitiveComponent.SetMaterial` (`StaticMeshActor.StaticMeshComponent` _target_5) _array_index_5 _array_element_5))
                      (`/Engine/EditorBlueprintResources/StandardMacros.IsValid` _target_6
                        (:`Is Valid`
                          (for (_array_element_6 _array_index_6) (`self.Original_Material_6`)
                            (`PrimitiveComponent.SetMaterial` (`StaticMeshActor.StaticMeshComponent` _target_6) _array_index_6 _array_element_6)))))))))))))))

(event `self.ReceiveActorEndOverlap`
  (params (OtherActor :type "Actor Object Reference"))
  (bind _asbp_character_base (cast `/Game/TSS_Game/Blueprints/System/BP_CharacterBase` OtherActor))
  (if (`Pawn.IsLocallyControlled` _asbp_character_base)
    (goto _label)))

(fn `UserConstructionScript`)