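; View blocker trigger that makes up to three linked static mesh actors transparent while the local player's character overlaps it.
; BeginPlay caches each target's materials, and overlap hard-swaps every slot to a shared transparent material instance.
; When the local character exits, originals return only if no BP_CharacterBase still overlaps.
; Target checks are nested, so each later target works only when the earlier ones are set.
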(event `self.ReceiveBeginPlay`
  (bind _target_1 (`self.Target_1`))
  (bind _target_2 (`self.Target_2`))
  (bind _target_3 (`self.Target_3`))
  (`/Engine/EditorBlueprintResources/StandardMacros.IsValid` _target_1
    (:`Is Valid`
      (for _array_element (`MeshComponent.GetMaterials` (`StaticMeshActor.StaticMeshComponent` _target_1))
        (`KismetArrayLibrary.Array_Add` (`self.Original_Material_1`) _array_element))
      (`/Engine/EditorBlueprintResources/StandardMacros.IsValid` _target_2
        (:`Is Valid`
          (for _array_element_2 (`MeshComponent.GetMaterials` (`StaticMeshActor.StaticMeshComponent` _target_2))
            (`KismetArrayLibrary.Array_Add` (`self.Original_Material_2`) _array_element_2))
          (`/Engine/EditorBlueprintResources/StandardMacros.IsValid` _target_3
            (:`Is Valid`
              (for _array_element_3 (`MeshComponent.GetMaterials` (`StaticMeshActor.StaticMeshComponent` _target_3))
                (`KismetArrayLibrary.Array_Add` (`self.Original_Material_3`) _array_element_3)))))))))

(event `self.ReceiveActorBeginOverlap`
  (params (OtherActor :type "Actor Object Reference"))
  (bind _target_1 (`self.Target_1`))
  (bind _target_2 (`self.Target_2`))
  (bind _target_3 (`self.Target_3`))
  (bind _staticmeshcomponent (`StaticMeshActor.StaticMeshComponent` _target_3))
  (bind _staticmeshcomponent_2 (`StaticMeshActor.StaticMeshComponent` _target_1))
  (bind _staticmeshcomponent_3 (`StaticMeshActor.StaticMeshComponent` _target_2))
  (bind _ascharacter (cast `Character` OtherActor))
  (if (`Pawn.IsLocallyControlled` _ascharacter)
    (`/Engine/EditorBlueprintResources/StandardMacros.IsValid` _target_1
      (:`Is Valid`
        (for (_ _array_index) (`MeshComponent.GetMaterials` _staticmeshcomponent_2)
          (`PrimitiveComponent.SetMaterial` _staticmeshcomponent_2 _array_index "/Game/TSS_Game/Materials/M_Transparent_Inst_v2.M_Transparent_Inst_v2"))
        (`/Engine/EditorBlueprintResources/StandardMacros.IsValid` _target_2
          (:`Is Valid`
            (for (_ _array_index_2) (`MeshComponent.GetMaterials` _staticmeshcomponent_3)
              (`PrimitiveComponent.SetMaterial` _staticmeshcomponent_3 _array_index_2 "/Game/TSS_Game/Materials/M_Transparent_Inst_v2.M_Transparent_Inst_v2"))
            (`/Engine/EditorBlueprintResources/StandardMacros.IsValid` _target_3
              (:`Is Valid`
                (for (_ _array_index_3) (`MeshComponent.GetMaterials` _staticmeshcomponent)
                  (`PrimitiveComponent.SetMaterial` _staticmeshcomponent _array_index_3 "/Game/TSS_Game/Materials/M_Transparent_Inst_v2.M_Transparent_Inst_v2"))))))))))

(event `self.ReceiveActorEndOverlap`
  (params (OtherActor :type "Actor Object Reference"))
  (bind _target_1 (`self.Target_1`))
  (bind _target_2 (`self.Target_2`))
  (bind _target_3 (`self.Target_3`))
  (bind _ascharacter (cast `Character` OtherActor))
  (if (`Pawn.IsLocallyControlled` _ascharacter)
    (if (not (> (`KismetArrayLibrary.Array_Length` (`self.GetOverlappingActors` "/Game/TSS_Game/Blueprints/System/BP_CharacterBase.BP_CharacterBase_C")) 0))
      (`/Engine/EditorBlueprintResources/StandardMacros.IsValid` _target_1
        (:`Is Valid`
          (for (_array_element _array_index) (`self.Original_Material_1`)
            (`PrimitiveComponent.SetMaterial` (`StaticMeshActor.StaticMeshComponent` _target_1) _array_index _array_element))
          (`/Engine/EditorBlueprintResources/StandardMacros.IsValid` _target_2
            (:`Is Valid`
              (for (_array_element_2 _array_index_2) (`self.Original_Material_2`)
                (`PrimitiveComponent.SetMaterial` (`StaticMeshActor.StaticMeshComponent` _target_2) _array_index_2 _array_element_2))
              (`/Engine/EditorBlueprintResources/StandardMacros.IsValid` _target_3
                (:`Is Valid`
                  (for (_array_element_3 _array_index_3) (`self.Original_Material_3`)
                    (`PrimitiveComponent.SetMaterial` (`StaticMeshActor.StaticMeshComponent` _target_3) _array_index_3 _array_element_3)))))))))))

(fn `UserConstructionScript`)