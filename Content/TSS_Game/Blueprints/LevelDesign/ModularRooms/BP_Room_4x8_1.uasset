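; A modular 4x8 room Blueprint that defines one randomizable piece of a procedurally linked level.
; Its construction script passes the room's contents to InitRoomActors, then calls the parent script.
; Wall actors, decals and floor decor are paired with shared replacement chances and default variant pools.
; It also registers actors hidable for the next room, a single blast-door exit with its arrow, an ammo crate, skulls and enemy pre-spawners.
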(fn `UserConstructionScript`
  (bind _defaultdecorations (`self.DefaultDecorations`))
  (bind _defaultwallspawners (`self.DefaultWallSpawners`))
  (bind _defaultdecals (`self.DefaultDecals`))
  (bind _actorschancetoreplace (`self.ActorsChanceToReplace`))
  (bind _decalchancetoreplace (`self.DecalChanceToReplace`))
  (bind _mesheschancetoreplace (`self.MeshesChanceToReplace`))
  (`self.InitRoomActors` :`IsServer?` true :`ActorReplacableVariants` (`|MakeArray` (make `/Game/TSS_Game/Blueprints/LevelDesign/ModularRooms/ST_RoomCompVariants` (`self.StaticMeshActor_210027`) _actorschancetoreplace _defaultwallspawners) (make `/Game/TSS_Game/Blueprints/LevelDesign/ModularRooms/ST_RoomCompVariants` (`self.StaticMeshActor_210030`) _actorschancetoreplace _defaultwallspawners) (make `/Game/TSS_Game/Blueprints/LevelDesign/ModularRooms/ST_RoomCompVariants` (`self.StaticMeshActor_210028`) _actorschancetoreplace _defaultwallspawners) (make `/Game/TSS_Game/Blueprints/LevelDesign/ModularRooms/ST_RoomCompVariants` (`self.StaticMeshActor_210029`) _actorschancetoreplace _defaultwallspawners) (make `/Game/TSS_Game/Blueprints/LevelDesign/ModularRooms/ST_RoomCompVariants` (`self.StaticMeshActor_181693`) _actorschancetoreplace _defaultwallspawners)) :`MeshReplacableVariants` (`|MakeArray` (make `/Game/TSS_Game/Blueprints/LevelDesign/ModularRooms/ST_RoomMeshVariants` (`self.Decal_2`) _decalchancetoreplace _defaultdecals) (make `/Game/TSS_Game/Blueprints/LevelDesign/ModularRooms/ST_RoomMeshVariants` (`self.Decal_3`) _decalchancetoreplace _defaultdecals) (make `/Game/TSS_Game/Blueprints/LevelDesign/ModularRooms/ST_RoomMeshVariants` (`self.Decal_4`) _decalchancetoreplace _defaultdecals) (make `/Game/TSS_Game/Blueprints/LevelDesign/ModularRooms/ST_RoomMeshVariants` (`self.Decal_5`) _decalchancetoreplace _defaultdecals) (make `/Game/TSS_Game/Blueprints/LevelDesign/ModularRooms/ST_RoomMeshVariants` (`self.Decal_1`) _decalchancetoreplace _defaultdecals) (make `/Game/TSS_Game/Blueprints/LevelDesign/ModularRooms/ST_RoomMeshVariants` (`self.Decal_6`) _decalchancetoreplace _defaultdecals) (make `/Game/TSS_Game/Blueprints/LevelDesign/ModularRooms/ST_RoomMeshVariants` (`self.DecorFloor2`) _mesheschancetoreplace _defaultdecorations) (make `/Game/TSS_Game/Blueprints/LevelDesign/ModularRooms/ST_RoomMeshVariants` (`self.DecorFloor3`) _mesheschancetoreplace _defaultdecorations) (make `/Game/TSS_Game/Blueprints/LevelDesign/ModularRooms/ST_RoomMeshVariants` (`self.DecorFloor4`) _mesheschancetoreplace _defaultdecorations) (make `/Game/TSS_Game/Blueprints/LevelDesign/ModularRooms/ST_RoomMeshVariants` (`self.DecorFloor1`) _mesheschancetoreplace _defaultdecorations) (make `/Game/TSS_Game/Blueprints/LevelDesign/ModularRooms/ST_RoomMeshVariants` (`self.DecorFloor5`) _mesheschancetoreplace _defaultdecorations)) :`ActorsHidable_NextRoom` (`|MakeArray` (`self.StaticMeshActor_181898`) (`self.StaticMeshActor_181896`) (`self.StaticMeshActor_181897`) (`self.StaticMeshActor_210033`) (`self.StaticMeshActor_210032`)) :`PossibleWays` (`|MakeArray` (make `/Game/TSS_Game/Blueprints/LevelDesign/ModularRooms/ST_ProcDoors_Pure` (`self.BP_ACT_BlastDoor_SingleLarge_C_219`) (`self.NextRoomArrow`))) :`AmmoCrates` (`|MakeArray` (`self.Ammo1`)) :`Skulls` (`|MakeArray` (`self.Skulls5`) (`self.Skulls4`) (`self.Skulls6`)) :`EnemiesPreSpawners` (`|MakeArray` (`self.EnemyPreSpawner_4`) (`self.EnemyPreSpawner_3`) (`self.EnemyPreSpawner_2`) (`self.EnemyPreSpawner_5`) (`self.EnemyPreSpawner_1`)))
  (`parent.UserConstructionScript`))