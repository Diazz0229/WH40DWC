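; BP_Room_Side_10x8_1 is a modular side room for procedural level building, with a single onward door, arrow and direction.
; Its construction script registers the room's components through InitRoomActors, then calls the parent construction script.
; It supplies chance-based variant pools for a wall actor, floor decorations and decals, plus hidable pieces, ammo crates, skulls, enemy spawners and pre-spawners.
; The event graph holds no active logic.
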(fn `UserConstructionScript`
  (bind _defaultdecorations (`self.DefaultDecorations`))
  (bind _defaultdecals (`self.DefaultDecals`))
  (bind _decalchancetoreplace (`self.DecalChanceToReplace`))
  (bind _mesheschancetoreplace (`self.MeshesChanceToReplace`))
  (`self.InitRoomActors` true (`|MakeArray` (make `/Game/TSS_Game/Blueprints/LevelDesign/ModularRooms/ST_RoomCompVariants` (`self.StaticMeshActor_524435`) (`self.ActorsChanceToReplace`) (`self.DefaultWallSpawners`))) (`|MakeArray` (make `/Game/TSS_Game/Blueprints/LevelDesign/ModularRooms/ST_RoomMeshVariants` (`self.DecorFloor2`) _mesheschancetoreplace _defaultdecorations) (make `/Game/TSS_Game/Blueprints/LevelDesign/ModularRooms/ST_RoomMeshVariants` (`self.DecorFloor3`) _mesheschancetoreplace _defaultdecorations) (make `/Game/TSS_Game/Blueprints/LevelDesign/ModularRooms/ST_RoomMeshVariants` (`self.DecorFloor1`) _mesheschancetoreplace _defaultdecorations) (make `/Game/TSS_Game/Blueprints/LevelDesign/ModularRooms/ST_RoomMeshVariants` (`self.DecorFloor4`) _mesheschancetoreplace _defaultdecorations) (make `/Game/TSS_Game/Blueprints/LevelDesign/ModularRooms/ST_RoomMeshVariants` (`self.DecorFloor5`) _mesheschancetoreplace _defaultdecorations) (make `/Game/TSS_Game/Blueprints/LevelDesign/ModularRooms/ST_RoomMeshVariants` (`self.Decal_2`) _decalchancetoreplace _defaultdecals) (make `/Game/TSS_Game/Blueprints/LevelDesign/ModularRooms/ST_RoomMeshVariants` (`self.Decal_1`) _decalchancetoreplace _defaultdecals) (make `/Game/TSS_Game/Blueprints/LevelDesign/ModularRooms/ST_RoomMeshVariants` (`self.Decal_4`) _decalchancetoreplace _defaultdecals) (make `/Game/TSS_Game/Blueprints/LevelDesign/ModularRooms/ST_RoomMeshVariants` (`self.Decal_5`) _decalchancetoreplace _defaultdecals) (make `/Game/TSS_Game/Blueprints/LevelDesign/ModularRooms/ST_RoomMeshVariants` (`self.Decal_3`) _decalchancetoreplace _defaultdecals) (make `/Game/TSS_Game/Blueprints/LevelDesign/ModularRooms/ST_RoomMeshVariants` (`self.Decal_6`) _decalchancetoreplace _defaultdecals) (make `/Game/TSS_Game/Blueprints/LevelDesign/ModularRooms/ST_RoomMeshVariants` (`self.DecorFloor6`) _mesheschancetoreplace _defaultdecorations) (make `/Game/TSS_Game/Blueprints/LevelDesign/ModularRooms/ST_RoomMeshVariants` (`self.DecorFloor7`) _mesheschancetoreplace _defaultdecorations)) (`|MakeArray` (`self.StaticMeshActor_524469`) (`self.StaticMeshActor_524504`) (`self.StaticMeshActor_524440`) (`self.StaticMeshActor_524470`) (`self.StaticMeshActor_524506`) (`self.StaticMeshActor_524463`) (`self.StaticMeshActor_524441`)) (`|MakeArray` (`self.StaticMeshActor_524439`) (`self.StaticMeshActor_524427`) (`self.StaticMeshActor_524425`) (`self.StaticMeshActor_524426`) (`self.StaticMeshActor_524465`)) (`|MakeArray` (make `/Game/TSS_Game/Blueprints/LevelDesign/ModularRooms/ST_ProcDoors_Pure` (`self.BP_ACT_BlastDoor_SingleLarge_C_3171`) (`self.NextRoomArrow`) "NewEnumerator1")) (`|MakeArray` (`self.Ammo3`) (`self.Ammo1`) (`self.Ammo2`)) (`|MakeArray` (`self.Skulls3`) (`self.Skulls2`) (`self.Skulls4`) (`self.Skulls1`)) (`|MakeArray` (`self.EnemySpawner_1`) (`self.EnemySpawner_2`) (`self.EnemySpawner_3`)) (`|MakeArray` (`self.EnemyPreSpawner_2`) (`self.EnemyPreSpawner_4`) (`self.EnemyPreSpawner_5`) (`self.EnemyPreSpawner_1`) (`self.EnemyPreSpawner_7`) (`self.EnemyPreSpawner_3`) (`self.EnemyPreSpawner_6`)))
  (`parent.UserConstructionScript`))