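; BP_Room_Start_4x4_1 is a modular start room Blueprint, apparently for procedural level layouts.
; Its construction script calls InitRoomActors, registering static meshes that can be hidden, one mesh hidable for the next room, and a single exit.
; That exit pairs a blast door with an arrow and a direction, then the parent construction script runs.
; The event graph has only disabled placeholder events.
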(fn `UserConstructionScript`
  ;[1 1 1] All replacable and dynamic actors in blueprint must be initialized here
  (`self.InitRoomActors` :`IsServer?` true :`ActorsHidable` (`|MakeArray` (`self.StaticMeshActor_5688`) (`self.StaticMeshActor_5690`) (`self.StaticMeshActor_5691`) (`self.StaticMeshActor_5687`)) :`ActorsHidable_NextRoom` (`|MakeArray` (`self.StaticMeshActor_5680`)) :`PossibleWays` (`|MakeArray` (make `/Game/TSS_Game/Blueprints/LevelDesign/ModularRooms/ST_ProcDoors_Pure` (`self.BP_ACT_BlastDoor_Single_C_9`) (`self.NextRoomArrow`))))
  (`parent.UserConstructionScript`))