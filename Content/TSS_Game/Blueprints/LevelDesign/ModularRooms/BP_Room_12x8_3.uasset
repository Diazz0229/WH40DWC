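; Modular 12x8 room variant (BP_Room_12x8_3) for procedural level layouts, configured entirely in its construction script.
; It passes its placed components to InitRoomActors: chance-based replacement sets for wall spawners, floor decorations and decals, plus hidable actor lists.
; The same call supplies one possible exit door with its next-room arrow, along with ammo crates, skulls and enemy pre-spawners, before running the parent construction script.
; The event graph holds no active logic.
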(fn `UserConstructionScript`
  (bind _defaultdecorations (`self.DefaultDecorations`))
  (bind _defaultwallspawners (`self.DefaultWallSpawners`))
  (bind _defaultdecals (`self.DefaultDecals`))
  (bind _actorschancetoreplace (`self.ActorsChanceToReplace`))
  (bind _decalchancetoreplace (`self.DecalChanceToReplace`))
  (bind _mesheschancetoreplace (`self.MeshesChanceToReplace`))
  (`self.InitRoomActors` :`IsServer?` true :`ActorReplacableVariants` (`|MakeArray` (make `/Game/TSS_Game/Blueprints/LevelDesign/ModularRooms/ST_RoomCompVariants` (`self.StaticMeshActor_328773`) _actorschancetoreplace _defaultwallspawners) (make `/Game/TSS_Game/Blueprints/LevelDesign/ModularRooms/ST_RoomCompVariants` (`self.StaticMeshActor_328764`) _actorschancetoreplace _defaultwallspawners) (make `/Game/TSS_Game/Blueprints/LevelDesign/ModularRooms/ST_RoomCompVariants` (`self.StaticMeshActor_328776`) _actorschancetoreplace _defaultwallspawners) (make `/Game/TSS_Game/Blueprints/LevelDesign/ModularRooms/ST_RoomCompVariants` (`self.StaticMeshActor_328761`) _actorschancetoreplace _defaultwallspawners) (make `/Game/TSS_Game/Blueprints/LevelDesign/ModularRooms/ST_RoomCompVariants` (`self.StaticMeshActor_328770`) _actorschancetoreplace _defaultwallspawners)) :`MeshReplacableVariants` (`|MakeArray` (make `/Game/TSS_Game/Blueprints/LevelDesign/ModularRooms/ST_RoomMeshVariants` (`self.DecorFloor2`) _mesheschancetoreplace _defaultdecorations) (make `/Game/TSS_Game/Blueprints/LevelDesign/ModularRooms/ST_RoomMeshVariants` (`self.DecorFloor3`) _mesheschancetoreplace _defaultdecorations) (make `/Game/TSS_Game/Blueprints/LevelDesign/ModularRooms/ST_RoomMeshVariants` (`self.DecorFloor1`) _mesheschancetoreplace _defaultdecorations) (make `/Game/TSS_Game/Blueprints/LevelDesign/ModularRooms/ST_RoomMeshVariants` (`self.DecorFloor4`) _mesheschancetoreplace _defaultdecorations) (make `/Game/TSS_Game/Blueprints/LevelDesign/ModularRooms/ST_RoomMeshVariants` (`self.DecorFloor5`) _mesheschancetoreplace _defaultdecorations) (make `/Game/TSS_Game/Blueprints/LevelDesign/ModularRooms/ST_RoomMeshVariants` (`self.Decal_2`) _decalchancetoreplace _defaultdecals) (make `/Game/TSS_Game/Blueprints/LevelDesign/ModularRooms/ST_RoomMeshVariants` (`self.Decal_1`) _decalchancetoreplace _defaultdecals) (make `/Game/TSS_Game/Blueprints/LevelDesign/ModularRooms/ST_RoomMeshVariants` (`self.Decal_4`) _decalchancetoreplace _defaultdecals) (make `/Game/TSS_Game/Blueprints/LevelDesign/ModularRooms/ST_RoomMeshVariants` (`self.Decal_5`) _decalchancetoreplace _defaultdecals) (make `/Game/TSS_Game/Blueprints/LevelDesign/ModularRooms/ST_RoomMeshVariants` (`self.Decal_3`) _decalchancetoreplace _defaultdecals) (make `/Game/TSS_Game/Blueprints/LevelDesign/ModularRooms/ST_RoomMeshVariants` (`self.Decal_6`) _decalchancetoreplace _defaultdecals)) :`ActorsHidable` (`|MakeArray` (`self.StaticMeshActor_328807`) (`self.StaticMeshActor_328809`) (`self.StaticMeshActor_328805`) (`self.StaticMeshActor_328819`) (`self.StaticMeshActor_328767`) (`self.StaticMeshActor_328893`) (`self.StaticMeshActor_328768`) (`self.StaticMeshActor_328769`) (`self.StaticMeshActor_328766`)) :`ActorsHidable_NextRoom` (`|MakeArray` (`self.StaticMeshActor_328855`) (`self.StaticMeshActor_328718`) (`self.StaticMeshActor_328717`) (`self.StaticMeshActor_328719`) (`self.StaticMeshActor_328778`) (`self.StaticMeshActor_328779`) (`self.StaticMeshActor_328854`)) :`PossibleWays` (`|MakeArray` (make `/Game/TSS_Game/Blueprints/LevelDesign/ModularRooms/ST_ProcDoors_Pure` (`self.BP_ACT_BlastDoor_SingleLarge_C_1970`) (`self.NextRoomArrow`))) :`AmmoCrates` (`|MakeArray` (`self.Ammo3`) (`self.Ammo1`) (`self.Ammo2`)) :`Skulls` (`|MakeArray` (`self.Skulls3`) (`self.Skulls2`) (`self.Skulls4`) (`self.Skulls1`)) :`EnemiesPreSpawners` (`|MakeArray` (`self.EnemyPreSpawner_2`) (`self.EnemyPreSpawner_4`) (`self.EnemyPreSpawner_5`) (`self.EnemyPreSpawner_1`) (`self.EnemyPreSpawner_7`) (`self.EnemyPreSpawner_6`) (`self.EnemyPreSpawner_3`)))
  (`parent.UserConstructionScript`))