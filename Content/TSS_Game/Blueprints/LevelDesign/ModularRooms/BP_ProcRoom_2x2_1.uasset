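; BP_ProcRoom_2x2_1 is a modular 2x2 procedural room variant built on a parent room Blueprint.
; Its construction script, on authority only, registers ammo crates, skulls and replaceable wall components, then calls the parent construction script.
; Two walls have a chance to become large tube spawner walls, while the mesh variants have zero replacement chance.
; A CalculateChance macro provides a random percentage roll with Success and Fail outputs.
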(event `self.ReceiveBeginPlay`
  (`parent.ReceiveBeginPlay`))

(fn `UserConstructionScript`
  (bind _array (`|MakeArray` "/Game/TSS_Game/Blueprints/LevelDesign/ModularRooms/BP_SpawnerWallTube_Large_01.BP_SpawnerWallTube_Large_01_C" :!type "Actor Class Reference"))
  (`/Engine/EditorBlueprintResources/ActorMacros.Switch Has Authority`
    (:`Authority`
      ;[1 1 1] All replacable and dynamic actors in blueprint must be initialized here
      (set `self.AmmoCrates` (`|MakeArray` (`self.Ammo1`) (`self.Ammo3`) (`self.Ammo2`) (`self.Ammo4`)))
      (set `self.Skulls` (`|MakeArray` (`self.Skulls1`) (`self.Skulls2`)))
      (set `self.ActorReplacableVariants` (`|MakeArray` (make `/Game/TSS_Game/Blueprints/LevelDesign/ModularRooms/ST_RoomCompVariants` (`self.Wall1`) 30.0 _array) (make `/Game/TSS_Game/Blueprints/LevelDesign/ModularRooms/ST_RoomCompVariants` (`self.Wall2`) 30.0 _array)))
      (set `self.MeshReplacableVariants` (`|MakeArray` (make `/Game/TSS_Game/Blueprints/LevelDesign/ModularRooms/ST_RoomMeshVariants` (`self.NewWall1`)) (make `/Game/TSS_Game/Blueprints/LevelDesign/ModularRooms/ST_RoomMeshVariants` (`self.NewWall2`))))
      (`parent.UserConstructionScript`))))