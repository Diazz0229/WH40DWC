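; A 4x4 modular level room with randomizable contents and a single blast-door exit to the next room.
; Its construction script registers the room's parts through InitRoomActors, then calls the parent construction script.
; Wall, floor and decoration slots get variant pools and replacement chances, alongside the exit, an actor hidable for the next room, ammo crates and enemy pre-spawners.
; The event graph holds no active logic.
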(fn `UserConstructionScript`
  (bind _defaultdecorations (`self.DefaultDecorations`))
  (bind _defaultwallspawners (`self.DefaultWallSpawners`))
  (bind _defaultfloortiles (`self.DefaultFloorTiles`))
  (bind _mesheschancetoreplace (`self.MeshesChanceToReplace`))
  (bind _mesheschancetoreplace_2 (`self.MeshesChanceToReplace`))
  (bind _actorschancetoreplace (`self.ActorsChanceToReplace`))
  ;[1 1 1] All replacable and dynamic actors in blueprint must be initialized here
  (`self.InitRoomActors` :`IsServer?` true :`ActorReplacableVariants` (`|MakeArray` (make `/Game/TSS_Game/Blueprints/LevelDesign/ModularRooms/ST_RoomCompVariants` (`self.StaticMeshActor_5676`) _actorschancetoreplace _defaultwallspawners) (make `/Game/TSS_Game/Blueprints/LevelDesign/ModularRooms/ST_RoomCompVariants` (`self.StaticMeshActor_5678`) _actorschancetoreplace _defaultwallspawners) (make `/Game/TSS_Game/Blueprints/LevelDesign/ModularRooms/ST_RoomCompVariants` (`self.StaticMeshActor_5660`) _mesheschancetoreplace_2 _defaultfloortiles) (make `/Game/TSS_Game/Blueprints/LevelDesign/ModularRooms/ST_RoomCompVariants` (`self.StaticMeshActor_5657`) _mesheschancetoreplace_2 _defaultfloortiles)) :`MeshReplacableVariants` (`|MakeArray` (make `/Game/TSS_Game/Blueprints/LevelDesign/ModularRooms/ST_RoomMeshVariants` (`self.DecorFloor2`) _mesheschancetoreplace _defaultdecorations) (make `/Game/TSS_Game/Blueprints/LevelDesign/ModularRooms/ST_RoomMeshVariants` (`self.DecorFloor3`) _mesheschancetoreplace _defaultdecorations) (make `/Game/TSS_Game/Blueprints/LevelDesign/ModularRooms/ST_RoomMeshVariants` (`self.DecorFloor1`) _mesheschancetoreplace _defaultdecorations) (make `/Game/TSS_Game/Blueprints/LevelDesign/ModularRooms/ST_RoomMeshVariants` (`self.DecorFloor5`) _mesheschancetoreplace _defaultdecorations) (make `/Game/TSS_Game/Blueprints/LevelDesign/ModularRooms/ST_RoomMeshVariants` (`self.DecorFloor4`) _mesheschancetoreplace _defaultdecorations)) :`ActorsHidable_NextRoom` (`|MakeArray` (`self.StaticMeshActor_5680`)) :`PossibleWays` (`|MakeArray` (make `/Game/TSS_Game/Blueprints/LevelDesign/ModularRooms/ST_ProcDoors_Pure` (`self.BP_ACT_BlastDoor_Single_C_9`) (`self.NextRoomArrow`))) :`AmmoCrates` (`|MakeArray` (`self.Ammo1`) (`self.Ammo2`)) :`EnemiesPreSpawners` (`|MakeArray` (`self.EnemyPreSpawner_1`) (`self.EnemyPreSpawner_2`)))
  (`parent.UserConstructionScript`))