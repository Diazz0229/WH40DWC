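; Side 5x5 modular room Blueprint with two possible ways onward, configured as a piece for procedural room layouts.
; The construction script fills arrays for ammo crates, skulls, replaceable mesh variants and walls with a chance to become tube spawner walls.
; It pairs two next-room arrows with the same blast door child actor, then calls the parent construction script.
; The event graph holds no active logic.
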(fn `UserConstructionScript`
  (bind _array (`|MakeArray` "/Game/TSS_Game/Blueprints/LevelDesign/ModularRooms/BP_SpawnerWallTube_Large_01.BP_SpawnerWallTube_Large_01_C" :!type "Actor Class Reference"))
  ;[1 1 1] All replacable and dynamic actors in blueprint must be initialized here
  (set `self.AmmoCrates` (`|MakeArray` null null null null :!type "StaticMeshComponent Object Reference"))
  (set `self.Skulls` (`|MakeArray` null null :!type "StaticMeshComponent Object Reference"))
  (set `self.ActorReplacableVariants` (`|MakeArray` (make `/Game/TSS_Game/Blueprints/LevelDesign/ModularRooms/ST_RoomCompVariants` null 30.0 _array) (make `/Game/TSS_Game/Blueprints/LevelDesign/ModularRooms/ST_RoomCompVariants` null 30.0 _array)))
  (set `self.MeshReplacableVariants` (`|MakeArray` (struct) (struct) :!type "/Game/TSS_Game/Blueprints/LevelDesign/ModularRooms/ST_RoomMeshVariants Structure"))
  (set `self.PossibleWays` (`|MakeArray` (make `/Game/TSS_Game/Blueprints/LevelDesign/ModularRooms/ST_ProcDoors` (cast `/Game/TSS_Game/Blueprints/LevelDesign/BP_Activatable_Base` (`ChildActorComponent.ChildActor` (`self.BP_ACT_BlastDoor_Single_C_3`)) :!pure true) (`self.NextRoom1`) null) (make `/Game/TSS_Game/Blueprints/LevelDesign/ModularRooms/ST_ProcDoors` (cast `/Game/TSS_Game/Blueprints/LevelDesign/BP_Activatable_Base` (`ChildActorComponent.ChildActor` (`self.BP_ACT_BlastDoor_Single_C_3`)) :!pure true) (`self.NextRoomArrow`) null)))
  (`parent.UserConstructionScript`))