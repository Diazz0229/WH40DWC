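; Modular mission room 04, a defend encounter with rising lava, enemy spawners and a boss.
; Construction script registers doors, props, random variants and spawners; BeginPlay links two defend areas to the defend controller.
; The trigger hides the previous room for local players; the server requests activation once overlapping characters match the living count.
; Activation starts lava, defend points and spawns; winning stops lava, flashes alert lights and checks the HeartofFire achievement.
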(event `self.ReceiveBeginPlay`
  (bind _room_defend_controller (`self.Room Defend Controller`))
  ;[1 1 1] Setup for room defend controller
  (bind _asbp_act_defend_controller (cast `/Game/TSS_Game/Blueprints/LevelDesign/MissionActors/BP_Act_DefendController` (`ChildActorComponent.ChildActor` (`self.BP_Act_DefendController_C_0`))))
  (set `self.Room Defend Controller` _asbp_act_defend_controller)
  (for _array_element (`|MakeArray` (`self.BP_Act_DefendArea_C_2`) (`self.BP_Act_DefendArea_C_1`))
    (bind _asbp_activatable_base (cast `/Game/TSS_Game/Blueprints/LevelDesign/BP_Activatable_Base` (`ChildActorComponent.ChildActor` _array_element)))
    (`KismetArrayLibrary.Array_AddUnique` (`/Game/TSS_Game/Blueprints/LevelDesign/BP_Activatable_Base.ChainActivatables` (`self.Room Defend Controller`)) _asbp_activatable_base))
  (set `/Game/TSS_Game/Blueprints/LevelDesign/MissionActors/BP_Act_DefendController.ParentRoom` self _room_defend_controller)
  (set `/Game/TSS_Game/Blueprints/LevelDesign/MissionActors/BP_Act_DefendController.RoomIndex` (`self.RoomIndex`) _room_defend_controller)
  (for _array_element_2 (`self.StaticMeshesHidable`)
    (`PrimitiveComponent.SetCustomPrimitiveDataFloat` _array_element_2 0 1.0))
  (`parent.ReceiveBeginPlay`))

(event `self.RoomSetVisibility`
  (params (`Hide?` :type Boolean))
  (`parent.RoomSetVisibility` `Hide?`))

(event `self.RoomIsActivated`
  (bind _asbp_raising_lava (cast `/Game/TSS_Game/Blueprints/LevelDesign/MissionActors/BP_RaisingLava` (`ChildActorComponent.ChildActor` (`self.BP_RaisingLava_C_1`))))
  (`/Game/TSS_Game/Blueprints/LevelDesign/MissionActors/BP_RaisingLava.StartLavaRaising` _asbp_raising_lava 0.2)
  (set `PrimitiveComponent.bGenerateOverlapEvents` false (`self.EnemiesActivator`))
  (`/Game/TSS_Game/Blueprints/LevelDesign/MissionActors/BP_Act_DefendController.MC_InitDefendPoints` (`self.Room Defend Controller`))
  (set `self.IsRoomActivated?` true)
  (`self.EnableRoomEnemySpawners`)
  (`self.SV_SpawnBoss`))

(event `self.EnemiesActivator.OnComponentBeginOverlap`
  (params (OverlappedComponent :type "PrimitiveComponent Object Reference") (OtherActor :type "Actor Object Reference") (OtherComp :type "PrimitiveComponent Object Reference") (OtherBodyIndex :type Integer) (bFromSweep :type Boolean) (SweepResult :type "HitResult Structure (by ref)"))
  (bind _as_bp_game_mode_base (`self.As BP Game Mode Base`))
  (bind _asbp_character_base (cast `/Game/TSS_Game/Blueprints/System/BP_CharacterBase` OtherActor))
  (if (`Pawn.IsLocallyControlled` _asbp_character_base)
    ;[1 1 1] Hide previous room and 2nd floor
    (`self.SendStartDialog`)
    (`/Game/TSS_Game/Blueprints/System/BP_CharacterBase.Speech_Say` _asbp_character_base "NewEnumerator5" false 30.0)
    (`self.RoomSetVisibility` (`|GetArrayItem` (`/Game/TSS_Game/Blueprints/System/BP_PlayerController.AllGeneratedRooms` (`/Game/TSS_Game/Blueprints/System/BP_CharacterBase.OwningPlayerController` _asbp_character_base)) (- (`self.RoomIndex`) 1)) true)
    (for _array_element (`|MakeArray` (`self.StaticMeshActor_738302`) (`self.StaticMeshActor_738303`) (`self.StaticMeshActor_738301`) (`self.StaticMeshActor_738306`) (`self.StaticMeshActor_738305`) (`self.StaticMeshActor_738304`) (`self.StaticMeshActor_738342`) (`self.StaticMeshActor_738340`) (`self.StaticMeshActor_738339`) (`self.StaticMeshActor_738343`) (`self.StaticMeshActor_738344`))
      (bind _asstatic_mesh_actor (cast `StaticMeshActor` (`ChildActorComponent.ChildActor` _array_element)))
      (`PrimitiveComponent.SetCustomPrimitiveDataFloat` (`StaticMeshActor.StaticMeshComponent` _asstatic_mesh_actor) 0 1.0)))
  (if (`KismetSystemLibrary.IsServer`)
    (`KismetArrayLibrary.Array_Clear` (`self.CharactersInZone`))
    (`KismetArrayLibrary.Array_Clear` (`self.CharactersAlive_0`))
    (`/Engine/EditorBlueprintResources/StandardMacros.IsValid` _as_bp_game_mode_base
      (:`Is Valid`
        (for _array_element_2 (`/Game/TSS_Game/Blueprints/System/BP_GameModeBase.AllCharacters` _as_bp_game_mode_base)
          (if (not (`/Game/TSS_Game/Blueprints/System/BP_CharacterBase.IsDead` _array_element_2))
            (`KismetArrayLibrary.Array_Add` (`self.CharactersAlive_0`) _array_element_2)))
        (for _array_element_3 (`PrimitiveComponent.GetOverlappingActors` (`self.EnemiesActivator`) "/Game/TSS_Game/Blueprints/System/BP_CharacterBase.BP_CharacterBase_C")
          (bind _asbp_character_base_2 (cast `/Game/TSS_Game/Blueprints/System/BP_CharacterBase` _array_element_3))
          (`KismetArrayLibrary.Array_Add` (`self.CharactersInZone`) _asbp_character_base_2))
        (if (== (`KismetArrayLibrary.Array_Length` (`self.CharactersInZone`)) (`KismetArrayLibrary.Array_Length` (`self.CharactersAlive_0`)))
          (`/Game/TSS_Game/Blueprints/System/BP_PlayerController.SV_RoomManualActivation` (`self.As BP Player Controller`) (`self.RoomIndex`))))
      (:`Is Not Valid`
        (`KismetSystemLibrary.PrintString` "BP_Room_Side_Mission_01: ERROR! Failed to cast to game mode base!!!" true true (struct :`R` 1.0 :`A` 1.0) 5.0)))))

(event `self.DisableRoomEnemySpawners`
  (`parent.DisableRoomEnemySpawners`))

(event `self.MC_WinConditionReached`
  (bind _array (`|MakeArray` (`self.BP_ACT_AlertLights_C_289`) (`self.BP_ACT_AlertLights_C_290`) (`self.BP_ACT_AlertLights_C_291`)))
  (bind _asbp_raising_lava (cast `/Game/TSS_Game/Blueprints/LevelDesign/MissionActors/BP_RaisingLava` (`ChildActorComponent.ChildActor` (`self.BP_RaisingLava_C_1`))))
  (`/Game/TSS_Game/Blueprints/LevelDesign/MissionActors/BP_RaisingLava.StopLavaRaising` _asbp_raising_lava)
  (for _array_element _array
    (bind _asbp_activatable_base (cast `/Game/TSS_Game/Blueprints/LevelDesign/BP_Activatable_Base` (`ChildActorComponent.ChildActor` _array_element)))
    (`/Game/TSS_Game/Blueprints/LevelDesign/BP_Activatable_Base.MC_Activate` _asbp_activatable_base))
  (`self.SpecialMissionAchievementChecker` "HeartofFire")
  (`KismetSystemLibrary.Delay` 3.0)
  (`parent.MC_WinConditionReached`)
  (`KismetSystemLibrary.Delay` 6.0)
  (for _array_element_2 _array
    (bind _asbp_activatable_base_2 (cast `/Game/TSS_Game/Blueprints/LevelDesign/BP_Activatable_Base` (`ChildActorComponent.ChildActor` _array_element_2)))
    (`/Game/TSS_Game/Blueprints/LevelDesign/BP_Activatable_Base.MC_Deactivate` _asbp_activatable_base_2)))

(fn `UserConstructionScript`
  (bind _array (`|MakeArray` "/Game/TSS_Game/Blueprints/LevelDesign/ModularRooms/BP_SpawnerWallTube_Large_01.BP_SpawnerWallTube_Large_01_C" "/Game/TSS_Game/Blueprints/LevelDesign/ModularRooms/BP_SpawnerWallTube_Large_02.BP_SpawnerWallTube_Large_02_C" "/Game/TSS_Game/Blueprints/LevelDesign/ModularRooms/BP_SpawnerWallTube_Large_03.BP_SpawnerWallTube_Large_03_C" :!type "Actor Class Reference"))
  (bind _defaultdecorations (`self.DefaultDecorations`))
  (bind _mesheschancetoreplace (`self.MeshesChanceToReplace`))
  (`self.InitRoomActors` :`IsServer?` true :`ActorReplacableVariants` (`|MakeArray` (make `/Game/TSS_Game/Blueprints/LevelDesign/ModularRooms/ST_RoomCompVariants` (`self.StaticMeshActor_738561`) 25.0 _array) (make `/Game/TSS_Game/Blueprints/LevelDesign/ModularRooms/ST_RoomCompVariants` (`self.StaticMeshActor_738314`) 25.0 _array) (make `/Game/TSS_Game/Blueprints/LevelDesign/ModularRooms/ST_RoomCompVariants` (`self.StaticMeshActor_738312`) 25.0 _array) (make `/Game/TSS_Game/Blueprints/LevelDesign/ModularRooms/ST_RoomCompVariants` (`self.StaticMeshActor_738324`) 25.0 _array)) :`MeshReplacableVariants` (`|MakeArray` (make `/Game/TSS_Game/Blueprints/LevelDesign/ModularRooms/ST_RoomMeshVariants` (`self.DecorFloor2`) _mesheschancetoreplace _defaultdecorations) (make `/Game/TSS_Game/Blueprints/LevelDesign/ModularRooms/ST_RoomMeshVariants` (`self.DecorFloor3`) _mesheschancetoreplace _defaultdecorations) (make `/Game/TSS_Game/Blueprints/LevelDesign/ModularRooms/ST_RoomMeshVariants` (`self.DecorFloor1`) _mesheschancetoreplace _defaultdecorations) (make `/Game/TSS_Game/Blueprints/LevelDesign/ModularRooms/ST_RoomMeshVariants` (`self.DecorFloor4`) _mesheschancetoreplace _defaultdecorations) (make `/Game/TSS_Game/Blueprints/LevelDesign/ModularRooms/ST_RoomMeshVariants` (`self.DecorFloor5`) _mesheschancetoreplace _defaultdecorations)) :`ActorsHidable` (`|MakeArray` (`self.StaticMeshActor_738297`) (`self.StaticMeshActor_738532`) (`self.StaticMeshActor_738295`) (`self.StaticMeshActor_738296`) (`self.StaticMeshActor_738333`) (`self.StaticMeshActor_738334`) (`self.StaticMeshActor_738298`)) :`ActorsHidable_NextRoom` (`|MakeArray` (`self.StaticMeshActor_738411`) (`self.StaticMeshActor_738413`) (`self.StaticMeshActor_738323`) (`self.StaticMeshActor_738394`) (`self.StaticMeshActor_738412`)) :`PossibleWays` (`|MakeArray` (make `/Game/TSS_Game/Blueprints/LevelDesign/ModularRooms/ST_ProcDoors_Pure` (`self.BP_ACT_BlastDoor_SingleLarge_C_4941`) (`self.NextRoomArrow`))) :`AmmoCrates` (`|MakeArray` (`self.Ammo3`) (`self.Ammo1`) (`self.Ammo2`) (`self.Ammo9`) (`self.Ammo7`) (`self.Ammo6`) (`self.Ammo5`) (`self.Ammo8`) (`self.Ammo4`) (`self.Ammo10`) (`self.Ammo11`)) :`Skulls` (`|MakeArray` (`self.Skulls3`) (`self.Skulls2`) (`self.Skulls4`) (`self.Skulls1`)) :`EnemySpawners` (`|MakeArray` (`self.EnemySpawner_1`) (`self.EnemySpawner_2`)) :`BossSpawners` (`|MakeArray` (`self.BossSpawner_1`)))
  (`parent.UserConstructionScript`))