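; Modular 10x8 room Blueprint for building levels from connected rooms, with randomized dressing and one exit to a next room.
; Its Construction Script registers the room's components through InitRoomActors, with IsServer fixed to true, then calls the parent script.
; Walls, floor tiles, decorations and decals get replacement chances and variant pools, alongside hidable actors, the exit door, ammo crates, skulls, enemy pre-spawners and respawn points.
; The event graph is inactive.
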(fn `UserConstructionScript`
  (bind _defaultdecorations (`self.DefaultDecorations`))
  (bind _defaultwallspawners (`self.DefaultWallSpawners`))
  (bind _defaultdecals (`self.DefaultDecals`))
  (bind _actorschancetoreplace (`self.ActorsChanceToReplace`))
  (bind _mesheschancetoreplace (`self.MeshesChanceToReplace`))
  (bind _decalchancetoreplace (`self.DecalChanceToReplace`))
  (bind _defaultfloortiles (`self.DefaultFloorTiles`))
  (bind _mesheschancetoreplace_2 (`self.MeshesChanceToReplace`))
  (`self.InitRoomActors` :`IsServer?` true :`ActorReplacableVariants` (`|MakeArray` (make `/Game/TSS_Game/Blueprints/LevelDesign/ModularRooms/ST_RoomCompVariants` (`self.StaticMeshActor_182038`) _actorschancetoreplace _defaultwallspawners) (make `/Game/TSS_Game/Blueprints/LevelDesign/ModularRooms/ST_RoomCompVariants` (`self.StaticMeshActor_182037`) _actorschancetoreplace _defaultwallspawners) (make `/Game/TSS_Game/Blueprints/LevelDesign/ModularRooms/ST_RoomCompVariants` (`self.StaticMeshActor_182229`) _actorschancetoreplace _defaultwallspawners) (make `/Game/TSS_Game/Blueprints/LevelDesign/ModularRooms/ST_RoomCompVariants` (`self.StaticMeshActor_182042`) _actorschancetoreplace _defaultwallspawners) (make `/Game/TSS_Game/Blueprints/LevelDesign/ModularRooms/ST_RoomCompVariants` (`self.StaticMeshActor_181241`) _mesheschancetoreplace _defaultfloortiles) (make `/Game/TSS_Game/Blueprints/LevelDesign/ModularRooms/ST_RoomCompVariants` (`self.StaticMeshActor_180529`) _mesheschancetoreplace _defaultfloortiles) (make `/Game/TSS_Game/Blueprints/LevelDesign/ModularRooms/ST_RoomCompVariants` (`self.StaticMeshActor_181313`) _mesheschancetoreplace _defaultfloortiles) (make `/Game/TSS_Game/Blueprints/LevelDesign/ModularRooms/ST_RoomCompVariants` (`self.StaticMeshActor_181314`) _mesheschancetoreplace _defaultfloortiles) (make `/Game/TSS_Game/Blueprints/LevelDesign/ModularRooms/ST_RoomCompVariants` (`self.StaticMeshActor_181401`) _mesheschancetoreplace _defaultfloortiles)) :`MeshReplacableVariants` (`|MakeArray` (make `/Game/TSS_Game/Blueprints/LevelDesign/ModularRooms/ST_RoomMeshVariants` (`self.DecorFloor2`) _mesheschancetoreplace_2 _defaultdecorations) (make `/Game/TSS_Game/Blueprints/LevelDesign/ModularRooms/ST_RoomMeshVariants` (`self.DecorFloor3`) _mesheschancetoreplace_2 _defaultdecorations) (make `/Game/TSS_Game/Blueprints/LevelDesign/ModularRooms/ST_RoomMeshVariants` null _mesheschancetoreplace_2 _defaultdecorations) (make `/Game/TSS_Game/Blueprints/LevelDesign/ModularRooms/ST_RoomMeshVariants` (`self.DecorFloor1`) _mesheschancetoreplace_2 _defaultdecorations) (make `/Game/TSS_Game/Blueprints/LevelDesign/ModularRooms/ST_RoomMeshVariants` (`self.DecorFloor5`) _mesheschancetoreplace_2 _defaultdecorations) (make `/Game/TSS_Game/Blueprints/LevelDesign/ModularRooms/ST_RoomMeshVariants` (`self.DecorFloor6`) _mesheschancetoreplace_2 _defaultdecorations) (make `/Game/TSS_Game/Blueprints/LevelDesign/ModularRooms/ST_RoomMeshVariants` (`self.Decal_2`) _decalchancetoreplace _defaultdecals) (make `/Game/TSS_Game/Blueprints/LevelDesign/ModularRooms/ST_RoomMeshVariants` (`self.Decal_3`) _decalchancetoreplace _defaultdecals) (make `/Game/TSS_Game/Blueprints/LevelDesign/ModularRooms/ST_RoomMeshVariants` (`self.Decal_4`) _decalchancetoreplace _defaultdecals) (make `/Game/TSS_Game/Blueprints/LevelDesign/ModularRooms/ST_RoomMeshVariants` (`self.Decal_5`) _decalchancetoreplace _defaultdecals) (make `/Game/TSS_Game/Blueprints/LevelDesign/ModularRooms/ST_RoomMeshVariants` (`self.Decal_1`) _decalchancetoreplace _defaultdecals) (make `/Game/TSS_Game/Blueprints/LevelDesign/ModularRooms/ST_RoomMeshVariants` (`self.DecorFloor7`) _mesheschancetoreplace_2 _defaultdecorations) (make `/Game/TSS_Game/Blueprints/LevelDesign/ModularRooms/ST_RoomMeshVariants` (`self.Decal_7`) _decalchancetoreplace _defaultdecals) (make `/Game/TSS_Game/Blueprints/LevelDesign/ModularRooms/ST_RoomMeshVariants` (`self.Decal_8`) _decalchancetoreplace _defaultdecals) (make `/Game/TSS_Game/Blueprints/LevelDesign/ModularRooms/ST_RoomMeshVariants` (`self.Decal_6`) _decalchancetoreplace _defaultdecals)) :`ActorsHidable` (`|MakeArray` (`self.StaticMeshActor_182255`) (`self.StaticMeshActor_182415`) (`self.StaticMeshActor_182431`) (`self.StaticMeshActor_182429`) (`self.StaticMeshActor_182393`) (`self.StaticMeshActor_182394`) (`self.StaticMeshActor_182401`) (`self.StaticMeshActor_182317`) (`self.StaticMeshActor_182239`) (`self.StaticMeshActor_182257`) (`self.StaticMeshActor_182402`) (`self.StaticMeshActor_182233`) (`self.StaticMeshActor_182279`) (`self.StaticMeshActor_182349`) (`self.StaticMeshActor_182053`) (`self.StaticMeshActor_182059`) (`self.StaticMeshActor_182358`) (`self.StaticMeshActor_182357`) (`self.StaticMeshActor_182359`) (`self.StaticMeshActor_182360`)) :`ActorsHidable_NextRoom` (`|MakeArray` (`self.StaticMeshActor_181353`) (`self.StaticMeshActor_181358`) (`self.StaticMeshActor_182352`) (`self.StaticMeshActor_182351`) (`self.StaticMeshActor_181359`)) :`PossibleWays` (`|MakeArray` (make `/Game/TSS_Game/Blueprints/LevelDesign/ModularRooms/ST_ProcDoors_Pure` (`self.BP_ACT_BlastDoor_SingleLarge_C_217`) (`self.NextRoomArrow`))) :`AmmoCrates` (`|MakeArray` (`self.Ammo3`) (`self.Ammo4`) (`self.Ammo2`)) :`Skulls` (`|MakeArray` (`self.Skulls7`) (`self.Skulls8`) (`self.Skulls4`) (`self.Skulls6`) (`self.Skulls5`)) :`EnemiesPreSpawners` (`|MakeArray` (`self.EnemyPreSpawner_2`) (`self.EnemyPreSpawner_4`) (`self.EnemyPreSpawner_5`) (`self.EnemyPreSpawner_6`) (`self.EnemyPreSpawner_7`) (`self.EnemyPreSpawner_1`) (`self.EnemyPreSpawner_3`) (`self.EnemyPreSpawner_9`) (`self.EnemyPreSpawner_8`)) :`RespawnPoints` (`|MakeArray` (`self.RespawnPoint_2`) (`self.RespawnPoint_3`) (`self.RespawnPoint_4`) (`self.RespawnPoint_5`) (`self.RespawnPoint_6`) (`self.RespawnPoint_1`)))
  (`parent.UserConstructionScript`))