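; Modular start room variant for procedurally connected levels, with one blast-door exit, ammo crates, skulls and respawn points.
; The construction script passes its placed actors to InitRoomActors with IsServer hardcoded true, then runs the parent construction script.
; That call also registers floor tiles for chance-based mesh replacement, two groups of hidable actors and the exit's door, arrow and direction.
; The event graph holds only disabled stubs.
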(fn `UserConstructionScript`
  (bind _mesheschancetoreplace (`self.MeshesChanceToReplace`))
  (bind _defaultfloortiles (`self.DefaultFloorTiles`))
  (`self.InitRoomActors` :`IsServer?` true :`ActorReplacableVariants` (`|MakeArray` (make `/Game/TSS_Game/Blueprints/LevelDesign/ModularRooms/ST_RoomCompVariants` (`self.StaticMeshActor_757949`) _mesheschancetoreplace _defaultfloortiles) (make `/Game/TSS_Game/Blueprints/LevelDesign/ModularRooms/ST_RoomCompVariants` (`self.StaticMeshActor_757962`) _mesheschancetoreplace _defaultfloortiles) (make `/Game/TSS_Game/Blueprints/LevelDesign/ModularRooms/ST_RoomCompVariants` (`self.StaticMeshActor_757957`) _mesheschancetoreplace _defaultfloortiles)) :`ActorsHidable` (`|MakeArray` (`self.StaticMeshActor_757982`) (`self.StaticMeshActor_757981`) (`self.StaticMeshActor_757991`) (`self.StaticMeshActor_758002`) (`self.StaticMeshActor_757983`)) :`ActorsHidable_NextRoom` (`|MakeArray` (`self.StaticMeshActor_758071`) (`self.StaticMeshActor_758066`) (`self.StaticMeshActor_758067`) (`self.StaticMeshActor_758072`) (`self.StaticMeshActor_758068`) (`self.StaticMeshActor_758058`) (`self.StaticMeshActor_757985`) (`self.StaticMeshActor_757989`) (`self.StaticMeshActor_758057`)) :`PossibleWays` (`|MakeArray` (make `/Game/TSS_Game/Blueprints/LevelDesign/ModularRooms/ST_ProcDoors_Pure` (`self.BP_ACT_BlastDoor_SingleLarge_C_3961`) (`self.NextRoomArrow`))) :`AmmoCrates` (`|MakeArray` (`self.Ammo1`) (`self.Ammo3`) (`self.Ammo2`)) :`Skulls` (`|MakeArray` (`self.Skulls4`)) :`RespawnPoints` (`|MakeArray` (`self.RespawnPoint_1`) (`self.RespawnPoint_3`) (`self.RespawnPoint_4`) (`self.RespawnPoint_2`)))
  (`parent.UserConstructionScript`))