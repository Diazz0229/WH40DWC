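; BP_Room_Side_2x2 is a side room piece for modular, procedurally linked level layouts, built on a parent room class.
; Its construction script feeds InitRoomActors three walls that can each swap to a tube spawner wall by chance, plus hidable actors, one exit arrow, ammo crates and enemy pre-spawners, then runs the parent script.
; A CalculateChance helper provides a percentage roll, and BeginPlay only calls the parent.
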(event `self.ReceiveBeginPlay`
  (`parent.ReceiveBeginPlay`))

(fn `UserConstructionScript`
  (bind _array (`|MakeArray` "/Game/TSS_Game/Blueprints/LevelDesign/ModularRooms/BP_SpawnerWallTube_Large_01.BP_SpawnerWallTube_Large_01_C" :!type "Actor Class Reference"))
  (`self.InitRoomActors` :`IsServer?` true :`ActorReplacableVariants` (`|MakeArray` (make `/Game/TSS_Game/Blueprints/LevelDesign/ModularRooms/ST_RoomCompVariants` (`self.Wall1`) 50.0 _array) (make `/Game/TSS_Game/Blueprints/LevelDesign/ModularRooms/ST_RoomCompVariants` (`self.Wall3`) 50.0 _array) (make `/Game/TSS_Game/Blueprints/LevelDesign/ModularRooms/ST_RoomCompVariants` (`self.Wall2`) 50.0 _array)) :`ActorsHidable` (`|MakeArray` null null :!type "ChildActorComponent Object Reference") :`ActorsHidable_NextRoom` (`|MakeArray` null :!type "ChildActorComponent Object Reference") :`PossibleWays` (`|MakeArray` (make `/Game/TSS_Game/Blueprints/LevelDesign/ModularRooms/ST_ProcDoors_Pure` null (`self.NextRoomArrow`))) :`AmmoCrates` (`|MakeArray` (`self.Ammo1`) (`self.Ammo2`)) :`EnemiesPreSpawners` (`|MakeArray` null null :!type "StaticMeshComponent Object Reference"))
  (`parent.UserConstructionScript`))