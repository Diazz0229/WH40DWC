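; Modular 10x8 corner room piece for procedurally generated levels, with two possible exits, each pairing a blast door with a next-room arrow and direction.
; The construction script registers its components through InitRoomActors, then calls the parent script.
; It supplies wall, floor decor and decal slots with replacement chances and default variant pools, plus hidable actors, ammo crates, skulls and enemy pre-spawners.
; The event graph holds no active logic.
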(fn `UserConstructionScript`
  (bind _defaultdecorations (`self.DefaultDecorations`))
  (bind _defaultwallspawners (`self.DefaultWallSpawners`))
  (bind _defaultdecals (`self.DefaultDecals`))
  (bind _actorschancetoreplace (`self.ActorsChanceToReplace`))
  (bind _decalchancetoreplace (`self.DecalChanceToReplace`))
  (bind _mesheschancetoreplace (`self.MeshesChanceToReplace`))
  (`self.InitRoomActors` :`IsServer?` true :`ActorReplacableVariants` (`|MakeArray` (make `/Game/TSS_Game/Blueprints/LevelDesign/ModularRooms/ST_RoomCompVariants` (`self.StaticMeshActor_529173`) _actorschancetoreplace _defaultwallspawners) (make `/Game/TSS_Game/Blueprints/LevelDesign/ModularRooms/ST_RoomCompVariants` (`self.StaticMeshActor_529174`) _actorschancetoreplace _defaultwallspawners) (make `/Game/TSS_Game/Blueprints/LevelDesign/ModularRooms/ST_RoomCompVariants` (`self.StaticMeshActor_529172`) _actorschancetoreplace _defaultwallspawners)) :`MeshReplacableVariants` (`|MakeArray` (make `/Game/TSS_Game/Blueprints/LevelDesign/ModularRooms/ST_RoomMeshVariants` (`self.DecorFloor2`) _mesheschancetoreplace _defaultdecorations) (make `/Game/TSS_Game/Blueprints/LevelDesign/ModularRooms/ST_RoomMeshVariants` (`self.DecorFloor3`) _mesheschancetoreplace _defaultdecorations) (make `/Game/TSS_Game/Blueprints/LevelDesign/ModularRooms/ST_RoomMeshVariants` (`self.DecorFloor1`) _mesheschancetoreplace _defaultdecorations) (make `/Game/TSS_Game/Blueprints/LevelDesign/ModularRooms/ST_RoomMeshVariants` (`self.DecorFloor4`) _mesheschancetoreplace _defaultdecorations) (make `/Game/TSS_Game/Blueprints/LevelDesign/ModularRooms/ST_RoomMeshVariants` (`self.DecorFloor5`) _mesheschancetoreplace _defaultdecorations) (make `/Game/TSS_Game/Blueprints/LevelDesign/ModularRooms/ST_RoomMeshVariants` (`self.Decal_2`) _decalchancetoreplace _defaultdecals) (make `/Game/TSS_Game/Blueprints/LevelDesign/ModularRooms/ST_RoomMeshVariants` (`self.Decal_1`) _decalchancetoreplace _defaultdecals) (make `/Game/TSS_Game/Blueprints/LevelDesign/ModularRooms/ST_RoomMeshVariants` (`self.Decal_4`) _decalchancetoreplace _defaultdecals) (make `/Game/TSS_Game/Blueprints/LevelDesign/ModularRooms/ST_RoomMeshVariants` (`self.Decal_5`) _decalchancetoreplace _defaultdecals) (make `/Game/TSS_Game/Blueprints/LevelDesign/ModularRooms/ST_RoomMeshVariants` (`self.Decal_3`) _decalchancetoreplace _defaultdecals) (make `/Game/TSS_Game/Blueprints/LevelDesign/ModularRooms/ST_RoomMeshVariants` (`self.Decal_6`) _decalchancetoreplace _defaultdecals) (make `/Game/TSS_Game/Blueprints/LevelDesign/ModularRooms/ST_RoomMeshVariants` (`self.DecorFloor6`) _mesheschancetoreplace _defaultdecorations) (make `/Game/TSS_Game/Blueprints/LevelDesign/ModularRooms/ST_RoomMeshVariants` (`self.DecorFloor7`) _mesheschancetoreplace _defaultdecorations)) :`ActorsHidable` (`|MakeArray` (`self.StaticMeshActor_529183`) (`self.StaticMeshActor_529184`) (`self.StaticMeshActor_529185`) (`self.StaticMeshActor_529220`) (`self.StaticMeshActor_529182`)) :`ActorsHidable_NextRoom` (`|MakeArray` (`self.StaticMeshActor_529163`) (`self.StaticMeshActor_529161`) (`self.StaticMeshActor_529162`) (`self.StaticMeshActor_529171`) (`self.StaticMeshActor_529264`) (`self.StaticMeshActor_529168`) (`self.StaticMeshActor_529166`) (`self.StaticMeshActor_529167`) (`self.StaticMeshActor_529195`) (`self.StaticMeshActor_529194`)) :`PossibleWays` (`|MakeArray` (make `/Game/TSS_Game/Blueprints/LevelDesign/ModularRooms/ST_ProcDoors_Pure` (`self.BP_ACT_BlastDoor_SingleLarge_C_3206`) (`self.NextRoomArrow`)) (make `/Game/TSS_Game/Blueprints/LevelDesign/ModularRooms/ST_ProcDoors_Pure` (`self.BP_ACT_BlastDoor_SingleLarge_C_3207`) (`self.NextRoomArrow2`) "NewEnumerator1")) :`AmmoCrates` (`|MakeArray` (`self.Ammo3`) (`self.Ammo1`) (`self.Ammo2`)) :`Skulls` (`|MakeArray` (`self.Skulls3`) (`self.Skulls2`) (`self.Skulls4`) (`self.Skulls1`)) :`EnemiesPreSpawners` (`|MakeArray` (`self.EnemyPreSpawner_2`) (`self.EnemyPreSpawner_4`) (`self.EnemyPreSpawner_5`) (`self.EnemyPreSpawner_1`) (`self.EnemyPreSpawner_6`) (`self.EnemyPreSpawner_3`)))
  (`parent.UserConstructionScript`))