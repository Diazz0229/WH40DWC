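; Modular 10x8 room variant that registers its placed contents for randomized, procedural level assembly.
; The construction script passes wall actors, floor decor and decals, each with replacement chances and variant pools, to InitRoomActors, then runs the parent script.
; The same call supplies hidable actors, one next-room blast door with arrow and direction, ammo crates, skulls and enemy pre-spawners.
; The event graph holds no active logic.
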(fn `UserConstructionScript`
  (bind _defaultdecorations (`self.DefaultDecorations`))
  (bind _defaultwallspawners (`self.DefaultWallSpawners`))
  (bind _defaultdecals (`self.DefaultDecals`))
  (bind _actorschancetoreplace (`self.ActorsChanceToReplace`))
  (bind _decalchancetoreplace (`self.DecalChanceToReplace`))
  (bind _mesheschancetoreplace (`self.MeshesChanceToReplace`))
  (`self.InitRoomActors` :`IsServer?` true :`ActorReplacableVariants` (`|MakeArray` (make `/Game/TSS_Game/Blueprints/LevelDesign/ModularRooms/ST_RoomCompVariants` (`self.StaticMeshActor_277010`) _actorschancetoreplace _defaultwallspawners) (make `/Game/TSS_Game/Blueprints/LevelDesign/ModularRooms/ST_RoomCompVariants` (`self.StaticMeshActor_276996`) _actorschancetoreplace _defaultwallspawners) (make `/Game/TSS_Game/Blueprints/LevelDesign/ModularRooms/ST_RoomCompVariants` (`self.StaticMeshActor_277012`) _actorschancetoreplace _defaultwallspawners) (make `/Game/TSS_Game/Blueprints/LevelDesign/ModularRooms/ST_RoomCompVariants` (`self.StaticMeshActor_276995`) _actorschancetoreplace _defaultwallspawners) (make `/Game/TSS_Game/Blueprints/LevelDesign/ModularRooms/ST_RoomCompVariants` (`self.StaticMeshActor_276999`) _actorschancetoreplace _defaultwallspawners)) :`MeshReplacableVariants` (`|MakeArray` (make `/Game/TSS_Game/Blueprints/LevelDesign/ModularRooms/ST_RoomMeshVariants` (`self.DecorFloor2`) _mesheschancetoreplace _defaultdecorations) (make `/Game/TSS_Game/Blueprints/LevelDesign/ModularRooms/ST_RoomMeshVariants` (`self.DecorFloor3`) _mesheschancetoreplace _defaultdecorations) (make `/Game/TSS_Game/Blueprints/LevelDesign/ModularRooms/ST_RoomMeshVariants` (`self.DecorFloor4`) _mesheschancetoreplace _defaultdecorations) (make `/Game/TSS_Game/Blueprints/LevelDesign/ModularRooms/ST_RoomMeshVariants` (`self.DecorFloor1`) _mesheschancetoreplace _defaultdecorations) (make `/Game/TSS_Game/Blueprints/LevelDesign/ModularRooms/ST_RoomMeshVariants` (`self.DecorFloor5`) _mesheschancetoreplace _defaultdecorations) (make `/Game/TSS_Game/Blueprints/LevelDesign/ModularRooms/ST_RoomMeshVariants` (`self.DecorFloor6`) _mesheschancetoreplace _defaultdecorations) (make `/Game/TSS_Game/Blueprints/LevelDesign/ModularRooms/ST_RoomMeshVariants` (`self.Decal_2`) _decalchancetoreplace _defaultdecals) (make `/Game/TSS_Game/Blueprints/LevelDesign/ModularRooms/ST_RoomMeshVariants` (`self.Decal_3`) _decalchancetoreplace _defaultdecals) (make `/Game/TSS_Game/Blueprints/LevelDesign/ModularRooms/ST_RoomMeshVariants` (`self.Decal_4`) _decalchancetoreplace _defaultdecals) (make `/Game/TSS_Game/Blueprints/LevelDesign/ModularRooms/ST_RoomMeshVariants` (`self.Decal_5`) _decalchancetoreplace _defaultdecals) (make `/Game/TSS_Game/Blueprints/LevelDesign/ModularRooms/ST_RoomMeshVariants` (`self.Decal_1`) _decalchancetoreplace _defaultdecals) (make `/Game/TSS_Game/Blueprints/LevelDesign/ModularRooms/ST_RoomMeshVariants` (`self.DecorFloor7`) _mesheschancetoreplace _defaultdecorations) (make `/Game/TSS_Game/Blueprints/LevelDesign/ModularRooms/ST_RoomMeshVariants` (`self.Decal_9`) _decalchancetoreplace _defaultdecals) (make `/Game/TSS_Game/Blueprints/LevelDesign/ModularRooms/ST_RoomMeshVariants` (`self.Decal_7`) _decalchancetoreplace _defaultdecals) (make `/Game/TSS_Game/Blueprints/LevelDesign/ModularRooms/ST_RoomMeshVariants` (`self.Decal_8`) _decalchancetoreplace _defaultdecals) (make `/Game/TSS_Game/Blueprints/LevelDesign/ModularRooms/ST_RoomMeshVariants` (`self.Decal_6`) _decalchancetoreplace _defaultdecals) (make `/Game/TSS_Game/Blueprints/LevelDesign/ModularRooms/ST_RoomMeshVariants` (`self.Decal_10`) _decalchancetoreplace _defaultdecals)) :`ActorsHidable` (`|MakeArray` (`self.StaticMeshActor_277016`) (`self.StaticMeshActor_276982`) (`self.StaticMeshActor_276986`) (`self.StaticMeshActor_277001`) (`self.StaticMeshActor_277011`) (`self.StaticMeshActor_276981`) (`self.StaticMeshActor_277019`) (`self.StaticMeshActor_277022`) (`self.StaticMeshActor_277005`) (`self.StaticMeshActor_277007`)) :`ActorsHidable_NextRoom` (`|MakeArray` (`self.StaticMeshActor_276992`) (`self.StaticMeshActor_276990`) (`self.StaticMeshActor_276991`) (`self.StaticMeshActor_277003`) (`self.StaticMeshActor_277002`)) :`PossibleWays` (`|MakeArray` (make `/Game/TSS_Game/Blueprints/LevelDesign/ModularRooms/ST_ProcDoors_Pure` (`self.BP_ACT_BlastDoor_SingleLarge_C_1528`) (`self.NextRoomArrow`))) :`AmmoCrates` (`|MakeArray` (`self.Ammo3`) (`self.Ammo1`) (`self.Ammo2`)) :`Skulls` (`|MakeArray` (`self.Skulls3`) (`self.Skulls2`) (`self.Skulls1`) (`self.Skulls1`)) :`EnemiesPreSpawners` (`|MakeArray` (`self.EnemyPreSpawner_2`) (`self.EnemyPreSpawner_4`) (`self.EnemyPreSpawner_5`) (`self.EnemyPreSpawner_6`) (`self.EnemyPreSpawner_7`) (`self.EnemyPreSpawner_1`) (`self.EnemyPreSpawner_3`)))
  (`parent.UserConstructionScript`))