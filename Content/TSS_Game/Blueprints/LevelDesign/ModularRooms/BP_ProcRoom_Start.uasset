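; Starting-room variant of the procedural modular room Blueprints used in level design.
; On BeginPlay it fills the ammo crate, skull and enemy spawner arrays with its own placed instances, then calls the parent BeginPlay.
; It adds no other logic, and its construction script only calls the parent's.
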(event `self.ReceiveBeginPlay`
  (set `self.AmmoCrates` (`|MakeArray` (`self.Ammo1`) (`self.Ammo3`) (`self.Ammo2`) (`self.Ammo4`)))
  (set `self.Skulls` (`|MakeArray` (`self.Skulls1`) (`self.Skulls2`)))
  (set `self.EnemySpawner` (`|MakeArray` (`self.EnemySpawner1`) (`self.EnemySpawner2`)))
  (`parent.ReceiveBeginPlay`))

(fn `UserConstructionScript`
  (`parent.UserConstructionScript`))