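; BP_AI_JumpPlatform is a level-design jump pad that launches BP_Enemy_BASE characters along a placed direction arrow.
; Enemies entering the TriggerBox have their capsule turned to LaunchDirection's yaw, their movement stopped, and are launched with randomized forward and upward velocity.
; A looping timer started on BeginPlay relaunches any enemies still overlapping the box, so none get stuck on it.
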(event `self.ReceiveBeginPlay`
  (`KismetSystemLibrary.K2_SetTimerDelegate` (delegate `LaunchAllStuck`) 0.8 true))

(event `LaunchAllStuck`
  (for _array_element (`PrimitiveComponent.GetOverlappingActors` (`self.TriggerBox`) "/Game/TSS_Game/Blueprints/Bonus/AI/BP_Enemy_BASE.BP_Enemy_BASE_C")
    (`self.LaunchCharacter` _array_element)))

(event `self.TriggerBox.OnComponentBeginOverlap`
  (params (OverlappedComponent :type "PrimitiveComponent Object Reference") (OtherActor :type "Actor Object Reference") (OtherComp :type "PrimitiveComponent Object Reference") (OtherBodyIndex :type Integer) (bFromSweep :type Boolean) (SweepResult :type "HitResult Structure (by ref)"))
  (`self.LaunchCharacter` OtherActor))

(event `LaunchCharacter`
  (params (Object :type "Object Object Reference"))
  (bind (_returnvalue_roll _returnvalue_pitch _returnvalue_yaw) (`KismetMathLibrary.BreakRotator` (`SceneComponent.K2_GetComponentRotation` (`self.LaunchDirection`))))
  (bind _asbp_enemy_base (cast `/Game/TSS_Game/Blueprints/Bonus/AI/BP_Enemy_BASE` Object))
  (`SceneComponent.K2_SetWorldRotation` (`Character.CapsuleComponent` _asbp_enemy_base) (`KismetMathLibrary.MakeRotator` 0.0 0.0 _returnvalue_yaw) false false)
  (`MovementComponent.StopMovementImmediately` (`Character.CharacterMovement` _asbp_enemy_base))
  (`Character.LaunchCharacter` _asbp_enemy_base (+ (* (`SceneComponent.GetForwardVector` (`self.LaunchDirection`)) (`KismetMathLibrary.RandomFloatInRange` 500.0 750.0)) (`KismetMathLibrary.MakeVector` 0.0 0.0 (`KismetMathLibrary.RandomFloatInRange` 250.0 400.0))) false false))

(fn `UserConstructionScript`)