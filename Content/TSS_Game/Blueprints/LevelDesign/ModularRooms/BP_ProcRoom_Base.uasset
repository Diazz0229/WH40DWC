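; Base actor for procedural modular rooms that randomizes their contents, runs a timed combat encounter and chains to the next room.
; The server randomly swaps placeholders, scatters pickups, picks an exit and records replacements by index for remote replay.
; Unlocking pre-spawns passive enemies; overlapping the activator aggroes them and starts timed, mutated wave spawners.
; Once all enemies die, the win condition opens the exit, unlocks the next room and updates hidden walls.
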(event `self.ReceiveBeginPlay`
  ;[1 1 1] Hide walls
  (for _array_element (`self.ActorsHidable`)
    (bind _asstatic_mesh_actor (cast `StaticMeshActor` (`ChildActorComponent.ChildActor` _array_element)))
    (`PrimitiveComponent.SetCustomPrimitiveDataFloat` (`StaticMeshActor.StaticMeshComponent` _asstatic_mesh_actor) 0 1.0))
  ;[1 1 1] Place eternal Enemy spawners
  (for _array_element_2 (`self.EnemySpawners_Eternal`)
    (bind _returnvalue (`|SpawnActorFromClass` "/Game/TSS_Game/Blueprints/LevelDesign/Spawners/BP_EnemySpawner.BP_EnemySpawner_C" (`KismetMathLibrary.MakeTransform` (`SceneComponent.K2_GetComponentLocation` _array_element_2)) "Undefined" "MultiplyWithRoot" null null))
    (`KismetArrayLibrary.Array_AddUnique` (`self.RoomEnemySpawners`) _returnvalue)))

(event `MC_WinConditionReached`
  (bind (_nextroomdoor _nextroomarrow _nextroom) (break `/Game/TSS_Game/Blueprints/LevelDesign/ModularRooms/ST_ProcDoors` (`self.ExitWay`)))
  (`/Game/TSS_Game/Blueprints/LevelDesign/BP_Activatable_Base.MC_Activate` _nextroomdoor)
  (`KismetSystemLibrary.PrintString` "ROOM_BASE: Win condition reached, show congrats message!" true true (struct :`R` 0.095554 :`G` 1.0 :`A` 1.0) :!pinned true) ; REPLACE TEMP
  (set `self.IsRoomActivated?` false)
  (`self.RoomIsUnlocked` _nextroom)
  ;[1 1 1] Hide walls that go after next room
  (for _array_element (`self.ActorsHidable_NextRoom`)
    (bind _asstatic_mesh_actor (cast `StaticMeshActor` (`ChildActorComponent.ChildActor` _array_element)))
    (`PrimitiveComponent.SetCustomPrimitiveDataFloat` (`StaticMeshActor.StaticMeshComponent` _asstatic_mesh_actor) 0 1.0)))

(event `EnableRoomEnemySpawners`
  (bind _as_bp_game_mode_base (`self.As BP Game Mode Base`))
  (if (`KismetSystemLibrary.IsServer`)
    (bind (_newmutation _mutationdescription) (`/Game/TSS_Game/Blueprints/System/BP_GameModeBase.DetermineNewMutation` _as_bp_game_mode_base))
    (for _array_element (`self.RoomEnemySpawners`)
      (set `/Game/TSS_Game/Blueprints/LevelDesign/Spawners/BP_EnemySpawner.IsActive?` true _array_element)
      (`/Game/TSS_Game/Blueprints/LevelDesign/Spawners/BP_EnemySpawner.BeginSpawns` _array_element 1 (`KismetMathLibrary.Clamp` (+ (* (`KismetArrayLibrary.Array_Length` (`/Game/TSS_Game/Blueprints/System/BP_GameModeBase.AllCharacters` _as_bp_game_mode_base)) 10) (`self.RoomIndex`)) 0 80) _newmutation (`self.WaveList`) 4.0 30.0)
      (`KismetSystemLibrary.PrintString` (`KismetStringLibrary.Concat_StrStr` "BP_Proc_Room_Base: New mutation: " (`KismetTextLibrary.Conv_TextToString` _mutationdescription)) true true (struct :`R` 1.0 :`B` 0.907107 :`A` 1.0) 4.0))))

(event `RoomIsUnlocked`
  (if (`KismetSystemLibrary.IsServer`)
    (`/Engine/EditorBlueprintResources/StandardMacros.DoOnce` false
      (:`Completed`
        (`self.EnemiesPreSpawnersInit`)))))

(event `EnemiesPreSpawnersInit`
  (bind (_enemyclass _spawnchance _behaviortree) (break `/Game/TSS_Game/Blueprints/Bonus/AI/ST_WaveList` (`self.WaveList`)))
  (bind (_outitem _outindex) (`KismetArrayLibrary.Array_Random` _enemyclass))
  (for _array_element (`self.EnemiesPreSpawners`)
    (bind _returnvalue (`AIBlueprintHelperLibrary.SpawnAIFromClass` _outitem (`|GetArrayItem` _behaviortree _outindex) (`SceneComponent.K2_GetComponentLocation` _array_element) (struct) false null))
    (bind _asbp_enemy_base (cast `/Game/TSS_Game/Blueprints/Bonus/AI/BP_Enemy_BASE` _returnvalue))
    (`KismetArrayLibrary.Array_AddUnique` (`self.EnemiesPreSpawned`) _asbp_enemy_base)
    (set `/Game/TSS_Game/Blueprints/Bonus/AI/BP_Enemy_BASE.AI_agressive` false _asbp_enemy_base)
    (`/Game/TSS_Game/Blueprints/Bonus/AI/BP_Enemy_BASE.SV_AgressiveStateChanged` _asbp_enemy_base)))

(event `self.EnemiesActivator.OnComponentBeginOverlap`
  (params (OverlappedComponent :type "PrimitiveComponent Object Reference") (OtherActor :type "Actor Object Reference") (OtherComp :type "PrimitiveComponent Object Reference") (OtherBodyIndex :type Integer) (bFromSweep :type Boolean) (SweepResult :type "HitResult Structure (by ref)"))
  (cast `/Game/TSS_Game/Blueprints/System/BP_CharacterBase` OtherActor)
  (switch `/Game/TSS_Game/Blueprints/LevelDesign/ModularRooms/E_ProcRoomWinCondition` (`self.WinCondition`)
    (:`NewEnumerator0`
      (if (`KismetSystemLibrary.IsServer`)
        (`self.RoomIsActivated`)
        (else
          (set `PrimitiveComponent.bGenerateOverlapEvents` false (`self.EnemiesActivator`)))))))

(event `MC_RoomIsActivated`
  (for _array_element (`self.StaticMeshesHidable`)
    (`PrimitiveComponent.SetCustomPrimitiveDataFloat` _array_element 0 1.0))
  (set `self.IsRoomActivated?` true))

(event `RoomIsActivated`
  (set `PrimitiveComponent.bGenerateOverlapEvents` false (`self.EnemiesActivator`))
  (for _array_element (`self.EnemiesPreSpawned`)
    (`/Engine/EditorBlueprintResources/StandardMacros.IsValid` _array_element
      (:`Is Valid`
        (set `/Game/TSS_Game/Blueprints/Bonus/AI/BP_Enemy_BASE.AI_agressive` true _array_element)
        (`/Game/TSS_Game/Blueprints/Bonus/AI/BP_Enemy_BASE.SV_AgressiveStateChanged` _array_element))))
  (`self.EnableRoomEnemySpawners`)
  (`KismetSystemLibrary.K2_SetTimerDelegate` (delegate `DisableRoomEnemySpawners`) (`self.RoomMissionTimer`))
  (`self.MC_RoomIsActivated`)
  (if (`KismetArrayLibrary.Array_IsEmpty` (`self.RoomEnemySpawners`))
    (`self.DisableRoomEnemySpawners`)
    (`KismetSystemLibrary.K2_PauseTimer` null "DisableRoomEnemySpawners")))

(event `DisableRoomEnemySpawners`
  (for _array_element (`self.RoomEnemySpawners`)
    (set `/Game/TSS_Game/Blueprints/LevelDesign/Spawners/BP_EnemySpawner.IsActive?` false _array_element)
    (`/Game/TSS_Game/Blueprints/System/BP_GameModeBase.EnemiesStartDeathTimer` (`self.As BP Game Mode Base`)))
  (`KismetSystemLibrary.K2_SetTimerDelegate` (delegate `CheckIfAllEnemiesAreDead`) 5.0 true))

(event `CheckIfAllEnemiesAreDead`
  (bind _as_bp_game_mode_base (`self.As BP Game Mode Base`))
  (bind _allenemiesdead (`/Game/TSS_Game/Blueprints/System/BP_GameModeBase.EnemiesDeadChecker` _as_bp_game_mode_base))
  (if _allenemiesdead
    (set `self.IsRoomClear?` true)
    (`KismetSystemLibrary.K2_PauseTimer` null "CheckIfAllEnemiesAreDead")
    (switch `/Game/TSS_Game/Blueprints/LevelDesign/ModularRooms/E_ProcRoomWinCondition` (`self.WinCondition`)
      (:`NewEnumerator0`
        (bind _asbp_player_controller (cast `/Game/TSS_Game/Blueprints/System/BP_PlayerController` (`GameplayStatics.GetPlayerController` 0)))
        (`/Game/TSS_Game/Blueprints/System/BP_PlayerController.SV_WinConditionReached` _asbp_player_controller (`self.RoomIndex`))))
    (else
      (switch `/Game/TSS_Game/Blueprints/LevelDesign/ModularRooms/E_ProcRoomWinCondition` (`self.WinCondition`)
        (:`NewEnumerator0`
          (`/Game/TSS_Game/Blueprints/System/BP_GameModeBase.UpdateWaveInfo` _as_bp_game_mode_base false))))))

(event `SV_SpawnBoss`
  (bind (_enemyclass _spawnchance _behaviortree _bossclass _bossammount _bossbehaviortree) (break `/Game/TSS_Game/Blueprints/Bonus/AI/ST_WaveList` (`self.WaveList`)))
  (bind (_outitem _outindex) (`KismetArrayLibrary.Array_Random` _bossclass))
  (for _array_element (`self.Boss Spawners`)
    (`AIBlueprintHelperLibrary.SpawnAIFromClass` (castclass `Pawn` _outitem :!pure true) (`|GetArrayItem` _bossbehaviortree _outindex) (`SceneComponent.K2_GetComponentLocation` _array_element) (struct) false null)))

(fn `InitRoomActors`
  (params (`IsServer?` :type Boolean) (ActorReplacableVariants :type "Array of /Game/TSS_Game/Blueprints/LevelDesign/ModularRooms/ST_RoomCompVariants Structure") (MeshReplacableVariants :type "Array of /Game/TSS_Game/Blueprints/LevelDesign/ModularRooms/ST_RoomMeshVariants Structure") (ActorsHidable :type "Array of ChildActorComponent Object Reference") (ActorsHidable_NextRoom :type "Array of ChildActorComponent Object Reference") (PossibleWays :type "Array of /Game/TSS_Game/Blueprints/LevelDesign/ModularRooms/ST_ProcDoors_Pure Structure") (AmmoCrates :type "Array of StaticMeshComponent Object Reference") (Skulls :type "Array of StaticMeshComponent Object Reference") (EnemySpawners :type "Array of StaticMeshComponent Object Reference") (EnemiesPreSpawners :type "Array of StaticMeshComponent Object Reference") (BossSpawners :type "Array of StaticMeshComponent Object Reference"))
  (returns (`Success?` :type Boolean))
  (if `IsServer?`
    (set `self.ActorReplacableVariants` ActorReplacableVariants)
    (set `self.MeshReplacableVariants` MeshReplacableVariants)
    (set `self.ActorsHidable` ActorsHidable)
    (set `self.ActorsHidable_NextRoom` ActorsHidable_NextRoom))
  (for (_array_element _array_index) PossibleWays
    (bind (_nextroomdoor _nextroomarrow _nextroomdirection) (break `/Game/TSS_Game/Blueprints/LevelDesign/ModularRooms/ST_ProcDoors_Pure` _array_element))
    (bind _asbp_activatable_base (cast `/Game/TSS_Game/Blueprints/LevelDesign/BP_Activatable_Base` (`ChildActorComponent.ChildActor` _nextroomdoor)))
    (`KismetArrayLibrary.Array_AddUnique` (`self.PossibleWays`) (make `/Game/TSS_Game/Blueprints/LevelDesign/ModularRooms/ST_ProcDoors` _asbp_activatable_base _nextroomarrow null _array_index _nextroomdirection)))
  (set `self.AmmoCrates` AmmoCrates)
  (set `self.Skulls` Skulls)
  (set `self.EnemySpawners_Eternal` EnemySpawners)
  (set `self.EnemiesPreSpawners` EnemiesPreSpawners)
  (set `self.Boss Spawners` BossSpawners)
  (return true))

(fn `Remote Generate Room Assets`
  (returns (`Success?` :type Boolean))
  (for _array_element (`self.Components to Replace`)
    (bind (_roomcomponent _newactor) (break `/Game/TSS_Game/Blueprints/LevelDesign/ModularRooms/ST_RoomComponentsReplacer` _array_element))
    (if (`KismetSystemLibrary.IsValidClass` _newactor)
      (bind _output (`|GetArrayItem` (`self.ChildActorReplacables`) _roomcomponent))
      (bind (_returnvalue_location _returnvalue_rotation) (`KismetMathLibrary.BreakTransform` (`SceneComponent.K2_GetComponentToWorld` _output)))
      (bind _returnvalue (`|SpawnActorFromClass` _newactor (`KismetMathLibrary.MakeTransform` _returnvalue_location _returnvalue_rotation) "AlwaysSpawn" "MultiplyWithRoot" null null))
      (bind _asbp_spawner_wall_tube_large_base (cast `/Game/TSS_Game/Blueprints/LevelDesign/ModularRooms/BP_SpawnerWallTube_LargeBase` _returnvalue)
        (:`then`
          (set `/Game/TSS_Game/Blueprints/LevelDesign/ModularRooms/BP_SpawnerWallTube_LargeBase.ParentRoom` self _asbp_spawner_wall_tube_large_base))
        (:`CastFailed`
          _)))
    (`ActorComponent.K2_DestroyComponent` _output))
  (for _array_element_2 (`self.Meshes to Replace`)
    (bind (_roomcomponent_2 _newactor_2) (break `/Game/TSS_Game/Blueprints/LevelDesign/ModularRooms/ST_RoomMeshesReplacer` _array_element_2))
    (if (`KismetSystemLibrary.IsValidClass` _newactor_2)
      (bind _output_2 (`|GetArrayItem` (`self.StaticMeshesReplacables`) _roomcomponent_2))
      (bind (_returnvalue_location_2 _returnvalue_rotation_2) (`KismetMathLibrary.BreakTransform` (`SceneComponent.K2_GetComponentToWorld` _output_2)))
      (bind _returnvalue_2 (`|SpawnActorFromClass` _newactor_2 (`KismetMathLibrary.MakeTransform` _returnvalue_location_2 _returnvalue_rotation_2) "AlwaysSpawn" "MultiplyWithRoot" null null))
      (bind _asbp_spawner_wall_tube_large_base_2 (cast `/Game/TSS_Game/Blueprints/LevelDesign/ModularRooms/BP_SpawnerWallTube_LargeBase` _returnvalue_2)
        (:`then`
          (set `/Game/TSS_Game/Blueprints/LevelDesign/ModularRooms/BP_SpawnerWallTube_LargeBase.ParentRoom` self _asbp_spawner_wall_tube_large_base_2))
        (:`CastFailed`
          _)))
    (`ActorComponent.K2_DestroyComponent` _output_2))
  (return true))

(fn `RemoteSetNextRoom`
  (params (`Exit Way Next Room` :type "/Game/TSS_Game/Blueprints/LevelDesign/ModularRooms/BP_ProcRoom_Base Object Reference"))
  (returns (`Success?` :type Boolean))
  (bind _exitdoorindex (`self.ExitDoorIndex`))
  (bind (_nextroomdoor _nextroomarrow _nextroom _nextroomdoorindex _nextroomdirection) (break `/Game/TSS_Game/Blueprints/LevelDesign/ModularRooms/ST_ProcDoors` (`|GetArrayItem` (`self.PossibleWays`) _exitdoorindex)))
  (set `self.ExitWay` (make `/Game/TSS_Game/Blueprints/LevelDesign/ModularRooms/ST_ProcDoors` _nextroomdoor _nextroomarrow `Exit Way Next Room` _exitdoorindex _nextroomdirection))
  (return true))

(fn `SV Generate New Room`
  (params (RoomClass :type "Actor Class Reference"))
  (returns (SpawnedRoom :type "/Game/TSS_Game/Blueprints/LevelDesign/ModularRooms/BP_ProcRoom_Base Object Reference"))
  (bind (_exitway_nextroomdoor _exitway_nextroomarrow) (break `/Game/TSS_Game/Blueprints/LevelDesign/ModularRooms/ST_ProcDoors` (`self.ExitWay`)))
  (bind (_exitway_nextroomdoor_2 _exitway_nextroomarrow_2 _exitway_nextroom _exitway_nextroomdoorindex _exitway_nextroomdirection) (break `/Game/TSS_Game/Blueprints/LevelDesign/ModularRooms/ST_ProcDoors` (`self.ExitWay`)))
  (bind _returnvalue (`|SpawnActorFromClass` RoomClass (`KismetMathLibrary.MakeTransform` (`SceneComponent.K2_GetComponentLocation` _exitway_nextroomarrow) (`SceneComponent.K2_GetComponentRotation` _exitway_nextroomarrow)) "AlwaysSpawn" "MultiplyWithRoot" null null))
  (bind _asbp_proc_room_base (cast `/Game/TSS_Game/Blueprints/LevelDesign/ModularRooms/BP_ProcRoom_Base` _returnvalue))
  (set `self.ExitWay` (make `/Game/TSS_Game/Blueprints/LevelDesign/ModularRooms/ST_ProcDoors` _exitway_nextroomdoor_2 _exitway_nextroomarrow_2 _asbp_proc_room_base _exitway_nextroomdoorindex _exitway_nextroomdirection))
  (return _asbp_proc_room_base))

(fn `SV Generate Room Assets`
  (returns (`Success?` :type Boolean))
  (bind (_nextroomdoor _nextroomarrow _nextroom _nextroomdoorindex _nextroomdirection) (break `/Game/TSS_Game/Blueprints/LevelDesign/ModularRooms/ST_ProcDoors` (`KismetArrayLibrary.Array_Random` (`self.PossibleWays`))))
  (for _array_element (`self.ActorReplacableVariants`)
    (bind (_actorcomponent _chancetobereplaced _replacablevariants) (break `/Game/TSS_Game/Blueprints/LevelDesign/ModularRooms/ST_RoomCompVariants` _array_element))
    (`self.CalculateChance` _chancetobereplaced
      (:`Success`
        (`self.SV Replace Child Actor BP` _actorcomponent (`KismetArrayLibrary.Array_Random` _replacablevariants) 100.0))))
  (for _array_element_2 (`self.MeshReplacableVariants`)
    (bind (_actorcomponent_2 _chancetobereplaced_2 _replacablevariants_2) (break `/Game/TSS_Game/Blueprints/LevelDesign/ModularRooms/ST_RoomMeshVariants` _array_element_2))
    (`self.CalculateChance` _chancetobereplaced_2
      (:`Success`
        (`self.SV Replace Meshes` _actorcomponent_2 (`KismetArrayLibrary.Array_Random` _replacablevariants_2) 100.0))))
  (`|ExecutionSequence`
    (:`then_0`
      (`/Engine/EditorBlueprintResources/StandardMacros.IsValid` _nextroomdoor
        (:`Is Valid`
          (set `self.ExitWay` (make `/Game/TSS_Game/Blueprints/LevelDesign/ModularRooms/ST_ProcDoors` _nextroomdoor _nextroomarrow null _nextroomdoorindex _nextroomdirection))
          (if (`KismetSystemLibrary.IsServer`)
            (bind _asbp_game_mode_base (cast `/Game/TSS_Game/Blueprints/System/BP_GameModeBase` (`GameplayStatics.GetGameMode`)))
            (bind _output_get (set `self.As BP Game Mode Base` _asbp_game_mode_base))
            (bind (_success_ _out_row) (`/Game/TSS_Game/Blueprints/System/BP_GameModeBase.Get wave table` _output_get (`self.RoomIndex`)))
            (set `self.WaveList` _out_row)))))
    (:`then_1`
      (if (`KismetArrayLibrary.Array_IsNotEmpty` (`self.AmmoCrates`))
        (`self.SV SpawnRandomAmmoCrates` true))
      (if (`KismetArrayLibrary.Array_IsNotEmpty` (`self.Skulls`))
        (`self.SV SpawnRandomSkulls` true 5.0))
      (return true))))

(fn `SV Replace Child Actor BP`
  (params (ChildToReplace :type "ChildActorComponent Object Reference (by ref)") (NewBlueprint :type "Actor Class Reference") (ChanceToReplace :type "Float (double-precision)"))
  (returns (`Success?` :type Boolean))
  (bind (_returnvalue_location _returnvalue_rotation) (`KismetMathLibrary.BreakTransform` (`SceneComponent.K2_GetComponentToWorld` ChildToReplace)))
  (`/Engine/EditorBlueprintResources/StandardMacros.IsValid` ChildToReplace
    (:`Is Valid`
      (if (`KismetSystemLibrary.IsValidClass` NewBlueprint)
        (`self.CalculateChance` ChanceToReplace
          (:`Success`
            (bind _returnvalue (`|SpawnActorFromClass` NewBlueprint (`KismetMathLibrary.MakeTransform` _returnvalue_location _returnvalue_rotation) "AlwaysSpawn" "MultiplyWithRoot" null null))
            (bind _asbp_spawner_wall_tube_large_base (cast `/Game/TSS_Game/Blueprints/LevelDesign/ModularRooms/BP_SpawnerWallTube_LargeBase` _returnvalue)
              (:`then`
                (set `/Game/TSS_Game/Blueprints/LevelDesign/ModularRooms/BP_SpawnerWallTube_LargeBase.ParentRoom` self _asbp_spawner_wall_tube_large_base))
              (:`CastFailed`
                _))
            (`KismetArrayLibrary.Array_AddUnique` (`self.Components to Replace`) (make `/Game/TSS_Game/Blueprints/LevelDesign/ModularRooms/ST_RoomComponentsReplacer` (`KismetArrayLibrary.Array_Find` (`self.ChildActorReplacables`) ChildToReplace) NewBlueprint))
            (`ActorComponent.K2_DestroyComponent` ChildToReplace :!label _label)
            (return true))
          (:`Fail`
            _))
        (else
          (goto _label))))
    (:`Is Not Valid`
      _))
  (return false))

(fn `SV Replace Meshes`
  (params (MeshToReplace :type "StaticMeshComponent Object Reference (by ref)") (NewActor :type "Actor Class Reference") (Chance :type "Float (double-precision)") (`ShouldHide?` :type Boolean))
  (returns (`Success?` :type Boolean))
  (bind (_returnvalue_location _returnvalue_rotation) (`KismetMathLibrary.BreakTransform` (`SceneComponent.K2_GetComponentToWorld` MeshToReplace)))
  (`/Engine/EditorBlueprintResources/StandardMacros.IsValid` MeshToReplace
    (:`Is Valid`
      (if (`KismetSystemLibrary.IsValidClass` NewActor)
        (`self.CalculateChance` Chance
          (:`Success`
            (bind _returnvalue (`|SpawnActorFromClass` NewActor (`KismetMathLibrary.MakeTransform` _returnvalue_location _returnvalue_rotation) "AlwaysSpawn" "MultiplyWithRoot" null null))
            (bind _asbp_spawner_wall_tube_large_base (cast `/Game/TSS_Game/Blueprints/LevelDesign/ModularRooms/BP_SpawnerWallTube_LargeBase` _returnvalue)
              (:`then`
                (set `/Game/TSS_Game/Blueprints/LevelDesign/ModularRooms/BP_SpawnerWallTube_LargeBase.ParentRoom` self _asbp_spawner_wall_tube_large_base))
              (:`CastFailed`
                _))
            (`KismetArrayLibrary.Array_AddUnique` (`self.Meshes to Replace`) (make `/Game/TSS_Game/Blueprints/LevelDesign/ModularRooms/ST_RoomMeshesReplacer` (`KismetArrayLibrary.Array_Find` (`self.StaticMeshesReplacables`) MeshToReplace) NewActor))
            (`ActorComponent.K2_DestroyComponent` MeshToReplace :!label _label)
            (return true))
          (:`Fail`
            _))
        (else
          (goto _label))))
    (:`Is Not Valid`
      _))
  (return false))

(fn `SV SpawnRandomAmmoCrates`
  (params (`IsNotFixedSpawn?` :type Boolean :default true) (`Chance to spawn` :type "Float (double-precision)" :default 20.0) (FixedItemsSpawned :type Integer))
  (returns (`Success?` :type Boolean))
  (locals (TEMPAmmoCrates :type "Array of StaticMeshComponent Object Reference"))
  (bind _outitem (`KismetArrayLibrary.Array_Random` (`local.TEMPAmmoCrates`)))
  (if `IsNotFixedSpawn?`
    (for _array_element (`self.AmmoCrates`)
      (if (>= `Chance to spawn` (`KismetMathLibrary.RandomIntegerInRange` 1 100))
        (`|SpawnActorFromClass` "/Game/TSS_Game/Blueprints/Pickup/BP_AmmoCrate.BP_AmmoCrate_C" (`SceneComponent.K2_GetComponentToWorld` _array_element) "Undefined" "MultiplyWithRoot" null null)))
    (else
      (bind _output_get (set `local.TEMPAmmoCrates` (`self.AmmoCrates`)))
      (for _ (range 1 (+ FixedItemsSpawned 1))
        (`|SpawnActorFromClass` "/Game/TSS_Game/Blueprints/Pickup/BP_AmmoCrate.BP_AmmoCrate_C" (`SceneComponent.K2_GetComponentToWorld` _outitem) "Undefined" "MultiplyWithRoot" null null)
        (`KismetArrayLibrary.Array_RemoveItem` _output_get _outitem))))
  (return true))

(fn `SV SpawnRandomSkulls`
  (params (`IsNotFixedSpawn?` :type Boolean :default true) (`Chance to spawn` :type "Float (double-precision)" :default 10.0) (FixedItemsSpawned :type Integer))
  (returns (`Success?` :type Boolean))
  (locals (TEMPSkulls :type "Array of StaticMeshComponent Object Reference"))
  (bind _outitem (`KismetArrayLibrary.Array_Random` (`local.TEMPSkulls`)))
  (if `IsNotFixedSpawn?`
    (for _array_element (`self.Skulls`)
      (if (>= `Chance to spawn` (`KismetMathLibrary.RandomIntegerInRange` 1 100))
        (bind _returnvalue (`|SpawnActorFromClass` "/Game/TSS_Game/Blueprints/LevelDesign/Spawners/BP_Spawn_ServoSkull01.BP_Spawn_ServoSkull01_C" (`SceneComponent.K2_GetComponentToWorld` _array_element) "Undefined" "MultiplyWithRoot" null null))
        (`/Game/TSS_Game/Blueprints/LevelDesign/Spawners/BP_Spawn_ServoSkull01.SpawnItem` _returnvalue)))
    (else
      (bind _output_get (set `local.TEMPSkulls` (`self.Skulls`)))
      (for _ (range 1 (+ FixedItemsSpawned 1))
        (bind _returnvalue_2 (`|SpawnActorFromClass` "/Game/TSS_Game/Blueprints/LevelDesign/Spawners/BP_Spawn_ServoSkull01.BP_Spawn_ServoSkull01_C" (`SceneComponent.K2_GetComponentToWorld` _outitem) "Undefined" "MultiplyWithRoot" null null))
        (`/Game/TSS_Game/Blueprints/LevelDesign/Spawners/BP_Spawn_ServoSkull01.SpawnItem` _returnvalue_2)
        (`KismetArrayLibrary.Array_RemoveItem` _output_get _outitem))))
  (return true))

(fn `UserConstructionScript`
  (for _array_element (`self.AmmoCrates`)
    (`/Engine/EditorBlueprintResources/StandardMacros.IsValid` _array_element
      (:`Is Valid`
        (`SceneComponent.SetHiddenInGame` _array_element true false)
        (`PrimitiveComponent.SetCollisionEnabled` _array_element "NoCollision"))))
  (for _array_element_2 (`self.Skulls`)
    (`/Engine/EditorBlueprintResources/StandardMacros.IsValid` _array_element_2
      (:`Is Valid`
        (`SceneComponent.SetHiddenInGame` _array_element_2 true false)
        (`PrimitiveComponent.SetCollisionEnabled` _array_element_2 "NoCollision"))))
  (for _array_element_3 (`self.ActorReplacableVariants`)
    (bind (_actorcomponent _chancetobereplaced _replacablevariants _shouldhide_) (break `/Game/TSS_Game/Blueprints/LevelDesign/ModularRooms/ST_RoomCompVariants` _array_element_3))
    (`/Engine/EditorBlueprintResources/StandardMacros.IsValid` _actorcomponent
      (:`Is Valid`
        (`KismetArrayLibrary.Array_AddUnique` (`self.ChildActorReplacables`) _actorcomponent)
        (bind _asstatic_mesh_actor (cast `StaticMeshActor` (`ChildActorComponent.ChildActor` _actorcomponent))))))
  (for _array_element_4 (`self.MeshReplacableVariants`)
    (bind (_actorcomponent_2 _chancetobereplaced_2 _replacablevariants_2 _shouldhide__2) (break `/Game/TSS_Game/Blueprints/LevelDesign/ModularRooms/ST_RoomMeshVariants` _array_element_4))
    (`/Engine/EditorBlueprintResources/StandardMacros.IsValid` _actorcomponent_2
      (:`Is Valid`
        (`KismetArrayLibrary.Array_AddUnique` (`self.StaticMeshesReplacables`) _actorcomponent_2)
        (if _shouldhide__2
          (`KismetArrayLibrary.Array_AddUnique` (`self.StaticMeshesHidable`) _actorcomponent_2))))))