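; Side mission 03 modular room: a boss encounter built on a parent room Blueprint.
; The construction script registers replaceable variants, hidable actors, the exit door, pickups and boss spawner.
; When all living characters overlap EnemiesActivator, the server requests activation, which enables blockers and spawners, spawns the boss and polls its death by timer.
; Boss death sets the win condition and stops spawners; the win event runs alert lights and an achievement check.
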(event `self.ReceiveBeginPlay`
  (for _array_element (`|MakeArray` (`self.BP_PlayerBlockerBox_C_4079`) (`self.BP_PlayerBlockerBox_C_4080`))
    (bind _asbp_player_blocker_box (cast `/Game/TSS_Game/Blueprints/LevelDesign/BP_PlayerBlockerBox` (`ChildActorComponent.ChildActor` _array_element)))
    (`PrimitiveComponent.SetCollisionEnabled` (`/Game/TSS_Game/Blueprints/LevelDesign/BP_PlayerBlockerBox.Cube` _asbp_player_blocker_box) "NoCollision"))
  (for _array_element_2 (`self.StaticMeshesHidable`)
    (`PrimitiveComponent.SetCustomPrimitiveDataFloat` _array_element_2 0 1.0))
  (`parent.ReceiveBeginPlay`))

(event `CheckBossDeadTimer`
  (bind _roomboss (`self.RoomBoss`))
  (`/Engine/EditorBlueprintResources/StandardMacros.IsValid` _roomboss
    (:`Is Valid`
      (if (`/Game/TSS_Game/Blueprints/Bonus/AI/BP_Enemy_BASE.isDead` _roomboss)
        (set `self.WinCondition` "NewEnumerator0" :!label _label)
        (`self.DisableRoomEnemySpawners`)
        (`KismetSystemLibrary.K2_PauseTimer` null "CheckBossDeadTimer")))
    (:`Is Not Valid`
      (goto _label))))

(event `self.RoomIsActivated`
  (for _array_element (`|MakeArray` (`self.BP_PlayerBlockerBox_C_4079`) (`self.BP_PlayerBlockerBox_C_4080`))
    (bind _asbp_player_blocker_box (cast `/Game/TSS_Game/Blueprints/LevelDesign/BP_PlayerBlockerBox` (`ChildActorComponent.ChildActor` _array_element)))
    (`PrimitiveComponent.SetCollisionEnabled` (`/Game/TSS_Game/Blueprints/LevelDesign/BP_PlayerBlockerBox.Cube` _asbp_player_blocker_box) "QueryAndPhysics"))
  (set `PrimitiveComponent.bGenerateOverlapEvents` false (`self.EnemiesActivator`))
  (set `self.IsRoomActivated?` true)
  (`self.EnableRoomEnemySpawners`)
  (if (`KismetSystemLibrary.IsServer`)
    (`self.SV_SpawnBoss`)
    (`KismetSystemLibrary.K2_SetTimerDelegate` (delegate `CheckBossDeadTimer`) 2.0 true)))

(event `self.DisableRoomEnemySpawners`
  (`parent.DisableRoomEnemySpawners`))

(event `self.EnemiesActivator.OnComponentBeginOverlap`
  (params (OverlappedComponent :type "PrimitiveComponent Object Reference") (OtherActor :type "Actor Object Reference") (OtherComp :type "PrimitiveComponent Object Reference") (OtherBodyIndex :type Integer) (bFromSweep :type Boolean) (SweepResult :type "HitResult Structure (by ref)"))
  (bind _as_bp_game_mode_base (`self.As BP Game Mode Base`))
  (bind _asbp_character_base (cast `/Game/TSS_Game/Blueprints/System/BP_CharacterBase` OtherActor))
  (if (`Pawn.IsLocallyControlled` _asbp_character_base)
    (`self.SendStartDialog`)
    (`/Game/TSS_Game/Blueprints/System/BP_CharacterBase.Speech_Say` _asbp_character_base "NewEnumerator5" false 30.0))
  (if (`KismetSystemLibrary.IsServer`)
    (`KismetArrayLibrary.Array_Clear` (`self.CharactersInZone`))
    (`KismetArrayLibrary.Array_Clear` (`self.CharactersAlive_0`))
    (`/Engine/EditorBlueprintResources/StandardMacros.IsValid` _as_bp_game_mode_base
      (:`Is Valid`
        (for _array_element (`/Game/TSS_Game/Blueprints/System/BP_GameModeBase.AllCharacters` _as_bp_game_mode_base)
          (if (not (`/Game/TSS_Game/Blueprints/System/BP_CharacterBase.IsDead` _array_element))
            (`KismetArrayLibrary.Array_Add` (`self.CharactersAlive_0`) _array_element)))
        (for _array_element_2 (`PrimitiveComponent.GetOverlappingActors` (`self.EnemiesActivator`) "/Game/TSS_Game/Blueprints/System/BP_CharacterBase.BP_CharacterBase_C")
          (bind _asbp_character_base_2 (cast `/Game/TSS_Game/Blueprints/System/BP_CharacterBase` _array_element_2))
          (`KismetArrayLibrary.Array_Add` (`self.CharactersInZone`) _asbp_character_base_2))
        (if (== (`KismetArrayLibrary.Array_Length` (`self.CharactersInZone`)) (`KismetArrayLibrary.Array_Length` (`self.CharactersAlive_0`)))
          (bind _asbp_player_controller (cast `/Game/TSS_Game/Blueprints/System/BP_PlayerController` (`GameplayStatics.GetPlayerController` 0)))
          (`/Game/TSS_Game/Blueprints/System/BP_PlayerController.SV_RoomManualActivation` _asbp_player_controller (`self.RoomIndex`))))
      (:`Is Not Valid`
        (`KismetSystemLibrary.PrintString` "BP_Room_Side_Mission_01: ERROR! Failed to cast to game mode base!!!" true true (struct :`R` 1.0 :`A` 1.0) 5.0)))))

(event `self.MC_WinConditionReached`
  (bind _array (`|MakeArray` (`self.BP_ACT_AlertLights`) (`self.BP_ACT_AlertLights1`)))
  (for _array_element _array
    (bind _asbp_activatable_base (cast `/Game/TSS_Game/Blueprints/LevelDesign/BP_Activatable_Base` (`ChildActorComponent.ChildActor` _array_element)))
    (`/Game/TSS_Game/Blueprints/LevelDesign/BP_Activatable_Base.MC_Activate` _asbp_activatable_base))
  (`self.SpecialMissionAchievementChecker` "UnderHisGaze")
  (`KismetSystemLibrary.Delay` 6.0)
  (`parent.MC_WinConditionReached`)
  (`KismetSystemLibrary.Delay` 6.0)
  (for _array_element_2 _array
    (bind _asbp_activatable_base_2 (cast `/Game/TSS_Game/Blueprints/LevelDesign/BP_Activatable_Base` (`ChildActorComponent.ChildActor` _array_element_2)))
    (`/Game/TSS_Game/Blueprints/LevelDesign/BP_Activatable_Base.MC_Deactivate` _asbp_activatable_base_2)))

(fn `UserConstructionScript`
  (bind _defaultdecorations (`self.DefaultDecorations`))
  (bind _mesheschancetoreplace (`self.MeshesChanceToReplace`))
  (`self.InitRoomActors` :`IsServer?` true :`ActorReplacableVariants` (`|MakeArray` (make `/Game/TSS_Game/Blueprints/LevelDesign/ModularRooms/ST_RoomCompVariants` (`self.StaticMeshActor_723068`) 90.0 (`|MakeArray` "/Game/TSS_Game/Blueprints/LevelDesign/ModularRooms/BP_SpawnerWallTube_Large_01.BP_SpawnerWallTube_Large_01_C" "/Game/TSS_Game/Blueprints/LevelDesign/ModularRooms/BP_SpawnerWallTube_Large_02.BP_SpawnerWallTube_Large_02_C" "/Game/TSS_Game/Blueprints/LevelDesign/ModularRooms/BP_SpawnerWallTube_Large_03.BP_SpawnerWallTube_Large_03_C" :!type "Actor Class Reference"))) :`MeshReplacableVariants` (`|MakeArray` (make `/Game/TSS_Game/Blueprints/LevelDesign/ModularRooms/ST_RoomMeshVariants` (`self.DecorFloor2`) _mesheschancetoreplace _defaultdecorations) (make `/Game/TSS_Game/Blueprints/LevelDesign/ModularRooms/ST_RoomMeshVariants` (`self.DecorFloor3`) _mesheschancetoreplace _defaultdecorations) (make `/Game/TSS_Game/Blueprints/LevelDesign/ModularRooms/ST_RoomMeshVariants` (`self.DecorFloor1`) _mesheschancetoreplace _defaultdecorations) (make `/Game/TSS_Game/Blueprints/LevelDesign/ModularRooms/ST_RoomMeshVariants` (`self.DecorFloor4`) _mesheschancetoreplace _defaultdecorations) (make `/Game/TSS_Game/Blueprints/LevelDesign/ModularRooms/ST_RoomMeshVariants` (`self.DecorFloor5`) _mesheschancetoreplace _defaultdecorations) (make `/Game/TSS_Game/Blueprints/LevelDesign/ModularRooms/ST_RoomMeshVariants` (`self.DecorFloor6`) _mesheschancetoreplace _defaultdecorations)) :`ActorsHidable` (`|MakeArray` (`self.StaticMeshActor_723039`) (`self.StaticMeshActor_723086`) (`self.StaticMeshActor_723111`) (`self.StaticMeshActor_723116`) (`self.StaticMeshActor_723087`) (`self.StaticMeshActor_723096`) (`self.StaticMeshActor_723089`) (`self.StaticMeshActor_723093`) (`self.StaticMeshActor_723085`) (`self.StaticMeshActor_723041`) (`self.StaticMeshActor_723045`) (`self.StaticMeshActor_723047`) (`self.StaticMeshActor_723042`) (`self.StaticMeshActor_723044`) (`self.StaticMeshActor_723038`) (`self.StaticMeshActor_723036`) (`self.StaticMeshActor_723088`) (`self.StaticMeshActor_723126`) (`self.StaticMeshActor_723110`) (`self.StaticMeshActor_722991`) (`self.StaticMeshActor_723072`) (`self.StaticMeshActor_723071`) (`self.StaticMeshActor_722988`) (`self.StaticMeshActor_723009`)) :`ActorsHidable_NextRoom` (`|MakeArray` (`self.StaticMeshActor_723090`) (`self.StaticMeshActor_723048`) (`self.StaticMeshActor_723050`)) :`PossibleWays` (`|MakeArray` (make `/Game/TSS_Game/Blueprints/LevelDesign/ModularRooms/ST_ProcDoors_Pure` (`self.BP_ACT_BlastDoor_SingleLarge_C_4869`) (`self.NextRoomArrow`) "NewEnumerator1")) :`AmmoCrates` (`|MakeArray` (`self.Ammo3`) (`self.Ammo1`) (`self.Ammo2`) (`self.Ammo9`) (`self.Ammo7`) (`self.Ammo6`) (`self.Ammo5`) (`self.Ammo8`) (`self.Ammo4`) (`self.Ammo11`) (`self.Ammo12`) (`self.Ammo10`)) :`Skulls` (`|MakeArray` (`self.Skulls3`) (`self.Skulls2`) (`self.Skulls4`) (`self.Skulls1`)) :`BossSpawners` (`|MakeArray` (`self.BossSpawner_1`)))
  (`parent.UserConstructionScript`))