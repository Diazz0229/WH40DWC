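; Corner room module for modular, procedurally linked levels, set up entirely in its Construction Script.
; It passes its placed components to InitRoomActors: wall pieces and floor decor with chance-based replacement variants, plus two lists of hidable pieces.
; The same call registers two exit doors with arrows and directions for next rooms, along with ammo crates, skulls and enemy pre-spawners, before running the parent construction script.
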(fn `UserConstructionScript`
  (bind _defaultdecorations (`self.DefaultDecorations`))
  (bind _defaultwallspawners (`self.DefaultWallSpawners`))
  (bind _actorschancetoreplace (`self.ActorsChanceToReplace`))
  (bind _mesheschancetoreplace (`self.MeshesChanceToReplace`))
  (`self.InitRoomActors` :`IsServer?` true :`ActorReplacableVariants` (`|MakeArray` (make `/Game/TSS_Game/Blueprints/LevelDesign/ModularRooms/ST_RoomCompVariants` (`self.StaticMeshActor_20774`) _actorschancetoreplace _defaultwallspawners) (make `/Game/TSS_Game/Blueprints/LevelDesign/ModularRooms/ST_RoomCompVariants` (`self.StaticMeshActor_20775`) _actorschancetoreplace _defaultwallspawners) (make `/Game/TSS_Game/Blueprints/LevelDesign/ModularRooms/ST_RoomCompVariants` (`self.StaticMeshActor_20750`) _actorschancetoreplace _defaultwallspawners) (make `/Game/TSS_Game/Blueprints/LevelDesign/ModularRooms/ST_RoomCompVariants` (`self.StaticMeshActor_20751`) _actorschancetoreplace _defaultwallspawners) (make `/Game/TSS_Game/Blueprints/LevelDesign/ModularRooms/ST_RoomCompVariants` (`self.StaticMeshActor_20752`) _actorschancetoreplace _defaultwallspawners)) :`MeshReplacableVariants` (`|MakeArray` (make `/Game/TSS_Game/Blueprints/LevelDesign/ModularRooms/ST_RoomMeshVariants` (`self.DecorFloor2`) _mesheschancetoreplace _defaultdecorations) (make `/Game/TSS_Game/Blueprints/LevelDesign/ModularRooms/ST_RoomMeshVariants` (`self.DecorFloor3`) _mesheschancetoreplace _defaultdecorations) (make `/Game/TSS_Game/Blueprints/LevelDesign/ModularRooms/ST_RoomMeshVariants` (`self.DecorFloor7`) _mesheschancetoreplace _defaultdecorations) (make `/Game/TSS_Game/Blueprints/LevelDesign/ModularRooms/ST_RoomMeshVariants` (`self.DecorFloor1`) _mesheschancetoreplace _defaultdecorations) (make `/Game/TSS_Game/Blueprints/LevelDesign/ModularRooms/ST_RoomMeshVariants` (`self.DecorFloor4`) _mesheschancetoreplace _defaultdecorations) (make `/Game/TSS_Game/Blueprints/LevelDesign/ModularRooms/ST_RoomMeshVariants` (`self.DecorFloor5`) _mesheschancetoreplace _defaultdecorations) (make `/Game/TSS_Game/Blueprints/LevelDesign/ModularRooms/ST_RoomMeshVariants` (`self.DecorFloor6`) _mesheschancetoreplace _defaultdecorations) (make `/Game/TSS_Game/Blueprints/LevelDesign/ModularRooms/ST_RoomMeshVariants` (`self.DecorFloor9`) _mesheschancetoreplace _defaultdecorations) (make `/Game/TSS_Game/Blueprints/LevelDesign/ModularRooms/ST_RoomMeshVariants` (`self.DecorFloor10`) _mesheschancetoreplace _defaultdecorations) (make `/Game/TSS_Game/Blueprints/LevelDesign/ModularRooms/ST_RoomMeshVariants` (`self.DecorFloor11`) _mesheschancetoreplace _defaultdecorations) (make `/Game/TSS_Game/Blueprints/LevelDesign/ModularRooms/ST_RoomMeshVariants` (`self.DecorFloor8`) _mesheschancetoreplace _defaultdecorations)) :`ActorsHidable` (`|MakeArray` (`self.StaticMeshActor_20777`) (`self.StaticMeshActor_20776`) (`self.StaticMeshActor_20779`) (`self.StaticMeshActor_20778`)) :`ActorsHidable_NextRoom` (`|MakeArray` (`self.StaticMeshActor_20767`) (`self.StaticMeshActor_20766`) (`self.StaticMeshActor_20756`) (`self.StaticMeshActor_20757`) (`self.StaticMeshActor_20764`)) :`PossibleWays` (`|MakeArray` (make `/Game/TSS_Game/Blueprints/LevelDesign/ModularRooms/ST_ProcDoors_Pure` (`self.BP_ACT_BlastDoor_SingleLarge_C_5`) (`self.NextRoomArrow`)) (make `/Game/TSS_Game/Blueprints/LevelDesign/ModularRooms/ST_ProcDoors_Pure` (`self.BP_ACT_BlastDoor_SingleLarge_C_10`) (`self.NextRoomArrow2`) "NewEnumerator1")) :`AmmoCrates` (`|MakeArray` (`self.Ammo2`) (`self.Ammo3`) (`self.Ammo1`)) :`Skulls` (`|MakeArray` (`self.Skulls1`) (`self.Skulls3`) (`self.Skulls4`) (`self.Skulls5`) (`self.Skulls2`)) :`EnemiesPreSpawners` (`|MakeArray` (`self.EnemyPreSpawner_4`) (`self.EnemyPreSpawner_3`) (`self.EnemyPreSpawner_2`) (`self.EnemyPreSpawner_6`) (`self.EnemyPreSpawner_1`) (`self.EnemyPreSpawner_5`)))
  (`parent.UserConstructionScript`))