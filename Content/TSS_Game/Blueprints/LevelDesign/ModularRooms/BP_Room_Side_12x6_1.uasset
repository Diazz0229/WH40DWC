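; A 12x6 side-room module, variant 1, for modular level building with a single possible exit to a next room.
; Its construction script registers the room's placed parts through InitRoomActors before calling the parent script, and the event graph holds no active logic.
; Walls, floor tiles, decorations and decals get replacement chances and default variant pools.
; Hidable actors, the exit door and arrow, ammo crates, skulls, enemy spawners and prespawners are also passed in.
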(fn `UserConstructionScript`
  (bind _defaultdecorations (`self.DefaultDecorations`))
  (bind _defaultdecals (`self.DefaultDecals`))
  (bind _mesheschancetoreplace (`self.MeshesChanceToReplace`))
  (bind _decalchancetoreplace (`self.DecalChanceToReplace`))
  (bind _defaultfloortiles (`self.DefaultFloorTiles`))
  (bind _mesheschancetoreplace_2 (`self.MeshesChanceToReplace`))
  (`self.InitRoomActors` true (`|MakeArray` (make `/Game/TSS_Game/Blueprints/LevelDesign/ModularRooms/ST_RoomCompVariants` (`self.StaticMeshActor_376652`) (`self.ActorsChanceToReplace`) (`self.DefaultWallSpawners`)) (make `/Game/TSS_Game/Blueprints/LevelDesign/ModularRooms/ST_RoomCompVariants` (`self.StaticMeshActor_376539`) _mesheschancetoreplace _defaultfloortiles) (make `/Game/TSS_Game/Blueprints/LevelDesign/ModularRooms/ST_RoomCompVariants` (`self.StaticMeshActor_376544`) _mesheschancetoreplace _defaultfloortiles)) (`|MakeArray` (make `/Game/TSS_Game/Blueprints/LevelDesign/ModularRooms/ST_RoomMeshVariants` (`self.DecorFloor2`) _mesheschancetoreplace_2 _defaultdecorations) (make `/Game/TSS_Game/Blueprints/LevelDesign/ModularRooms/ST_RoomMeshVariants` (`self.DecorFloor3`) _mesheschancetoreplace_2 _defaultdecorations) (make `/Game/TSS_Game/Blueprints/LevelDesign/ModularRooms/ST_RoomMeshVariants` (`self.DecorFloor1`) _mesheschancetoreplace_2 _defaultdecorations) (make `/Game/TSS_Game/Blueprints/LevelDesign/ModularRooms/ST_RoomMeshVariants` (`self.DecorFloor4`) _mesheschancetoreplace_2 _defaultdecorations) (make `/Game/TSS_Game/Blueprints/LevelDesign/ModularRooms/ST_RoomMeshVariants` (`self.DecorFloor5`) _mesheschancetoreplace_2 _defaultdecorations) (make `/Game/TSS_Game/Blueprints/LevelDesign/ModularRooms/ST_RoomMeshVariants` (`self.Decal_2`) _decalchancetoreplace _defaultdecals) (make `/Game/TSS_Game/Blueprints/LevelDesign/ModularRooms/ST_RoomMeshVariants` (`self.Decal_1`) _decalchancetoreplace _defaultdecals) (make `/Game/TSS_Game/Blueprints/LevelDesign/ModularRooms/ST_RoomMeshVariants` (`self.Decal_4`) _decalchancetoreplace _defaultdecals) (make `/Game/TSS_Game/Blueprints/LevelDesign/ModularRooms/ST_RoomMeshVariants` (`self.Decal_5`) _decalchancetoreplace _defaultdecals) (make `/Game/TSS_Game/Blueprints/LevelDesign/ModularRooms/ST_RoomMeshVariants` (`self.Decal_3`) _decalchancetoreplace _defaultdecals) (make `/Game/TSS_Game/Blueprints/LevelDesign/ModularRooms/ST_RoomMeshVariants` (`self.Decal_6`) _decalchancetoreplace _defaultdecals)) (`|MakeArray` (`self.StaticMeshActor_376576`) (`self.StaticMeshActor_376644`) (`self.StaticMeshActor_376645`) (`self.StaticMeshActor_376646`) (`self.StaticMeshActor_376647`) (`self.StaticMeshActor_376586`) (`self.StaticMeshActor_376611`) (`self.StaticMeshActor_376718`)) (`|MakeArray` (`self.StaticMeshActor_376588`) (`self.StaticMeshActor_376587`) (`self.StaticMeshActor_376715`)) (`|MakeArray` (make `/Game/TSS_Game/Blueprints/LevelDesign/ModularRooms/ST_ProcDoors_Pure` (`self.BP_ACT_BlastDoor_SingleLarge_C_2245`) (`self.NextRoomArrow`) "NewEnumerator1")) (`|MakeArray` (`self.Ammo3`) (`self.Ammo1`) (`self.Ammo2`)) (`|MakeArray` (`self.Skulls3`) (`self.Skulls2`) (`self.Skulls4`) (`self.Skulls1`)) (`|MakeArray` (`self.EnemySpawner_1`) (`self.EnemySpawner_2`) (`self.EnemySpawner_3`)) (`|MakeArray` (`self.EnemyPreSpawner_2`) (`self.EnemyPreSpawner_4`) (`self.EnemyPreSpawner_5`) (`self.EnemyPreSpawner_1`) (`self.EnemyPreSpawner_6`) (`self.EnemyPreSpawner_3`)))
  (`parent.UserConstructionScript`))