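; BP_StreetLight_v1 is a level-design street light Blueprint with logic that tracks how many players overlap it.
; PlayerOverlapCalculation increments or decrements a counter on overlap begin or end, clamped between zero and the GameState PlayerArray size.
; It returns true when the count equals the number of players, meaning everyone is overlapping.
; The construction script is empty, and no overlap events or light changes appear in these graphs.
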(fn `PlayerOverlapCalculation`
  (params (BeginOverlap :type Boolean))
  (returns (AllPlayersPresent :type Boolean))
  (if BeginOverlap
    (bind _output_get (set `self.PlayerOverlap` (`KismetMathLibrary.Clamp` (+ (`self.PlayerOverlap`) 1) 0 (`KismetArrayLibrary.Array_Length` (`GameStateBase.PlayerArray` (`GameplayStatics.GetGameState`))))))
    (return (== _output_get (`KismetArrayLibrary.Array_Length` (`GameStateBase.PlayerArray` (`GameplayStatics.GetGameState`)))))
    (else
      (bind _output_get_2 (set `self.PlayerOverlap` (`KismetMathLibrary.Clamp` (- (`self.PlayerOverlap`) 1) 0 (`KismetArrayLibrary.Array_Length` (`GameStateBase.PlayerArray` (`GameplayStatics.GetGameState`))))))
      (return (== _output_get_2 (`KismetArrayLibrary.Array_Length` (`GameStateBase.PlayerArray` (`GameplayStatics.GetGameState`))))))))

(fn `UserConstructionScript`)