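; BP_Candles_light is a level lighting actor that makes two candle lights flicker.
; A self-restarting timer picks random intensity targets at random sub-second intervals, and Tick eases both lights toward the first target using DeltaSeconds as lerp alpha.
; The second target is generated but never read.
; PlayerOverlapCalculation keeps a clamped overlap count and reports whether it equals the player count, but nothing here calls it.
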(event `self.ReceiveBeginPlay`
  (`KismetSystemLibrary.K2_SetTimerDelegate` (delegate `FlameTimer`) 0.5))

(event `FlameTimer`
  (set `self.CandleIntensity1` (`KismetMathLibrary.RandomFloatInRange` 0.0 30000.0))
  (set `self.CandleIntensity2` (`KismetMathLibrary.RandomFloatInRange` 0.0 30000.0))
  (`KismetSystemLibrary.K2_SetTimerDelegate` (delegate `FlameTimer`) (`KismetMathLibrary.RandomFloatInRange` 0.05 0.5)))

(event `self.ReceiveTick`
  (params (DeltaSeconds :type "Float (single-precision)"))
  (bind _candlelight1 (`self.CandleLight1`))
  (bind _candlelight (`self.CandleLight`))
  (`LightComponent.SetIntensity` _candlelight1 (`KismetMathLibrary.Lerp` (`LightComponentBase.Intensity` _candlelight1) (`self.CandleIntensity1`) DeltaSeconds))
  (`LightComponent.SetIntensity` _candlelight (`KismetMathLibrary.Lerp` (`LightComponentBase.Intensity` _candlelight) (`self.CandleIntensity1`) DeltaSeconds)))

(fn `PlayerOverlapCalculation`
  (params (BeginOverlap :type Boolean))
  (returns (AllPlayersPresent :type Boolean))
  (if BeginOverlap
    (bind _output_get (set `self.PlayerOverlap` (`KismetMathLibrary.Clamp` (+ (`self.PlayerOverlap`) 1) 0 (`KismetArrayLibrary.Array_Length` (`GameStateBase.PlayerArray` (`GameplayStatics.GetGameState`))))))
    (return (== _output_get (`KismetArrayLibrary.Array_Length` (`GameStateBase.PlayerArray` (`GameplayStatics.GetGameState`)))))
    (else
      (bind _output_get_2 (set `self.PlayerOverlap` (`KismetMathLibrary.Clamp` (- (`self.PlayerOverlap`) 1) 0 (`KismetArrayLibrary.Array_Length` (`GameStateBase.PlayerArray` (`GameplayStatics.GetGameState`))))))
      (return (== _output_get_2 (`KismetArrayLibrary.Array_Length` (`GameStateBase.PlayerArray` (`GameplayStatics.GetGameState`))))))))

(fn `UserConstructionScript`)