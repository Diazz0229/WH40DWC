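; BP_MoveCameraUp is a level-design trigger that swings a BP_CharacterBase camera to a top view while the character overlaps it.
; On begin overlap, a timeline lerps the spring arm's relative rotation from the character's default to its top rotation.
; On end overlap, a second timeline blends back, and each plays from the start, so interrupted blends do not resume.
; Spring arm length lerps exist but are unconnected.
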(event `self.ReceiveBeginPlay`)

(event `self.ReceiveActorBeginOverlap`
  (params (OtherActor :type "Actor Object Reference"))
  (bind _asbp_character_base (cast `/Game/TSS_Game/Blueprints/System/BP_CharacterBase` OtherActor))
  (bind (_direction _alpha) (`Timeline|Timeline_Springarm` :!via `PlayFromStart`)
    (:`Update`
      (`SceneComponent.K2_SetRelativeRotation` (`/Game/TSS_Game/Blueprints/System/BP_CharacterBase.SpringArm` _asbp_character_base) (`KismetMathLibrary.RLerp` (`/Game/TSS_Game/Blueprints/System/BP_CharacterBase.CamSpringArmDefRotation` _asbp_character_base) (`/Game/TSS_Game/Blueprints/System/BP_CharacterBase.CamSpringArmTopRotation` _asbp_character_base) _alpha) false false))))

(event `self.ReceiveActorEndOverlap`
  (params (OtherActor :type "Actor Object Reference"))
  (bind _asbp_character_base (cast `/Game/TSS_Game/Blueprints/System/BP_CharacterBase` OtherActor))
  (bind (_direction _alpha) (`Timeline|Timeline_0` :!via `PlayFromStart`)
    (:`Update`
      (`SceneComponent.K2_SetRelativeRotation` (`/Game/TSS_Game/Blueprints/System/BP_CharacterBase.SpringArm` _asbp_character_base) (`KismetMathLibrary.RLerp` (`/Game/TSS_Game/Blueprints/System/BP_CharacterBase.CamSpringArmTopRotation` _asbp_character_base) (`/Game/TSS_Game/Blueprints/System/BP_CharacterBase.CamSpringArmDefRotation` _asbp_character_base) _alpha) false false))))

(fn `UserConstructionScript`)