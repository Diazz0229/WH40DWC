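; BP_NPC is an objective-system NPC that shows a name label and opens dialogue when the InteractwithWeapon event fires.
; The construction script writes NPCName to the TextRender, and Tick holds it at a fixed world rotation meant to face the camera.
; Interaction creates a new W_Dialogue widget filled with NPCText and adds it to the viewport.
; BeginPlay caches the singleplayer player character, though nothing shown uses it.
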(event `self.ReceiveBeginPlay`
  (bind _asbp_character_base_singleplayer (cast `/Game/TSS_Game/Blueprints/System/BP_CharacterBase_Singleplayer` (`GameplayStatics.GetPlayerCharacter` 0)))
  (set `self.PlayerCast` _asbp_character_base_singleplayer))

(event `/Game/TSS_Game/Blueprints/System/BPI_Interactive.InteractWithWeapon`
  (params (CharacterReference :type "/Game/TSS_Game/Blueprints/System/BP_CharacterBase Object Reference"))
  (bind _returnvalue (`|CreateWidget` "/Game/TSS_Game/Blueprints/Objective_System/NPC/W_Dialogue.W_Dialogue_C"))
  (`TextBlock.SetText` (`/Game/TSS_Game/Blueprints/Objective_System/NPC/W_Dialogue.NPC_Text` _returnvalue) (`self.NPC_Text`))
  (`UserWidget.AddToViewport` _returnvalue 0))

(event `self.ReceiveTick`
  (params (DeltaSeconds :type "Float (single-precision)"))
  (`SceneComponent.K2_SetWorldRotation` (`self.TextRender`) (struct :`Pitch` 45.0 :`Yaw` 180.0) false false) ; Rotates the text to face the camera
)

(fn `UserConstructionScript`
  (`TextRenderComponent.K2_SetText` (`self.TextRender`) (`self.NPC_Name`)))