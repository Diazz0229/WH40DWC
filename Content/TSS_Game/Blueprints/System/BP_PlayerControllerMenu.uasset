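; Player controller for the menu that opens the main menu, or a disclaimer screen on the first visit as tracked by the game instance's AlreadyPlayed flag.
; On BeginPlay it also switches existing crosshair cursor widgets to another switcher state.
; Separate events toggle shadow casting on sky, directional, point and rect light arrays supplied by the map Blueprint, with the init event disabling shadows at lowest shadow quality.
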(event `self.ReceiveBeginPlay`
  (if (`self.IsLocalPlayerController`)
    (bind _asbp_game_instance_with_settings (cast `/Game/TSS_Game/Blueprints/GameInstanceSettings/BP_GameInstanceWithSettings` (`GameplayStatics.GetGameInstance`))
      (:`then`
        (if (`/Game/TSS_Game/Blueprints/GameInstanceSettings/BP_GameInstanceWithSettings.AlreadyPlayed?` _asbp_game_instance_with_settings)
          (bind _returnvalue (`|CreateWidget` "/Game/TSS_Game/UI/W_MainMenu.W_MainMenu_C"))
          (`UserWidget.AddToViewport` _returnvalue 0)
          (else
            (bind _returnvalue_2 (`|CreateWidget` "/Game/TSS_Game/UI/W_DisclaimerScreen.W_DisclaimerScreen_C"))
            (`UserWidget.AddToViewport` _returnvalue_2 0)
            (set `/Game/TSS_Game/Blueprints/GameInstanceSettings/BP_GameInstanceWithSettings.AlreadyPlayed?` true _asbp_game_instance_with_settings)))
        (bind _foundwidgets (`WidgetBlueprintLibrary.GetAllWidgetsOfClass` "/Game/TSS_Game/UI/W_CursorCrosshair.W_CursorCrosshair_C" false))
        (for _array_element _foundwidgets
          (bind _output_get (set `self.CursorRef` _array_element))
          (set `WidgetSwitcher.ActiveWidgetIndex` 1 (`/Game/TSS_Game/UI/W_CursorCrosshair.WidgetSwitcher_79` _output_get))))
      (:`CastFailed`
        (`KismetSystemLibrary.PrintString` "PlControllerMenu: Instance cast failed!")))))

(event `LightSourcesCastingShadow_Init`
  ;[1 1 1] Light controls
  (bind _returnvalue (`GameUserSettings.GetGameUserSettings`))
  (if (== (`GameUserSettings.GetShadowQuality` _returnvalue) 0)
    (`self.ToggleShadowCast` false)
    (else
      (`self.ToggleShadowCast` true))))

(event `ToggleShadowCast`
  (params (`ShadowCastOn?` :type Boolean))
  ;[1 1 1] Light controls
  (for _array_element (`self.SkylightsShadow`)
    (bind _lightcomponent (`SkyLight.LightComponent` _array_element))
    (`LightComponentBase.SetCastShadows` _lightcomponent `ShadowCastOn?`)
    (`KismetSystemLibrary.PrintString` (`KismetSystemLibrary.GetDisplayName` _lightcomponent)))
  (for _array_element_2 (`self.DitectionalLightsShadow`)
    (`LightComponentBase.SetCastShadows` (`Light.LightComponent` _array_element_2) `ShadowCastOn?`))
  (for _array_element_3 (`self.PointLightsShadow`)
    (`LightComponentBase.SetCastShadows` (`PointLight.PointLightComponent` _array_element_3) `ShadowCastOn?`))
  (for _array_element_4 (`self.RectLightsShadow`)
    (`LightComponentBase.SetCastShadows` (`RectLight.RectLightComponent` _array_element_4) `ShadowCastOn?`)))

(fn `UserConstructionScript`)