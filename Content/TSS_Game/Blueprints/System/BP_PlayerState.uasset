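; Player state that relays lobby data between server and clients and keeps a simple player score.
; SV_ events pass slot resets, customization, ready status and level to MC_ events, which update the local lobby player controller.
; Customization entries are stored in an array, replaced by player number.
; Character ready and player-left events both call the game mode's SVPlayerReady; leaving also destroys the character after a delay.
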(event `self.ReceiveBeginPlay`)

(event `Start`
  (bind _asbp_character_base (cast `/Game/TSS_Game/Blueprints/System/BP_CharacterBase` (`GameplayStatics.GetPlayerCharacter` 0)))
  (set `self.PlayerCast` _asbp_character_base))

(event `/Game/TSS_Game/Blueprints/System/BPI_Interactive.Interact With Actor`
  (params (CharacterReference :type "/Game/TSS_Game/Blueprints/System/BP_CharacterBase Object Reference"))
  (`self.AddScore`))

(event `SV_Lobby_ResetPlayerSlotsForAll`
  (`self.MC_Lobby_ResetPlayerSlotsForAll`))

(event `MC_Lobby_ResetPlayerSlotsForAll`
  (bind _asbp_player_controller_lobby (cast `/Game/TSS_Game/Blueprints/System/BP_PlayerControllerLobby` (`GameplayStatics.GetPlayerController` 0)))
  (`/Game/TSS_Game/Blueprints/System/BP_PlayerControllerLobby.ResetAllPlayerSlots` _asbp_player_controller_lobby)
  (`/Game/TSS_Game/Blueprints/System/BP_PlayerControllerLobby.UpdatePlayerList` _asbp_player_controller_lobby))

(event `SV_GetPlayerCustInfo`
  (params (CustomizationToSend :type "/Game/TSS_Game/Blueprints/Customization/ST_All_PlayerInfo Structure"))
  (`self.MC_GetPlayerCustInfo` CustomizationToSend))

(event `MC_GetPlayerCustInfo`
  (params (CustomizationToSend :type "/Game/TSS_Game/Blueprints/Customization/ST_All_PlayerInfo Structure"))
  (bind _customizationofallplayers (`self.CustomizationOfAllPlayers`))
  (for _array_element _customizationofallplayers
    (if (== (`.PlayerNumber_34_824720D5414883DC0CD17497DCE998B0` (break `/Game/TSS_Game/Blueprints/Customization/ST_All_PlayerInfo` _array_element)) (`.PlayerNumber_34_824720D5414883DC0CD17497DCE998B0` (break `/Game/TSS_Game/Blueprints/Customization/ST_All_PlayerInfo` CustomizationToSend)))
      (`KismetArrayLibrary.Array_RemoveItem` (`self.CustomizationOfAllPlayers`) _array_element)))
  (`KismetArrayLibrary.Array_AddUnique` _customizationofallplayers CustomizationToSend)
  (bind _asbp_player_controller_lobby (cast `/Game/TSS_Game/Blueprints/System/BP_PlayerControllerLobby` (`GameplayStatics.GetPlayerController` 0)))
  (`/Game/TSS_Game/Blueprints/System/BP_PlayerControllerLobby.GetAllPlayersCustomization` _asbp_player_controller_lobby _customizationofallplayers))

(event `SV_GetPlayerReadyStatus`
  (params (NewReadyStatus :type Boolean) (PlayerNumber :type Integer))
  ;[1 1 1] PlayersReadyStatus (LOBBY)
  (`self.MC_GetPlayerReadyStatus` NewReadyStatus PlayerNumber))

(event `SV_CharacterIsReady`
  (params (CharacterRef :type "/Game/TSS_Game/Blueprints/System/BP_CharacterBase Object Reference"))
  (bind _asbp_game_mode_base (cast `/Game/TSS_Game/Blueprints/System/BP_GameModeBase` (`GameplayStatics.GetGameMode`)))
  (`/Game/TSS_Game/Blueprints/System/BP_GameModeBase.SV_PlayerReady` _asbp_game_mode_base CharacterRef))

(event `MC_GetPlayerReadyStatus`
  (params (NewReadyStatus :type Boolean) (PlayerNumber :type Integer))
  ;[1 1 1] PlayersReadyStatus (LOBBY)
  (bind _asbp_player_controller_lobby (cast `/Game/TSS_Game/Blueprints/System/BP_PlayerControllerLobby` (`GameplayStatics.GetPlayerController` 0)))
  (`/Game/TSS_Game/Blueprints/System/BP_PlayerControllerLobby.UpdatePlayerSlotReadyStatus` _asbp_player_controller_lobby PlayerNumber NewReadyStatus))

(event `SV_PlayerLeft`
  (params (CharacterRef :type "/Game/TSS_Game/Blueprints/System/BP_CharacterBase Object Reference"))
  (bind _asbp_game_mode_base (cast `/Game/TSS_Game/Blueprints/System/BP_GameModeBase` (`GameplayStatics.GetGameMode`)))
  (`/Game/TSS_Game/Blueprints/System/BP_GameModeBase.SV_PlayerReady` _asbp_game_mode_base CharacterRef)
  (`KismetSystemLibrary.Delay` 3.0)
  (`self.K2_DestroyActor` CharacterRef))

(event `SV_SendPlayerLevelUpdate`
  (params (PlayerNumber :type Integer) (PlayerLevel :type Integer))
  ;[1 1 1] PlayersReadyStatus (LOBBY)
  (`self.MC_SendPlayerLevelUpdate` PlayerNumber PlayerLevel))

(event `MC_SendPlayerLevelUpdate`
  (params (PlayerNumber :type Integer) (PlayerLevel :type Integer))
  ;[1 1 1] PlayersReadyStatus (LOBBY)
  (bind _asbp_player_controller_lobby (cast `/Game/TSS_Game/Blueprints/System/BP_PlayerControllerLobby` (`GameplayStatics.GetPlayerController` 0)))
  (`/Game/TSS_Game/Blueprints/System/BP_PlayerControllerLobby.UpdatePlayerLevel` _asbp_player_controller_lobby PlayerNumber PlayerLevel))

(fn `AddScore`
  (set `self.PlayerScore` (+ (`self.PlayerScore`) 1)))

(fn `UserConstructionScript`)