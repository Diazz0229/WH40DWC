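; Game mode for co-op missions in Survival and Quarantine modes, tracking players, tokens, mission win or failure, and kicks.
; Once all players are ready, Survival runs timed waves from a data table through enemy spawners, with bosses spawned inside RenewPlayerStates.
; Cleared waves revive players, award tokens, roll a random mutation and restock pickups before the next.
; Quarantine relays room completion, activation and unlock events to player controllers.
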(event `MissionSuccess`
  ;[1 1 1] Mission fail / win
  (`self.AddPointsToAllPlayers` (`self.TokensAddedForVictory`))
  (for _array_element (`self.PlayerControllers`)
    (`/Game/TSS_Game/Blueprints/System/BP_PlayerController.MissionSuccess` _array_element)))

(event `CheckPlayersAlive`
  (params (AskedController :type "/Game/TSS_Game/Blueprints/System/BP_PlayerController Object Reference"))
  ;[1 1 1] Mission fail / win
  (set `self.DeadPlayers` 0)
  (for _array_element (`self.PlayerControllers`)
    (if (`/Game/TSS_Game/Blueprints/System/BP_CharacterBase.IsDead` (`/Game/TSS_Game/Blueprints/System/BP_PlayerController.CharacterCast` _array_element))
      (`/Engine/EditorBlueprintResources/StandardMacros.IncrementInt` (`self.DeadPlayers`))))
  (if (== (`KismetArrayLibrary.Array_Length` (`GameStateBase.PlayerArray` (`GameplayStatics.GetGameState`))) (`self.DeadPlayers`))
    (`KismetSystemLibrary.Delay` 3.0)
    (for _array_element_2 (`self.PlayerControllers`)
      (`/Game/TSS_Game/Blueprints/System/BP_PlayerController.MissionFailed` _array_element_2))))

(event `self.ReceiveBeginPlay`
  (bind _asbp_game_instance_with_settings (cast `/Game/TSS_Game/Blueprints/GameInstanceSettings/BP_GameInstanceWithSettings` (`GameplayStatics.GetGameInstance`))
    (:`then`
      (if (not (`/Game/TSS_Game/Blueprints/GameInstanceSettings/BP_GameInstanceWithSettings.IsLocalCoopGame` _asbp_game_instance_with_settings))
        (for _array_element (`GameStateBase.PlayerArray` (`GameplayStatics.GetGameState`))
          (bind _asbp_player_state (cast `/Game/TSS_Game/Blueprints/System/BP_PlayerState` _array_element))
          (bind _asplayer_controller (cast `PlayerController` (`self.GetOwner` _asbp_player_state)))
          (if (not (== (`GameplayStatics.GetPlayerControllerID` _asplayer_controller) 0))
            (`GameplayStatics.RemovePlayer` _asplayer_controller true)))))
    (:`CastFailed`
      (`KismetSystemLibrary.PrintString` "GameMode: Failed to cast Game Instance" true true (struct :`G` 0.66 :`B` 1.0 :`A` 1.0) 10.0))))

(event `self.K2_PostLogin`
  (params (NewPlayer :type "PlayerController Object Reference"))
  (`/Engine/EditorBlueprintResources/StandardMacros.IsValid` NewPlayer :!label _label
    (:`Is Valid`
      (bind _asbp_player_controller (cast `/Game/TSS_Game/Blueprints/System/BP_PlayerController` NewPlayer :!label _label_2)
        (:`then`
          (`KismetArrayLibrary.Array_Add` (`self.PlayerControllers`) _asbp_player_controller))
        (:`CastFailed`
          (`KismetSystemLibrary.PrintString` "GameMode: Failed to cast to player controller bp. Retrying..." true true (struct :`G` 0.66 :`B` 1.0 :`A` 1.0) 10.0)
          (`KismetSystemLibrary.Delay` 1.0)
          (goto _label_2))))
    (:`Is Not Valid`
      (`KismetSystemLibrary.PrintString` "GameMode: Failed to get player controller. Retrying..." true true (struct :`G` 0.66 :`B` 1.0 :`A` 1.0) 10.0)
      (`KismetSystemLibrary.Delay` 0.3)
      (goto _label))))

(event `SV_PlayerReady`
  (params (CharacterRef :type "/Game/TSS_Game/Blueprints/System/BP_CharacterBase Object Reference"))
  ;[1 1 1] Players status control
  (`/Engine/EditorBlueprintResources/StandardMacros.IsValid` CharacterRef
    (:`Is Valid`
      (`KismetArrayLibrary.Array_AddUnique` (`self.AllCharacters`) CharacterRef)
      (bind _asbp_player_controller (cast `/Game/TSS_Game/Blueprints/System/BP_PlayerController` (`Pawn.GetController` CharacterRef) :!label _label_3)
        (:`then`
          (`KismetArrayLibrary.Array_AddUnique` (`self.PlayerControllers`) _asbp_player_controller)
          (`self.ChekIfAllPawnsAreControlled`)
          (`self.CheckPlayers`))
        (:`CastFailed`
          (`KismetSystemLibrary.PrintString` "GameMode: Failed to get player controller while player is ready. Retrying..." true true (struct :`G` 0.66 :`B` 1.0 :`A` 1.0) 10.0)
          (`KismetSystemLibrary.Delay` 0.3)
          (goto _label_3))))))

(event `EnableSpawns`
  (bind _allcharacters (`self.AllCharacters`))
  ;[1 1 1] WaveControl (Survival)
  (`KismetSystemLibrary.Delay` 5.0)
  (`KismetSystemLibrary.K2_SetTimerDelegate` (delegate `CheckIfAllEnemiesAreDead`) 5.0 true)
  (set `self.WaveStopped` false)
  (set `self.RestTime` false)
  (bind (_success_ _out_row) (`self.Get wave table` (- (`self.CurWaveNumber`) 1)))
  (set `self.WaveList` _out_row)
  (bind _outactors (`GameplayStatics.GetAllActorsOfClass` "/Game/TSS_Game/Blueprints/LevelDesign/Spawners/BP_EnemySpawner.BP_EnemySpawner_C"))
  (for _array_element _outactors
    (set `/Game/TSS_Game/Blueprints/LevelDesign/Spawners/BP_EnemySpawner.IsActive?` true _array_element)
    (`KismetArrayLibrary.Array_Clear` (`self.AllEnemiesArray`))
    (`/Game/TSS_Game/Blueprints/LevelDesign/Spawners/BP_EnemySpawner.BeginSpawns` _array_element (`KismetMathLibrary.RandomIntegerInRange` (* (`KismetArrayLibrary.Array_Length` _allcharacters) 3) 10) (`KismetMathLibrary.Clamp` (+ (* (`KismetArrayLibrary.Array_Length` _allcharacters) 5) (`self.CurWaveNumber`)) 0 80) (`self.New Mutation`) (`self.WaveList`) 1.0 30.0))
  (`KismetSystemLibrary.K2_SetTimerDelegate` (delegate `WaveStop`) (+ (* (`self.CurWaveNumber`) 2) 20.0))
  (`self.UpdateWaveInfo` true)
  (`self.Init_SpawnItems`)
  (`self.RenewPlayerStates`))

(event `SV_PlayerLeft`
  (params (Character :type "/Game/TSS_Game/Blueprints/System/BP_CharacterBase Object Reference (by ref)"))
  ;[1 1 1] Players status control
  (`KismetArrayLibrary.Array_RemoveItem` (`self.AllCharacters`) Character)
  (`self.CheckPlayers`))

(event `KickPlayer`
  (params (PlayerID :type Integer))
  ;[1 1 1] Kicks a player (Press P/ESC to open the menu)
  (for (_array_element _array_index) (`self.PlayerControllers`)
    (if (== _array_index PlayerID)
      (`/Engine/EditorBlueprintResources/StandardMacros.IsValid` _array_element
        (:`Is Valid`
          (`/Game/TSS_Game/Blueprints/System/BP_PlayerController.Kick` _array_element))))))

(event `WaveStop`
  ;[1 1 1] WaveControl (Survival)
  (set `self.WaveStopped` true)
  (bind _outactors (`GameplayStatics.GetAllActorsOfClass` "/Game/TSS_Game/Blueprints/LevelDesign/Spawners/BP_EnemySpawner.BP_EnemySpawner_C"))
  (for _array_element _outactors
    (set `/Game/TSS_Game/Blueprints/LevelDesign/Spawners/BP_EnemySpawner.IsActive?` false _array_element))
  (`self.EnemiesStartDeathTimer`))

(event `CheckPlayers`
  ;[1 1 1] Players status control
  (if (and (== (`KismetArrayLibrary.Array_Length` (`self.AllCharacters`)) (`KismetArrayLibrary.Array_Length` (`GameStateBase.PlayerArray` (`GameplayStatics.GetGameState`)))) (`self.WaveStopped`))
    (switch `/Game/TSS_Game/Blueprints/System/E_GameModeType` (`self.GameModeType`)
      (:`NewEnumerator0`
        (`self.EnableSpawns`))
      (:`NewEnumerator1`
        (`self.RenewPlayerStates`)
        (`KismetSystemLibrary.Delay` 5.0)
        (for _array_element (`self.PlayerControllers`)
          (`/Game/TSS_Game/Blueprints/System/BP_PlayerController.SV_WinConditionReached` _array_element 0))))))

(event `RenewPlayerStates`
  (bind (_enemyclass _spawnchance _behaviortree _bossclass _bossammount _bossbehaviortree) (break `/Game/TSS_Game/Blueprints/Bonus/AI/ST_WaveList` (`self.WaveList`)))
  ;[1 1 1] WaveControl (Survival)
  ;;[1 1 1] RenewPlayerstates
  (`KismetArrayLibrary.Array_Clear` (`self.AllPlayerStates`))
  (for _array_element (`GameStateBase.PlayerArray` (`GameplayStatics.GetGameState`))
    (`/Engine/EditorBlueprintResources/StandardMacros.IsValid` _array_element
      (:`Is Valid`
        (bind _asbp_player_state (cast `/Game/TSS_Game/Blueprints/System/BP_PlayerState` _array_element))
        (`KismetArrayLibrary.Array_AddUnique` (`self.AllPlayerStates`) _asbp_player_state))))
  ;;[1 1 1] Spawn N bosses at random spawns
  (for (_array_element_2 _array_index) _bossclass
    (for _ (range 1 (+ _bossammount 1))
      (bind _outactors (`GameplayStatics.GetAllActorsOfClass` "/Game/TSS_Game/Blueprints/LevelDesign/Spawners/BP_EnemySpawner.BP_EnemySpawner_C"))
      (`AIBlueprintHelperLibrary.SpawnAIFromClass` (castclass `Pawn` _array_element_2 :!pure true) (`|GetArrayItem` _bossbehaviortree _array_index) (`self.K2_GetActorLocation` (`KismetArrayLibrary.Array_Random` _outactors)) (struct) false null))))

(event `ServerTravel`
  (params (MapName :type String))
  (`KismetSystemLibrary.ExecuteConsoleCommand` (`KismetStringLibrary.Concat_StrStr` "servertravel " MapName) (`GameplayStatics.GetPlayerController` 0))
  (`UpdateSessionCallbackProxyAdvanced.UpdateSession` :`bAllowInvites` true))

(event `CheckIfAllEnemiesAreDead`
  ;[1 1 1] WaveControl (Survival)
  (if (`self.WaveStopped`)
    (bind _allenemiesdead (`self.EnemiesDeadChecker`))
    (if _allenemiesdead
      (if (not (`self.RestTime`))
        (`self.WaveCompleted`))
      (else
        (`self.UpdateWaveInfo` false)))))

(event `UpdateWaveInfo`
  (params (`IsNewWave?` :type Boolean))
  ;[1 1 1] WaveControl (Survival)
  (for _array_element (`self.AllCharacters`)
    (`/Game/TSS_Game/Blueprints/System/BP_PlayerController.SV_UpdateWaveInfo` (`/Game/TSS_Game/Blueprints/System/BP_CharacterBase.OwningPlayerController` _array_element) (`self.CurWaveNumber`) (`KismetArrayLibrary.Array_Length` (`self.AllEnemiesArray`)) `IsNewWave?` (`self.MutationDescription`))))

(event `EnemiesStartDeathTimer`
  (for _array_element (`self.AllEnemiesArray`)
    (bind _asbp_enemy_base (cast `/Game/TSS_Game/Blueprints/Bonus/AI/BP_Enemy_BASE` _array_element))
    (`/Game/TSS_Game/Blueprints/Bonus/AI/BP_Enemy_BASE.StartDeathTimer` _asbp_enemy_base)))

(event `AddPointsToPlayer`
  (params (PointsToAdd :type Integer) (PlayerController :type "PlayerController Object Reference"))
  ;[1 1 1] WaveControl (Survival)
  (bind _asbp_player_state (cast `/Game/TSS_Game/Blueprints/System/BP_PlayerState` (`Controller.PlayerState` PlayerController)))
  (set `/Game/TSS_Game/Blueprints/System/BP_PlayerState.PlayerTokensEarned` (+ (`/Game/TSS_Game/Blueprints/System/BP_PlayerState.PlayerTokensEarned` _asbp_player_state) PointsToAdd) _asbp_player_state)
  (bind _asbp_player_controller (cast `/Game/TSS_Game/Blueprints/System/BP_PlayerController` PlayerController))
  (`/Game/TSS_Game/Blueprints/System/BP_PlayerController.LC_TokensGained` _asbp_player_controller PointsToAdd))

(event `CollectSkull`
  (params (PlController :type "Controller Object Reference"))
  ;[1 1 1] WaveControl (Survival)
  (bind _asbp_player_state (cast `/Game/TSS_Game/Blueprints/System/BP_PlayerState` (`Controller.PlayerState` PlController)))
  (bind _result (`/Engine/EditorBlueprintResources/StandardMacros.IncrementInt` (`/Game/TSS_Game/Blueprints/System/BP_PlayerState.PlayerSkullsCollected` _asbp_player_state))
    (:`  `
      (bind _asbp_player_controller (cast `/Game/TSS_Game/Blueprints/System/BP_PlayerController` PlController))
      (`/Game/TSS_Game/Blueprints/System/BP_PlayerController.LC_SkullCollected` _asbp_player_controller _result))))

(event `AddPointsToAllPlayers`
  (params (PointsToAdd :type Integer))
  ;[1 1 1] WaveControl (Survival)
  (for _array_element (`self.AllPlayerStates`)
    (set `/Game/TSS_Game/Blueprints/System/BP_PlayerState.PlayerTokensEarned` (+ (`/Game/TSS_Game/Blueprints/System/BP_PlayerState.PlayerTokensEarned` _array_element) PointsToAdd) _array_element))
  (for _array_element_2 (`self.PlayerControllers`)
    (`/Game/TSS_Game/Blueprints/System/BP_PlayerController.LC_TokensGained` _array_element_2 PointsToAdd)))

(event `WaveCompleted`
  (bind _cratespawnersavailable (`self.CrateSpawnersAvailable`))
  ;[1 1 1] WaveControl (Survival)
  (set `self.RestTime` true)
  (for _array_element (`self.AllCharacters`)
    (`/Game/TSS_Game/Blueprints/System/BP_PlayerController.LC_WaveCompleted` (`/Game/TSS_Game/Blueprints/System/BP_CharacterBase.OwningPlayerController` _array_element)))
  (`self.ReviveAllDeadPlayers`)
  (`self.AddPointsToAllPlayers` (`KismetMathLibrary.Clamp` (* (`self.CurWaveNumber`) 10) 0 50))
  (`KismetSystemLibrary.Delay` 15.0)
  (`/Engine/EditorBlueprintResources/StandardMacros.IncrementInt` (`self.CurWaveNumber`) ; NextWave
    (:`  `
      (for _array_element_2 (`self.AllCharacters`)
        (`/Game/TSS_Game/Blueprints/System/BP_PlayerController.SV_UpdateWaveInfo` (`/Game/TSS_Game/Blueprints/System/BP_CharacterBase.OwningPlayerController` _array_element_2) (`self.CurWaveNumber`) 0 false ""))
      (`|ExecutionSequence`
        (:`then_0`
          (`self.EnableSpawns`)
          (`self.DetermineNewMutation`)
          ;;[1 1 1] Clear skulls
          (bind _outactors (`GameplayStatics.GetAllActorsOfClass` "/Game/TSS_Game/Blueprints/LevelDesign/Spawners/BP_Spawn_ServoSkull01.BP_Spawn_ServoSkull01_C"))
          (for _array_element_3 _outactors
            (bind _attacheditem (`/Game/TSS_Game/Blueprints/LevelDesign/Spawners/BP_Spawn_ServoSkull01.AttachedItem` _array_element_3))
            (`/Engine/EditorBlueprintResources/StandardMacros.IsValid` _attacheditem
              (:`Is Valid`
                (`self.K2_DestroyActor` _attacheditem)
                (set `/Game/TSS_Game/Blueprints/LevelDesign/Spawners/BP_Spawn_ServoSkull01.AttachedItem` null _array_element_3)))))
        (:`then_1`
          ;;[1 1 1] Spawn ammo crates
          (bind _outactors_2 (`GameplayStatics.GetAllActorsOfClass` "/Game/TSS_Game/Blueprints/Pickup/BP_AmmoCrate.BP_AmmoCrate_C" :!label _label_4))
          (bind _returnvalue (`KismetArrayLibrary.Array_Length` _outactors_2))
          (if (< _returnvalue (`self.MaxAmmoCratesAvailable`))
            (`KismetArrayLibrary.Array_Clear` (`self.CrateSpawnersAvailable`))
            (bind _outactors_3 (`GameplayStatics.GetAllActorsOfClass` "/Game/TSS_Game/Blueprints/LevelDesign/Spawners/BP_Spawn_AmmoCrates.BP_Spawn_AmmoCrates_C"))
            (for _array_element_4 _outactors_3
              (bind _iscratevalid (`/Game/TSS_Game/Blueprints/LevelDesign/Spawners/BP_Spawn_AmmoCrates.Crate Validation` _array_element_4))
              (if (not _iscratevalid)
                (`KismetArrayLibrary.Array_AddUnique` (`self.CrateSpawnersAvailable`) _array_element_4)))
            (if (`KismetArrayLibrary.Array_IsNotEmpty` _cratespawnersavailable)
              (for _ (range 1 (+ (- (`self.MaxAmmoCratesAvailable`) _returnvalue) 1))
                (bind _output_get (set `self.TEMP_AmmoSpawnerRef` (`KismetArrayLibrary.Array_Random` _cratespawnersavailable)))
                (`/Game/TSS_Game/Blueprints/LevelDesign/Spawners/BP_Spawn_AmmoCrates.SpawnAmmoCrate` _output_get)
                (`KismetArrayLibrary.Array_RemoveItem` _cratespawnersavailable _output_get)))))))))

(event `ReviveAllDeadPlayers`
  ;[1 1 1] WaveControl (Survival)
  (for _array_element (`self.AllCharacters`)
    (if (`/Game/TSS_Game/Blueprints/System/BP_CharacterBase.IsDead` _array_element)
      (`/Game/TSS_Game/Blueprints/System/BP_CharacterBase.SV_ReviveCharacter` _array_element))))

(event `Init_SpawnItems`
  (bind _skullspawnersavailable (`self.SkullSpawnersAvailable`))
  ;[1 1 1] WaveControl (Survival)
  (`|ExecutionSequence`
    (:`then_0`
      (goto _label_4))
    (:`then_1`
      ;;[1 1 1] Spawn skulls
      (set `self.CurSkullsAvailable` (`KismetMathLibrary.RandomIntegerInRange` 0 (`self.MaxSkullsAvailable`)))
      (bind _outactors (`GameplayStatics.GetAllActorsOfClass` "/Game/TSS_Game/Blueprints/Pickup/BP_ItemPickup_ServoSkull_Badge.BP_ItemPickup_ServoSkull_Badge_C"))
      (bind _returnvalue (`KismetArrayLibrary.Array_Length` _outactors))
      (if (< _returnvalue (`self.CurSkullsAvailable`))
        (`KismetArrayLibrary.Array_Clear` (`self.CrateSpawnersAvailable`))
        (bind _outactors_2 (`GameplayStatics.GetAllActorsOfClass` "/Game/TSS_Game/Blueprints/LevelDesign/Spawners/BP_Spawn_ServoSkull01.BP_Spawn_ServoSkull01_C"))
        (for _array_element _outactors_2
          (bind _iscratevalid (`/Game/TSS_Game/Blueprints/LevelDesign/Spawners/BP_Spawn_ServoSkull01.Item Validation` _array_element))
          (if (not _iscratevalid)
            (`KismetArrayLibrary.Array_AddUnique` (`self.SkullSpawnersAvailable`) _array_element)))
        (if (`KismetArrayLibrary.Array_IsNotEmpty` _skullspawnersavailable)
          (for _ (range 1 (+ (- (`self.CurSkullsAvailable`) _returnvalue) 1))
            (bind _output_get (set `self.TEMP_SkullSpawnerRef` (`KismetArrayLibrary.Array_Random` _skullspawnersavailable)))
            (`/Game/TSS_Game/Blueprints/LevelDesign/Spawners/BP_Spawn_ServoSkull01.SpawnItem` _output_get)
            (`KismetArrayLibrary.Array_RemoveItem` _skullspawnersavailable _output_get)))))))

(event `RoomWinConditionComplete`
  (params (RoomIndex :type Integer))
  ;[1 1 1] Wave control (Quarantine)
  (for _array_element (`self.AllCharacters`)
    (`/Game/TSS_Game/Blueprints/System/BP_PlayerController.LC_WinConditionReached` (`/Game/TSS_Game/Blueprints/System/BP_CharacterBase.OwningPlayerController` _array_element) RoomIndex)
    (if (> RoomIndex 5)
      (`self.AddPointsToAllPlayers` 5))))

(event `RoomManualActivation`
  (params (RoomIndex :type Integer))
  ;[1 1 1] Wave control (Quarantine)
  (for _array_element (`self.AllCharacters`)
    (`/Game/TSS_Game/Blueprints/System/BP_PlayerController.LC_RoomManualActivation` (`/Game/TSS_Game/Blueprints/System/BP_CharacterBase.OwningPlayerController` _array_element) RoomIndex)))

(event `SV_UnlockNextRoom`
  (params (RoomIndex :type Integer))
  ;[1 1 1] Wave control (Quarantine)
  (for _array_element (`self.AllCharacters`)
    (`/Game/TSS_Game/Blueprints/System/BP_PlayerController.LC_UnlockNextDoor` (`/Game/TSS_Game/Blueprints/System/BP_CharacterBase.OwningPlayerController` _array_element) RoomIndex)))

(fn `ChekIfAllPawnsAreControlled`
  (bind _outactors (`GameplayStatics.GetAllActorsOfClass` "/Game/TSS_Game/Blueprints/System/BP_Character_Cust_v1.BP_Character_Cust_v1_C"))
  (for _array_element _outactors
    (if (not (`Pawn.IsPlayerControlled` _array_element))
      (`self.K2_DestroyActor` _array_element)))
  (return))

(fn `DetermineNewMutation`
  (returns (NewMutation :type "/Game/TSS_Game/Blueprints/AbilitySystem/EnemyMutations/Base/AC_Mutation_BASE Class Reference") (MutationDescription :type Text))
  (bind _outrownames (`DataTableFunctionLibrary.GetDataTableRowNames` "/Game/TSS_Game/Blueprints/AbilitySystem/EnemyMutations/DT_MutationsList.DT_MutationsList"))
  (bind _returnvalue (`|GetDataTableRow` "/Game/TSS_Game/Blueprints/AbilitySystem/EnemyMutations/DT_MutationsList.DT_MutationsList" (`KismetArrayLibrary.Array_Random` _outrownames))
    (:`then`
      (bind (_bp_component _description) (break `/Game/TSS_Game/Blueprints/AbilitySystem/EnemyMutations/Base/ST_MutationList` _returnvalue))
      (bind _output_get (set `self.New Mutation` _bp_component))
      (bind _output_get_2 (set `self.MutationDescription` _description))
      (return _output_get _output_get_2))))

(fn `EnemiesDeadChecker`
  (returns (AllEnemiesDead :type Boolean))
  (bind _allenemiesarray (`self.AllEnemiesArray`))
  (for _array_element _allenemiesarray
    (`/Engine/EditorBlueprintResources/StandardMacros.IsValid` _array_element
      (:`Is Valid`
        (bind _asbp_enemy_base (cast `/Game/TSS_Game/Blueprints/Bonus/AI/BP_Enemy_BASE` _array_element)
          (:`then`
            (if (`/Game/TSS_Game/Blueprints/Bonus/AI/BP_Enemy_BASE.isDead` _asbp_enemy_base)
              (`KismetArrayLibrary.Array_RemoveItem` _allenemiesarray _array_element :!label _label)))
          (:`CastFailed`
            (goto _label))))
      (:`Is Not Valid`
        (goto _label))))
  (if (`KismetArrayLibrary.Array_IsNotEmpty` _allenemiesarray)
    (return false)
    (else
      (return true))))

(fn `Get wave table`
  (params (WaveListRow :type Integer))
  (returns (`Success?` :type Boolean) (`Out Row` :type "/Game/TSS_Game/Blueprints/Bonus/AI/ST_WaveList Structure"))
  (bind _outrownames (`DataTableFunctionLibrary.GetDataTableRowNames` "/Game/TSS_Game/Blueprints/Bonus/AI/DT_WaveList_Survival_1.DT_WaveList_Survival_1"))
  (bind _returnvalue (`|GetDataTableRow` "/Game/TSS_Game/Blueprints/Bonus/AI/DT_WaveList_Survival_1.DT_WaveList_Survival_1" (`|GetArrayItem` _outrownames (- WaveListRow 1)))
    (:`then`
      (return true _returnvalue))
    (:`RowNotFound`
      (bind _returnvalue_2 (`|GetDataTableRow` "/Game/TSS_Game/Blueprints/Bonus/AI/DT_WaveList_Survival_1.DT_WaveList_Survival_1" (`|GetArrayItem` _outrownames (`KismetArrayLibrary.Array_Length` _outrownames))) ; Get last wave data if waves are above described in table
        (:`then`
          (return true _returnvalue_2))))))

(fn `UserConstructionScript`)