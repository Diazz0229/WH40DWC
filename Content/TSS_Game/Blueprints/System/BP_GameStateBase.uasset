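; Game state Blueprint that sends achievement and tech-log messages to Discord webhooks through VaRest.
; SendDiscord_MSG loads and caches the SavedSettings save once, retrying on a delay while it is missing.
; Global achievements reach the achievement webhook only when important, allowed in settings and in a distribution build.
; Other achievements get a PrivateLog prefix and share the second webhook with tech logs.
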(event `CalledURL1`
  (params (Request :type "VaRestRequestJSON Object Reference"))
  ;[1 1 1] Discord msg
)

(event `SendDiscord_MSG`
  (params (StringSent :type String) (MSG_type :type "/Game/TSS_Game/Blueprints/System/E_DiscordMSG Enum" :default "NewEnumerator0") (`IsImportantAch?` :type Boolean))
  (bind _returnvalue (subsystem `VaRestSubsystem`))
  (bind _returnvalue_2 (subsystem `VaRestSubsystem`))
  (set `self.String Sent` StringSent)
  ;[1 1 1] Find save game
  (bind _returnvalue_3 (`GameplayStatics.DoesSaveGameExist` "SavedSettings" :!label _label))
  (if _returnvalue_3
    (`|ExecutionSequence`
      (:`then_0`
        (`/Engine/EditorBlueprintResources/StandardMacros.DoOnce` false
          (:`Completed`
            (bind _returnvalue_4 (`GameplayStatics.LoadGameFromSlot` "SavedSettings"))
            (bind _asbp_settings_save (cast `/Game/TSS_Game/Blueprints/GameInstanceSettings/BP_SettingsSave` _returnvalue_4))
            (set `self.As BP Settings Save` _asbp_settings_save))))
      (:`then_1`
        (switch `/Game/TSS_Game/Blueprints/System/E_DiscordMSG` MSG_type
          (:`NewEnumerator0`
            (if (and (`/Game/TSS_Game/Blueprints/GameInstanceSettings/BP_SettingsSave.Saved_AllowDiscordAchievements` (`self.As BP Settings Save`)) (`KismetSystemLibrary.IsPackagedForDistribution`) `IsImportantAch?`)
              ;[1 1 1] Discord msg
              (bind _returnvalue_5 (`VaRestSubsystem.ConstructVaRestJsonObject` _returnvalue_2))
              (`VaRestJsonObject.SetStringField` _returnvalue_5 "content" (`self.String Sent`))
              (`VaRestSubsystem.CallURL` _returnvalue_2 "https://discord.com/api/webhooks/1399314856414285888/dCdXN1sLo3v9aFWRrolGqO8M5EMXOFubHbzubwEFk9EKeZoDAxZxcC8TSgFn-brsRsHr" "POST" "json" _returnvalue_5 (delegate `CalledURL1`))
              (else
                (set `self.String Sent` (`KismetStringLibrary.Concat_StrStr` "PrivateLog: " (`self.String Sent`)))
                ;[1 1 1] Discord msg
                (bind _returnvalue_6 (`VaRestSubsystem.ConstructVaRestJsonObject` _returnvalue :!label _label_2))
                (`VaRestJsonObject.SetStringField` _returnvalue_6 "content" (`self.String Sent`))
                (`VaRestSubsystem.CallURL` _returnvalue "https://discord.com/api/webhooks/1399315802905378916/yXVcU1y5VYJS0KU8ye7jAVo5oG-8M-HUqsw3wGZ2Qi_s4icEjLJ-2f5w_qNBVum54wpe" "POST" "json" _returnvalue_6 (delegate `CalledURL2`)))))
          (:`NewEnumerator1`
            (goto _label_2)))))
    (else
      (`KismetSystemLibrary.PrintString` "BP_GameStateBase: Failed to loadSettings file. Retrying in 5sec..." true true (struct :`R` 1.0 :`A` 1.0) 4.0)
      (`KismetSystemLibrary.Delay` 5.0)
      (goto _label))))

(event `CalledURL2`
  (params (Request :type "VaRestRequestJSON Object Reference"))
  ;[1 1 1] Discord msg
)

(fn `UserConstructionScript`)