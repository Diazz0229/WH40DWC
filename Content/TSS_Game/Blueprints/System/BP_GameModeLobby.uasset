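; Lobby game mode that manages joining and leaving players, readiness and travel to the match map.
; It numbers players on login, refreshes client lists, and unreadies everyone on any join or non-travel logout.
; It relays customization and ready status through every PlayerState, starting countdowns on lobby controllers once all are ready.
; ServerTravel flags travel to skip logout handling, shows loading screens, then runs the servertravel console command.
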(event `self.ReceiveBeginPlay`
  (bind _asbp_game_instance_with_settings (cast `/Game/TSS_Game/Blueprints/GameInstanceSettings/BP_GameInstanceWithSettings` (`GameplayStatics.GetGameInstance`)))
  (bind _output_get (set `self.GameInstanceCast` _asbp_game_instance_with_settings))
  (`/Game/TSS_Game/Blueprints/GameInstanceSettings/BP_GameInstanceWithSettings.LoadSettings` _output_get)
  (`KismetSystemLibrary.ExecuteConsoleCommand` (`KismetStringLibrary.Concat_StrStr` "r.SetRes " (`/Game/TSS_Game/Blueprints/GameInstanceSettings/BP_GameInstanceWithSettings.Settings_Resolution` _output_get) (select `bool` (`/Game/TSS_Game/Blueprints/GameInstanceSettings/BP_GameInstanceWithSettings.Settings_Resolution_Mode` _output_get) :`false` "w" :`true` "f")) null))

(event `self.K2_OnLogout`
  (params (ExitingController :type "Controller Object Reference"))
  ;[1 1 1] Player login or logout event
  (if (not (`self.IsMapTravelling`))
    (`self.Chat_PlayerLog` (`PlayerState.GetPlayerName` (`Controller.PlayerState` ExitingController)))
    (`KismetSystemLibrary.Delay` 0.2)
    (for _array_element (`GameStateBase.PlayerArray` (`GameplayStatics.GetGameState`))
      (bind _asbp_player_state (cast `/Game/TSS_Game/Blueprints/System/BP_PlayerState` _array_element))
      (`/Game/TSS_Game/Blueprints/System/BP_PlayerState.SV_Lobby_ResetPlayerSlotsForAll` _asbp_player_state))
    (`self.ForceAllUnready`)))

(event `self.K2_PostLogin`
  (params (NewPlayer :type "PlayerController Object Reference"))
  (bind _playerstate (`Controller.PlayerState` NewPlayer))
  ;[1 1 1] Player login or logout event
  (bind _result (`/Engine/EditorBlueprintResources/StandardMacros.IncrementInt` (`self.PlayerIndex`))
    (:`  `
      (bind _asbp_player_controller_lobby (cast `/Game/TSS_Game/Blueprints/System/BP_PlayerControllerLobby` NewPlayer))
      (bind _output_get (set `/Game/TSS_Game/Blueprints/System/BP_PlayerControllerLobby.PlayerNumber` _result _asbp_player_controller_lobby))
      (bind _asbp_player_state (cast `/Game/TSS_Game/Blueprints/System/BP_PlayerState` _playerstate))
      (set `/Game/TSS_Game/Blueprints/System/BP_PlayerState.PlayerNumber` _output_get _asbp_player_state)
      (`/Game/TSS_Game/Blueprints/System/BP_PlayerControllerLobby.InitPlayer` _asbp_player_controller_lobby)
      (set `/Game/TSS_Game/Blueprints/System/BP_PlayerControllerLobby.Player Name` (`KismetTextLibrary.Conv_StringToText` (`PlayerState.GetPlayerName` _playerstate)) _asbp_player_controller_lobby)
      (`self.UpdateClientsPlayerInfo`)
      (`self.ForceAllUnready`))))

(event `ForceAllUnready`
  ;[1 1 1] Player login or logout event
  (for _array_element (`GameStateBase.PlayerArray` (`GameplayStatics.GetGameState`))
    (bind _asbp_player_controller_lobby (cast `/Game/TSS_Game/Blueprints/System/BP_PlayerControllerLobby` (`PlayerState.GetPlayerController` _array_element)))
    (`/Game/TSS_Game/Blueprints/System/BP_PlayerControllerLobby.ForceUnready` _asbp_player_controller_lobby)))

(event `UpdateClientsPlayerInfo`
  ;[1 1 1] Player login or logout event
  (for _array_element (`GameStateBase.PlayerArray` (`GameplayStatics.GetGameState`))
    (bind _asbp_player_controller_lobby (cast `/Game/TSS_Game/Blueprints/System/BP_PlayerControllerLobby` (`PlayerState.GetPlayerController` _array_element)))
    (`/Game/TSS_Game/Blueprints/System/BP_PlayerControllerLobby.UpdatePlayerList` _asbp_player_controller_lobby)))

(event `Chat_PlayerLog`
  (params (PlayerName :type String) (`Joined?` :type Boolean))
  ;[1 1 1] Chat
  (bind _asbp_player_controller_lobby (cast `/Game/TSS_Game/Blueprints/System/BP_PlayerControllerLobby` (`GameplayStatics.GetPlayerController` 0)))
  (if `Joined?`
    (`/Game/TSS_Game/Blueprints/System/BP_PlayerControllerLobby.SendChatMessage` _asbp_player_controller_lobby (`KismetStringLibrary.Concat_StrStr` PlayerName " joined the squad!") "SYSTEM")
    (else
      (`/Game/TSS_Game/Blueprints/System/BP_PlayerControllerLobby.SendChatMessage` _asbp_player_controller_lobby (`KismetStringLibrary.Concat_StrStr` PlayerName " left the squad!") "SYSTEM"))))

(event `TransferPlayerCustomization`
  (params (CustomizationToTransfer :type "Array of /Game/TSS_Game/Blueprints/Customization/ST_CustomizationItem Structure") (PlayerNumber :type Integer) (`All Player Info to Transfer Player Name` :type Text) (EquipmentToTransfer :type "Array of /Game/TSS_Game/Blueprints/Customization/ST_Equipment_Item Structure") (PlayerClass :type "/Game/TSS_Game/Blueprints/Customization/E_PlayerClass Enum" :default "NewEnumerator0"))
  ;[1 1 1] Customization transfer
  (set `self.AllPlayerInfoToTransfer` (make `/Game/TSS_Game/Blueprints/Customization/ST_All_PlayerInfo` PlayerNumber CustomizationToTransfer `All Player Info to Transfer Player Name` EquipmentToTransfer PlayerClass))
  (for _array_element (`GameStateBase.PlayerArray` (`GameplayStatics.GetGameState`))
    (bind _asbp_player_state (cast `/Game/TSS_Game/Blueprints/System/BP_PlayerState` _array_element))
    (`/Game/TSS_Game/Blueprints/System/BP_PlayerState.SV_GetPlayerCustInfo` _asbp_player_state (`self.AllPlayerInfoToTransfer`))))

(event `SV_TransferReadyStatus`
  (params (NewReadyStatus :type Boolean) (PlayerNumber :type Integer))
  (bind _playerstotal (`self.PlayersTotal`))
  (bind _playersready (`self.PlayersReady`))
  ;[1 1 1] Player Ready status and server map travel
  (for _array_element (`GameStateBase.PlayerArray` (`GameplayStatics.GetGameState`))
    (bind _asbp_player_state (cast `/Game/TSS_Game/Blueprints/System/BP_PlayerState` _array_element))
    (`/Game/TSS_Game/Blueprints/System/BP_PlayerState.SV_GetPlayerReadyStatus` _asbp_player_state NewReadyStatus PlayerNumber))
  (`KismetSystemLibrary.Delay` 0.5)
  (if NewReadyStatus
    (set `self.PlayersTotal` 0)
    (set `self.PlayersReady` 0)
    (for _array_element_2 (`GameStateBase.PlayerArray` (`GameplayStatics.GetGameState`))
      (`/Engine/EditorBlueprintResources/StandardMacros.IncrementInt` (`self.PlayersTotal`)
        (:`  `
          (bind _asbp_player_state_2 (cast `/Game/TSS_Game/Blueprints/System/BP_PlayerState` _array_element_2))
          (if (`/Game/TSS_Game/Blueprints/System/BP_PlayerState.IsReady` _asbp_player_state_2)
            (`/Engine/EditorBlueprintResources/StandardMacros.IncrementInt` (`self.PlayersReady`))))))
    (if (== _playerstotal _playersready)
      (for _array_element_3 (`GameStateBase.PlayerArray` (`GameplayStatics.GetGameState`))
        (bind _asbp_player_controller_lobby (cast `/Game/TSS_Game/Blueprints/System/BP_PlayerControllerLobby` (`PlayerState.GetPlayerController` _array_element_3)))
        (`/Game/TSS_Game/Blueprints/System/BP_PlayerControllerLobby.ReadyStartCountdown` _asbp_player_controller_lobby))
      (else
        (`KismetSystemLibrary.PrintString` (`KismetStringLibrary.Concat_StrStr` "Not enough ready players: " (`KismetStringLibrary.Conv_IntToString` _playersready) " of " (`KismetStringLibrary.Conv_IntToString` _playerstotal)))))))

(event `ServerTravel`
  (params (MapName :type String))
  ;[1 1 1] Player Ready status and server map travel
  (set `self.IsMapTravelling` true)
  (for _array_element (`GameStateBase.PlayerArray` (`GameplayStatics.GetGameState`))
    (bind _asbp_player_controller_lobby (cast `/Game/TSS_Game/Blueprints/System/BP_PlayerControllerLobby` (`PlayerState.GetPlayerController` _array_element)))
    (`/Game/TSS_Game/Blueprints/System/BP_PlayerControllerLobby.MC_LoadscreenShow` _asbp_player_controller_lobby))
  (`KismetSystemLibrary.ExecuteConsoleCommand` (`KismetStringLibrary.Concat_StrStr` "servertravel " MapName) (`GameplayStatics.GetPlayerController` 0)))

(fn `UserConstructionScript`)