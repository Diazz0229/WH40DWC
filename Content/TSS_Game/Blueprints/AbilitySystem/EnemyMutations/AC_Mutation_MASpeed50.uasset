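; Enemy mutation component that gives its BP_Enemy_BASE owner a temporary movement and attack speed buff.
; On BeginPlay it raises max walk speed by a fraction scaled from mutation level, offsets attack delay and play rate, and attaches a red Niagara effect to the head socket.
; When a one-shot timer ends, it subtracts the stored bonuses, destroys the effect and removes itself.
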(event `self.ReceiveBeginPlay`
  (bind _ownerenemycast (`self.OwnerEnemyCast`))
  (bind _asbp_enemy_base (cast `/Game/TSS_Game/Blueprints/Bonus/AI/BP_Enemy_BASE` (`self.GetOwner`)))
  (set `self.OwnerEnemyCast` _asbp_enemy_base)
  (bind _charactermovement (`Character.CharacterMovement` _asbp_enemy_base))
  (bind _maxwalkspeed (`CharacterMovementComponent.MaxWalkSpeed` _charactermovement))
  (bind _output_get (set `self.StatAdded` (* _maxwalkspeed (* (`self.Mutation Level`) (`self.SpeedMultiplier`)))))
  (set `CharacterMovementComponent.MaxWalkSpeed` (+ _maxwalkspeed _output_get) _charactermovement)
  (`KismetSystemLibrary.K2_SetTimerDelegate` (delegate `RemoveBuff`) (`self.BuffTime`))
  (set `/Game/TSS_Game/Blueprints/Bonus/AI/BP_Enemy_BASE.AttacksDelay` (+ (`/Game/TSS_Game/Blueprints/Bonus/AI/BP_Enemy_BASE.AttacksDelay` _ownerenemycast) (`self.AttacksDealyMinus`)) _ownerenemycast)
  (set `/Game/TSS_Game/Blueprints/Bonus/AI/BP_Enemy_BASE.AttacksPlayRate` (+ (`/Game/TSS_Game/Blueprints/Bonus/AI/BP_Enemy_BASE.AttacksPlayRate` _ownerenemycast) (`self.AttacksPlaySpeedPlus`)) _ownerenemycast)
  (bind _returnvalue (`NiagaraFunctionLibrary.SpawnSystemAttached` "/Game/VFX/PowerUps/N_floatingToCenter_red.N_floatingToCenter_red" (`Character.Mesh` (`self.OwnerEnemyCast`)) "HeadSocket" (0.0 0.0 0.0) (struct) "SnapToTarget"))
  (set `self.AttachedNiagara` _returnvalue))

(event `RemoveBuff`
  (bind _attachedniagara (`self.AttachedNiagara`))
  (bind _ownerenemycast (`self.OwnerEnemyCast`))
  (bind _charactermovement (`Character.CharacterMovement` (`self.OwnerEnemyCast`)))
  (set `CharacterMovementComponent.MaxWalkSpeed` (- (`CharacterMovementComponent.MaxWalkSpeed` _charactermovement) (`self.StatAdded`)) _charactermovement)
  (set `/Game/TSS_Game/Blueprints/Bonus/AI/BP_Enemy_BASE.AttacksDelay` (- (`/Game/TSS_Game/Blueprints/Bonus/AI/BP_Enemy_BASE.AttacksDelay` _ownerenemycast) (`self.AttacksDealyMinus`)) _ownerenemycast)
  (set `/Game/TSS_Game/Blueprints/Bonus/AI/BP_Enemy_BASE.AttacksPlayRate` (- (`/Game/TSS_Game/Blueprints/Bonus/AI/BP_Enemy_BASE.AttacksPlayRate` _ownerenemycast) (`self.AttacksPlaySpeedPlus`)) _ownerenemycast)
  (`/Engine/EditorBlueprintResources/StandardMacros.IsValid` _attachedniagara
    (:`Is Valid`
      (`self.K2_DestroyComponent` _attachedniagara))
    (:`Is Not Valid`
      _))
  (`self.K2_DestroyComponent`))