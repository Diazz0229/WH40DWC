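; Enemy mutation actor component that temporarily boosts the owning BP_Enemy_BASE's movement speed.
; On BeginPlay it adds a bonus to MaxWalkSpeed, computed from the current speed scaled by mutation level and a speed multiplier.
; A one-shot timer then subtracts that stored bonus after the buff time and destroys the component.
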(event `self.ReceiveBeginPlay`
  (bind _asbp_enemy_base (cast `/Game/TSS_Game/Blueprints/Bonus/BP_Enemy_BASE` (`self.GetOwner`)))
  (set `self.OwnerEnemyCast` _asbp_enemy_base)
  (bind _charactermovement (`Character.CharacterMovement` _asbp_enemy_base))
  (bind _maxwalkspeed (`CharacterMovementComponent.MaxWalkSpeed` _charactermovement))
  (bind _output_get (set `self.StatAdded` (* _maxwalkspeed (* (`self.Mutation Level`) (`self.SpeedMultiplier`)))))
  (set `CharacterMovementComponent.MaxWalkSpeed` (+ _maxwalkspeed _output_get) _charactermovement)
  (`KismetSystemLibrary.K2_SetTimerDelegate` (delegate `RemoveBuff`) (`self.BuffTime`)))

(event `RemoveBuff`
  (bind _charactermovement (`Character.CharacterMovement` (`self.OwnerEnemyCast`)))
  (set `CharacterMovementComponent.MaxWalkSpeed` (- (`CharacterMovementComponent.MaxWalkSpeed` _charactermovement) (`self.StatAdded`)) _charactermovement)
  (`self.K2_DestroyComponent`))