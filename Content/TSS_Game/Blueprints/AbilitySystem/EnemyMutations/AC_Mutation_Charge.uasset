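; AC_Mutation_Charge is an enemy mutation component that gives its owning BP_Enemy_BASE a temporary charge speed buff.
; On BeginPlay it raises max walk speed in proportion to mutation level, adds flat acceleration, and attaches a red Niagara effect to the head socket.
; A timer then subtracts the stored bonuses, clears the enemy's IsCharging flag, and destroys both the effect and the component.
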(event `self.ReceiveBeginPlay`
  (bind _asbp_enemy_base (cast `/Game/TSS_Game/Blueprints/Bonus/AI/BP_Enemy_BASE` (`self.GetOwner`)))
  (set `self.OwnerEnemyCast` _asbp_enemy_base)
  (bind _charactermovement (`Character.CharacterMovement` _asbp_enemy_base))
  (bind _maxwalkspeed (`CharacterMovementComponent.MaxWalkSpeed` _charactermovement))
  (bind _output_get (set `self.SpeedAdded` (* _maxwalkspeed (* (`self.Mutation Level`) (`self.SpeedMultiplier`)))))
  (set `CharacterMovementComponent.MaxWalkSpeed` (+ _maxwalkspeed _output_get) _charactermovement)
  (set `CharacterMovementComponent.MaxAcceleration` (+ (`CharacterMovementComponent.MaxAcceleration` _charactermovement) (`self.AccelerationAdded`)) _charactermovement)
  (`KismetSystemLibrary.K2_SetTimerDelegate` (delegate `RemoveBuff`) (`self.BuffTime`))
  (bind _returnvalue (`NiagaraFunctionLibrary.SpawnSystemAttached` "/Game/VFX/PowerUps/N_floatingToCenter_red.N_floatingToCenter_red" (`Character.Mesh` (`self.OwnerEnemyCast`)) "HeadSocket" (0.0 0.0 0.0) (struct) "SnapToTarget"))
  (set `self.AttachedNiagara` _returnvalue))

(event `RemoveBuff`
  (bind _charactermovement (`Character.CharacterMovement` (`self.OwnerEnemyCast`)))
  (set `CharacterMovementComponent.MaxWalkSpeed` (- (`CharacterMovementComponent.MaxWalkSpeed` _charactermovement) (`self.SpeedAdded`)) _charactermovement)
  (set `CharacterMovementComponent.MaxAcceleration` (- (`CharacterMovementComponent.MaxAcceleration` _charactermovement) (`self.AccelerationAdded`)) _charactermovement)
  (set `/Game/TSS_Game/Blueprints/Bonus/AI/BP_Enemy_BASE.IsCharging` false (`self.OwnerEnemyCast`))
  (`self.K2_DestroyComponent` (`self.AttachedNiagara`))
  (`self.K2_DestroyComponent`))