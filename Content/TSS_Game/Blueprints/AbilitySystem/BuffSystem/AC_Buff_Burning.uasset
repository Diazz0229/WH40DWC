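; Burning buff component that applies damage over time and a walk-speed debuff to the buffed actor.
; On BeginPlay it scales an enemy's speed change by buff level, attaches fire Niagara, and enables damage only where the local player controls the actor's or buff owner's instigator.
; Each activation tick routes random, crit-capable damage through that PlayerController, or destroys the buff if the target is Dead, reversing the stored speed change.
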(event `self.ReceiveBeginPlay`
  (bind _buffedactor (`self.BuffedActor`))
  (bind _buffowner (`self.BuffOwner`))
  (bind _returnvalue (`Pawn.GetController` (`Actor.Instigator` _buffedactor)))
  (bind _returnvalue_2 (`Pawn.GetController` (`Actor.Instigator` _buffowner)))
  (`parent.ReceiveBeginPlay`)
  (`/Engine/EditorBlueprintResources/StandardMacros.IsValid` _buffedactor
    (:`Is Valid`
      (`self.ApplySpeedDebuff`)
      (`/Engine/EditorBlueprintResources/StandardMacros.IsValid` _returnvalue
        (:`Is Valid`
          (if (== (`GameplayStatics.GetPlayerController` 0) _returnvalue)
            (set `self.ShouldDealDamage?` true :!label _label)
            (bind _asbp_player_controller (cast `/Game/TSS_Game/Blueprints/System/BP_PlayerController` (`GameplayStatics.GetPlayerController` 0)))
            (set `self.LocalPlayerController` _asbp_player_controller)
            (else
              (`/Engine/EditorBlueprintResources/StandardMacros.IsValid` _buffowner :!label _label_2
                (:`Is Valid`
                  (`/Engine/EditorBlueprintResources/StandardMacros.IsValid` _returnvalue_2
                    (:`Is Valid`
                      (if (== _returnvalue_2 (`GameplayStatics.GetPlayerController` 0))
                        (goto _label)))))))))
        (:`Is Not Valid`
          (goto _label_2))))))

(event `ApplySpeedDebuff`
  ;[1 1 1] Speed penalty
  (bind _asbp_enemy_base (cast `/Game/TSS_Game/Blueprints/Bonus/AI/BP_Enemy_BASE` (`self.BuffedActor`)))
  (bind _charactermovement (`Character.CharacterMovement` _asbp_enemy_base))
  (bind _maxwalkspeed (`CharacterMovementComponent.MaxWalkSpeed` _charactermovement))
  (bind _output_get (set `self.ResultedDebuff` (* _maxwalkspeed (* (`self.BuffLevel`) (`self.SpeedDebuff`)))))
  (set `CharacterMovementComponent.MaxWalkSpeed` (+ _output_get _maxwalkspeed) _charactermovement)
  (bind _returnvalue (`NiagaraFunctionLibrary.SpawnSystemAttached` "/Game/M5VFXVOL2/Niagara/Fire/NFire_03.NFire_03" (`Actor.RootComponent` (`self.BuffedActor`)) "None" (0.0 0.0 0.0) (struct) "KeepRelativeOffset"))
  (set `self.ShownNiagara` _returnvalue))

(event `self.ActivateTick`
  (bind _buffedactor (`self.BuffedActor`))
  (bind _localplayercontroller (`self.LocalPlayerController`))
  (`/Engine/EditorBlueprintResources/StandardMacros.IsValid` _localplayercontroller
    (:`Is Valid`
      (if (`self.ShouldDealDamage?`)
        (if (`Actor.ActorHasTag` (`self.BuffedActor`) "Dead")
          (`self.DestroyBuff`)
          (else
            (bind _asbp_character_base (cast `/Game/TSS_Game/Blueprints/System/BP_CharacterBase` (`self.BuffOwner`))
              (:`then`
                (`self.CheckCritAndDealDamage` _buffedactor _localplayercontroller _asbp_character_base))
              (:`CastFailed`
                (`self.CheckCritAndDealDamage` _buffedactor _localplayercontroller)))))))))

(event `DestroySpeedBuff`
  ;[1 1 1] Speed penalty
  (bind _asbp_enemy_base (cast `/Game/TSS_Game/Blueprints/Bonus/AI/BP_Enemy_BASE` (`self.BuffedActor`)))
  (bind _charactermovement (`Character.CharacterMovement` _asbp_enemy_base))
  (set `CharacterMovementComponent.MaxWalkSpeed` (- (`CharacterMovementComponent.MaxWalkSpeed` _charactermovement) (`self.ResultedDebuff`)) _charactermovement))

(event `self.DestroyBuff`
  (`self.DestroySpeedBuff`)
  (`parent.DestroyBuff`))

(fn `CheckCritAndDealDamage`
  (params (DamageTarget :type "Actor Object Reference") (`Pl Controller` :type "/Game/TSS_Game/Blueprints/System/BP_PlayerController Object Reference") (Source :type "/Game/TSS_Game/Blueprints/System/BP_CharacterBase Object Reference"))
  (if (<= (`KismetMathLibrary.RandomFloatInRange` 0.0 100.0) (`self.CritChance`))
    (`/Game/TSS_Game/Blueprints/System/BP_PlayerController.DealDamage` `Pl Controller` DamageTarget (* (`KismetMathLibrary.RandomFloatInRange` (`self.DamageMin`) (`self.DamageMax`)) (`self.CritMultiplier`)) Source true (`self.DamageType`) 0.0 0.0)
    (else
      (`/Game/TSS_Game/Blueprints/System/BP_PlayerController.DealDamage` `Pl Controller` DamageTarget (`KismetMathLibrary.RandomFloatInRange` (`self.DamageMin`) (`self.DamageMax`)) Source false (`self.DamageType`) 0.0 0.0))))