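; Base buff component for the ability system, attached to the actor it affects and meant to be subclassed for specific buffs.
; On BeginPlay it caches its owner and starts optional timers: a looping activation tick and a one-shot expiry padded slightly past the buff duration.
; Expiry removes any Cascade or Niagara effect and notifies the owner to detach the buff.
; Tick, activate, attach-request and detach events are empty hooks.
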(event `self.ReceiveBeginPlay`
  (bind _bufftime (`self.BuffTime`))
  (bind _buffactivatetime (`self.BuffActivateTime`))
  (set `self.BuffedActor` (`self.GetOwner`))
  (if (> _bufftime 0.0)
    (`KismetSystemLibrary.K2_SetTimerDelegate` (delegate `DestroyBuff`) (+ _bufftime 0.2)))
  (if (> _buffactivatetime 0.0)
    (`KismetSystemLibrary.K2_SetTimerDelegate` (delegate `ActivateTick`) _buffactivatetime true)))

(event `ActivateTick`)

(event `DestroyBuff`
  (bind _showncascade (`self.ShownCascade`))
  (bind _shownniagara (`self.ShownNiagara`))
  (`/Engine/EditorBlueprintResources/StandardMacros.IsValid` _showncascade
    (:`Is Valid`
      (`self.K2_DestroyComponent` _showncascade))
    (:`Is Not Valid`
      _))
  (`/Engine/EditorBlueprintResources/StandardMacros.IsValid` _shownniagara
    (:`Is Valid`
      (`self.K2_DestroyComponent` _shownniagara))
    (:`Is Not Valid`
      _))
  (message `/Game/TSS_Game/Blueprints/AbilitySystem/BuffSystem/Base/BPI_Buffable.DetachBuff` (`self.BuffedActor`) self))

(event `/Game/TSS_Game/Blueprints/AbilitySystem/BuffSystem/Base/BPI_Buffable.DetachBuff`
  (params (Buff :type "/Game/TSS_Game/Blueprints/AbilitySystem/BuffSystem/Base/AC_Buff_BASE Object Reference")))

(event `/Game/TSS_Game/Blueprints/AbilitySystem/BuffSystem/Base/BPI_Buffable.ActivateBuff`
  (params (Buff :type "/Game/TSS_Game/Blueprints/AbilitySystem/BuffSystem/Base/AC_Buff_BASE Class Reference")))

(event `/Game/TSS_Game/Blueprints/AbilitySystem/BuffSystem/Base/BPI_Buffable.Attach Buff Request`
  (params (`Buff Settings` :type "/Game/TSS_Game/Blueprints/AbilitySystem/BuffSystem/ST_BuffSettingsMSG Structure")))