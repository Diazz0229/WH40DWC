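; Bleeding buff component that attaches a bleeding Niagara effect to the buffed actor and deals damage over time.
; On BeginPlay it enables damage only if the local player's controller is behind the buffed actor or, failing that, the buff owner.
; Each ActivateTick then sends a random damage amount within the configured range as a multicast damage message, crediting the buff owner as source.
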(event `self.ReceiveBeginPlay`
  (bind _buffedactor (`self.BuffedActor`))
  (bind _buffowner (`self.BuffOwner`))
  (bind _returnvalue (`Pawn.GetController` (`Actor.Instigator` _buffedactor)))
  (bind _returnvalue_2 (`Pawn.GetController` (`Actor.Instigator` _buffowner)))
  (`parent.ReceiveBeginPlay`)
  (bind _returnvalue_3 (`NiagaraFunctionLibrary.SpawnSystemAttached` "/Game/VFX/PowerUps/N_Bleeding.N_Bleeding" (`Actor.RootComponent` (`self.BuffedActor`)) "None" (0.0 0.0 100.0) (struct) "KeepRelativeOffset" true))
  (set `self.ShownNiagara` _returnvalue_3)
  (`/Engine/EditorBlueprintResources/StandardMacros.IsValid` _buffedactor
    (:`Is Valid`
      (`/Engine/EditorBlueprintResources/StandardMacros.IsValid` _buffedactor
        (:`Is Valid`
          (`/Engine/EditorBlueprintResources/StandardMacros.IsValid` _returnvalue
            (:`Is Valid`
              (if (== (`GameplayStatics.GetPlayerController` 0) _returnvalue)
                (set `self.ShouldDealDamage?` true :!label _label)
                (bind _asbp_player_controller (cast `/Game/TSS_Game/Blueprints/System/BP_PlayerController` (`GameplayStatics.GetPlayerController` 0)))
                (set `self.LocalPlayerController` _asbp_player_controller)
                (else
                  (`/Engine/EditorBlueprintResources/StandardMacros.IsValid` _buffowner :!label _label_2
                    (:`Is Valid`
                      (`/Engine/EditorBlueprintResources/StandardMacros.IsValid` _returnvalue_2
                        (:`Is Valid`
                          (if (== _returnvalue_2 (`GameplayStatics.GetPlayerController` 0))
                            (goto _label)))))))))
            (:`Is Not Valid`
              (goto _label_2))))))))

(event `self.ActivateTick`
  (`/Engine/EditorBlueprintResources/StandardMacros.IsValid` (`self.LocalPlayerController`)
    (:`Is Valid`
      (if (`self.ShouldDealDamage?`)
        (message `/Game/TSS_Game/Blueprints/System/BPI_Damagable.DamageIntercation` (`self.BuffedActor`) (`KismetMathLibrary.RandomFloatInRange` (`self.DamageMin`) (`self.DamageMax`)) (`self.BuffOwner`) true (`self.DamageType`))))))