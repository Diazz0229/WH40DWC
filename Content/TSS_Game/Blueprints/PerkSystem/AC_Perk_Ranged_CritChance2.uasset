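; Ranged perk component that raises the critical hit chance of a character's weapons.
; AttachPerk calls the parent implementation, then adds a flat bonus directly to CritChance on each valid primary and secondary weapon.
; The bonus is a one-time change to the weapons held at attach time, with no removal or reapplication logic in this graph.
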(event `self.AttachPerk`
  (params (CharacterRef :type "/Game/TSS_Game/Blueprints/System/BP_CharacterBase Object Reference"))
  (bind _wpn_primary (`/Game/TSS_Game/Blueprints/System/BP_CharacterBase.WPN_Primary` CharacterRef))
  (bind _wpn_secondary (`/Game/TSS_Game/Blueprints/System/BP_CharacterBase.WPN_Secondary` CharacterRef))
  (`parent.AttachPerk` CharacterRef)
  (`/Engine/EditorBlueprintResources/StandardMacros.IsValid` _wpn_primary
    (:`Is Valid`
      (set `/Game/TSS_Game/Blueprints/Weapons/Base/BP_WeaponBase.CritChance` (+ (`/Game/TSS_Game/Blueprints/Weapons/Base/BP_WeaponBase.CritChance` _wpn_primary) 2.0) _wpn_primary))
    (:`Is Not Valid`
      _))
  (`/Engine/EditorBlueprintResources/StandardMacros.IsValid` _wpn_secondary
    (:`Is Valid`
      (set `/Game/TSS_Game/Blueprints/Weapons/Base/BP_WeaponBase.CritChance` (+ (`/Game/TSS_Game/Blueprints/Weapons/Base/BP_WeaponBase.CritChance` _wpn_secondary) 2.0) _wpn_secondary))))