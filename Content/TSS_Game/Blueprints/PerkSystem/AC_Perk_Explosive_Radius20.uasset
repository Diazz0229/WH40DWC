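; Perk component that increases explosive effect radius by 20% for the character it attaches to.
; On AttachPerk it calls the parent, then scans the character's equipment slots, UT inventory, and valid primary and secondary weapons for a matching perk class tag.
; Matching equipment gets its ActiveRadius multiplied, while inventory items and weapons get their SplashRadius multiplied.
; The change is applied directly at attach time, with no revert logic in this graph.
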(event `self.AttachPerk`
  (params (CharacterRef :type "/Game/TSS_Game/Blueprints/System/BP_CharacterBase Object Reference"))
  (bind _temp_aceqpbaseref (`self.TEMP_ACEQPBaseRef`))
  (bind _wpn_primary (`/Game/TSS_Game/Blueprints/System/BP_CharacterBase.WPN_Primary` CharacterRef))
  (bind _wpn_secondary (`/Game/TSS_Game/Blueprints/System/BP_CharacterBase.WPN_Secondary` CharacterRef))
  (`parent.AttachPerk` CharacterRef)
  (for _array_element (`/Game/TSS_Game/Blueprints/System/BP_CharacterBase.EQP_Slots` CharacterRef)
    (bind _asac_eqp_base (cast `/Game/TSS_Game/Blueprints/Equipment/AC_EQP_Base` _array_element))
    (bind _output_get (set `self.TEMP_ACEQPBaseRef` _asac_eqp_base))
    (if (`KismetArrayLibrary.Array_Contains` (`/Game/TSS_Game/Blueprints/Equipment/AC_EQP_Base.PerkClasses` _output_get) "NewEnumerator13")
      (set `/Game/TSS_Game/Blueprints/Equipment/AC_EQP_Base.ActiveRadius` (* (`/Game/TSS_Game/Blueprints/Equipment/AC_EQP_Base.ActiveRadius` _temp_aceqpbaseref) 1.2) _temp_aceqpbaseref)))
  (for _array_element_2 (`/Game/TSS_Game/Blueprints/System/BP_CharacterBase.UT_Inventory` CharacterRef)
    (if (`KismetArrayLibrary.Array_Contains` (`/Game/TSS_Game/Blueprints/Weapons/Base/BP_WeaponBase.PerkClasses` _array_element_2) "NewEnumerator13")
      (set `/Game/TSS_Game/Blueprints/Weapons/Base/BP_WeaponBase.Splash Radius` (* (`/Game/TSS_Game/Blueprints/Weapons/Base/BP_WeaponBase.Splash Radius` _array_element_2) 1.2) _array_element_2)))
  (`/Engine/EditorBlueprintResources/StandardMacros.IsValid` _wpn_primary
    (:`Is Valid`
      (if (`KismetArrayLibrary.Array_Contains` (`/Game/TSS_Game/Blueprints/Weapons/Base/BP_WeaponBase.PerkClasses` _wpn_primary) "NewEnumerator13")
        (set `/Game/TSS_Game/Blueprints/Weapons/Base/BP_WeaponBase.Splash Radius` (* (`/Game/TSS_Game/Blueprints/Weapons/Base/BP_WeaponBase.Splash Radius` _wpn_primary) 1.2) _wpn_primary)))
    (:`Is Not Valid`
      _))
  (`/Engine/EditorBlueprintResources/StandardMacros.IsValid` _wpn_secondary
    (:`Is Valid`
      (if (`KismetArrayLibrary.Array_Contains` (`/Game/TSS_Game/Blueprints/Weapons/Base/BP_WeaponBase.PerkClasses` _wpn_secondary) "NewEnumerator13")
        (set `/Game/TSS_Game/Blueprints/Weapons/Base/BP_WeaponBase.Splash Radius` (* (`/Game/TSS_Game/Blueprints/Weapons/Base/BP_WeaponBase.Splash Radius` _wpn_secondary) 1.2) _wpn_secondary)))))