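; Perk component that turns the owning character's primary weapon into a Dragonfire weapon with area-of-effect splash, paired with a 30% damage reduction for one damage class.
; On attach, it runs the parent attach logic and applies the class-based damage change through the character.
; If a primary weapon is valid, it swaps in the Dragonfire projectile and red shotgun shell, enlarges the splash radius, and tags the weapon with a perk class.
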(event `self.AttachPerk`
  (params (CharacterRef :type "/Game/TSS_Game/Blueprints/System/BP_CharacterBase Object Reference"))
  (bind _wpn_primary (`/Game/TSS_Game/Blueprints/System/BP_CharacterBase.WPN_Primary` CharacterRef))
  (`parent.AttachPerk` CharacterRef)
  (`/Game/TSS_Game/Blueprints/System/BP_CharacterBase.Perks_ChangeAllDamageByClass` CharacterRef "NewEnumerator30" -0.3)
  (`/Engine/EditorBlueprintResources/StandardMacros.IsValid` _wpn_primary
    (:`Is Valid`
      (set `/Game/TSS_Game/Blueprints/Weapons/Base/BP_WeaponBase.ProjectileToFire` "/Game/TSS_Game/Blueprints/Weapons/Base/BP_ProjectileDragonfire.BP_ProjectileDragonfire_C" _wpn_primary)
      (set `/Game/TSS_Game/Blueprints/Weapons/Base/BP_WeaponBase.ShellType` "/Game/TSS_Game/Blueprints/Weapons/Base/BP_ShellShotgun_red.BP_ShellShotgun_red_C" _wpn_primary)
      (set `/Game/TSS_Game/Blueprints/Weapons/Base/BP_WeaponBase.Splash Radius` (+ (`/Game/TSS_Game/Blueprints/Weapons/Base/BP_WeaponBase.Splash Radius` _wpn_primary) 150.0) _wpn_primary)
      (`KismetArrayLibrary.Array_AddUnique` (`/Game/TSS_Game/Blueprints/Weapons/Base/BP_WeaponBase.PerkClasses` _wpn_primary) "NewEnumerator13"))))