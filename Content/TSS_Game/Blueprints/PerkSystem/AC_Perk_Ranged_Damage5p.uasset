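; Perk component that raises a character's ranged weapon damage by five percent when attached.
; On AttachPerk it calls the parent, then adds five percent of each weapon's default minimum and maximum damage to the current values of the primary and secondary weapons.
; The bonus is based on the default values rather than the current ones, so it adds flatly instead of compounding.
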(event `self.AttachPerk`
  (params (CharacterRef :type "/Game/TSS_Game/Blueprints/System/BP_CharacterBase Object Reference"))
  (bind _wpn_secondary (`/Game/TSS_Game/Blueprints/System/BP_CharacterBase.WPN_Secondary` CharacterRef))
  (bind _wpn_primary (`/Game/TSS_Game/Blueprints/System/BP_CharacterBase.WPN_Primary` CharacterRef))
  (`parent.AttachPerk` CharacterRef)
  (set `/Game/TSS_Game/Blueprints/Weapons/Base/BP_WeaponBase.DamageMin` (+ (`/Game/TSS_Game/Blueprints/Weapons/Base/BP_WeaponBase.DamageMin` _wpn_primary) (* (`/Game/TSS_Game/Blueprints/Weapons/Base/BP_WeaponBase.DamageMin_Default` _wpn_primary) 0.05)) _wpn_primary)
  (set `/Game/TSS_Game/Blueprints/Weapons/Base/BP_WeaponBase.DamageMax` (+ (`/Game/TSS_Game/Blueprints/Weapons/Base/BP_WeaponBase.DamageMax` _wpn_primary) (* (`/Game/TSS_Game/Blueprints/Weapons/Base/BP_WeaponBase.DamageMax_Default` _wpn_primary) 0.05)) _wpn_primary)
  (set `/Game/TSS_Game/Blueprints/Weapons/Base/BP_WeaponBase.DamageMin` (+ (`/Game/TSS_Game/Blueprints/Weapons/Base/BP_WeaponBase.DamageMin` _wpn_secondary) (* (`/Game/TSS_Game/Blueprints/Weapons/Base/BP_WeaponBase.DamageMin_Default` _wpn_secondary) 0.05)) _wpn_secondary)
  (set `/Game/TSS_Game/Blueprints/Weapons/Base/BP_WeaponBase.DamageMax` (+ (`/Game/TSS_Game/Blueprints/Weapons/Base/BP_WeaponBase.DamageMax` _wpn_secondary) (* (`/Game/TSS_Game/Blueprints/Weapons/Base/BP_WeaponBase.DamageMax_Default` _wpn_secondary) 0.05)) _wpn_secondary))