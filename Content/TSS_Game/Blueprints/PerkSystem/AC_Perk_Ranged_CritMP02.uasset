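; Perk component that grants a ranged critical hit multiplier bonus to the character it attaches to.
; On AttachPerk it runs the parent attach logic, then adds a flat amount to CritMultiplier on the character's primary and secondary weapons, skipping any that are not valid.
; The bonus is applied directly to the weapon instances present at attach time.
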(event `self.AttachPerk`
  (params (CharacterRef :type "/Game/TSS_Game/Blueprints/System/BP_CharacterBase Object Reference"))
  (bind _wpn_primary (`/Game/TSS_Game/Blueprints/System/BP_CharacterBase.WPN_Primary` CharacterRef))
  (bind _wpn_secondary (`/Game/TSS_Game/Blueprints/System/BP_CharacterBase.WPN_Secondary` CharacterRef))
  (`parent.AttachPerk` CharacterRef)
  (`/Engine/EditorBlueprintResources/StandardMacros.IsValid` _wpn_primary
    (:`Is Valid`
      (set `/Game/TSS_Game/Blueprints/Weapons/Base/BP_WeaponBase.CritMultiplier` (+ (`/Game/TSS_Game/Blueprints/Weapons/Base/BP_WeaponBase.CritMultiplier` _wpn_primary) 0.2) _wpn_primary))
    (:`Is Not Valid`
      _))
  (`/Engine/EditorBlueprintResources/StandardMacros.IsValid` _wpn_secondary
    (:`Is Valid`
      (set `/Game/TSS_Game/Blueprints/Weapons/Base/BP_WeaponBase.CritMultiplier` (+ (`/Game/TSS_Game/Blueprints/Weapons/Base/BP_WeaponBase.CritMultiplier` _wpn_secondary) 0.2) _wpn_secondary))))