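; AC_Perk_Resist_Ranged3 is a perk component that raises the owning character's resistance to a damage type, by its name the third tier of ranged resistance.
; On AttachPerk it calls the parent, then searches the character's DamageResistances for the entry matching ResistToChange.
; It adds ResistancePercentAdded to that entry's percent, writes the struct back and stops; with no matching entry, nothing changes.
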(event `self.AttachPerk`
  (params (CharacterRef :type "/Game/TSS_Game/Blueprints/System/BP_CharacterBase Object Reference"))
  (bind _damageresistances (`/Game/TSS_Game/Blueprints/System/BP_CharacterBase.DamageResistances` CharacterRef))
  (bind _resisttochange (`self.ResistToChange`))
  (`parent.AttachPerk` CharacterRef)
  (for (_array_element _array_index) _damageresistances
    (bind (_damagetyperesistance _resistancepercent) (break `/Game/TSS_Game/Blueprints/Weapons/ST_DamageResistance` _array_element))
    (if (`|EnumEquality` _damagetyperesistance _resisttochange)
      (`KismetArrayLibrary.Array_Set` _damageresistances _array_index (make `/Game/TSS_Game/Blueprints/Weapons/ST_DamageResistance` _resisttochange (+ _resistancepercent (`self.ResistancePercentAdded`))))
      (break))))