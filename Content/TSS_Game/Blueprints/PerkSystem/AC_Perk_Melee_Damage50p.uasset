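; Perk component that raises the owning character's melee weapon damage by 50 percent.
; On AttachPerk it calls the parent attach logic, then adds half of the melee weapon's default minimum and maximum damage to the current values.
; Because the bonus is based on the default values rather than the current ones, it adds linearly to other damage modifiers instead of compounding.
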(event `self.AttachPerk`
  (params (CharacterRef :type "/Game/TSS_Game/Blueprints/System/BP_CharacterBase Object Reference"))
  (bind _wpn_melee (`/Game/TSS_Game/Blueprints/System/BP_CharacterBase.WPN_Melee` CharacterRef))
  (`parent.AttachPerk` CharacterRef)
  (set `/Game/TSS_Game/Blueprints/Weapons/Base/BP_WeaponBase.DamageMin` (+ (`/Game/TSS_Game/Blueprints/Weapons/Base/BP_WeaponBase.DamageMin` _wpn_melee) (* (`/Game/TSS_Game/Blueprints/Weapons/Base/BP_WeaponBase.DamageMin_Default` _wpn_melee) 0.5)) _wpn_melee)
  (set `/Game/TSS_Game/Blueprints/Weapons/Base/BP_WeaponBase.DamageMax` (+ (`/Game/TSS_Game/Blueprints/Weapons/Base/BP_WeaponBase.DamageMax` _wpn_melee) (* (`/Game/TSS_Game/Blueprints/Weapons/Base/BP_WeaponBase.DamageMax_Default` _wpn_melee) 0.5)) _wpn_melee))