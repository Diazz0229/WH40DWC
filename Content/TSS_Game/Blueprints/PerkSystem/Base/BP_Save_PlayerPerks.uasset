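; Save object for player perks that keeps the list of unlocked perk row names.
; InitBasePerks scans DT_PerksList and adds every row flagged IsBase to that list without duplicates.
; A workaround lookup function finds an equipment row by name by trying six weapon, equipment and chapter tables in turn, printing an error when none match.
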(event `InitBasePerks`
  (bind _outrownames (`DataTableFunctionLibrary.GetDataTableRowNames` "/Game/TSS_Game/Blueprints/PerkSystem/Base/DT_PerksList.DT_PerksList"))
  (for _array_element _outrownames
    (bind _returnvalue (`|GetDataTableRow` "/Game/TSS_Game/Blueprints/PerkSystem/Base/DT_PerksList.DT_PerksList" _array_element)
      (:`then`
        (if (`.IsBase_29_9A62C66B4C205D8FBE2E2EAF1EE5EBA0` (break `/Game/TSS_Game/Blueprints/PerkSystem/Base/ST_PerkInfo` _returnvalue))
          (`KismetArrayLibrary.Array_AddUnique` (`self.UnlockedPerkRowNames`) _array_element))))))

(fn `F_GetEquipmentTableRow_Workaround`
  (params (RowName :type Name))
  (returns (`ST Equipment` :type "/Game/TSS_Game/Blueprints/Customization/ST_Equipment_Item Structure"))
  (bind _returnvalue (`|GetDataTableRow` "/Game/TSS_Game/Blueprints/Customization/DT_EQP_WPN_Primary.DT_EQP_WPN_Primary" RowName)
    (:`then`
      (return _returnvalue))
    (:`RowNotFound`
      (bind _returnvalue_2 (`|GetDataTableRow` "/Game/TSS_Game/Blueprints/Customization/DT_EQP_WPN_SecondaryMelee.DT_EQP_WPN_SecondaryMelee" RowName)
        (:`then`
          (return _returnvalue_2))
        (:`RowNotFound`
          (bind _returnvalue_3 (`|GetDataTableRow` "/Game/TSS_Game/Blueprints/Customization/DT_EQP_Equipment.DT_EQP_Equipment" RowName)
            (:`then`
              (return _returnvalue_3))
            (:`RowNotFound`
              (bind _returnvalue_4 (`|GetDataTableRow` "/Game/TSS_Game/Blueprints/Customization/DT_EQP_Chapter.DT_EQP_Chapter" RowName)
                (:`then`
                  (return _returnvalue_4))
                (:`RowNotFound`
                  (bind _returnvalue_5 (`|GetDataTableRow` "/Game/TSS_Game/Blueprints/Customization/DT_EQP_ChapOther.DT_EQP_ChapOther" RowName)
                    (:`then`
                      (return _returnvalue_5))
                    (:`RowNotFound`
                      (bind _returnvalue_6 (`|GetDataTableRow` "/Game/TSS_Game/Blueprints/Customization/DT_EQP_WPN_SecondaryPistols.DT_EQP_WPN_SecondaryPistols" RowName)
                        (:`then`
                          (return _returnvalue_6))
                        (:`RowNotFound`
                          (`KismetSystemLibrary.PrintString` null "BP_Save_PlayerCust: Could not get player equipment from any table!" true true (struct :`R` 1.0 :`A` 1.0) 4.0))))))))))))))