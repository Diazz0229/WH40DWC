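; SaveGame object that stores unlocked perks and achievement counters.
; InitBasePerks stores the slot name and unlocks perks flagged as base in DT_PerksList.
; When achievement counts differ from DT_AchievementsList, InitAchievmentsList appends missing rows with zeroed counters, keeping existing progress, then refreshes the name list and saves itself.
; A workaround helper, uncalled here, finds equipment rows by searching six DataTables in sequence.
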(event `InitBasePerks`
  (params (SavePerksSlotName :type String))
  (set `self.SavePerksSlotName` SavePerksSlotName)
  (bind _outrownames (`DataTableFunctionLibrary.GetDataTableRowNames` "/Game/TSS_Game/Blueprints/PerkSystem/Base/DT_PerksList.DT_PerksList"))
  (for _array_element _outrownames
    (bind _returnvalue (`|GetDataTableRow` "/Game/TSS_Game/Blueprints/PerkSystem/Base/DT_PerksList.DT_PerksList" _array_element)
      (:`then`
        (if (`.IsBase_29_9A62C66B4C205D8FBE2E2EAF1EE5EBA0` (break `/Game/TSS_Game/Blueprints/PerkSystem/Base/ST_PerkInfo` _returnvalue))
          (`KismetArrayLibrary.Array_AddUnique` (`self.UnlockedPerkRowNames`) _array_element))))))

(event `InitAchievmentsList`
  (params (SaveVersion :type Integer))
  (set `self.SaveVersion` SaveVersion)
  (bind _outrownames (`DataTableFunctionLibrary.GetDataTableRowNames` "/Game/TSS_Game/Blueprints/AchievementSystem/DT_AchievementsList.DT_AchievementsList"))
  (if (not (== (`KismetArrayLibrary.Array_Length` _outrownames) (`KismetArrayLibrary.Array_Length` (`self.Ach_Counters`))))
    (`self.F_MergeOldAndNewAchievments`)
    (`KismetArrayLibrary.Array_Clear` (`self.Ach_Namelist`))
    (for (_array_element _array_index) (`self.Ach_Counters`)
      (`KismetArrayLibrary.Array_Set` (`self.Ach_Namelist`) _array_index (`.AchRowName_2_DA82240E4D4BE977A08B7DBBBC6C3FC1` (break `/Game/TSS_Game/Blueprints/AchievementSystem/ST_AchCounters` _array_element)) true))
    (`GameplayStatics.SaveGameToSlot` self (`self.SavePerksSlotName`))))

(fn `F_GetEquipmentTableRow_Workaround`
  (params (RowName :type Name))
  (returns (`ST Equipment` :type "/Game/TSS_Game/Blueprints/Customization/ST_EQP_Item Structure"))
  (bind _returnvalue (`|GetDataTableRow` "/Game/TSS_Game/Blueprints/Customization/DT_EQP_WPN_Primary.DT_EQP_WPN_Primary" RowName)
    (:`then`
      (return _returnvalue))
    (:`RowNotFound`
      (bind _returnvalue_2 (`|GetDataTableRow` "/Game/TSS_Game/Blueprints/Customization/DT_EQP_WPN_SecondaryMelee.DT_EQP_WPN_SecondaryMelee" RowName)
        (:`then`
          (return _returnvalue_2))
        (:`RowNotFound`
          (bind _returnvalue_3 (`|GetDataTableRow` "/Game/TSS_Game/Blueprints/Customization/DT_EQP_Equipment.DT_EQP_Equipment" RowName)
            (:`then`
              (return _returnvalue_3))
            (:`RowNotFound`
              (bind _returnvalue_4 (`|GetDataTableRow` "/Game/TSS_Game/Blueprints/Customization/DT_EQP_Chapter.DT_EQP_Chapter" RowName)
                (:`then`
                  (return _returnvalue_4))
                (:`RowNotFound`
                  (bind _returnvalue_5 (`|GetDataTableRow` "/Game/TSS_Game/Blueprints/Customization/DT_EQP_ChapOther.DT_EQP_ChapOther" RowName)
                    (:`then`
                      (return _returnvalue_5))
                    (:`RowNotFound`
                      (bind _returnvalue_6 (`|GetDataTableRow` "/Game/TSS_Game/Blueprints/Customization/DT_EQP_WPN_SecondaryPistols.DT_EQP_WPN_SecondaryPistols" RowName)
                        (:`then`
                          (return _returnvalue_6))
                        (:`RowNotFound`
                          (`KismetSystemLibrary.PrintString` null "BP_Save_PlayerCust: Could not get player equipment from any table!" true true (struct :`R` 1.0 :`A` 1.0) 4.0))))))))))))))

(fn `F_MergeOldAndNewAchievments`
  (returns (`Success?` :type Boolean))
  (locals (AllCurAchNames :type "Array of Name"))
  (bind _outrownames (`DataTableFunctionLibrary.GetDataTableRowNames` "/Game/TSS_Game/Blueprints/AchievementSystem/DT_AchievementsList.DT_AchievementsList"))
  (bind _output_get (set `local.AllCurAchNames` _outrownames))
  (for _array_element (`self.Ach_Counters`)
    (bind _achrowname (break `/Game/TSS_Game/Blueprints/AchievementSystem/ST_AchCounters` _array_element))
    (if (`KismetArrayLibrary.Array_Contains` _output_get _achrowname)
      (`KismetArrayLibrary.Array_RemoveItem` (`local.AllCurAchNames`) _achrowname)))
  (for _array_element_2 (`local.AllCurAchNames`)
    (bind _returnvalue (`|GetDataTableRow` "/Game/TSS_Game/Blueprints/AchievementSystem/DT_AchievementsList.DT_AchievementsList" _array_element_2)
      (:`then`
        (`KismetArrayLibrary.Array_AddUnique` (`self.Ach_Counters`) (make `/Game/TSS_Game/Blueprints/AchievementSystem/ST_AchCounters` _array_element_2 0 (`.AchCounter_12_90B628D44146A182103C13BC12D4BEBC` (break `/Game/TSS_Game/Blueprints/AchievementSystem/ST_AchievementInfo` _returnvalue)))))))
  (return true))