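; Stalker perk component that trades primary weapon damage for extra target penetration.
; On attach, it calls the parent perk logic, then, if the character's primary weapon is valid, lets it pierce three more targets.
; It also lowers minimum and maximum damage by 15% of their default values, subtracting from current values rather than scaling them.
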(event `self.AttachPerk`
  (params (CharacterRef :type "/Game/TSS_Game/Blueprints/System/BP_CharacterBase Object Reference"))
  (bind _wpn_primary (`/Game/TSS_Game/Blueprints/System/BP_CharacterBase.WPN_Primary` CharacterRef))
  (`parent.AttachPerk` CharacterRef)
  (`/Engine/EditorBlueprintResources/StandardMacros.IsValid` _wpn_primary
    (:`Is Valid`
      (set `/Game/TSS_Game/Blueprints/Weapons/Base/BP_WeaponBase.PiercedTargets` (+ (`/Game/TSS_Game/Blueprints/Weapons/Base/BP_WeaponBase.PiercedTargets` _wpn_primary) 3) _wpn_primary)
      (set `/Game/TSS_Game/Blueprints/Weapons/Base/BP_WeaponBase.DamageMin` (- (`/Game/TSS_Game/Blueprints/Weapons/Base/BP_WeaponBase.DamageMin` _wpn_primary) (* (`/Game/TSS_Game/Blueprints/Weapons/Base/BP_WeaponBase.DamageMin_Default` _wpn_primary) 0.15)) _wpn_primary)
      (set `/Game/TSS_Game/Blueprints/Weapons/Base/BP_WeaponBase.DamageMax` (- (`/Game/TSS_Game/Blueprints/Weapons/Base/BP_WeaponBase.DamageMax` _wpn_primary) (* (`/Game/TSS_Game/Blueprints/Weapons/Base/BP_WeaponBase.DamageMax_Default` _wpn_primary) 0.15)) _wpn_primary))))