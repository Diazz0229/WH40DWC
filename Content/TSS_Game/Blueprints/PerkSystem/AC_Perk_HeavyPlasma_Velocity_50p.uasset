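; Perk component that upgrades the Heavy Plasma primary weapon with faster projectiles.
; On attach it runs the parent attach logic, then checks that the character's primary weapon lists the matching perk class.
; If so, it swaps the weapon's projectile to the fast Heavy Plasma variant and raises crit chance by a fraction of its default.
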(event `self.AttachPerk`
  (params (CharacterRef :type "/Game/TSS_Game/Blueprints/System/BP_CharacterBase Object Reference"))
  (bind _wpn_primary (`/Game/TSS_Game/Blueprints/System/BP_CharacterBase.WPN_Primary` CharacterRef))
  (`parent.AttachPerk` CharacterRef)
  (if (`KismetArrayLibrary.Array_Contains` (`/Game/TSS_Game/Blueprints/Weapons/Base/BP_WeaponBase.PerkClasses` _wpn_primary) "NewEnumerator31")
    (`/Engine/EditorBlueprintResources/StandardMacros.IsValid` _wpn_primary
      (:`Is Valid`
        (set `/Game/TSS_Game/Blueprints/Weapons/Base/BP_WeaponBase.ProjectileToFire` "/Game/TSS_Game/Blueprints/Weapons/Base/BP_Projectile_HeavyPlasma_Fast.BP_Projectile_HeavyPlasma_Fast_C" _wpn_primary)
        (set `/Game/TSS_Game/Blueprints/Weapons/Base/BP_WeaponBase.CritChance` (+ (`/Game/TSS_Game/Blueprints/Weapons/Base/BP_WeaponBase.CritChance` _wpn_primary) (* (`/Game/TSS_Game/Blueprints/Weapons/Base/BP_WeaponBase.CritChance_Default` _wpn_primary) 0.1)) _wpn_primary)))))