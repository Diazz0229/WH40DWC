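; Static attachable Blueprint for the rapid bolter weapon, assembling its visual model from modular parts.
; The construction script adds static mesh components for muzzle, bayonet slot, handle, magazine, sight, grip, Godwyn top and aquila decoration, attaching each to a named SkeletalMesh socket.
; Each added part renders custom depth and ignores all collision channels.
; A visor scope branch is disconnected and never runs, and the event graph has no active logic.
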(fn `UserConstructionScript`
  (bind _skeletalmesh (`self.SkeletalMesh`))
  (bind _returnvalue (`AddComponent|NODE_AddStaticMeshComponent-15` :`bManualAttachment` true))
  (`PrimitiveComponent.SetRenderCustomDepth` _returnvalue true)
  (`StaticMeshComponent.SetStaticMesh` _returnvalue "/Game/WH40Assets/Weapons/SM_XX_Bolter_Godwyn01/SM_XX_Bolter_XX_MDmuzzle03_ATmuzzle01.SM_XX_Bolter_XX_MDmuzzle03_ATmuzzle01")
  (`SceneComponent.K2_AttachToComponent` _returnvalue _skeletalmesh "ATmuzzle01" "KeepRelative" "KeepRelative" "KeepRelative" true)
  (`PrimitiveComponent.SetCollisionResponseToAllChannels` _returnvalue "ECR_Ignore")
  (bind _returnvalue_2 (`AddComponent|NODE_AddStaticMeshComponent-16` :`bManualAttachment` true))
  (`PrimitiveComponent.SetRenderCustomDepth` _returnvalue_2 true)
  (`StaticMeshComponent.SetStaticMesh` _returnvalue_2 "/Game/WH40Assets/Weapons/SM_XX_Bolter_Godwyn01/SM_XX_Bolter_XX_MDbayonetslot01_ATbayonetslot01.SM_XX_Bolter_XX_MDbayonetslot01_ATbayonetslot01")
  (`SceneComponent.K2_AttachToComponent` _returnvalue_2 _skeletalmesh "ATbayonetslot01" "KeepRelative" "KeepRelative" "KeepRelative" true)
  (`PrimitiveComponent.SetCollisionResponseToAllChannels` _returnvalue_2 "ECR_Ignore")
  (bind _returnvalue_3 (`AddComponent|NODE_AddStaticMeshComponent-17` :`bManualAttachment` true))
  (`PrimitiveComponent.SetRenderCustomDepth` _returnvalue_3 true)
  (`StaticMeshComponent.SetStaticMesh` _returnvalue_3 "/Game/WH40Assets/Weapons/SM_XX_Bolter_Godwyn01/SM_XX_Bolter_XX_MDhandle01_AThandle01.SM_XX_Bolter_XX_MDhandle01_AThandle01")
  (`SceneComponent.K2_AttachToComponent` _returnvalue_3 _skeletalmesh "AThandle01" "KeepRelative" "KeepRelative" "KeepRelative" true)
  (`PrimitiveComponent.SetCollisionResponseToAllChannels` _returnvalue_3 "ECR_Ignore")
  (bind _returnvalue_4 (`AddComponent|NODE_AddStaticMeshComponent-18` :`bManualAttachment` true))
  (`PrimitiveComponent.SetRenderCustomDepth` _returnvalue_4 true)
  (`StaticMeshComponent.SetStaticMesh` _returnvalue_4 "/Game/WH40Assets/Weapons/SM_XX_Bolter_Godwyn01/SM_XX_Bolter_XX_MDmag01_ATmag01.SM_XX_Bolter_XX_MDmag01_ATmag01")
  (`SceneComponent.K2_AttachToComponent` _returnvalue_4 _skeletalmesh "ATmag01" "KeepRelative" "KeepRelative" "KeepRelative" true)
  (`PrimitiveComponent.SetCollisionResponseToAllChannels` _returnvalue_4 "ECR_Ignore")
  (bind _returnvalue_5 (`AddComponent|NODE_AddStaticMeshComponent-19` :`bManualAttachment` true))
  (`PrimitiveComponent.SetRenderCustomDepth` _returnvalue_5 true)
  (`StaticMeshComponent.SetStaticMesh` _returnvalue_5 "/Game/WH40Assets/Weapons/SM_XX_Bolter_Godwyn01/SM_XX_Bolter_XX_MDsight02_ATsight01.SM_XX_Bolter_XX_MDsight02_ATsight01")
  (`SceneComponent.K2_AttachToComponent` _returnvalue_5 _skeletalmesh "ATsight01" "KeepRelative" "KeepRelative" "KeepRelative" true)
  (`PrimitiveComponent.SetCollisionResponseToAllChannels` _returnvalue_5 "ECR_Ignore")
  (bind _returnvalue_6 (`AddComponent|NODE_AddStaticMeshComponent-20` :`bManualAttachment` true))
  (`PrimitiveComponent.SetRenderCustomDepth` _returnvalue_6 true)
  (`StaticMeshComponent.SetStaticMesh` _returnvalue_6 "/Game/WH40Assets/Weapons/SM_XX_Bolter_Godwyn01/CM_XX_Bolter_XX_MDgrip01_ATgrip01.CM_XX_Bolter_XX_MDgrip01_ATgrip01")
  (`SceneComponent.K2_AttachToComponent` _returnvalue_6 _skeletalmesh "ATgrip01" "KeepRelative" "KeepRelative" "KeepRelative" true)
  (`PrimitiveComponent.SetCollisionResponseToAllChannels` _returnvalue_6 "ECR_Ignore")
  (bind _returnvalue_7 (`AddComponent|NODE_AddStaticMeshComponent-22` :`bManualAttachment` true))
  (`PrimitiveComponent.SetRenderCustomDepth` _returnvalue_7 true)
  (`StaticMeshComponent.SetStaticMesh` _returnvalue_7 "/Game/WH40Assets/Weapons/SM_XX_Bolter_Godwyn01/SM_XX_Bolter_Godwyn01_MDtop01_ATtop01.SM_XX_Bolter_Godwyn01_MDtop01_ATtop01")
  (`SceneComponent.K2_AttachToComponent` _returnvalue_7 _skeletalmesh "ATtop01" "KeepRelative" "KeepRelative" "KeepRelative" true)
  (`PrimitiveComponent.SetCollisionResponseToAllChannels` _returnvalue_7 "ECR_Ignore")
  (bind _returnvalue_8 (`AddComponent|NODE_AddStaticMeshComponent-23` :`bManualAttachment` true))
  (`PrimitiveComponent.SetRenderCustomDepth` _returnvalue_8 true)
  (`StaticMeshComponent.SetStaticMesh` _returnvalue_8 "/Game/WH40Assets/Weapons/SM_XX_Bolter_Godwyn01/SM_XX_XX_XX_VSaquilaroman01_ATdeco01.SM_XX_XX_XX_VSaquilaroman01_ATdeco01")
  (`SceneComponent.K2_AttachToComponent` _returnvalue_8 _skeletalmesh "ATdecoRT01" "KeepRelative" "KeepRelative" "KeepRelative" true)
  (`PrimitiveComponent.SetCollisionResponseToAllChannels` _returnvalue_8 "ECR_Ignore"))