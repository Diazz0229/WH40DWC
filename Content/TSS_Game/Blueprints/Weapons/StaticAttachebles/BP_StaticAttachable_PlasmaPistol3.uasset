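; Static attachable plasma pistol variant that assembles its cosmetic weapon parts in the construction script.
; It adds muzzle, rear and handle meshes plus two copies of a red Inquisition decoration, each attached to a named socket on SkeletalMesh1.
; Every added part renders to custom depth and ignores all collision channels.
; The event graph holds only disabled default events, so there is no runtime logic.
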(fn `UserConstructionScript`
  (bind _skeletalmesh1 (`self.SkeletalMesh1`))
  (bind _returnvalue (`AddComponent|NODE_AddStaticMeshComponent-11` :`bManualAttachment` true))
  (`PrimitiveComponent.SetRenderCustomDepth` _returnvalue true)
  (`StaticMeshComponent.SetStaticMesh` _returnvalue "/Game/WH40Assets/Weapons/SM_XX_Plasma_Plasmapistol01/SM_XX_Plasma_Plasmapistol01_MDmuzzle01_ATmuzzle03.SM_XX_Plasma_Plasmapistol01_MDmuzzle01_ATmuzzle03")
  (`SceneComponent.K2_AttachToComponent` _returnvalue _skeletalmesh1 "ATmuzzle01" "KeepRelative" "KeepRelative" "KeepRelative" true)
  (`PrimitiveComponent.SetCollisionResponseToAllChannels` _returnvalue "ECR_Ignore")
  (bind _returnvalue_2 (`AddComponent|NODE_AddStaticMeshComponent-12` :`bManualAttachment` true))
  (`PrimitiveComponent.SetRenderCustomDepth` _returnvalue_2 true)
  (`StaticMeshComponent.SetStaticMesh` _returnvalue_2 "/Game/WH40Assets/Weapons/SM_XX_Plasma_Plasmapistol01/SM_XX_Plasma_Plasmapistol01_MDrear01_ATrear01.SM_XX_Plasma_Plasmapistol01_MDrear01_ATrear01")
  (`SceneComponent.K2_AttachToComponent` _returnvalue_2 _skeletalmesh1 "ATrear01" "KeepRelative" "KeepRelative" "KeepRelative" true)
  (`PrimitiveComponent.SetCollisionResponseToAllChannels` _returnvalue_2 "ECR_Ignore")
  (bind _returnvalue_3 (`AddComponent|NODE_AddStaticMeshComponent-13` :`bManualAttachment` true))
  (`PrimitiveComponent.SetRenderCustomDepth` _returnvalue_3 true)
  (`StaticMeshComponent.SetStaticMesh` _returnvalue_3 "/Game/WH40Assets/Weapons/SM_XX_Plasma_Plasmagun01/SM_XX_Plasma_XX_MDhandle01_AThandle01.SM_XX_Plasma_XX_MDhandle01_AThandle01")
  (`SceneComponent.K2_AttachToComponent` _returnvalue_3 _skeletalmesh1 "AThandle01" "KeepRelative" "KeepRelative" "KeepRelative" true)
  (`PrimitiveComponent.SetCollisionResponseToAllChannels` _returnvalue_3 "ECR_Ignore")
  (bind _returnvalue_4 (`AddComponent|NODE_AddStaticMeshComponent-14` :`bManualAttachment` true))
  (`PrimitiveComponent.SetRenderCustomDepth` _returnvalue_4 true)
  (`StaticMeshComponent.SetStaticMesh` _returnvalue_4 "/Game/Characters/SpaceMarine/BodyPart/Legs/SM_XX_LegRT_Mkvii01/SM_XX_LegRT_XX_VSinquisition_ATlegfrontRT01ATlegfrontRT01_red.SM_XX_LegRT_XX_VSinquisition_ATlegfrontRT01ATlegfrontRT01_red")
  (`SceneComponent.K2_AttachToComponent` _returnvalue_4 _skeletalmesh1 "ATdecoRT02_Inquisition_0" "KeepRelative" "KeepRelative" "KeepRelative" true)
  (`PrimitiveComponent.SetCollisionResponseToAllChannels` _returnvalue_4 "ECR_Ignore")
  (bind _returnvalue_5 (`AddComponent|NODE_AddStaticMeshComponent-15` :`bManualAttachment` true))
  (`PrimitiveComponent.SetRenderCustomDepth` _returnvalue_5 true)
  (`StaticMeshComponent.SetStaticMesh` _returnvalue_5 "/Game/Characters/SpaceMarine/BodyPart/Legs/SM_XX_LegRT_Mkvii01/SM_XX_LegRT_XX_VSinquisition_ATlegfrontRT01ATlegfrontRT01_red.SM_XX_LegRT_XX_VSinquisition_ATlegfrontRT01ATlegfrontRT01_red")
  (`SceneComponent.K2_AttachToComponent` _returnvalue_5 _skeletalmesh1 "ATdecoRT02_Inquisition" "KeepRelative" "KeepRelative" "KeepRelative" true)
  (`PrimitiveComponent.SetCollisionResponseToAllChannels` _returnvalue_5 "ECR_Ignore"))