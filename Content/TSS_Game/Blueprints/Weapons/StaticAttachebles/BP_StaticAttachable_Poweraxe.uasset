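; Static attachable power axe weapon Blueprint that assembles its modular visual model from separate club-set mesh parts.
; The construction script adds static mesh components for the axe tip, head, pommel and force pack, attaching each to its named socket on WeaponMesh.
; Each part renders custom depth and ignores all collision channels.
; The parent construction script is not called, and the event graph has no active logic.
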(fn `UserConstructionScript`
  (bind _weaponmesh (`self.WeaponMesh`))
  (bind _returnvalue (`AddComponent|NODE_AddStaticMeshComponent-10` :`bManualAttachment` true))
  (`PrimitiveComponent.SetRenderCustomDepth` _returnvalue true)
  (`StaticMeshComponent.SetStaticMesh` _returnvalue "/Game/WH40Assets/Weapons/SM_XX_Club_Club01/SM_XX_Club_XX_MDaxeLarge01_ATtip01.SM_XX_Club_XX_MDaxeLarge01_ATtip01")
  (`SceneComponent.K2_AttachToComponent` _returnvalue _weaponmesh "ATtip01" "KeepRelative" "KeepRelative" "KeepRelative" true)
  (`PrimitiveComponent.SetCollisionResponseToAllChannels` _returnvalue "ECR_Ignore")
  (bind _returnvalue_2 (`AddComponent|NODE_AddStaticMeshComponent-11` :`bManualAttachment` true))
  (`PrimitiveComponent.SetRenderCustomDepth` _returnvalue_2 true)
  (`StaticMeshComponent.SetStaticMesh` _returnvalue_2 "/Game/WH40Assets/Weapons/SM_XX_Club_Club01/SM_XX_Club_XX_MDhead03_AThead01AThead02.SM_XX_Club_XX_MDhead03_AThead01AThead02")
  (`SceneComponent.K2_AttachToComponent` _returnvalue_2 _weaponmesh "AThead02" "KeepRelative" "KeepRelative" "KeepRelative" true)
  (`PrimitiveComponent.SetCollisionResponseToAllChannels` _returnvalue_2 "ECR_Ignore")
  (bind _returnvalue_3 (`AddComponent|NODE_AddStaticMeshComponent-12` :`bManualAttachment` true))
  (`PrimitiveComponent.SetRenderCustomDepth` _returnvalue_3 true)
  (`StaticMeshComponent.SetStaticMesh` _returnvalue_3 "/Game/WH40Assets/Weapons/SM_XX_Club_Club01/SM_XX_Club_XX_MDpommel02_ATpommel01.SM_XX_Club_XX_MDpommel02_ATpommel01")
  (`SceneComponent.K2_AttachToComponent` _returnvalue_3 _weaponmesh "ATpommel01" "KeepRelative" "KeepRelative" "KeepRelative" true)
  (`PrimitiveComponent.SetCollisionResponseToAllChannels` _returnvalue_3 "ECR_Ignore")
  (bind _returnvalue_4 (`AddComponent|NODE_AddStaticMeshComponent-13` :`bManualAttachment` true))
  (`PrimitiveComponent.SetRenderCustomDepth` _returnvalue_4 true)
  (`StaticMeshComponent.SetStaticMesh` _returnvalue_4 "/Game/WH40Assets/Weapons/SM_XX_Club_Club01/SM_XX_Club_XX_MDforcepack01_ATpack01.SM_XX_Club_XX_MDforcepack01_ATpack01")
  (`SceneComponent.K2_AttachToComponent` _returnvalue_4 _weaponmesh "ATpack01" "KeepRelative" "KeepRelative" "KeepRelative" true)
  (`PrimitiveComponent.SetCollisionResponseToAllChannels` _returnvalue_4 "ECR_Ignore"))