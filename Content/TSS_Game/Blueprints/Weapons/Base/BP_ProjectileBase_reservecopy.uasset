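; Base weapon projectile that copies damage and penetration from its owner's equipped weapon and destroys multicast-shot copies for the local shooter.
; Hit spawns a Niagara or emitter effect, then deals damage through the PlayerController, either to a sphere-traced splash area or to the locally hit damageable actor.
; Damaging hits push physics bodies and spend penetration before deactivation and delayed destruction.
; Piercing works by restoring initial rotation and velocity whenever projectile movement stops.
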(event `self.ReceiveBeginPlay`)

(event `ProjectileInit`
  (bind _ownercharacter (`self.OwnerCharacter`))
  (bind _equippedweapon (`/Game/TSS_Game/Blueprints/System/BP_CharacterBase.EquippedWeapon` _ownercharacter))
  (`/Engine/EditorBlueprintResources/StandardMacros.IsValid` _ownercharacter
    (:`Is Valid`
      (if (and (`Pawn.IsLocallyControlled` _ownercharacter) (`self.IsMCShot`))
        (`self.K2_DestroyActor`)
        (else
          (`SceneComponent.SetVisibility` (`self.Sphere1`) true true)
          (set `self.ProjectileDamage` (`/Game/TSS_Game/Blueprints/Weapons/Base/BP_WeaponBase.Damage` _equippedweapon))
          (set `self.PenetrateTargets` (`/Game/TSS_Game/Blueprints/Weapons/Base/BP_WeaponBase.PenetratedTargets` _equippedweapon))
          (set `self.InitRotation` (`self.K2_GetActorRotation`))
          (set `self.InitVelocity` (`KismetMathLibrary.MakeVector` (`ProjectileMovementComponent.InitialSpeed` (`self.ProjectileMovement`)))))))
    (:`Is Not Valid`
      (`KismetSystemLibrary.PrintString` "BP_ProjectileBase: PLayer controller is not valid"))))

(event `self.ReceiveHit`
  (params (MyComp :type "PrimitiveComponent Object Reference") (Other :type "Actor Object Reference") (OtherComp :type "PrimitiveComponent Object Reference") (bSelfMoved :type Boolean) (HitLocation :type "Vector Structure") (HitNormal :type "Vector Structure") (NormalImpulse :type "Vector Structure") (Hit :type "HitResult Structure (by ref)"))
  (bind _ownercharacter (`self.OwnerCharacter`))
  (bind _penetratetargets (`self.PenetrateTargets`))
  (bind _splashradius (`self.SplashRadius`))
  (bind _ownercharacter_2 (`self.OwnerCharacter`))
  (bind _ownercharacter_3 (`self.OwnerCharacter`))
  (bind _bulletmesh (`self.BulletMesh`))
  (set `self.Hit Actor` (`.HitActor` (`GameplayStatics.BreakHitResult` Hit)))
  (if (`self.IsHitByNiagara`)
    (`NiagaraFunctionLibrary.SpawnSystemAtLocation` (`self.NiagaraHitEffect`) HitLocation)
    (else
      (`GameplayStatics.SpawnEmitterAtLocation` (`self.HitEmitter`) HitLocation (struct) (0.5 0.5 0.5))))
  (`/Engine/EditorBlueprintResources/StandardMacros.IsValid` _ownercharacter
    (:`Is Valid`
      (if (> _splashradius 0.0)
        (bind _outhits (`KismetSystemLibrary.SphereTraceMulti` HitLocation HitLocation _splashradius "TraceTypeQuery1"))
        (for _array_element _outhits
          (bind (_bblockinghit _binitialoverlap _time _distance _location _impactpoint _normal _impactnormal _physmat _hitactor) (`GameplayStatics.BreakHitResult` _array_element))
          (`/Engine/EditorBlueprintResources/StandardMacros.IsValid` _hitactor
            (:`Is Valid`
              (if (not (`KismetArrayLibrary.Array_Contains` (`self.Enemies to Hit`) _hitactor))
                (`KismetArrayLibrary.Array_AddUnique` (`self.Enemies to Hit`) _hitactor)))))
        (for _array_element_2 (`self.Enemies to Hit`)
          (if (`KismetSystemLibrary.DoesImplementInterface` _array_element_2 "/Game/TSS_Game/Blueprints/System/BPI_Damagable.BPI_Damagable_C")
            (bind _asbp_player_controller (cast `/Game/TSS_Game/Blueprints/System/BP_PlayerController` (`Pawn.GetController` _ownercharacter_2)))
            (`/Game/TSS_Game/Blueprints/System/BP_PlayerController.DealDamage` _asbp_player_controller _array_element_2 (`self.ProjectileDamage`) _ownercharacter_2)))
        (`self.ApplyPhysics` OtherComp :!label _label)
        (if (> _penetratetargets 0)
          (`/Engine/EditorBlueprintResources/StandardMacros.DecrementInt` _penetratetargets)
          (else
            (`ActorComponent.Deactivate` (`self.ProjectileMovement`) :!label _label_2)
            (`ActorComponent.Deactivate` _bulletmesh)
            (`SceneComponent.ToggleVisibility` _bulletmesh false)
            (`KismetSystemLibrary.Delay` 2.0)
            (`self.K2_DestroyActor`)))
        (elif (and (`Pawn.IsLocallyControlled` _ownercharacter) (`KismetSystemLibrary.DoesImplementInterface` (`self.Hit Actor`) "/Game/TSS_Game/Blueprints/System/BPI_Damagable.BPI_Damagable_C"))
          (bind _asbp_player_controller_2 (cast `/Game/TSS_Game/Blueprints/System/BP_PlayerController` (`Pawn.GetController` _ownercharacter_3)))
          (`/Game/TSS_Game/Blueprints/System/BP_PlayerController.DealDamage` _asbp_player_controller_2 (`self.Hit Actor`) (`self.ProjectileDamage`) _ownercharacter_3)
          (goto _label)
          (else
            (goto _label_2)))))
    (:`Is Not Valid`
      (goto _label_2))))

(event `self.ProjectileMovement.OnProjectileStop`
  (params (ImpactResult :type "HitResult Structure (by ref)"))
  (bind _projectilemovement (`self.ProjectileMovement`))
  (`MovementComponent.SetUpdatedComponent` _projectilemovement (`self.RootComponent`))
  (`self.K2_SetActorRotation` (`self.InitRotation`) true)
  (`KismetSystemLibrary.Delay` 0.02)
  (`ProjectileMovementComponent.SetVelocityInLocalSpace` _projectilemovement (`self.InitVelocity`)))

(fn `ApplyPhysics`
  (params (OtherComponent :type "PrimitiveComponent Object Reference"))
  (`/Engine/EditorBlueprintResources/StandardMacros.IsValid` OtherComponent
    (:`Is Valid`
      (if (`SceneComponent.IsSimulatingPhysics` OtherComponent "None")
        (`PrimitiveComponent.AddImpulseAtLocation` OtherComponent (* (`self.GetVelocity`) (`self.ProjectileImpulseStrenght`)) (`self.K2_GetActorLocation`) "None")
        (return)
        (else
          (return))))
    (:`Is Not Valid`
      (return))))

(fn `UserConstructionScript`)