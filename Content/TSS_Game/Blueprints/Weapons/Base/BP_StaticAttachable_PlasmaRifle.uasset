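; Plasma rifle static attachable Blueprint that assembles the weapon model from modular parts.
; The Construction Script spawns static mesh components for muzzle, rear, grip, bottom, handle and sight, attaching each to its matching socket on SkeletalMesh1.
; Each part renders custom depth and ignores all collision channels.
; The event graph holds only disabled placeholder events, so it adds no runtime logic.
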(fn `UserConstructionScript`
  (bind _returnvalue (`AddComponent|NODE_AddStaticMeshComponent-5` :`bManualAttachment` true))
  (`PrimitiveComponent.SetRenderCustomDepth` _returnvalue true)
  (`StaticMeshComponent.SetStaticMesh` _returnvalue "/Game/WH40Assets/Weapons/SM_XX_Plasma_Plasmagun01/SM_XX_Plasma_Plasmagun01_MDmuzzle01_ATmuzzle01.SM_XX_Plasma_Plasmagun01_MDmuzzle01_ATmuzzle01")
  (`SceneComponent.K2_AttachToComponent` _returnvalue (`self.SkeletalMesh1`) "ATmuzzle01" "KeepRelative" "KeepRelative" "KeepRelative" true)
  (`PrimitiveComponent.SetCollisionResponseToAllChannels` _returnvalue "ECR_Ignore")
  (bind _returnvalue_2 (`AddComponent|NODE_AddStaticMeshComponent-6` :`bManualAttachment` true))
  (`PrimitiveComponent.SetRenderCustomDepth` _returnvalue_2 true)
  (`StaticMeshComponent.SetStaticMesh` _returnvalue_2 "/Game/WH40Assets/Weapons/SM_XX_Plasma_Plasmagun01/SM_XX_Plasma_XX_MDrear01_ATrear01.SM_XX_Plasma_XX_MDrear01_ATrear01")
  (`SceneComponent.K2_AttachToComponent` _returnvalue_2 (`self.SkeletalMesh1`) "ATrear01" "KeepRelative" "KeepRelative" "KeepRelative" true)
  (`PrimitiveComponent.SetCollisionResponseToAllChannels` _returnvalue_2 "ECR_Ignore")
  (bind _returnvalue_3 (`AddComponent|NODE_AddStaticMeshComponent-7` :`bManualAttachment` true))
  (`PrimitiveComponent.SetRenderCustomDepth` _returnvalue_3 true)
  (`StaticMeshComponent.SetStaticMesh` _returnvalue_3 "/Game/WH40Assets/Weapons/SM_XX_Plasma_Plasmagun01/SM_XX_Plasma_XX_MDgrip01_ATgrip01.SM_XX_Plasma_XX_MDgrip01_ATgrip01")
  (`SceneComponent.K2_AttachToComponent` _returnvalue_3 (`self.SkeletalMesh1`) "ATgrip01" "KeepRelative" "KeepRelative" "KeepRelative" true)
  (`PrimitiveComponent.SetCollisionResponseToAllChannels` _returnvalue_3 "ECR_Ignore")
  (bind _returnvalue_4 (`AddComponent|NODE_AddStaticMeshComponent-8` :`bManualAttachment` true))
  (`PrimitiveComponent.SetRenderCustomDepth` _returnvalue_4 true)
  (`StaticMeshComponent.SetStaticMesh` _returnvalue_4 "/Game/WH40Assets/Weapons/SM_XX_Plasma_Plasmagun01/SM_XX_Plasma_XX_MDbottom01_ATbottom01.SM_XX_Plasma_XX_MDbottom01_ATbottom01")
  (`SceneComponent.K2_AttachToComponent` _returnvalue_4 (`self.SkeletalMesh1`) "ATbottom01" "KeepRelative" "KeepRelative" "KeepRelative" true)
  (`PrimitiveComponent.SetCollisionResponseToAllChannels` _returnvalue_4 "ECR_Ignore")
  (bind _returnvalue_5 (`AddComponent|NODE_AddStaticMeshComponent-9` :`bManualAttachment` true))
  (`PrimitiveComponent.SetRenderCustomDepth` _returnvalue_5 true)
  (`StaticMeshComponent.SetStaticMesh` _returnvalue_5 "/Game/WH40Assets/Weapons/SM_XX_Plasma_Plasmagun01/SM_XX_Plasma_XX_MDhandle01_AThandle01.SM_XX_Plasma_XX_MDhandle01_AThandle01")
  (`SceneComponent.K2_AttachToComponent` _returnvalue_5 (`self.SkeletalMesh1`) "AThandle01" "KeepRelative" "KeepRelative" "KeepRelative" true)
  (`PrimitiveComponent.SetCollisionResponseToAllChannels` _returnvalue_5 "ECR_Ignore")
  (bind _returnvalue_6 (`AddComponent|NODE_AddStaticMeshComponent-10` :`bManualAttachment` true))
  (`PrimitiveComponent.SetRenderCustomDepth` _returnvalue_6 true)
  (`StaticMeshComponent.SetStaticMesh` _returnvalue_6 "/Game/WH40Assets/Weapons/SM_XX_Plasma_Plasmagun01/SM_XX_Plasma_Plasmagun01_MDsight01_ATsight01.SM_XX_Plasma_Plasmagun01_MDsight01_ATsight01")
  (`SceneComponent.K2_AttachToComponent` _returnvalue_6 (`self.SkeletalMesh1`) "ATsight01" "KeepRelative" "KeepRelative" "KeepRelative" true)
  (`PrimitiveComponent.SetCollisionResponseToAllChannels` _returnvalue_6 "ECR_Ignore"))