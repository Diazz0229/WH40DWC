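; Frag grenade explosion actor that spawns the blast effect and sound, deals area damage, then fades out its decal and destroys itself.
; For a brief window after spawn, sphere overlaps damage each living damageable, non-BP_CharacterBase actor once.
; Only the locally controlled owner's instance rolls random damage and crits, routing hits through the owning player's DealDamage.
; A delayed looping timer lowers the decal's dynamic material opacity before cleanup.
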(event `self.ReceiveBeginPlay`
  (`SphereComponent.SetSphereRadius` (`self.Sphere`) (`self.Sphere Radius`) true)
  (`NiagaraFunctionLibrary.SpawnSystemAttached` "/Game/NiagaraExplosion01/Niagaras/Air/N_ExplosionAir_004.N_ExplosionAir_004" (`self.DefaultSceneRoot`) "None" (0.0 0.0 0.0) (struct) "KeepRelativeOffset" true)
  (`GameplayStatics.SpawnSoundAtLocation` "/Game/TSS_Game/SFX/Explosions/SC_LArgeExplosion.SC_LArgeExplosion" (`self.K2_GetActorLocation`) (struct) 1.0 0.2 0.0 null null)
  (bind _returnvalue (`DecalComponent.CreateDynamicMaterialInstance` (`self.Decal`)))
  (set `self.DynamicMaterial` _returnvalue)
  (`KismetSystemLibrary.Delay` 0.2)
  (set `self.IsActive?` false)
  (`KismetSystemLibrary.Delay` 3.0)
  (`KismetSystemLibrary.K2_SetTimerDelegate` (delegate `LowerOpacity`) 0.1 true))

(event `LowerOpacity`
  (bind _dynamicmaterial (`self.DynamicMaterial`))
  (bind _returnvalue (`MaterialInstanceDynamic.K2_GetScalarParameterValue` _dynamicmaterial "Opacity"))
  (if (>= _returnvalue 0.0)
    (`MaterialInstanceDynamic.SetScalarParameterValue` _dynamicmaterial "Opacity" (- _returnvalue 0.1))
    (else
      (`KismetSystemLibrary.K2_PauseTimer` null "LowerOpacity")
      (`self.K2_DestroyActor`))))

(event `self.ReceiveActorBeginOverlap`
  (params (OtherActor :type "Actor Object Reference"))
  (bind _ownercharacter (`self.OwnerCharacter`))
  (if (`self.IsActive?`)
    (`/Engine/EditorBlueprintResources/StandardMacros.IsValid` _ownercharacter
      (:`Is Valid`
        (if (`Pawn.IsLocallyControlled` _ownercharacter)
          (cast `/Game/TSS_Game/Blueprints/System/BP_CharacterBase` OtherActor
            (:`CastFailed`
              (if (`KismetSystemLibrary.DoesImplementInterface` OtherActor "/Game/TSS_Game/Blueprints/System/BPI_Damagable.BPI_Damagable_C")
                (if (not (or (`self.ActorHasTag` OtherActor "Dead") (`KismetArrayLibrary.Array_Contains` (`self.DamagedActors`) OtherActor)))
                  (`KismetArrayLibrary.Array_Add` (`self.DamagedActors`) OtherActor)
                  (`self.CheckCritAndDealDamage` OtherActor (`self.OwnerPlayer`) (`self.OwnerCharacter`)))))))))))

(fn `CheckCritAndDealDamage`
  (params (DamageTarget :type "Actor Object Reference") (PlController :type "/Game/TSS_Game/Blueprints/System/BP_PlayerController Object Reference") (Source :type "/Game/TSS_Game/Blueprints/System/BP_CharacterBase Object Reference"))
  (bind _damagedealt (`self.DamageDealt`))
  (set `self.DamageDealt` (`KismetMathLibrary.Conv_IntToDouble` (`KismetMathLibrary.RandomIntegerInRange` (`KismetMathLibrary.FTrunc` (`self.DamageMin`)) (`KismetMathLibrary.FTrunc` (`self.DamageMax`)))))
  (if (<= (`KismetMathLibrary.RandomFloatInRange` 0.0 100.0) (`self.CritChance`))
    (set `self.DamageDealt` (* (`self.DamageDealt`) (`self.CritMultiplier`)))
    (`/Game/TSS_Game/Blueprints/System/BP_PlayerController.DealDamage` PlController DamageTarget _damagedealt Source true (`self.Damage Type`) 0.0 0.0)
    (else
      (`/Game/TSS_Game/Blueprints/System/BP_PlayerController.DealDamage` PlController DamageTarget _damagedealt Source false (`self.Damage Type`) 0.0 0.0))))

(fn `UserConstructionScript`)