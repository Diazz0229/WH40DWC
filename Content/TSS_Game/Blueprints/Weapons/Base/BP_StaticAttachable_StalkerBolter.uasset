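; Static attachable Stalker Bolter weapon actor that assembles its modular look from separate part meshes.
; The construction script adds static mesh components for muzzle, scope, bayonet slot, handle and magazine, attaching each to its matching socket on the skeletal mesh with collision responses set to ignore.
; A sixth component on the sight socket has no mesh assigned.
; The event graph holds no active logic.
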(fn `UserConstructionScript`
  (bind _skeletalmesh (`self.SkeletalMesh`))
  (bind _returnvalue (`AddComponent|NODE_AddStaticMeshComponent-10` :`bManualAttachment` true))
  (`StaticMeshComponent.SetStaticMesh` _returnvalue "/Game/WH40Assets/Weapons/SM_XX_Bolter_Godwyn01/SM_XX_Bolter_XX_MDmuzzle05_ATmuzzle01.SM_XX_Bolter_XX_MDmuzzle05_ATmuzzle01")
  (`SceneComponent.K2_AttachToComponent` _returnvalue _skeletalmesh "ATmuzzle01" "KeepRelative" "KeepRelative" "KeepRelative" true)
  (`PrimitiveComponent.SetCollisionResponseToAllChannels` _returnvalue "ECR_Ignore")
  (bind _returnvalue_2 (`AddComponent|NODE_AddStaticMeshComponent-15` :`bManualAttachment` true))
  (`StaticMeshComponent.SetStaticMesh` _returnvalue_2 "/Game/WH40Assets/Weapons/SM_XX_Bolter_Godwyn01/SM_XX_XX_XX_MDscope03_ATvisor01.SM_XX_XX_XX_MDscope03_ATvisor01")
  (`SceneComponent.K2_AttachToComponent` _returnvalue_2 _skeletalmesh "ATvisor01" "KeepRelative" "KeepRelative" "KeepRelative" true)
  (`PrimitiveComponent.SetCollisionResponseToAllChannels` _returnvalue_2 "ECR_Ignore")
  (bind _returnvalue_3 (`AddComponent|NODE_AddStaticMeshComponent-11` :`bManualAttachment` true))
  (`StaticMeshComponent.SetStaticMesh` _returnvalue_3 "/Game/WH40Assets/Weapons/SM_XX_Bolter_Godwyn01/SM_XX_Bolter_XX_MDbayonetslot01_ATbayonetslot01.SM_XX_Bolter_XX_MDbayonetslot01_ATbayonetslot01")
  (`SceneComponent.K2_AttachToComponent` _returnvalue_3 _skeletalmesh "ATbayonetslot01" "KeepRelative" "KeepRelative" "KeepRelative" true)
  (`PrimitiveComponent.SetCollisionResponseToAllChannels` _returnvalue_3 "ECR_Ignore")
  (bind _returnvalue_4 (`AddComponent|NODE_AddStaticMeshComponent-12` :`bManualAttachment` true))
  (`StaticMeshComponent.SetStaticMesh` _returnvalue_4 "/Game/WH40Assets/Weapons/SM_XX_Bolter_Godwyn01/SM_XX_Bolter_XX_MDhandle02_AThandle01.SM_XX_Bolter_XX_MDhandle02_AThandle01")
  (`SceneComponent.K2_AttachToComponent` _returnvalue_4 _skeletalmesh "AThandle01" "KeepRelative" "KeepRelative" "KeepRelative" true)
  (`PrimitiveComponent.SetCollisionResponseToAllChannels` _returnvalue_4 "ECR_Ignore")
  (bind _returnvalue_5 (`AddComponent|NODE_AddStaticMeshComponent-13` :`bManualAttachment` true))
  (`StaticMeshComponent.SetStaticMesh` _returnvalue_5 "/Game/WH40Assets/Weapons/SM_XX_Bolter_Godwyn01/SM_XX_Bolter_XX_MDmag01_ATmag01.SM_XX_Bolter_XX_MDmag01_ATmag01")
  (`SceneComponent.K2_AttachToComponent` _returnvalue_5 _skeletalmesh "ATmag01" "KeepRelative" "KeepRelative" "KeepRelative" true)
  (`PrimitiveComponent.SetCollisionResponseToAllChannels` _returnvalue_5 "ECR_Ignore")
  (bind _returnvalue_6 (`AddComponent|NODE_AddStaticMeshComponent-14` :`bManualAttachment` true))
  (`StaticMeshComponent.SetStaticMesh` _returnvalue_6 null)
  (`SceneComponent.K2_AttachToComponent` _returnvalue_6 _skeletalmesh "ATsight01" "KeepRelative" "KeepRelative" "KeepRelative" true)
  (`PrimitiveComponent.SetCollisionResponseToAllChannels` _returnvalue_6 "ECR_Ignore"))