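; BP_Explosion is a short-lived explosion actor in the weapons base folder that plays effects and damages actors that overlap it.
; On BeginPlay it calls a server event, which calls a multicast event to spawn the big explosion particle and a pitched-down grenade launcher sound.
; The multicast event then destroys the actor after a brief delay.
; Overlapping actors take a small flat damage, credited to the instigator's controller.
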(event `Multicast_Effects`
  (bind _returnvalue (`self.K2_GetActorLocation`))
  (`GameplayStatics.SpawnEmitterAtLocation` "/Game/TSS_Game/Particles/P_Explosion_Big.P_Explosion_Big" _returnvalue)
  (`GameplayStatics.SpawnSoundAtLocation` "/Game/TSS_Game/SFX/Weapon/SC_GrenadeLauncherExplosion.SC_GrenadeLauncherExplosion" _returnvalue (struct) 1.0 0.2 0.0 null null)
  (`KismetSystemLibrary.Delay` 0.2)
  (`self.K2_DestroyActor`))

(event `Server_Effects`
  (`self.Multicast_Effects`))

(event `self.ReceiveBeginPlay`
  (`self.Server_Effects`))

(event `self.ReceiveActorBeginOverlap`
  (params (OtherActor :type "Actor Object Reference"))
  (`GameplayStatics.ApplyDamage` OtherActor 0.5 (`self.GetInstigatorController`) self))

(fn `UserConstructionScript`)