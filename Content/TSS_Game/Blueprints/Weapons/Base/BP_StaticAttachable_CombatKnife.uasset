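; Static attachable combat knife weapon Blueprint, assembled from modular mesh parts.
; The construction script adds guard and blade static mesh components and attaches them to their joint sockets on the inherited WeaponMesh.
; Both parts render custom depth and ignore all collision channels.
; The event graph holds only disabled placeholder events, so it adds no runtime logic.
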(fn `UserConstructionScript`
  (`parent.UserConstructionScript`)
  (bind _returnvalue (`AddComponent|NODE_AddStaticMeshComponent-0` :`bManualAttachment` true))
  (`PrimitiveComponent.SetRenderCustomDepth` _returnvalue true)
  (`StaticMeshComponent.SetStaticMesh` _returnvalue "/Game/WH40Assets/Weapons/Knife/SM_XX_Combatknife_XX_MDguard01_ATguard01.SM_XX_Combatknife_XX_MDguard01_ATguard01")
  (`SceneComponent.K2_AttachToComponent` _returnvalue (`self.WeaponMesh`) "joint_guard" "KeepRelative" "KeepRelative" "KeepRelative" true)
  (`PrimitiveComponent.SetCollisionResponseToAllChannels` _returnvalue "ECR_Ignore")
  (bind _returnvalue_2 (`AddComponent|NODE_AddStaticMeshComponent-1` :`bManualAttachment` true))
  (`PrimitiveComponent.SetRenderCustomDepth` _returnvalue_2 true)
  (`StaticMeshComponent.SetStaticMesh` _returnvalue_2 "/Game/WH40Assets/Weapons/Knife/SM_XX_Combatknife_XX_MDblade01_ATblade01.SM_XX_Combatknife_XX_MDblade01_ATblade01")
  (`SceneComponent.K2_AttachToComponent` _returnvalue_2 (`self.WeaponMesh`) "joint_blade" "KeepRelative" "KeepRelative" "KeepRelative" true)
  (`PrimitiveComponent.SetCollisionResponseToAllChannels` _returnvalue_2 "ECR_Ignore"))