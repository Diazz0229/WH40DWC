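; Static attachable Bolter weapon Blueprint that assembles the gun's visual model from modular parts.
; Its construction script adds static meshes for muzzle, bayonet slot, handle, magazine and sight, attaching each to its named socket on the SkeletalMesh.
; Collision is set to ignore all channels on the skeletal mesh and every part except the sight, which keeps its default responses.
; The event graph holds no active logic.
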(fn `UserConstructionScript`
  (bind _skeletalmesh (`self.SkeletalMesh`))
  (bind _returnvalue (`AddComponent|NODE_AddStaticMeshComponent-0` :`bManualAttachment` true))
  (`StaticMeshComponent.SetStaticMesh` _returnvalue "/Game/WH40Assets/Weapons/SM_XX_Bolter_Godwyn01/SM_XX_Bolter_XX_MDmuzzle04_ATmuzzle01.SM_XX_Bolter_XX_MDmuzzle04_ATmuzzle01")
  (`SceneComponent.K2_AttachToComponent` _returnvalue _skeletalmesh "ATmuzzle01" "KeepRelative" "KeepRelative" "KeepRelative" true)
  (`PrimitiveComponent.SetCollisionResponseToAllChannels` _returnvalue "ECR_Ignore")
  (bind _returnvalue_2 (`AddComponent|NODE_AddStaticMeshComponent-1` :`bManualAttachment` true))
  (`StaticMeshComponent.SetStaticMesh` _returnvalue_2 "/Game/WH40Assets/Weapons/SM_XX_Bolter_Godwyn01/SM_XX_Bolter_XX_MDbayonetslot01_ATbayonetslot01.SM_XX_Bolter_XX_MDbayonetslot01_ATbayonetslot01")
  (`SceneComponent.K2_AttachToComponent` _returnvalue_2 _skeletalmesh "ATbayonetslot01" "KeepRelative" "KeepRelative" "KeepRelative" true)
  (`PrimitiveComponent.SetCollisionResponseToAllChannels` _returnvalue_2 "ECR_Ignore")
  (bind _returnvalue_3 (`AddComponent|NODE_AddStaticMeshComponent-2` :`bManualAttachment` true))
  (`StaticMeshComponent.SetStaticMesh` _returnvalue_3 "/Game/WH40Assets/Weapons/SM_XX_Bolter_Godwyn01/SM_XX_Bolter_XX_MDhandle01_AThandle01.SM_XX_Bolter_XX_MDhandle01_AThandle01")
  (`SceneComponent.K2_AttachToComponent` _returnvalue_3 _skeletalmesh "AThandle01" "KeepRelative" "KeepRelative" "KeepRelative" true)
  (`PrimitiveComponent.SetCollisionResponseToAllChannels` _returnvalue_3 "ECR_Ignore")
  (bind _returnvalue_4 (`AddComponent|NODE_AddStaticMeshComponent-3` :`bManualAttachment` true))
  (`StaticMeshComponent.SetStaticMesh` _returnvalue_4 "/Game/WH40Assets/Weapons/SM_XX_Bolter_Godwyn01/SM_XX_Bolter_XX_MDmag01_ATmag01.SM_XX_Bolter_XX_MDmag01_ATmag01")
  (`SceneComponent.K2_AttachToComponent` _returnvalue_4 _skeletalmesh "ATmag01" "KeepRelative" "KeepRelative" "KeepRelative" true)
  (`PrimitiveComponent.SetCollisionResponseToAllChannels` _returnvalue_4 "ECR_Ignore")
  (bind _returnvalue_5 (`AddComponent|NODE_AddStaticMeshComponent-4` :`bManualAttachment` true))
  (`StaticMeshComponent.SetStaticMesh` _returnvalue_5 "/Game/WH40Assets/Weapons/SM_XX_Bolter_Godwyn01/SM_XX_Bolter_XX_MDsight01_ATsight01.SM_XX_Bolter_XX_MDsight01_ATsight01")
  (`SceneComponent.K2_AttachToComponent` _returnvalue_5 _skeletalmesh "ATsight01" "KeepRelative" "KeepRelative" "KeepRelative" true)
  (`PrimitiveComponent.SetCollisionResponseToAllChannels` _skeletalmesh "ECR_Ignore"))