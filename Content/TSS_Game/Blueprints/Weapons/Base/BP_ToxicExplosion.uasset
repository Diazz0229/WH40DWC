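; BP_ToxicExplosion is a short-lived toxic blast actor that harms non-enemy characters within its sphere.
; On BeginPlay it plays a hit sound, waits briefly, then sends damage to overlapping characters that are not dead, enemy-tagged or evading.
; Victims whose instigator controller is the first player controller also get a stackable toxins buff requested through that controller.
; It destroys itself about a second later.
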(event `self.ReceiveBeginPlay`
  (`GameplayStatics.SpawnSoundAtLocation` "/Game/TSS_Game/SFX/Characters/Tyranids/Weapons/SC_TYR_ToxicHit.SC_TYR_ToxicHit" (`self.K2_GetActorLocation`) (struct) 1.0 1.0 0.0 null null)
  (`KismetSystemLibrary.Delay` 0.05)
  (for _array_element (`PrimitiveComponent.GetOverlappingActors` (`self.Sphere`) "/Game/TSS_Game/Blueprints/System/BP_CharacterBase.BP_CharacterBase_C")
    (if (not (or (`self.ActorHasTag` _array_element "Dead") (`self.ActorHasTag` _array_element "Enemy") (`/Game/TSS_Game/Blueprints/System/BP_CharacterBase.IsEvading?` (cast `/Game/TSS_Game/Blueprints/System/BP_CharacterBase` _array_element :!pure true))))
      (message `/Game/TSS_Game/Blueprints/System/BPI_Damagable.DamageIntercation` _array_element (`self.Damage Dealt`) null true (`self.Damage Type`))
      (bind _returnvalue (`self.GetInstigatorController` _array_element))
      (`/Engine/EditorBlueprintResources/StandardMacros.IsValid` _returnvalue
        (:`Is Valid`
          (if (== _returnvalue (`GameplayStatics.GetPlayerController` 0))
            (message `/Game/TSS_Game/Blueprints/AbilitySystem/BuffSystem/Base/BPI_Buffable.Attach Buff Request` _returnvalue (make `/Game/TSS_Game/Blueprints/AbilitySystem/BuffSystem/ST_BuffSettingsMSG` _array_element "/Game/TSS_Game/Blueprints/AbilitySystem/BuffSystem/AC_Buff_Toxins.AC_Buff_Toxins_C" 1 (`self.Buff Owner`) true 5.0 10.0 20.0 5.0)))))))
  (`KismetSystemLibrary.Delay` 1.0)
  (`self.K2_DestroyActor`))

(fn `UserConstructionScript`)