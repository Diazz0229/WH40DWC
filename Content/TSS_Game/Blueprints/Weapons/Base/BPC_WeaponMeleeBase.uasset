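; Base melee weapon that runs combo attacks for the player, swapping to the secondary weapon and optionally back to primary afterwards.
; The locally controlled player cycles attack montages, whose notifies open and close the damage window and Niagara effect.
; DamageCollision overlaps hit each living BPI_Damagable actor once per swing, dealing damage through the player or its controller.
; Server-to-multicast events replay attack animation, sound and impact effects for other players.
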(event `SV_Melee`
  (`self.MC_MeleeAttack`))

(event `MC_MeleeAttack`
  (bind _attackmontageindex (`self.AttackMontageIndex`))
  (bind _playercast (`self.PlayerCast`))
  (`/Engine/EditorBlueprintResources/StandardMacros.IsValid` _playercast
    (:`Is Valid`
      (if (not (`Pawn.IsLocallyControlled` _playercast))
        (`/Game/TSS_Game/Blueprints/System/BP_CharacterBase.InstantRotationToMouse` _playercast)
        (`KismetSystemLibrary.Delay` 0.01)
        (`ActorComponent.SetActive` (`self.Niagara`) true true)
        (`|PlayMontage` (`Character.Mesh` (`self.PlayerCast`)) (`|GetArrayItem` (`self.AttackMontagesFast`) (`self.AttackMontageIndex`)) (`self.MeleeAttackSpeed`)
          (:`then`
            (`GameplayStatics.SpawnSoundAtLocation` (`self.FiringSound`) (`self.K2_GetActorLocation`) (struct) 1.0 1.0 0.0 null null :!label _label) ; Firing Sound
            (`/Engine/EditorBlueprintResources/StandardMacros.IncrementInt` _attackmontageindex
              (:`  `
                (if (> _attackmontageindex (`KismetArrayLibrary.Array_LastIndex` (`self.AttackMontagesFast`)))
                  (set `self.AttackMontageIndex` 0))))))))))

(event `MeleeResetAnimations`
  (set `self.AttackMontageIndex` 0))

(event `MeleeDealDamage`
  (params (`Damage Target` :type "Actor Object Reference"))
  (bind _playercast (`self.PlayerCast`))
  (bind _asbp_player_controller (cast `/Game/TSS_Game/Blueprints/System/BP_PlayerController` (`Pawn.GetController` _playercast)))
  (`/Game/TSS_Game/Blueprints/System/BP_PlayerController.DealDamage` _asbp_player_controller `Damage Target` (`self.Damage`) _playercast)
  (`self.SV_BloodAndSound` `Damage Target`))

(event `self.DamageCollision.OnComponentBeginOverlap`
  (params (OverlappedComponent :type "PrimitiveComponent Object Reference") (OtherActor :type "Actor Object Reference") (OtherComp :type "PrimitiveComponent Object Reference") (OtherBodyIndex :type Integer) (bFromSweep :type Boolean) (SweepResult :type "HitResult Structure (by ref)"))
  (bind _playercast (`self.PlayerCast`))
  (bind _actorshit (`self.ActorsHit`))
  (`/Engine/EditorBlueprintResources/StandardMacros.IsValid` _playercast
    (:`Is Valid`
      (if (and (`/Game/TSS_Game/Blueprints/System/BP_CharacterBase.IsMeleeDamaging?` _playercast) (not (`/Game/TSS_Game/Blueprints/System/BP_CharacterBase.IsDead` _playercast)))
        (bind _output_get (set `self.Other Actor` OtherActor))
        (if (and (not (`KismetArrayLibrary.Array_Contains` _actorshit _output_get)) (not (`self.ActorHasTag` _output_get "Dead")) (`KismetSystemLibrary.DoesImplementInterface` _output_get "/Game/TSS_Game/Blueprints/System/BPI_Damagable.BPI_Damagable_C"))
          (`KismetArrayLibrary.Array_Add` _actorshit _output_get)
          (`self.MeleeDealDamage` _output_get))))))

(event `SV_BloodAndSound`
  (params (`Damage Target` :type "Actor Object Reference"))
  (`/Engine/EditorBlueprintResources/StandardMacros.IsValid` `Damage Target`
    (:`Is Valid`
      (`self.MC_BloodAndSound` `Damage Target`))))

(event `MC_BloodAndSound`
  (params (`Damage Target` :type "Actor Object Reference"))
  (bind _returnvalue (`self.K2_GetActorLocation` `Damage Target`))
  (`/Engine/EditorBlueprintResources/StandardMacros.IsValid` `Damage Target`
    (:`Is Valid`
      (`GameplayStatics.SpawnSoundAtLocation` (`self.HitSound`) _returnvalue (struct) 1.0 1.0 0.0 null null)
      (`GameplayStatics.SpawnEmitterAtLocation` "/Game/TSS_Game/Particles/P_body_bullet_impact.P_Body_Bullet_Impact" _returnvalue (struct) (5.0 5.0 5.0)))))

(event `MeleeStopComplete`
  (bind _playercast (`self.PlayerCast`))
  (bind _playercast_2 (`self.PlayerCast`))
  (bind _wpn_primary (`/Game/TSS_Game/Blueprints/System/BP_CharacterBase.WPN_Primary` _playercast_2))
  (`self.MeleeResetAnimations`)
  (`ActorComponent.SetActive` (`self.Niagara`) false true)
  (set `/Game/TSS_Game/Blueprints/System/BP_CharacterBase.IsMeleeAttacking` false _playercast)
  (set `/Game/TSS_Game/Blueprints/System/BP_CharacterBase.IsMeleeDamaging?` false _playercast)
  (`KismetArrayLibrary.Array_Clear` (`self.ActorsHit`))
  (if (`/Game/TSS_Game/Blueprints/System/BP_CharacterBase.ShouldSwitchBackToMain?` _playercast_2)
    (if (== (`/Game/TSS_Game/Blueprints/System/BP_CharacterBase.EquippedWeapon` _playercast_2) _wpn_primary)
      (`KismetSystemLibrary.PrintString` "WeaponMeleeBase: Equiped is already primary")
      (else
        (`/Game/TSS_Game/Blueprints/System/BP_CharacterBase.Equip_From_Inventory` _playercast_2 (`KismetArrayLibrary.Array_Find` (`/Game/TSS_Game/Blueprints/System/BP_CharacterBase.UT_Inventory` _playercast_2) _wpn_primary))))
    (else
      (`KismetSystemLibrary.PrintString` "WeaponMeleeBase: Should not switch back"))))

(event `self.Fire`
  (bind _playercast (`self.PlayerCast`))
  (bind _playercast_2 (`self.PlayerCast`))
  (bind _playercast_3 (`self.PlayerCast`))
  (bind _playercast_4 (`self.PlayerCast`))
  (bind _equippedweapon (`/Game/TSS_Game/Blueprints/System/BP_CharacterBase.EquippedWeapon` _playercast_4))
  (`/Engine/EditorBlueprintResources/StandardMacros.IsValid` _playercast_4
    (:`Is Valid`
      (if (`Pawn.IsLocallyControlled` _playercast_4)
        (if (or (`/Game/TSS_Game/Blueprints/System/BP_CharacterBase.IsMeleeAttacking` _playercast_4) (`/Game/TSS_Game/Blueprints/System/BP_CharacterBase.IsDead` _playercast_4))
          (`KismetSystemLibrary.PrintString` "WeaponMeleeBase: Dead or Damaging")
          (else
            (set `/Game/TSS_Game/Blueprints/System/BP_CharacterBase.IsMeleeAttacking` true _playercast_4)
            (if (`/Game/TSS_Game/Blueprints/Weapons/Base/BP_WeaponBase.isReloading` _equippedweapon)
              (set `/Game/TSS_Game/Blueprints/Weapons/Base/BP_WeaponBase.isReloading` false _equippedweapon))
            (if (not (== _equippedweapon (`/Game/TSS_Game/Blueprints/System/BP_CharacterBase.WPN_Secondary` _playercast_4)))
              (`/Game/TSS_Game/Blueprints/System/BP_CharacterBase.Equip_From_Inventory` _playercast (`KismetArrayLibrary.Array_Find` (`/Game/TSS_Game/Blueprints/System/BP_CharacterBase.UT_Inventory` _playercast) (`/Game/TSS_Game/Blueprints/System/BP_CharacterBase.WPN_Secondary` _playercast))))
            (if (`/Game/TSS_Game/Blueprints/System/BP_CharacterBase.IsSprinting?` _playercast_4)
              (`/Game/TSS_Game/Blueprints/System/BP_CharacterBase.SprintEnd` _playercast_4 true false))
            (`KismetArrayLibrary.Array_Clear` (`self.ActorsHit`))
            (for _array_element (`PrimitiveComponent.GetOverlappingActors` (`self.DamageCollision`) null)
              (if (and (`KismetSystemLibrary.DoesImplementInterface` _array_element "/Game/TSS_Game/Blueprints/System/BPI_Damagable.BPI_Damagable_C") (not (`self.ActorHasTag` _array_element "Dead")))
                (`KismetArrayLibrary.Array_Add` (`self.ActorsHit`) _array_element)
                (`/Game/TSS_Game/Blueprints/System/BP_CharacterBase.MeleeDealDamage` (`self.PlayerCast`) _array_element)))
            (`/Game/TSS_Game/Blueprints/System/BP_CharacterBase.InstantRotationToMouse` (`self.PlayerCast`))
            (`KismetSystemLibrary.Delay` 0.01)
            (`ActorComponent.SetActive` (`self.Niagara`) true true)
            (bind _notifyname (`|PlayMontage` (`Character.Mesh` (`self.PlayerCast`)) (`|GetArrayItem` (`self.AttackMontagesFast`) (`self.AttackMontageIndex`)) (`self.MeleeAttackSpeed`))
              (:`then`
                (`/Engine/EditorBlueprintResources/StandardMacros.IsValid` _playercast_2
                  (:`Is Valid`
                    (`/Game/TSS_Game/Blueprints/System/BP_CharacterBase.SV_StartMeleeAttack` _playercast_2)
                    (goto _label))))
              (:`OnCompleted`
                (`self.MeleeStopComplete`))
              (:`OnNotifyBegin`
                (if (== _notifyname "Melee_end")
                  (set `/Game/TSS_Game/Blueprints/System/BP_CharacterBase.IsMeleeDamaging?` false _playercast_3)
                  (set `/Game/TSS_Game/Blueprints/System/BP_CharacterBase.IsMeleeAttacking` false _playercast_3)
                  (`ActorComponent.SetActive` (`self.Niagara`) false true)
                  (elif (== _notifyname "Melee_start")
                    (set `/Game/TSS_Game/Blueprints/System/BP_CharacterBase.IsMeleeDamaging?` true _playercast_3)))))))))))

(fn `UserConstructionScript`
  (`parent.UserConstructionScript`))