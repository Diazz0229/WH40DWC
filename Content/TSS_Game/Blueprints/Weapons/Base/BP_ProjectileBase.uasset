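; Base weapon projectile that takes damage and pierce count from the owner's equipped weapon.
; On hit or overlap, it damages BPI_Damagable targets through the owner's BP_PlayerController, using a sphere trace for splash or a locally controlled check for single hits.
; Impacts spawn Niagara or Cascade effects and push physics bodies.
; Piercing relaunches it by switching collision to Overlap and replacing the movement component; otherwise it hides and self-destroys after a delay.
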(event `self.ReceiveBeginPlay`
  (`ProjectileMovementComponent.SetVelocityInLocalSpace` (`self.ProjectileMovement`) (10000.0 0.0 0.0))
  (`PrimitiveComponent.SetCollisionResponseToChannel` (`self.Sphere1`) "ECC_WorldDynamic" "ECR_Block")
  (set `self.ProjectileMovementComponent` (`self.ProjectileMovement`)))

(event `ProjectileInit`
  (bind _ownercharacter (`self.OwnerCharacter`))
  (bind _equippedweapon (`/Game/TSS_Game/Blueprints/System/BP_CharacterBase.EquippedWeapon` _ownercharacter))
  (`/Engine/EditorBlueprintResources/StandardMacros.IsValid` _ownercharacter
    (:`Is Valid`
      (if (and (`Pawn.IsLocallyControlled` _ownercharacter) (`self.IsMCShot`))
        (`self.K2_DestroyActor`)
        (else
          (`SceneComponent.SetVisibility` (`self.Sphere1`) true true)
          (set `self.ProjectileDamage` (`/Game/TSS_Game/Blueprints/Weapons/Base/BP_WeaponBase.Damage` _equippedweapon))
          (set `self.PierceTargets` (`/Game/TSS_Game/Blueprints/Weapons/Base/BP_WeaponBase.PenetratedTargets` _equippedweapon)))))
    (:`Is Not Valid`
      (`KismetSystemLibrary.PrintString` "BP_ProjectileBase: PLayer controller is not valid"))))

(event `self.ReceiveHit`
  (params (MyComp :type "PrimitiveComponent Object Reference") (Other :type "Actor Object Reference") (OtherComp :type "PrimitiveComponent Object Reference") (bSelfMoved :type Boolean) (HitLocation :type "Vector Structure") (HitNormal :type "Vector Structure") (NormalImpulse :type "Vector Structure") (Hit :type "HitResult Structure (by ref)"))
  (bind (_bblockinghit _binitialoverlap _time _distance _location _impactpoint _normal _impactnormal _physmat _hitactor) (`GameplayStatics.BreakHitResult` Hit))
  (bind _ownercharacter (`self.OwnerCharacter`))
  (bind _hit_actor (`self.Hit Actor`))
  (bind _piercetargets (`self.PierceTargets`))
  (bind _splashradius (`self.SplashRadius`))
  (bind _ownercharacter_2 (`self.OwnerCharacter`))
  (bind _projectilemovementcomponent (`self.ProjectileMovementComponent`))
  (bind _ownercharacter_3 (`self.OwnerCharacter`))
  (bind _bulletmesh (`self.BulletMesh`))
  (bind _impactlocation (`self.ImpactLocation`))
  (bind _hit_actor_2 (`self.Hit Actor`))
  (set `self.Other Comp` MyComp)
  (set `self.Hit Actor` _hitactor)
  (set `self.ImpactLocation` _location)
  (`/Engine/EditorBlueprintResources/StandardMacros.IsValid` _ownercharacter :!label _label
    (:`Is Valid`
      (if (> _splashradius 0.0)
        (bind _outhits (`KismetSystemLibrary.SphereTraceMulti` _impactlocation _impactlocation _splashradius "TraceTypeQuery1"))
        (for _array_element _outhits
          (bind (_bblockinghit_2 _binitialoverlap_2 _time_2 _distance_2 _location_2 _impactpoint_2 _normal_2 _impactnormal_2 _physmat_2 _hitactor_2) (`GameplayStatics.BreakHitResult` _array_element))
          (`/Engine/EditorBlueprintResources/StandardMacros.IsValid` _hitactor_2
            (:`Is Valid`
              (if (not (`KismetArrayLibrary.Array_Contains` (`self.Enemies to Hit`) _hitactor_2))
                (`KismetArrayLibrary.Array_AddUnique` (`self.Enemies to Hit`) _hitactor_2)))))
        (for _array_element_2 (`self.Enemies to Hit`)
          (if (`KismetSystemLibrary.DoesImplementInterface` _array_element_2 "/Game/TSS_Game/Blueprints/System/BPI_Damagable.BPI_Damagable_C")
            (bind _asbp_player_controller (cast `/Game/TSS_Game/Blueprints/System/BP_PlayerController` (`Pawn.GetController` _ownercharacter_2)))
            (`/Game/TSS_Game/Blueprints/System/BP_PlayerController.DealDamage` _asbp_player_controller _array_element_2 (`self.ProjectileDamage`) _ownercharacter_2)))
        (`self.SpawnHitEmitter` :!label _label_2)
        (`self.ApplyPhysics` (`self.Other Comp`))
        (if (> _piercetargets 0) :!label _label_3
          (`/Engine/EditorBlueprintResources/StandardMacros.DecrementInt` _piercetargets
            (:`  `
              (`self.LaunchProjectileAgain`)))
          (else
            (`self.SpawnHitEmitter` :!label _label_4)
            (`/Engine/EditorBlueprintResources/StandardMacros.IsValid` _projectilemovementcomponent
              (:`Is Valid`
                (`ActorComponent.Deactivate` _projectilemovementcomponent))
              (:`Is Not Valid`
                _))
            (`ActorComponent.Deactivate` _bulletmesh)
            (`SceneComponent.SetVisibility` _bulletmesh false false)
            (`KismetSystemLibrary.Delay` (`self.LifeTime_AfterHit`))
            (`self.K2_DestroyActor`)))
        (else
          (`/Engine/EditorBlueprintResources/StandardMacros.DoOnce` false :!label _label_5
            (:`Completed`
              (if (and (`Pawn.IsLocallyControlled` _ownercharacter) (`KismetSystemLibrary.DoesImplementInterface` _hit_actor_2 "/Game/TSS_Game/Blueprints/System/BPI_Damagable.BPI_Damagable_C"))
                (if (`KismetArrayLibrary.Array_Contains` (`self.EnemiesAlreadyHit`) _hit_actor_2)
                  (`self.LaunchProjectileAgain`)
                  (else
                    (bind _asbp_player_controller_2 (cast `/Game/TSS_Game/Blueprints/System/BP_PlayerController` (`Pawn.GetController` _ownercharacter_3)))
                    (`/Game/TSS_Game/Blueprints/System/BP_PlayerController.DealDamage` _asbp_player_controller_2 _hit_actor (`self.ProjectileDamage`) _ownercharacter_3)
                    (`KismetArrayLibrary.Array_AddUnique` (`self.EnemiesAlreadyHit`) _hit_actor)
                    (goto _label_2)))
                (else
                  (goto _label_3))))))))
    (:`Is Not Valid`
      (goto _label_4))))

(event `ResetDamageAbility`
  (goto _label_5 :!via `Reset`))

(event `self.Sphere1.OnComponentBeginOverlap`
  (params (OverlappedComponent :type "PrimitiveComponent Object Reference") (OtherActor :type "Actor Object Reference") (OtherComp :type "PrimitiveComponent Object Reference") (OtherBodyIndex :type Integer) (bFromSweep :type Boolean) (SweepResult :type "HitResult Structure (by ref)"))
  (bind (_bblockinghit _binitialoverlap _time _distance _location _impactpoint _normal _impactnormal _physmat _hitactor) (`GameplayStatics.BreakHitResult` SweepResult))
  (set `self.Other Comp` OtherComp)
  (set `self.Hit Actor` _hitactor)
  (set `self.ImpactLocation` _location)
  (goto _label))

(event `SpawnHitEmitter`
  (bind _impactlocation (`self.ImpactLocation`))
  ;[1 1 1] HitEmitter
  (if (`self.IsHitByNiagara`)
    (`NiagaraFunctionLibrary.SpawnSystemAtLocation` (`self.NiagaraHitEffect`) _impactlocation)
    (else
      (`GameplayStatics.SpawnEmitterAtLocation` (`self.HitEmitter`) _impactlocation (struct) (0.5 0.5 0.5)))))

(event `LaunchProjectileAgain`
  (`PrimitiveComponent.SetCollisionResponseToChannel` (`self.Sphere1`) "ECC_WorldDynamic" "ECR_Overlap")
  (`ActorComponent.K2_DestroyComponent` (`self.ProjectileMovementComponent`))
  (bind _returnvalue (`AddComponent|NODE_AddProjectileMovementComponent-0`))
  (bind _output_get (set `self.ProjectileMovementComponent` _returnvalue))
  (`ProjectileMovementComponent.SetVelocityInLocalSpace` _output_get (`self.ProjectileVelocity`))
  (`self.ResetDamageAbility`))

(fn `ApplyPhysics`
  (params (OtherComponent :type "PrimitiveComponent Object Reference"))
  (`/Engine/EditorBlueprintResources/StandardMacros.IsValid` OtherComponent
    (:`Is Valid`
      (if (`SceneComponent.IsSimulatingPhysics` OtherComponent "None")
        (`PrimitiveComponent.AddImpulseAtLocation` OtherComponent (* (`self.GetVelocity`) (`self.ProjectileImpulseStrenght`)) (`self.K2_GetActorLocation`) "None")
        (return)
        (else
          (return))))
    (:`Is Not Valid`
      (return))))

(fn `UserConstructionScript`)