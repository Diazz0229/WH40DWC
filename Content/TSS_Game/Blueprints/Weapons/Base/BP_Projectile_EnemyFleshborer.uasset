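; Enemy Fleshborer projectile that damages BPI_Damagable actors on hit or sphere overlap, then spawns impact effects and destroys itself after a delay.
; Direct hits skip Enemy-tagged and already-hit actors, apply physics impulses, and pierce by replacing the movement component.
; Splash mode gathers targets by sphere trace, but its loop damages the original HitActor each time.
; CheckCritAndDealDamage defines crit rolls but is not called here.
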(event `self.ReceiveBeginPlay`
  (`ProjectileMovementComponent.SetVelocityInLocalSpace` (`self.ProjectileMovement`) (`self.ProjectileVelocity`))
  (`PrimitiveComponent.SetCollisionResponseToChannel` (`self.Sphere1`) "ECC_WorldDynamic" "ECR_Block")
  (set `self.ProjectileMovementComponent` (`self.ProjectileMovement`))
  (`GameplayStatics.SpawnSoundAttached` "/Game/TSS_Game/SFX/Characters/Tyranids/Weapons/SC_TYR_Fleshstings.SC_TYR_Fleshstings" (`self.BulletMesh`) "None" (0.0 0.0 0.0) (struct) "KeepRelativeOffset" false 1.0 1.0 0.0 null null)
  (`GameplayStatics.SpawnEmitterAtLocation` (`self.HitEmitter`) (`self.K2_GetActorLocation` self)))

(event `ProjectileInit`)

(event `self.ReceiveHit`
  (params (MyComp :type "PrimitiveComponent Object Reference") (Other :type "Actor Object Reference") (OtherComp :type "PrimitiveComponent Object Reference") (bSelfMoved :type Boolean) (HitLocation :type "Vector Structure") (HitNormal :type "Vector Structure") (NormalImpulse :type "Vector Structure") (Hit :type "HitResult Structure (by ref)"))
  (bind (_bblockinghit _binitialoverlap _time _distance _location _impactpoint _normal _impactnormal _physmat _hitactor) (`GameplayStatics.BreakHitResult` Hit))
  (bind _piercetargets (`self.PierceTargets`))
  (bind _hit_actor (`self.Hit Actor`))
  (bind _projectilemovementcomponent (`self.ProjectileMovementComponent`))
  (bind _bulletmesh (`self.BulletMesh`))
  (bind _impactlocation (`self.ImpactLocation`))
  (bind _splashradius (`self.SplashRadius`))
  (bind _returnvalue (`KismetSystemLibrary.DoesImplementInterface` _hit_actor "/Game/TSS_Game/Blueprints/System/BPI_Damagable.BPI_Damagable_C"))
  (set `self.Other Comp` MyComp)
  (set `self.Hit Actor` _hitactor)
  (set `self.ImpactLocation` _location)
  (if _returnvalue :!label _label
    (if (> _splashradius 0.0)
      (bind _outhits (`KismetSystemLibrary.SphereTraceMulti` _impactlocation _impactlocation _splashradius "TraceTypeQuery1"))
      (for _array_element _outhits
        (bind (_bblockinghit_2 _binitialoverlap_2 _time_2 _distance_2 _location_2 _impactpoint_2 _normal_2 _impactnormal_2 _physmat_2 _hitactor_2) (`GameplayStatics.BreakHitResult` _array_element))
        (`/Engine/EditorBlueprintResources/StandardMacros.IsValid` _hitactor_2
          (:`Is Valid`
            (if (not (`KismetArrayLibrary.Array_Contains` (`self.Enemies to Hit`) _hitactor_2))
              (`KismetArrayLibrary.Array_AddUnique` (`self.Enemies to Hit`) _hitactor_2)))))
      (for _array_element_2 (`self.Enemies to Hit`)
        (if (`KismetSystemLibrary.DoesImplementInterface` _array_element_2 "/Game/TSS_Game/Blueprints/System/BPI_Damagable.BPI_Damagable_C")
          (message `/Game/TSS_Game/Blueprints/System/BPI_Damagable.DamageIntercation` (`self.Hit Actor`) (`self.ProjectileDamage`) (`self.OwnerCharacter`) true (`self.Damage Type`))))
      (`self.ApplyPhysics` (`self.Other Comp`) :!label _label_2)
      (if (> _piercetargets 0) :!label _label_3
        (`/Engine/EditorBlueprintResources/StandardMacros.DecrementInt` _piercetargets
          (:`  `
            (`self.LaunchProjectileAgain`)))
        (else
          (`self.SpawnHitEmitter` :!label _label_4)
          (`/Engine/EditorBlueprintResources/StandardMacros.IsValid` _projectilemovementcomponent
            (:`Is Valid`
              (`ActorComponent.Deactivate` _projectilemovementcomponent))
            (:`Is Not Valid`
              _))
          (`SceneComponent.SetVisibility` _bulletmesh false false)
          (`ActorComponent.Deactivate` _bulletmesh)
          (`ActorComponent.Deactivate` (`self.NS_BulletTrail_1_b`))
          (`KismetSystemLibrary.Delay` (`self.LifeTime_AfterHit`))
          (`self.K2_DestroyActor`)))
      (else
        (`/Engine/EditorBlueprintResources/StandardMacros.DoOnce` false :!label _label_5
          (:`Completed`
            (if _returnvalue
              (if (or (`KismetArrayLibrary.Array_Contains` (`self.EnemiesAlreadyHit`) _hit_actor) (`self.ActorHasTag` _hit_actor "Enemy"))
                (`self.LaunchProjectileAgain`)
                (else
                  (message `/Game/TSS_Game/Blueprints/System/BPI_Damagable.DamageIntercation` (`self.Hit Actor`) (`self.ProjectileDamage`) (`self.OwnerCharacter`) true (`self.Damage Type`))
                  (`KismetArrayLibrary.Array_AddUnique` (`self.EnemiesAlreadyHit`) (`self.Hit Actor`))
                  (goto _label_2)))
              (else
                (goto _label_3)))))))
    (else
      (goto _label_4))))

(event `ResetDamageAbility`
  (goto _label_5 :!via `Reset`))

(event `self.Sphere1.OnComponentBeginOverlap`
  (params (OverlappedComponent :type "PrimitiveComponent Object Reference") (OtherActor :type "Actor Object Reference") (OtherComp :type "PrimitiveComponent Object Reference") (OtherBodyIndex :type Integer) (bFromSweep :type Boolean) (SweepResult :type "HitResult Structure (by ref)"))
  (bind (_bblockinghit _binitialoverlap _time _distance _location _impactpoint _normal _impactnormal _physmat _hitactor) (`GameplayStatics.BreakHitResult` SweepResult))
  (set `self.Other Comp` OtherComp)
  (set `self.Hit Actor` _hitactor)
  (set `self.ImpactLocation` _location)
  (goto _label))

(event `LaunchProjectileAgain`
  (`PrimitiveComponent.SetCollisionResponseToChannel` (`self.Sphere1`) "ECC_WorldDynamic" "ECR_Overlap")
  (`ActorComponent.K2_DestroyComponent` (`self.ProjectileMovementComponent`))
  (bind _returnvalue (`AddComponent|NODE_AddProjectileMovementComponent-0`))
  (bind _output_get (set `self.ProjectileMovementComponent` _returnvalue))
  (`ProjectileMovementComponent.SetVelocityInLocalSpace` _output_get (`self.ProjectileVelocity`))
  (`self.ResetDamageAbility`))

(event `SpawnHitEmitter`
  (bind _impactlocation (`self.ImpactLocation`))
  ;[1 1 1] HitEmitter
  (if (`self.IsHitByNiagara`)
    (`NiagaraFunctionLibrary.SpawnSystemAtLocation` (`self.NiagaraHitEffect`) _impactlocation)
    (else
      (`GameplayStatics.SpawnEmitterAtLocation` (`self.HitEmitter`) _impactlocation (struct) (3.0 3.0 3.0)))))

(fn `ApplyPhysics`
  (params (OtherComponent :type "PrimitiveComponent Object Reference"))
  (`/Engine/EditorBlueprintResources/StandardMacros.IsValid` OtherComponent
    (:`Is Valid`
      (if (`SceneComponent.IsSimulatingPhysics` OtherComponent "None")
        (`PrimitiveComponent.AddImpulseAtLocation` OtherComponent (* (`self.GetVelocity`) (`self.ProjectileImpulseStrenght`)) (`self.K2_GetActorLocation`) "None")
        (return)
        (else
          (return))))
    (:`Is Not Valid`
      (return))))

(fn `CheckCritAndDealDamage`
  (params (DamageTarget :type "Actor Object Reference") (Target :type "/Game/TSS_Game/Blueprints/System/BP_PlayerController Object Reference") (Source :type "/Game/TSS_Game/Blueprints/System/BP_CharacterBase Object Reference"))
  (bind _projectiledamage (`self.ProjectileDamage`))
  (if (<= (`KismetMathLibrary.RandomFloatInRange` 0.0 100.0) (`self.Crit Chance`))
    (set `self.ProjectileDamage` (* (`self.ProjectileDamage`) (`self.Crit Multiplier`)))
    (`/Game/TSS_Game/Blueprints/System/BP_PlayerController.DealDamage` Target DamageTarget _projectiledamage Source true (`self.Damage Type`))
    (else
      (`/Game/TSS_Game/Blueprints/System/BP_PlayerController.DealDamage` Target DamageTarget _projectiledamage Source false (`self.Damage Type`)))))

(fn `UserConstructionScript`)