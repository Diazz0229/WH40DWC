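; Plasma pistol weapon Blueprint, a variant assembled from modular meshes, with firing left to the parent class.
; The construction script attaches muzzle, rear and handle parts, plus two red Inquisition decoration meshes, to WeaponMesh sockets.
; Each added component renders custom depth and ignores all collision channels.
; The parent construction script is never called, and Fire only forwards to the parent.
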(event `self.Fire`
  (`parent.Fire`))

(fn `UserConstructionScript`
  (bind _returnvalue (`AddComponent|NODE_AddStaticMeshComponent-0` :`bManualAttachment` true))
  (`PrimitiveComponent.SetRenderCustomDepth` _returnvalue true)
  (`StaticMeshComponent.SetStaticMesh` _returnvalue "/Game/WH40Assets/Weapons/SM_XX_Plasma_Plasmapistol01/SM_XX_Plasma_Plasmapistol01_MDmuzzle01_ATmuzzle03.SM_XX_Plasma_Plasmapistol01_MDmuzzle01_ATmuzzle03")
  (`SceneComponent.K2_AttachToComponent` _returnvalue (`self.WeaponMesh`) "ATmuzzle01" "KeepRelative" "KeepRelative" "KeepRelative" true)
  (`PrimitiveComponent.SetCollisionResponseToAllChannels` _returnvalue "ECR_Ignore")
  (bind _returnvalue_2 (`AddComponent|NODE_AddStaticMeshComponent-1` :`bManualAttachment` true))
  (`PrimitiveComponent.SetRenderCustomDepth` _returnvalue_2 true)
  (`StaticMeshComponent.SetStaticMesh` _returnvalue_2 "/Game/WH40Assets/Weapons/SM_XX_Plasma_Plasmapistol01/SM_XX_Plasma_Plasmapistol01_MDrear01_ATrear01.SM_XX_Plasma_Plasmapistol01_MDrear01_ATrear01")
  (`SceneComponent.K2_AttachToComponent` _returnvalue_2 (`self.WeaponMesh`) "ATrear01" "KeepRelative" "KeepRelative" "KeepRelative" true)
  (`PrimitiveComponent.SetCollisionResponseToAllChannels` _returnvalue_2 "ECR_Ignore")
  (bind _returnvalue_3 (`AddComponent|NODE_AddStaticMeshComponent-2` :`bManualAttachment` true))
  (`PrimitiveComponent.SetRenderCustomDepth` _returnvalue_3 true)
  (`StaticMeshComponent.SetStaticMesh` _returnvalue_3 "/Game/WH40Assets/Weapons/SM_XX_Plasma_Plasmagun01/SM_XX_Plasma_XX_MDhandle01_AThandle01.SM_XX_Plasma_XX_MDhandle01_AThandle01")
  (`SceneComponent.K2_AttachToComponent` _returnvalue_3 (`self.WeaponMesh`) "AThandle01" "KeepRelative" "KeepRelative" "KeepRelative" true)
  (`PrimitiveComponent.SetCollisionResponseToAllChannels` _returnvalue_3 "ECR_Ignore")
  (bind _returnvalue_4 (`AddComponent|NODE_AddStaticMeshComponent-4` :`bManualAttachment` true))
  (`PrimitiveComponent.SetRenderCustomDepth` _returnvalue_4 true)
  (`StaticMeshComponent.SetStaticMesh` _returnvalue_4 "/Game/Characters/SpaceMarine/BodyPart/Legs/SM_XX_LegRT_Mkvii01/SM_XX_LegRT_XX_VSinquisition_ATlegfrontRT01ATlegfrontRT01_red.SM_XX_LegRT_XX_VSinquisition_ATlegfrontRT01ATlegfrontRT01_red")
  (`SceneComponent.K2_AttachToComponent` _returnvalue_4 (`self.WeaponMesh`) "ATdecoRT02_Inquisition_0" "KeepRelative" "KeepRelative" "KeepRelative" true)
  (`PrimitiveComponent.SetCollisionResponseToAllChannels` _returnvalue_4 "ECR_Ignore")
  (bind _returnvalue_5 (`AddComponent|NODE_AddStaticMeshComponent-5` :`bManualAttachment` true))
  (`PrimitiveComponent.SetRenderCustomDepth` _returnvalue_5 true)
  (`StaticMeshComponent.SetStaticMesh` _returnvalue_5 "/Game/Characters/SpaceMarine/BodyPart/Legs/SM_XX_LegRT_Mkvii01/SM_XX_LegRT_XX_VSinquisition_ATlegfrontRT01ATlegfrontRT01_red.SM_XX_LegRT_XX_VSinquisition_ATlegfrontRT01ATlegfrontRT01_red")
  (`SceneComponent.K2_AttachToComponent` _returnvalue_5 (`self.WeaponMesh`) "ATdecoRT02_Inquisition" "KeepRelative" "KeepRelative" "KeepRelative" true)
  (`PrimitiveComponent.SetCollisionResponseToAllChannels` _returnvalue_5 "ECR_Ignore"))