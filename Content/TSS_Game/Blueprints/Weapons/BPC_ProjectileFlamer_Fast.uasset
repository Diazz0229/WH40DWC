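; Fast flamer projectile Blueprint that sets its hit target on fire, extending a parent projectile class.
; On hit it runs the parent damage logic, then, only if the owning character is locally controlled, sends a burning buff request through the player controller.
; The short-lived burn takes its damage range from the owner's equipped weapon.
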(event `self.DealDamageOnHit`
  (params (DamageTarget :type "Actor Object Reference") (PlController :type "/Game/TSS_Game/Blueprints/System/BP_PlayerController Object Reference") (Source :type "/Game/TSS_Game/Blueprints/System/BP_CharacterBase Object Reference"))
  (bind _equippedweapon (`/Game/TSS_Game/Blueprints/System/BP_CharacterBase.EquippedWeapon` (`self.OwnerCharacter`)))
  (`parent.DealDamageOnHit` DamageTarget PlController Source)
  (if (`Pawn.IsLocallyControlled` (`self.OwnerCharacter`))
    (message `/Game/TSS_Game/Blueprints/AbilitySystem/BuffSystem/Base/BPI_Buffable.Attach Buff Request` PlController (make `/Game/TSS_Game/Blueprints/AbilitySystem/BuffSystem/ST_BuffSettingsMSG` DamageTarget "/Game/TSS_Game/Blueprints/AbilitySystem/BuffSystem/AC_Buff_Burning.AC_Buff_Burning_C" 1 Source false (`/Game/TSS_Game/Blueprints/Weapons/Base/BP_WeaponBase.DamageMin` _equippedweapon) (`/Game/TSS_Game/Blueprints/Weapons/Base/BP_WeaponBase.DamageMax` _equippedweapon) 3.0 0.25))))

(fn `UserConstructionScript`
  (`parent.UserConstructionScript`))