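; Pistol weapon Blueprint variant that adds a decorative bolter skull mesh to the gun.
; The Construction Script runs the parent's setup, then creates a static mesh component attached to the "joint_DecoLT" socket on PistolMesh.
; That mesh renders to custom depth and ignores all collision channels.
; Fire only forwards to the parent, and BeginPlay is disabled.
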(event `self.Fire`
  (`parent.Fire`))

(fn `UserConstructionScript`
  (`parent.UserConstructionScript`)
  (bind _returnvalue (`AddComponent|NODE_AddStaticMeshComponent-0` :`bManualAttachment` true))
  (`PrimitiveComponent.SetRenderCustomDepth` _returnvalue true)
  (`StaticMeshComponent.SetStaticMesh` _returnvalue "/Game/WH40Assets/Weapons/SM_XX_Bolter_Godwyn01/IM_XX_Bolter_XX_VSskull01_ATdeco01ATdeco02ATdeco03.IM_XX_Bolter_XX_VSskull01_ATdeco01ATdeco02ATdeco03")
  (`SceneComponent.K2_AttachToComponent` _returnvalue (`self.Pistol_Mesh`) "joint_DecoLT" "KeepRelative" "KeepRelative" "KeepRelative" true)
  (`PrimitiveComponent.SetCollisionResponseToAllChannels` _returnvalue "ECR_Ignore"))