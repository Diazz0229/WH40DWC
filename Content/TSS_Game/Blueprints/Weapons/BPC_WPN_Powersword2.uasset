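; Power sword weapon Blueprint, a child class that builds its look from modular sword meshes.
; The construction script adds guard, power blade and pommel static meshes and attaches each to its named socket on WeaponMesh.
; Each part renders custom depth and ignores all collision channels.
; BeginPlay only calls the parent; a leftover chainsword idle sound setup is disconnected and never runs.
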(event `self.ReceiveBeginPlay`
  (`parent.ReceiveBeginPlay`))

(fn `UserConstructionScript`
  (bind _weaponmesh (`self.WeaponMesh`))
  (bind _returnvalue (`AddComponent|NODE_AddStaticMeshComponent-0` :`bManualAttachment` true))
  (`PrimitiveComponent.SetRenderCustomDepth` _returnvalue true)
  (`StaticMeshComponent.SetStaticMesh` _returnvalue "/Game/WH40Assets/Weapons/PoweSword/SM_XX_Sword_Sword01/IM_XX_Sword_XX_MDGuard01_ATguard01.IM_XX_Sword_XX_MDGuard01_ATguard01")
  (`SceneComponent.K2_AttachToComponent` _returnvalue _weaponmesh "ATguard01" "KeepRelative" "KeepRelative" "KeepRelative" true)
  (`PrimitiveComponent.SetCollisionResponseToAllChannels` _returnvalue "ECR_Ignore")
  (bind _returnvalue_2 (`AddComponent|NODE_AddStaticMeshComponent-1` :`bManualAttachment` true))
  (`PrimitiveComponent.SetRenderCustomDepth` _returnvalue_2 true)
  (`StaticMeshComponent.SetStaticMesh` _returnvalue_2 "/Game/WH40Assets/Weapons/PoweSword/SM_XX_Sword_Sword01/SM_XX_Sword_XX_MDpower01_ATblade01.SM_XX_Sword_XX_MDpower01_ATblade01")
  (`SceneComponent.K2_AttachToComponent` _returnvalue_2 _weaponmesh "ATblade01" "KeepRelative" "KeepRelative" "KeepRelative" true)
  (`PrimitiveComponent.SetCollisionResponseToAllChannels` _returnvalue_2 "ECR_Ignore")
  (bind _returnvalue_3 (`AddComponent|NODE_AddStaticMeshComponent-2` :`bManualAttachment` true))
  (`PrimitiveComponent.SetRenderCustomDepth` _returnvalue_3 true)
  (`StaticMeshComponent.SetStaticMesh` _returnvalue_3 "/Game/WH40Assets/Weapons/PoweSword/SM_XX_Sword_Sword01/SM_XX_Sword_XX_MDpommel03_ATpommel01.SM_XX_Sword_XX_MDpommel03_ATpommel01")
  (`SceneComponent.K2_AttachToComponent` _returnvalue_3 _weaponmesh "ATpommel01" "KeepRelative" "KeepRelative" "KeepRelative" true)
  (`PrimitiveComponent.SetCollisionResponseToAllChannels` _returnvalue_3 "ECR_Ignore"))