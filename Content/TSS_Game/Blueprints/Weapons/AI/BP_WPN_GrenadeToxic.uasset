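; AI toxic grenade projectile that spawns BP_ToxicExplosion on impact, passing it the damage and damage type, then destroys itself shortly after.
; Hits on damageable enemies, corpses or itself don't detonate; it switches its sphere to overlap WorldDynamic and relaunches by replacing its projectile movement component.
; Crit-damage and physics-impulse helpers are defined but not called within this Blueprint.
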(event `self.ReceiveBeginPlay`
  (`ProjectileMovementComponent.SetVelocityInLocalSpace` (`self.ProjectileMovement`) (`self.ProjectileVelocity`))
  (`PrimitiveComponent.SetCollisionResponseToChannel` (`self.Sphere1`) "ECC_WorldDynamic" "ECR_Block")
  (set `self.ProjectileMovementComponent` (`self.ProjectileMovement`))
  (`GameplayStatics.SpawnEmitterAtLocation` null (`self.K2_GetActorLocation` self)))

(event `self.ReceiveHit`
  (params (MyComp :type "PrimitiveComponent Object Reference") (Other :type "Actor Object Reference") (OtherComp :type "PrimitiveComponent Object Reference") (bSelfMoved :type Boolean) (HitLocation :type "Vector Structure") (HitNormal :type "Vector Structure") (NormalImpulse :type "Vector Structure") (Hit :type "HitResult Structure (by ref)"))
  (bind (_bblockinghit _binitialoverlap _time _distance _location _impactpoint _normal _impactnormal _physmat _hitactor) (`GameplayStatics.BreakHitResult` Hit))
  (bind (_returnvalue_location _returnvalue_rotation) (`KismetMathLibrary.BreakTransform` (`self.GetTransform`)))
  (bind _projectilemovement (`self.ProjectileMovement`))
  (bind _hit_actor (`self.Hit Actor`))
  (bind _returnvalue (`ActorComponent.GetOwner` (`self.Other Comp`)))
  (set `self.Other Comp` OtherComp)
  (set `self.Hit Actor` _hitactor)
  (set `self.ImpactLocation` _location)
  (if (`KismetSystemLibrary.DoesImplementInterface` _hit_actor "/Game/TSS_Game/Blueprints/System/BPI_Damagable.BPI_Damagable_C")
    (`/Engine/EditorBlueprintResources/StandardMacros.DoOnce` false :!label _label
      (:`Completed`
        (if (or (`self.ActorHasTag` _hit_actor "Enemy") (`self.ActorHasTag` _hit_actor "Dead") (== (`self.Hit Actor`) self) (`self.ActorHasTag` _returnvalue "Enemy") (`self.ActorHasTag` _returnvalue "Dead"))
          (`self.LaunchProjectileAgain`)
          (else
            (`/Engine/EditorBlueprintResources/StandardMacros.DoOnce` false :!label _label_2
              (:`Completed`
                (`/Engine/EditorBlueprintResources/StandardMacros.IsValid` _projectilemovement
                  (:`Is Valid`
                    (`ActorComponent.Deactivate` _projectilemovement))
                  (:`Is Not Valid`
                    _))
                (`|SpawnActorFromClass` "/Game/TSS_Game/Blueprints/Weapons/Base/BP_ToxicExplosion.BP_ToxicExplosion_C" (`KismetMathLibrary.MakeTransform` _returnvalue_location _returnvalue_rotation) "Undefined" "MultiplyWithRoot" null (`self.GrenadeDamage`) (`self.Damage Type`) null null)
                (`KismetSystemLibrary.Delay` 0.5)
                (`self.K2_DestroyActor`)))))))
    (else
      (goto _label_2))))

(event `ResetDamageAbility`
  (goto _label :!via `Reset`))

(event `self.Sphere1.OnComponentBeginOverlap`
  (params (OverlappedComponent :type "PrimitiveComponent Object Reference") (OtherActor :type "Actor Object Reference") (OtherComp :type "PrimitiveComponent Object Reference") (OtherBodyIndex :type Integer) (bFromSweep :type Boolean) (SweepResult :type "HitResult Structure (by ref)")))

(event `LaunchProjectileAgain`
  (`PrimitiveComponent.SetCollisionResponseToChannel` (`self.Sphere1`) "ECC_WorldDynamic" "ECR_Overlap")
  (`ActorComponent.K2_DestroyComponent` (`self.ProjectileMovementComponent`))
  (bind _returnvalue (`AddComponent|NODE_AddProjectileMovementComponent-1`))
  (bind _output_get (set `self.ProjectileMovementComponent` _returnvalue))
  (`ProjectileMovementComponent.SetVelocityInLocalSpace` _output_get (`self.ProjectileVelocity`))
  (`self.ResetDamageAbility`))

(fn `ApplyPhysics`
  (params (OtherComponent :type "PrimitiveComponent Object Reference"))
  (`/Engine/EditorBlueprintResources/StandardMacros.IsValid` OtherComponent
    (:`Is Valid`
      (if (`SceneComponent.IsSimulatingPhysics` OtherComponent "None")
        (`PrimitiveComponent.AddImpulseAtLocation` OtherComponent (* (`self.GetVelocity`) (`self.ProjectileImpulseStrenght`)) (`self.K2_GetActorLocation`) "None")
        (return)
        (else
          (return))))
    (:`Is Not Valid`
      (return))))

(fn `CheckCritAndDealDamage`
  (params (DamageTarget :type "Actor Object Reference") (Target :type "/Game/TSS_Game/Blueprints/System/BP_PlayerController Object Reference") (Source :type "/Game/TSS_Game/Blueprints/System/BP_CharacterBase Object Reference"))
  (bind _grenadedamage (`self.GrenadeDamage`))
  (if (<= (`KismetMathLibrary.RandomFloatInRange` 0.0 100.0) (`self.Crit Chance`))
    (set `self.GrenadeDamage` (* (`self.GrenadeDamage`) (`self.Crit Multiplier`)))
    (`/Game/TSS_Game/Blueprints/System/BP_PlayerController.DealDamage` Target DamageTarget _grenadedamage Source true (`self.Damage Type`) 0.0 0.0)
    (else
      (`/Game/TSS_Game/Blueprints/System/BP_PlayerController.DealDamage` Target DamageTarget _grenadedamage Source false (`self.Damage Type`) 0.0 0.0))))

(fn `UserConstructionScript`)