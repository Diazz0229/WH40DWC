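; Sniper weapon Blueprint that assembles a scoped bolter variant from modular parts on top of its parent weapon class.
; The construction script adds static meshes for muzzle, bayonet slot, handle, magazine, sight, grip, scope and top, each attached to its named socket on WeaponMesh.
; Every part renders custom depth and ignores all collision channels.
; BeginPlay only calls the parent, and a skull decoration is left unconnected.
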(event `self.ReceiveBeginPlay`
  (`parent.ReceiveBeginPlay`))

(fn `UserConstructionScript`
  (bind _weaponmesh (`self.WeaponMesh`))
  (`parent.UserConstructionScript`)
  (bind _returnvalue (`AddComponent|NODE_AddStaticMeshComponent-11` :`bManualAttachment` true))
  (`PrimitiveComponent.SetRenderCustomDepth` _returnvalue true)
  (`StaticMeshComponent.SetStaticMesh` _returnvalue "/Game/WH40Assets/Weapons/SM_XX_Bolter_Godwyn01/SM_XX_Bolter_XX_MDmuzzle05_ATmuzzle01.SM_XX_Bolter_XX_MDmuzzle05_ATmuzzle01")
  (`SceneComponent.K2_AttachToComponent` _returnvalue _weaponmesh "ATmuzzle01" "KeepRelative" "KeepRelative" "KeepRelative" true)
  (`PrimitiveComponent.SetCollisionResponseToAllChannels` _returnvalue "ECR_Ignore")
  (bind _returnvalue_2 (`AddComponent|NODE_AddStaticMeshComponent-12` :`bManualAttachment` true))
  (`PrimitiveComponent.SetRenderCustomDepth` _returnvalue_2 true)
  (`StaticMeshComponent.SetStaticMesh` _returnvalue_2 "/Game/WH40Assets/Weapons/SM_XX_Bolter_Godwyn01/SM_XX_Bolter_XX_MDbayonetslot01_ATbayonetslot01.SM_XX_Bolter_XX_MDbayonetslot01_ATbayonetslot01")
  (`SceneComponent.K2_AttachToComponent` _returnvalue_2 _weaponmesh "ATbayonetslot01" "KeepRelative" "KeepRelative" "KeepRelative" true)
  (`PrimitiveComponent.SetCollisionResponseToAllChannels` _returnvalue_2 "ECR_Ignore")
  (bind _returnvalue_3 (`AddComponent|NODE_AddStaticMeshComponent-13` :`bManualAttachment` true))
  (`PrimitiveComponent.SetRenderCustomDepth` _returnvalue_3 true)
  (`StaticMeshComponent.SetStaticMesh` _returnvalue_3 "/Game/WH40Assets/Weapons/SM_XX_Bolter_Godwyn01/SM_XX_Bolter_XX_MDhandle01_AThandle01.SM_XX_Bolter_XX_MDhandle01_AThandle01")
  (`SceneComponent.K2_AttachToComponent` _returnvalue_3 _weaponmesh "AThandle01" "KeepRelative" "KeepRelative" "KeepRelative" true)
  (`PrimitiveComponent.SetCollisionResponseToAllChannels` _returnvalue_3 "ECR_Ignore")
  (bind _returnvalue_4 (`AddComponent|NODE_AddStaticMeshComponent-14` :`bManualAttachment` true))
  (`PrimitiveComponent.SetRenderCustomDepth` _returnvalue_4 true)
  (`StaticMeshComponent.SetStaticMesh` _returnvalue_4 "/Game/WH40Assets/Weapons/SM_XX_Bolter_Godwyn01/SM_XX_Bolter_XX_MDmag01_ATmag01.SM_XX_Bolter_XX_MDmag01_ATmag01")
  (`SceneComponent.K2_AttachToComponent` _returnvalue_4 _weaponmesh "ATmag01" "KeepRelative" "KeepRelative" "KeepRelative" true)
  (`PrimitiveComponent.SetCollisionResponseToAllChannels` _returnvalue_4 "ECR_Ignore")
  (bind _returnvalue_5 (`AddComponent|NODE_AddStaticMeshComponent-15` :`bManualAttachment` true))
  (`PrimitiveComponent.SetRenderCustomDepth` _returnvalue_5 true)
  (`StaticMeshComponent.SetStaticMesh` _returnvalue_5 "/Game/WH40Assets/Weapons/SM_XX_Bolter_Godwyn01/SM_XX_Bolter_XX_MDsight01_ATsight01.SM_XX_Bolter_XX_MDsight01_ATsight01")
  (`SceneComponent.K2_AttachToComponent` _returnvalue_5 _weaponmesh "ATsight01" "KeepRelative" "KeepRelative" "KeepRelative" true)
  (`PrimitiveComponent.SetCollisionResponseToAllChannels` _returnvalue_5 "ECR_Ignore")
  (bind _returnvalue_6 (`AddComponent|NODE_AddStaticMeshComponent-16` :`bManualAttachment` true))
  (`PrimitiveComponent.SetRenderCustomDepth` _returnvalue_6 true)
  (`StaticMeshComponent.SetStaticMesh` _returnvalue_6 "/Game/WH40Assets/Weapons/SM_XX_Bolter_Godwyn01/CM_XX_Bolter_XX_MDgrip01_ATgrip01.CM_XX_Bolter_XX_MDgrip01_ATgrip01")
  (`SceneComponent.K2_AttachToComponent` _returnvalue_6 _weaponmesh "ATgrip01" "KeepRelative" "KeepRelative" "KeepRelative" true)
  (`PrimitiveComponent.SetCollisionResponseToAllChannels` _returnvalue_6 "ECR_Ignore")
  (bind _returnvalue_7 (`AddComponent|NODE_AddStaticMeshComponent-17` :`bManualAttachment` true))
  (`PrimitiveComponent.SetRenderCustomDepth` _returnvalue_7 true)
  (`StaticMeshComponent.SetStaticMesh` _returnvalue_7 "/Game/WH40Assets/Weapons/SM_XX_Bolter_Godwyn01/SM_XX_XX_XX_MDscope03_ATvisor01.SM_XX_XX_XX_MDscope03_ATvisor01")
  (`SceneComponent.K2_AttachToComponent` _returnvalue_7 _weaponmesh "ATvisor01" "KeepRelative" "KeepRelative" "KeepRelative" true)
  (`PrimitiveComponent.SetCollisionResponseToAllChannels` _returnvalue_7 "ECR_Ignore")
  (bind _returnvalue_8 (`AddComponent|NODE_AddStaticMeshComponent-18` :`bManualAttachment` true))
  (`PrimitiveComponent.SetRenderCustomDepth` _returnvalue_8 true)
  (`StaticMeshComponent.SetStaticMesh` _returnvalue_8 "/Game/WH40Assets/Weapons/SM_XX_Bolter_Godwyn01/SM_XX_Bolter_Godwyn01_MDtop01_ATtop01.SM_XX_Bolter_Godwyn01_MDtop01_ATtop01")
  (`SceneComponent.K2_AttachToComponent` _returnvalue_8 _weaponmesh "ATtop01" "KeepRelative" "KeepRelative" "KeepRelative" true)
  (`PrimitiveComponent.SetCollisionResponseToAllChannels` _returnvalue_8 "ECR_Ignore"))