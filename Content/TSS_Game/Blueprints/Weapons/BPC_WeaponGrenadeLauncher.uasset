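; Grenade launcher weapon Blueprint that assembles its visual model from modular Bolter parts on top of a parent weapon class.
; After the parent construction script, it adds muzzle, bayonet slot, handle, magazine and sight static meshes, attached to matching WeaponMesh sockets.
; The weapon mesh and every added part except the sight are set to ignore all collision channels.
; BeginPlay only calls the parent, and no firing logic is defined here.
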(event `self.ReceiveBeginPlay`
  (`parent.ReceiveBeginPlay`))

(fn `UserConstructionScript`
  (`parent.UserConstructionScript`)
  (bind _returnvalue (`AddComponent|NODE_AddStaticMeshComponent-5` :`bManualAttachment` true))
  (`StaticMeshComponent.SetStaticMesh` _returnvalue "/Game/WH40Assets/Weapons/SM_XX_Bolter_Godwyn01/SM_XX_Bolter_XX_MDmuzzle03_ATmuzzle01.SM_XX_Bolter_XX_MDmuzzle03_ATmuzzle01")
  (`SceneComponent.K2_AttachToComponent` _returnvalue (`self.WeaponMesh`) "ATmuzzle01" "KeepRelative" "KeepRelative" "KeepRelative" true)
  (`PrimitiveComponent.SetCollisionResponseToAllChannels` _returnvalue "ECR_Ignore")
  (bind _returnvalue_2 (`AddComponent|NODE_AddStaticMeshComponent-6` :`bManualAttachment` true))
  (`StaticMeshComponent.SetStaticMesh` _returnvalue_2 "/Game/WH40Assets/Weapons/SM_XX_Bolter_Godwyn01/SM_XX_Bolter_XX_MDbayonetslot01_ATbayonetslot01.SM_XX_Bolter_XX_MDbayonetslot01_ATbayonetslot01")
  (`SceneComponent.K2_AttachToComponent` _returnvalue_2 (`self.WeaponMesh`) "ATbayonetslot01" "KeepRelative" "KeepRelative" "KeepRelative" true)
  (`PrimitiveComponent.SetCollisionResponseToAllChannels` _returnvalue_2 "ECR_Ignore")
  (bind _returnvalue_3 (`AddComponent|NODE_AddStaticMeshComponent-7` :`bManualAttachment` true))
  (`StaticMeshComponent.SetStaticMesh` _returnvalue_3 "/Game/WH40Assets/Weapons/SM_XX_Bolter_Godwyn01/SM_XX_Bolter_XX_MDhandle01_AThandle01.SM_XX_Bolter_XX_MDhandle01_AThandle01")
  (`SceneComponent.K2_AttachToComponent` _returnvalue_3 (`self.WeaponMesh`) "AThandle01" "KeepRelative" "KeepRelative" "KeepRelative" true)
  (`PrimitiveComponent.SetCollisionResponseToAllChannels` _returnvalue_3 "ECR_Ignore")
  (bind _returnvalue_4 (`AddComponent|NODE_AddStaticMeshComponent-8` :`bManualAttachment` true))
  (`StaticMeshComponent.SetStaticMesh` _returnvalue_4 "/Game/WH40Assets/Weapons/SM_XX_Bolter_Godwyn01/SM_XX_Bolter_XX_MDmag05_ATmag01.SM_XX_Bolter_XX_MDmag05_ATmag01")
  (`SceneComponent.K2_AttachToComponent` _returnvalue_4 (`self.WeaponMesh`) "ATmag01" "KeepRelative" "KeepRelative" "KeepRelative" true)
  (`PrimitiveComponent.SetCollisionResponseToAllChannels` _returnvalue_4 "ECR_Ignore")
  (bind _returnvalue_5 (`AddComponent|NODE_AddStaticMeshComponent-9` :`bManualAttachment` true))
  (`StaticMeshComponent.SetStaticMesh` _returnvalue_5 "/Game/WH40Assets/Weapons/SM_XX_Bolter_Godwyn01/SM_XX_Bolter_XX_MDsight02_ATsight01.SM_XX_Bolter_XX_MDsight02_ATsight01")
  (`SceneComponent.K2_AttachToComponent` _returnvalue_5 (`self.WeaponMesh`) "ATsight01" "KeepRelative" "KeepRelative" "KeepRelative" true)
  (`PrimitiveComponent.SetCollisionResponseToAllChannels` (`self.WeaponMesh`) "ECR_Ignore"))