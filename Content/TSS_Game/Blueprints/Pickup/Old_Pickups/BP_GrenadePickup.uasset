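; A grenade pickup actor that adds one grenade to an overlapping character's count and then destroys itself.
; BeginPlay sets the floating name text, and Tick holds it at a fixed world rotation intended to face the camera.
; Overlap casts the other actor to BP_CharacterBase and clamps the new grenade count to a maximum, so it is consumed even when the character is already full.
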(event `self.ReceiveBeginPlay`
  (`TextRenderComponent.K2_SetText` (`self.Name_TXT`) (`self.Name`)))

(event `self.ReceiveTick`
  (params (DeltaSeconds :type "Float (single-precision)"))
  (`SceneComponent.K2_SetWorldRotation` (`self.Name_TXT`) (struct :`Pitch` 45.0 :`Yaw` 180.0) false false) ; Rotates the text to face the camera
)

(event `self.ReceiveActorBeginOverlap`
  (params (OtherActor :type "Actor Object Reference"))
  (bind _asbp_character_base (cast `/Game/TSS_Game/Blueprints/System/BP_CharacterBase` OtherActor))
  (set `/Game/TSS_Game/Blueprints/System/BP_CharacterBase.Grenades` (`KismetMathLibrary.Clamp` (+ (`/Game/TSS_Game/Blueprints/System/BP_CharacterBase.Grenades` _asbp_character_base) 1) 0 5) _asbp_character_base)
  (`self.K2_DestroyActor`))

(fn `UserConstructionScript`)