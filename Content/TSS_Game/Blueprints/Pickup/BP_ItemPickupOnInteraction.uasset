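; BP_ItemPickupOnInteraction is an item pickup actor that shows an interaction prompt while a locally controlled character is nearby.
; A looping half-second timer polls the sphere's overlapping characters and toggles the widget's visibility.
; InteractwithActor only stores the valid interacting character, and ActivationSuccess is empty, so this graph contains no pickup logic itself.
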(event `MessageCheck`
  (bind _interactionwidget (`self.InteractionWidget`))
  (set `self.ShouldShowWidget` false)
  (for _array_element (`PrimitiveComponent.GetOverlappingActors` (`self.Sphere`) "/Game/TSS_Game/Blueprints/System/BP_CharacterBase.BP_CharacterBase_C")
    (bind _asbp_character_base (cast `/Game/TSS_Game/Blueprints/System/BP_CharacterBase` _array_element))
    (bind _owningplayercontroller (`/Game/TSS_Game/Blueprints/System/BP_CharacterBase.OwningPlayerController` _asbp_character_base))
    (`/Engine/EditorBlueprintResources/StandardMacros.IsValid` _owningplayercontroller
      (:`Is Valid`
        (if (`Controller.IsLocalPlayerController` _owningplayercontroller)
          (set `self.ShouldShowWidget` true)))))
  (if (`self.ShouldShowWidget`)
    (`SceneComponent.SetVisibility` _interactionwidget true false)
    (else
      (`SceneComponent.SetVisibility` _interactionwidget false false))))

(event `self.ReceiveBeginPlay`
  (`KismetSystemLibrary.K2_SetTimerDelegate` (delegate `MessageCheck`) 0.5 true)
  (`SceneComponent.SetVisibility` (`self.InteractionWidget`) false false))

(event `self.Interact With Actor`
  (params (CharacterReference :type "/Game/TSS_Game/Blueprints/System/BP_CharacterBase Object Reference"))
  (`/Engine/EditorBlueprintResources/StandardMacros.IsValid` CharacterReference
    (:`Is Valid`
      (set `self.Character` CharacterReference))))

(event `ActivationSuccess`)

(fn `UserConstructionScript`)