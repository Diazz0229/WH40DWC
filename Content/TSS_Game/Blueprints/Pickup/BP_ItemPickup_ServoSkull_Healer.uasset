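; Servo skull pickup that heals the character who collects it and awards points to all players.
; Extends a parent pickup: activation has the character play an interact montage via InteractPickable.
; On multicast success it plays a sound, then the authority credits points and the skull through the game mode.
; The server also requests a stackable timed healing buff, expressed as negative damage, and destroys the pickup.
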(event `self.ActivationSuccess`
  (bind _character (`self.Character`))
  (bind _returnvalue (`Pawn.GetController` _character))
  (`parent.ActivationSuccess`)
  (`GameplayStatics.PlaySoundAtLocation` "/Game/TSS_Game/SFX/Pickup/SFX_Coin_Cue.SFX_Coin_Cue" (`self.K2_GetActorLocation`) (struct) 1.0 1.0 0.0 null null null null)
  (`/Engine/EditorBlueprintResources/ActorMacros.Switch Has Authority`
    (:`Authority`
      (bind _asbp_game_mode_base (cast `/Game/TSS_Game/Blueprints/System/BP_GameModeBase` (`GameplayStatics.GetGameMode`)))
      (`/Game/TSS_Game/Blueprints/System/BP_GameModeBase.AddPointsToAllPlayers` _asbp_game_mode_base (`self.Points to Add`))
      (`/Game/TSS_Game/Blueprints/System/BP_GameModeBase.CollectSkull` _asbp_game_mode_base _returnvalue)
      (message `/Game/TSS_Game/Blueprints/AbilitySystem/BuffSystem/Base/BPI_Buffable.Attach Buff Request` _returnvalue (make `/Game/TSS_Game/Blueprints/AbilitySystem/BuffSystem/ST_BuffSettingsMSG` _character "/Game/TSS_Game/Blueprints/AbilitySystem/BuffSystem/AC_Buff_Healing.AC_Buff_Healing_C" 1 _character true -2.0 -2.0 5.0 1.0))
      (`self.K2_DestroyActor`))))

(event `self.MC_Activate`
  (params (InputObject :type "Object Object Reference"))
  (`parent.MC_Activate` InputObject)
  (`/Game/TSS_Game/Blueprints/System/BP_CharacterBase.InteractPickable` (`self.Character`) self (`self.AnimMontage`)))

(fn `UserConstructionScript`
  (`parent.UserConstructionScript`))