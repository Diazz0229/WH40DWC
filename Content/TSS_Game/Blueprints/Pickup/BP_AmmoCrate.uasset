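; Limited-use ammo crate pickup that replenishes a character's equipment and non-melee weapons, then destroys itself once depleted.
; A looping timer checks sphere overlaps to show the interaction widget for local players.
; Interaction passes a DoOnce gate into the character's crate interaction and hides the light until the authority re-enables the crate.
; MC_AmmoRestored applies the refill, spawns floating text, advances the light color and reduces remaining supply.
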(event `MessageCheck`
  (bind _interactionwidget (`self.InteractionWidget`))
  (set `self.ShouldShowWidget` false)
  (for _array_element (`PrimitiveComponent.GetOverlappingActors` (`self.Sphere`) "/Game/TSS_Game/Blueprints/System/BP_CharacterBase.BP_CharacterBase_C")
    (bind _asbp_character_base (cast `/Game/TSS_Game/Blueprints/System/BP_CharacterBase` _array_element))
    (bind _owningplayercontroller (`/Game/TSS_Game/Blueprints/System/BP_CharacterBase.OwningPlayerController` _asbp_character_base))
    (`/Engine/EditorBlueprintResources/StandardMacros.IsValid` _owningplayercontroller
      (:`Is Valid`
        (if (`Controller.IsLocalPlayerController` _owningplayercontroller)
          (set `self.ShouldShowWidget` true)))))
  (if (`self.ShouldShowWidget`)
    (`SceneComponent.SetVisibility` _interactionwidget true false)
    (else
      (`SceneComponent.SetVisibility` _interactionwidget false false))))

(event `self.ReceiveBeginPlay`
  (`KismetSystemLibrary.K2_SetTimerDelegate` (delegate `MessageCheck`) 0.5 true)
  (`SceneComponent.SetVisibility` (`self.InteractionWidget`) false false))

(event `self.Interact With Actor`
  (params (CharacterReference :type "/Game/TSS_Game/Blueprints/System/BP_CharacterBase Object Reference"))
  (`self.ActivateObject` CharacterReference))

(event `MC_CrateAvailable`
  (`SceneComponent.SetVisibility` (`self.Light`) true false)
  (goto _label :!via `Reset`))

(event `ActivateObject`
  (params (InputObject :type "Object Object Reference"))
  (`/Engine/EditorBlueprintResources/StandardMacros.IsValid` InputObject
    (:`Is Valid`
      (bind _asbp_character_base (cast `/Game/TSS_Game/Blueprints/System/BP_CharacterBase` InputObject))
      (`/Engine/EditorBlueprintResources/StandardMacros.DoOnce` false :!label _label
        (:`Completed`
          (bind _output_get (set `self.Character` _asbp_character_base))
          (`/Game/TSS_Game/Blueprints/System/BP_CharacterBase.StartInteractingWithCrate` _output_get self)
          (`SceneComponent.SetVisibility` (`self.Light`) false false)
          (`/Engine/EditorBlueprintResources/ActorMacros.Switch Has Authority`
            (:`Authority`
              (`KismetSystemLibrary.Delay` 3.0)
              (`self.MC_CrateAvailable`))))))))

(event `MC_AmmoRestored`
  (params (Target :type "/Game/TSS_Game/Blueprints/System/BP_CharacterBase Object Reference"))
  (bind _output_get (set `self.TEMP_RestoredChar` Target))
  (for _array_element (`/Game/TSS_Game/Blueprints/System/BP_CharacterBase.EQP_Slots` _output_get)
    (bind _asac_eqp_base (cast `/Game/TSS_Game/Blueprints/Equipment/AC_EQP_Base` _array_element))
    (set `/Game/TSS_Game/Blueprints/Equipment/AC_EQP_Base.AmmoCur` (`KismetMathLibrary.Clamp` (+ (`/Game/TSS_Game/Blueprints/Equipment/AC_EQP_Base.AmmoCur` _asac_eqp_base) 1) 0 (`/Game/TSS_Game/Blueprints/Equipment/AC_EQP_Base.AmmoMax` _asac_eqp_base)) _asac_eqp_base))
  (for _array_element_2 (`/Game/TSS_Game/Blueprints/System/BP_CharacterBase.UT_Inventory` _output_get)
    (`/Engine/EditorBlueprintResources/StandardMacros.IsValid` _array_element_2
      (:`Is Valid`
        (if (not (`/Game/TSS_Game/Blueprints/Weapons/Base/BP_WeaponBase.IsMelee?` _array_element_2))
          (if (`/Game/TSS_Game/Blueprints/Weapons/Base/BP_WeaponBase.SingleMag?` _array_element_2)
            (bind _ammomax (`/Game/TSS_Game/Blueprints/Weapons/Base/BP_WeaponBase.AmmoMax` _array_element_2))
            (bind _output_get_2 (set `/Game/TSS_Game/Blueprints/Weapons/Base/BP_WeaponBase.AmmoCurrent` (`KismetMathLibrary.Clamp` (+ (stale _output_get_2) (/ _ammomax 2)) 0 _ammomax) _array_element_2)) ; Restore percent of current mag
            (else
              (bind _ammoinreservemax (`/Game/TSS_Game/Blueprints/Weapons/Base/BP_WeaponBase.AmmoInReserveMax` _array_element_2))
              (set `/Game/TSS_Game/Blueprints/Weapons/Base/BP_WeaponBase.AmmoInReserve` (`KismetMathLibrary.Clamp` (+ (`/Game/TSS_Game/Blueprints/Weapons/Base/BP_WeaponBase.AmmoInReserve` _array_element_2) (/ _ammoinreservemax 2)) 0 _ammoinreservemax) _array_element_2) ; Restore percent of ammo
              (set `/Game/TSS_Game/Blueprints/Weapons/Base/BP_WeaponBase.AmmoCurrent` (`/Game/TSS_Game/Blueprints/Weapons/Base/BP_WeaponBase.AmmoMax` _array_element_2) _array_element_2) ; Restore current mag
            ))
          (`/Game/TSS_Game/Blueprints/Weapons/Base/BP_WeaponBase.ReloadWarningCheck` _array_element_2)
          (bind _returnvalue (`|SpawnActorFromClass` "/Game/TSS_Game/UI/FloatingText/FloatingText_AmmoRestored.FloatingText_AmmoRestored_C" (`KismetMathLibrary.Conv_VectorToTransform` (`self.K2_GetActorLocation` self)) "Undefined" "MultiplyWithRoot" null null))
          (`/Game/TSS_Game/UI/FloatingText/FloatingText_AmmoRestored.Init` _returnvalue)))))
  (`/Engine/EditorBlueprintResources/StandardMacros.IncrementInt` (`self.NewColorIndex`)
    (:`  `
      (`LightComponent.SetLightColor` (`self.Light`) (`|GetArrayItem` (`self.New Light Color`) (`self.NewColorIndex`)) true)
      (bind _output_get_3 (set `self.AmmoLeftPercent` (- (`self.AmmoLeftPercent`) (`self.AmmoUsedPerUse`))))
      (if (> _output_get_3 0.0)
        (`/Engine/EditorBlueprintResources/ActorMacros.Switch Has Authority`
          (:`Authority`
            (`self.MC_CrateAvailable`)))
        (else
          (`self.K2_DestroyActor`))))))

(fn `UserConstructionScript`)