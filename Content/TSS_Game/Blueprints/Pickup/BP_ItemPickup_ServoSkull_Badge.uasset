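; Servo skull badge pickup that rewards all players with points and EXP and registers a collected skull for the interacting character's controller.
; MCActivate extends the parent behavior by having the character play a pickup interaction montage through InteractPickable.
; The multicast ActivationSuccess plays a coin sound at the pickup, while only the authority calls BP_GameModeBase for rewards and skull collection, then destroys the actor.
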(event `self.ActivationSuccess`
  (`parent.ActivationSuccess`)
  (`GameplayStatics.PlaySoundAtLocation` "/Game/TSS_Game/SFX/Pickup/SFX_Coin_Cue.SFX_Coin_Cue" (`self.K2_GetActorLocation`) (struct) 1.0 1.0 0.0 null null null null)
  (`/Engine/EditorBlueprintResources/ActorMacros.Switch Has Authority`
    (:`Authority`
      (bind _asbp_game_mode_base (cast `/Game/TSS_Game/Blueprints/System/BP_GameModeBase` (`GameplayStatics.GetGameMode`)))
      (`/Game/TSS_Game/Blueprints/System/BP_GameModeBase.AddPointsToAllPlayers` _asbp_game_mode_base (`self.Points to Add`))
      (`/Game/TSS_Game/Blueprints/System/BP_GameModeBase.AddEXP_ToAllPlayers` _asbp_game_mode_base (`self.EXP_To_Add`))
      (`/Game/TSS_Game/Blueprints/System/BP_GameModeBase.CollectSkull` _asbp_game_mode_base (`Pawn.GetController` (`self.Character`)))
      (`self.K2_DestroyActor`))))

(event `self.MC_Activate`
  (params (InputObject :type "Object Object Reference"))
  (`parent.MC_Activate` InputObject)
  (`/Game/TSS_Game/Blueprints/System/BP_CharacterBase.InteractPickable` (`self.Character`) self (`self.AnimMontage`)))

(fn `UserConstructionScript`
  (`parent.UserConstructionScript`))