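; Severed Hormagant head gore actor that gets flung, spurts blood, then dissolves and destroys itself.
; Construction randomizes spin and upward-sideways launch velocity for its rotating and projectile movement components.
; On BeginPlay it creates dynamic materials, stops spinning after a second, and re-triggers blood particles on timers at lengthening intervals.
; A timeline finally drives the materials' Appearance parameter before destroying the actor.
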(event `self.ReceiveBeginPlay`
  (bind _staticmesh (`self.StaticMesh`))
  (for (_array_element _array_index) (`MeshComponent.GetMaterials` _staticmesh)
    (bind _returnvalue (`KismetMaterialLibrary.CreateDynamicMaterialInstance` _array_element))
    (`KismetArrayLibrary.Array_AddUnique` (`self.Materials_Dissolved`) _returnvalue)
    (`PrimitiveComponent.SetMaterial` _staticmesh _array_index _returnvalue))
  (`KismetSystemLibrary.K2_SetTimerDelegate` (delegate `ActivateBlood`) 0.4 true)
  (`KismetSystemLibrary.Delay` 1.0)
  (`ActorComponent.Deactivate` (`self.RotatingMovement`))
  (`KismetSystemLibrary.Delay` 4.0)
  (`SceneComponent.SetWorldScale3D` (`self.P_Body_Bullet_Impact`) (1.0 1.0 1.0))
  (`KismetSystemLibrary.K2_SetTimerDelegate` (delegate `ActivateBlood`) 1.1 true)
  (`KismetSystemLibrary.Delay` 3.0)
  (`KismetSystemLibrary.K2_SetTimerDelegate` (delegate `ActivateBlood`) 2.0 true)
  ;[1 1 1] DissolveEffect
  (bind (_direction _duration) (`Timeline|Timeline` :!via `PlayFromStart`)
    (:`Update`
      (for _array_element_2 (`self.Materials_Dissolved`)
        (`MaterialInstanceDynamic.SetScalarParameterValue` _array_element_2 "Appearance" (`KismetMathLibrary.Lerp` 0.0 1.0 _duration))))
    (:`Finished`
      (`self.K2_DestroyActor`))))

(event `ActivateBlood`
  (`ActorComponent.Activate` (`self.P_Body_Bullet_Impact`) false))

(fn `UserConstructionScript`
  (set `RotatingMovementComponent.RotationRate` (`KismetMathLibrary.RandomRotator` false) (`self.RotatingMovement`))
  (set `MovementComponent.Velocity` (`KismetMathLibrary.MakeVector` 0.0 (`KismetMathLibrary.RandomFloatInRange` 50.0 300.0) (`KismetMathLibrary.RandomFloatInRange` 300.0 600.0)) (`self.ProjectileMovement`)))