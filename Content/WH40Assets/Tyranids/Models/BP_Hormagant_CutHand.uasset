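; BP_Hormagant_CutHand is a severed Hormagant hand that flies off spurting blood, then destroys itself after about eight seconds.
; The construction script randomizes its rotation rate and launches it sideways and upward through ProjectileMovement.
; Spinning stops after one second, while a looping timer keeps re-activating the PBodyBulletImpact effect.
; Later the effect's world scale is set to one and the spurt interval lengthens.
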(event `self.ReceiveBeginPlay`
  (`KismetSystemLibrary.K2_SetTimerDelegate` (delegate `ActivateBlood`) 0.4 true)
  (`KismetSystemLibrary.Delay` 1.0)
  (`ActorComponent.Deactivate` (`self.RotatingMovement`))
  (`KismetSystemLibrary.Delay` 4.0)
  (`SceneComponent.SetWorldScale3D` (`self.P_Body_Bullet_Impact`) (1.0 1.0 1.0))
  (`KismetSystemLibrary.K2_SetTimerDelegate` (delegate `ActivateBlood`) 1.1 true)
  (`KismetSystemLibrary.Delay` 3.0)
  (`KismetSystemLibrary.K2_SetTimerDelegate` (delegate `ActivateBlood`) 2.0 true)
  (`self.K2_DestroyActor`))

(event `ActivateBlood`
  (`ActorComponent.Activate` (`self.P_Body_Bullet_Impact`) false))

(fn `UserConstructionScript`
  (set `RotatingMovementComponent.RotationRate` (`KismetMathLibrary.RandomRotator` false) (`self.RotatingMovement`))
  (set `MovementComponent.Velocity` (`KismetMathLibrary.MakeVector` 0.0 (`KismetMathLibrary.RandomFloatInRange` 50.0 300.0) (`KismetMathLibrary.RandomFloatInRange` 300.0 600.0)) (`self.ProjectileMovement`)))